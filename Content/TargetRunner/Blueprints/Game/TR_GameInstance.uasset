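; TargetRunner's game instance, which persists game settings and player progress and handles level travel and LAN sessions.
; Init restores save slot and difficulty from the global save and creates the GoodsDropper, all only if that load succeeds; Shutdown writes it back, without mode records yet.
; Player data saves per slot, and OnNewGameMode reloads the GoodsDropper's drop tables from the game mode.
; Events cover local and server travel, session host/join/destroy, and error printouts.
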(event Custom|ServerHostNewSesssion
  (params (HostPlayerController :type TR%20Player%20Controller%20Base%20Object%20Reference) (DifficultyMultiplier :type Float%20%28single-precision%29) (Seed :type Integer))
  ;[1 1 1] ServerHostNewSession
  (Variables|Default|SetCurrentDifficultyMultiplier DifficultyMultiplier)
  (Variables|Default|SetGameSeed Seed)
  (|Session HostPlayerController 3 true
    (:OnSuccess
      (Game|OpenLevel(byName) "LobbyMap01" true "listen"))
    (:OnFailure
      (Development|PrintString "Failed to create session." true true "(R=0.875000,G=0.000000,B=0.000000,A=1.000000)" 1e+01))))

(event Custom|ServerJoinSession
  (params (JoiningPlayerController :type TR%20Player%20Controller%20Base%20Object%20Reference))
  ;[1 1 1] Server Join Session
  (bind _results (|FindSessions JoiningPlayerController 1 true)
    (:OnSuccess
      (bind _array_element (Utilities|Array|ForEachLoopwithBreak _results :!label _label)
        (:LoopBody
          (Development|PrintString (Class|FindSessionsCallbackProxy|GetServerName _array_element))
          (Utilities|FlowControl|Delay 2.0)
          (|JoinSession JoiningPlayerController _array_element
            (:then
              (goto _label Break))))))
    (:OnFailure
      (Development|PrintString "Session search failed." true true "(R=0.875000,G=0.000000,B=0.000000,A=1.000000)" 1e+01))))

(event Custom|ServerTravelToLevel
  (params (LevelName :type String) (InitiatingPlayerController :type TR%20Player%20Controller%20Base%20Object%20Reference))
  ;[1 1 1] Server Travel To Level
  (Development|ExecuteConsoleCommand (Utilities|String|Append "servertravel " LevelName) InitiatingPlayerController))

(event Custom|DestroyPlayerSession
  (params (PlayerController :type Player%20Controller%20Object%20Reference))
  ;[1 1 1] Destroy Player Session
  (|DestroySession self PlayerController))

(event Custom|OnNewGameMode
  ;[1 1 1] OnNewGameMode
  (Class|GoodsDropper|ClearDropTableLibrary (Variables|Default|GetGoodsDropper))
  (bind _astr_game_mode_base_bp (Utilities|Casting|CastToTR_GameMode_Base_BP (Game|GetGameMode)))
  (Class|GoodsDropper|AddDropTableDatatoLibrary (Variables|Default|GetGoodsDropper) (Variables|/Game/TargetRunner/Blueprints/Game/TR_GameMode_Base_BP.TR_GameMode_Base_BP_C|GetGoodsDropTables _astr_game_mode_base_bp)))

(event Custom|LocalTravelToLevel
  (params (LevelName :type Name))
  ;[1 1 1] Local (single player) level travel
  (Game|OpenLevel(byName) LevelName))

(event Custom|LocalTravelToGameStart
  (params (Difficulty :type Float%20%28single-precision%29) (Seed :type Integer))
  ;[1 1 1] Local (single player) level travel
  (Variables|Default|SetCurrentDifficultyMultiplier Difficulty)
  (Variables|Default|SetGameSeed Seed)
  (CallFunction|LocalTraveltoLevel (Variables|Default|GetSinglePlayerGameLevel)))

(event Custom|LocalTravelToGameMenu
  ;[1 1 1] Local (single player) level travel
  (CallFunction|LocalTraveltoLevel (Variables|Default|GetGameMenuLevel)) ; Game menu level blueprint will trigger new player menu(s)
)

(event EventHandleNetworkError
  (params (FailureType :type ENetworkFailure%20Enum :default "NetDriverAlreadyExists") (bIsServer :type Boolean))
  ;[1 1 1] Network & Travel Errors
  (Development|PrintString (Utilities|String|Append "Network error: " (Utilities|String|EnumtoString FailureType)) true true "(R=0.875000,G=0.000000,B=0.000000,A=1.000000)"))

(event EventHandleTravelError
  (params (FailureType :type ETravelFailure%20Enum :default "NoLevel"))
  ;[1 1 1] Network & Travel Errors
  (Development|PrintString (Utilities|String|Append "Travel error: " (Utilities|String|EnumtoString FailureType)) true true "(R=0.875000,G=0.000000,B=0.000000,A=1.000000)"))

(event EventInit
  ;[1 1 1] Init
  (|CallParentFunction)
  (bind (_successful _globalgamesavedata) (CallFunction|GetSavedGlobalGameData))
  (if _successful
    (Utilities|FlowControl|Sequence
      (:then_0
        (Variables|Default|SetSaveSlot (select (>= (.LastSelectedSaveSlot (Utilities|Struct|BreakGlobalGameSaveData _globalgamesavedata)) 0.0) (Math|Float|Truncate (.LastSelectedSaveSlot (Utilities|Struct|BreakGlobalGameSaveData _globalgamesavedata))) 0)))
      (:then_1
        (Variables|Default|SetCurrentDifficultyMultiplier (select (> (.GameDifficulty (Utilities|Struct|BreakGlobalGameSaveData _globalgamesavedata)) 0.0) (.GameDifficulty (Utilities|Struct|BreakGlobalGameSaveData _globalgamesavedata)) 1.0)))
      (:then_2
        (bind _returnvalue (Game|ConstructObjectfromClass "/Script/TargetRunner.GoodsDropper" self))
        (bind _output_get (Variables|Default|SetGoodsDropper _returnvalue))
        (Class|GoodsDropper|AddDropTableDatatoLibrary _output_get)))))

(event EventShutdown
  ;[1 1 1] Shutdown
  (CallFunction|SaveGlobalGameData)
  (|CallParentFunction))

(fn GetSavedGlobalGameData
  (bind _returnvalue (SaveGame|DoesSaveGameExist (Variables|Default|GetGlobalGameDataSlotName)))
  (if _returnvalue
    (bind _returnvalue_2 (SaveGame|LoadGamefromSlot (Variables|Default|GetGlobalGameDataSlotName)))
    (bind _astr_global_game_save (Utilities|Casting|CastToTR_GlobalGameSave _returnvalue_2)
      (:then
        (return true (Utilities|Struct|MakeGlobalGameSaveData (.LastSelectedSaveSlot (Utilities|Struct|BreakGlobalGameSaveData (Variables|/Game/TargetRunner/Blueprints/Game/SaveLoad/TR_GlobalGameSave.TR_GlobalGameSave_C|GetGlobalGameSaveData _astr_global_game_save))) (.LastGameMode (Utilities|Struct|BreakGlobalGameSaveData (Variables|/Game/TargetRunner/Blueprints/Game/SaveLoad/TR_GlobalGameSave.TR_GlobalGameSave_C|GetGlobalGameSaveData _astr_global_game_save))) (.GameDifficulty (Utilities|Struct|BreakGlobalGameSaveData (Variables|/Game/TargetRunner/Blueprints/Game/SaveLoad/TR_GlobalGameSave.TR_GlobalGameSave_C|GetGlobalGameSaveData _astr_global_game_save))) (.GameModeRecords (Utilities|Struct|BreakGlobalGameSaveData (Variables|/Game/TargetRunner/Blueprints/Game/SaveLoad/TR_GlobalGameSave.TR_GlobalGameSave_C|GetGlobalGameSaveData _astr_global_game_save))))))
      (:CastFailed
        _)))
  (return false (Utilities|Struct|MakeGlobalGameSaveData 0.0 "/Game/TargetRunner/Blueprints/Game/TR_FPGameMode_BP.TR_FPGameMode_BP_C" 1.0 (Utilities|Array|MakeArray))))

(fn SaveGlobalGameData
  (bind _returnvalue (SaveGame|CreateSaveGameObject "/Game/TargetRunner/Blueprints/Game/SaveLoad/TR_GlobalGameSave.TR_GlobalGameSave_C"))
  (LocalVariables|SettmpSaveGame _returnvalue)
  (Default|SetGlobalGameStateValues (LocalVariables|GettmpSaveGame) (Math|Conversions|ToFloat(Integer) (Variables|Default|GetSaveSlot)) (Variables|Default|GetLastGameMode) (Variables|Default|GetCurrentDifficultyMultiplier) (Utilities|Array|MakeArray))
  (bind _returnvalue_2 (SaveGame|SaveGametoSlot (LocalVariables|GettmpSaveGame) (Variables|Default|GetGlobalGameDataSlotName)))
  (return _returnvalue_2))

(fn SavePlayerGameData
  (params (PlayerState :type TR%20Player%20State%20Object%20Reference) (PlayerIndex :type Integer))
  (bind _returnvalue (SaveGame|CreateSaveGameObject "/Game/TargetRunner/Blueprints/Game/SaveLoad/TR_PlayerSlotSave.TR_PlayerSlotSave_C"))
  (LocalVariables|SettmpSaveGame _returnvalue)
  (bind _playersavedata (Default|GetPlayerSaveData PlayerState))
  (Default|SetPlayerSaveData (LocalVariables|GettmpSaveGame) _playersavedata)
  (bind _returnvalue_2 (SaveGame|SaveGametoSlot (LocalVariables|GettmpSaveGame) (Utilities|String|Append (Variables|Default|GetPlayerSaveSlotPrefix) (Utilities|String|ToString(Integer) (Variables|Default|GetSaveSlot))) PlayerIndex))
  (return _returnvalue_2))

(fn LoadPlayerGameData
  (params (PlayerIndex :type Integer))
  (bind _saveslot (Variables|Default|GetSaveSlot))
  (bind _playersaveslotprefix (Variables|Default|GetPlayerSaveSlotPrefix))
  (bind _returnvalue (Utilities|String|ToString(Integer) _saveslot))
  (bind _returnvalue_2 (Utilities|String|Append _playersaveslotprefix _returnvalue))
  (bind _returnvalue_3 (SaveGame|DoesSaveGameExist _returnvalue_2 PlayerIndex))
  (if _returnvalue_3
    (bind _returnvalue_4 (SaveGame|LoadGamefromSlot _returnvalue_2 PlayerIndex))
    (bind _astr_player_slot_save (Utilities|Casting|CastToTR_PlayerSlotSave _returnvalue_4)
      (:then
        (return true _astr_player_slot_save))
      (:CastFailed
        _))
    (else
      (Development|PrintString "No Save Game Found" true true "(R=1.000000,G=0.014578,B=0.000000,A=1.000000)")))
  (return false 0))
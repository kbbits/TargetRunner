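; Game instance for TargetRunner, handling local and server level travel, LAN session hosting and joining, and save slots.
; Caches each player's run stats by PlayerArray index before travel, for level-complete summaries afterwards.
; Owns a GoodsDropper that loads drop tables from the platforms game mode and resolves drops into goods data.
; Saves global data on shutdown (loaded data goes unapplied) and fails the run when all players' Animus is depleted.
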(event Custom|ServerHostNewSesssion
  (params (HostPlayerController :type TR%20Player%20Controller%20Base%20BP%20Object%20Reference) (GameLevel :type Float%20%28single-precision%29) (Seed :type Integer))
  ;[1 1 1] ServerHostNewSession
  (Variables|Default|SetCurrentGameLevel GameLevel)
  (Variables|Default|SetGameSeed Seed)
  (|Session HostPlayerController 3 true
    (:OnSuccess
      (Variables|Default|SetisMultiplayerSession true)
      (Game|OpenLevel(byName) "LobbyMap01" true "listen"))
    (:OnFailure
      (Variables|Default|SetisMultiplayerSession false)
      (Development|PrintString "Failed to create session." true true "(R=0.875000,G=0.000000,B=0.000000,A=1.000000)" 1e+01))))

(event Custom|ServerJoinSession
  (params (JoiningPlayerController :type TR%20Player%20Controller%20Base%20BP%20Object%20Reference))
  ;[1 1 1] Server Join Session - Needs much improvement
  (bind _results (|FindSessions JoiningPlayerController 1 true)
    (:OnSuccess
      (bind _array_element (Utilities|Array|ForEachLoopwithBreak _results :!label _label)
        (:LoopBody
          (Development|PrintString (Class|FindSessionsCallbackProxy|GetServerName _array_element))
          (Utilities|FlowControl|Delay 2.0)
          (|JoinSession JoiningPlayerController _array_element
            (:then
              (goto _label Break))))))
    (:OnFailure
      (Development|PrintString "Session search failed." true true "(R=0.875000,G=0.000000,B=0.000000,A=1.000000)" 1e+01))))

(event Custom|ServerTravelToLevel
  (params (LevelName :type String) (InitiatingPlayerController :type Player%20Controller%20Object%20Reference))
  ;[1 1 1] Server Travel To Level
  (Utilities|CachePlayerRunStats
    (:Out
      (Development|ExecuteConsoleCommand (Utilities|String|Append "servertravel " LevelName) InitiatingPlayerController))))

(event Custom|DestroyPlayerSession
  (params (PlayerController :type Player%20Controller%20Object%20Reference))
  ;[1 1 1] Destroy Player Session
  (if (Ability|HasAuthority PlayerController)
    (Variables|Default|SetisMultiplayerSession false))
  (|DestroySession self PlayerController))

(event Custom|OnNewGameMode
  ;[1 1 1] OnNewGameMode
  (Class|GoodsDropper|ClearDropTableLibrary (Variables|Default|GetGoodsDropper))
  (bind _astr_game_mode_platforms_bp (Utilities|Casting|CastToTR_GameModePlatforms_BP (Game|GetGameMode)))
  (Class|GoodsDropper|AddDropTableDatatoLibrary (Variables|Default|GetGoodsDropper) (Variables|/Game/TargetRunner/Blueprints/Game/TR_GameModePlatforms_BP.TR_GameModePlatforms_BP_C|GetGoodsDropTables _astr_game_mode_platforms_bp)))

(event Custom|ServerTravelToGameStart
  (params (GameLevel :type Float%20%28single-precision%29) (GameSeed :type Integer) (InitiatingPlayerController :type Player%20Controller%20Object%20Reference))
  ;[1 1 1] Server Travel To Game Level
  (Variables|Default|SetCurrentGameLevel GameLevel)
  (Variables|Default|SetGameSeed GameSeed)
  (CallFunction|ServerTraveltoLevel (Utilities|String|ToString(Name) (Variables|Default|GetMainGameLevel)) InitiatingPlayerController))

(event Custom|LocalTravelToLevel
  (params (LevelName :type Name))
  ;[1 1 1] Local (single player) level travel
  (Variables|Default|SetisMultiplayerSession false)
  (Utilities|CachePlayerRunStats
    (:Out
      (Game|OpenLevel(byName) LevelName))))

(event Custom|LocalTravelToGameStart
  (params (GameLevel :type Float%20%28single-precision%29) (Seed :type Integer))
  ;[1 1 1] Local (single player) level travel
  (Variables|Default|SetCurrentGameLevel GameLevel)
  (Variables|Default|SetGameSeed Seed)
  (CallFunction|LocalTraveltoLevel (Variables|Default|GetMainGameLevel)))

(event Custom|LocalTravelToRunComplete
  ;[1 1 1] Local (single player) level travel
  (CallFunction|LocalTraveltoLevel (Variables|Default|GetSinglePlayerRunCompleteLevel)) ; Game menu level blueprint will trigger new player menu(s)
)

(event EventHandleNetworkError
  (params (FailureType :type ENetworkFailure%20Enum :default "NetDriverAlreadyExists") (bIsServer :type Boolean))
  ;[1 1 1] Network & Travel Errors
  (Development|PrintString (Utilities|String|Append "Network error: " (Utilities|String|EnumtoString FailureType)) true true "(R=0.875000,G=0.000000,B=0.000000,A=1.000000)"))

(event EventHandleTravelError
  (params (FailureType :type ETravelFailure%20Enum :default "NoLevel"))
  ;[1 1 1] Network & Travel Errors
  (Development|PrintString (Utilities|String|Append "Travel error: " (Utilities|String|EnumtoString FailureType)) true true "(R=0.875000,G=0.000000,B=0.000000,A=1.000000)"))

(event EventInit
  ;[1 1 1] Init
  (|CallParentFunction)
  (bind (_successful _globalgamesavedata) (CallFunction|GetSavedGlobalGameData))
  (bind _returnvalue (Game|ConstructObjectfromClass "/Script/TargetRunner.GoodsDropper" self))
  (Variables|Default|SetGoodsDropper _returnvalue))

(event EventShutdown
  ;[1 1 1] Shutdown
  (CallFunction|SaveGlobalGameData)
  (|CallParentFunction))

(fn GetSavedGlobalGameData
  (bind _returnvalue (SaveGame|DoesSaveGameExist (Variables|Default|GetGlobalGameDataSlotName)))
  (if _returnvalue
    (bind _returnvalue_2 (SaveGame|LoadGamefromSlot (Variables|Default|GetGlobalGameDataSlotName)))
    (bind _astr_global_game_save (Utilities|Casting|CastToTR_GlobalGameSave _returnvalue_2)
      (:then
        (return true (Utilities|Struct|MakeGlobalGameSaveData (.LastSelectedSaveSlot (Utilities|Struct|BreakGlobalGameSaveData (Variables|/Game/TargetRunner/Blueprints/Game/SaveLoad/TR_GlobalGameSave.TR_GlobalGameSave_C|GetGlobalGameSaveData _astr_global_game_save))) (.LastGameMode (Utilities|Struct|BreakGlobalGameSaveData (Variables|/Game/TargetRunner/Blueprints/Game/SaveLoad/TR_GlobalGameSave.TR_GlobalGameSave_C|GetGlobalGameSaveData _astr_global_game_save))) (.GameDifficulty (Utilities|Struct|BreakGlobalGameSaveData (Variables|/Game/TargetRunner/Blueprints/Game/SaveLoad/TR_GlobalGameSave.TR_GlobalGameSave_C|GetGlobalGameSaveData _astr_global_game_save))) (.GameModeRecords (Utilities|Struct|BreakGlobalGameSaveData (Variables|/Game/TargetRunner/Blueprints/Game/SaveLoad/TR_GlobalGameSave.TR_GlobalGameSave_C|GetGlobalGameSaveData _astr_global_game_save))))))
      (:CastFailed
        _)))
  (return false (Utilities|Struct|MakeGlobalGameSaveData 0.0 "/Game/TargetRunner/Blueprints/Game/TR_FPGameMode_BP.TR_FPGameMode_BP_C" 1.0 (Utilities|Array|MakeArray))))

(fn SaveGlobalGameData
  (bind _returnvalue (SaveGame|CreateSaveGameObject "/Game/TargetRunner/Blueprints/Game/SaveLoad/TR_GlobalGameSave.TR_GlobalGameSave_C"))
  (LocalVariables|SettmpSaveGame _returnvalue)
  (Default|SetGlobalGameStateValues (LocalVariables|GettmpSaveGame) (Math|Conversions|ToFloat(Integer) (Variables|Default|GetSaveSlot)) (Variables|Default|GetLastGameMode) (Variables|Default|GetCurrentGameLevel) (Utilities|Array|MakeArray))
  (bind _returnvalue_2 (SaveGame|SaveGametoSlot (LocalVariables|GettmpSaveGame) (Variables|Default|GetGlobalGameDataSlotName)))
  (return _returnvalue_2))

(fn SavePlayerGameData
  (params (PlayerIndex :type Integer) (PlayerSaveData :type Player%20Save%20Data%20Structure))
  (bind _returnvalue (SaveGame|CreateSaveGameObject "/Game/TargetRunner/Blueprints/Game/SaveLoad/TR_PlayerSlotSave.TR_PlayerSlotSave_C"))
  (LocalVariables|SettmpSaveGame _returnvalue)
  (Default|SetPlayerSaveData (LocalVariables|GettmpSaveGame) PlayerSaveData)
  (bind _returnvalue_2 (SaveGame|SaveGametoSlot (LocalVariables|GettmpSaveGame) (Utilities|String|Append (Variables|Default|GetPlayerSaveSlotPrefix) (Utilities|String|ToString(Integer) (Variables|Default|GetSaveSlot))) PlayerIndex))
  (return _returnvalue_2))

(fn LoadPlayerSaveData
  (params (PlayerIndex :type Integer))
  (bind _saveslot (Variables|Default|GetSaveSlot))
  (bind _playersaveslotprefix (Variables|Default|GetPlayerSaveSlotPrefix))
  (bind _returnvalue (Utilities|String|ToString(Integer) _saveslot))
  (bind _returnvalue_2 (Utilities|String|Append _playersaveslotprefix _returnvalue))
  (bind _returnvalue_3 (SaveGame|DoesSaveGameExist _returnvalue_2 PlayerIndex))
  (if _returnvalue_3
    (bind _returnvalue_4 (SaveGame|LoadGamefromSlot _returnvalue_2 PlayerIndex))
    (bind _astr_player_slot_save (Utilities|Casting|CastToTR_PlayerSlotSave _returnvalue_4)
      (:then
        (return true _astr_player_slot_save))
      (:CastFailed
        _))
    (else
      (Development|PrintString "No Save Game Found" true true "(R=1.000000,G=0.014578,B=0.000000,A=1.000000)")))
  (return false 0))

(fn EvaluateGoodsDropData
  (params (RandStream :type Random%20Stream%20Structure%20%28by%20ref%29) (DropTableName :type Name%20%28by%20ref%29) (Level :type Float%20%28single-precision%29))
  (bind _returnvalue (Class|GoodsDropper|EvaluateGoodsDropTablebyName (Variables|Default|GetGoodsDropper) RandStream DropTableName Level))
  (for _array_element _returnvalue
    (if (.Found (Default|GetGoodsData (Variables|Default|GetMyGameState) (.Name (Utilities|Struct|BreakGoodsQuantity _array_element))))
      (Utilities|Array|Add (LocalVariables|GettmpGoodsToDrop) (Utilities|Struct|MakeGoodsTypeQuantity (.Quantity (Utilities|Struct|BreakGoodsQuantity _array_element)) (.GoodsData (Default|GetGoodsData (Variables|Default|GetMyGameState) (.Name (Utilities|Struct|BreakGoodsQuantity _array_element))))))))
  (return (LocalVariables|GettmpGoodsToDrop)))

(fn CheckAllDead
  (LocalVariables|SettmpAllDead true)
  (bind _array_element (Utilities|Array|ForEachLoopwithBreak (Variables|Default|GetLoggedInPlayers) :!label _label)
    (:LoopBody
      (bind _astr_player_controller_base_bp (Utilities|Casting|CastToTR_PlayerController_Base_BP _array_element))
      (Utilities|IsValid (Variables|/Game/TargetRunner/Blueprints/Player/TR_PlayerController_Base_BP.TR_PlayerController_Base_BP_C|GetMyPlayerState _astr_player_controller_base_bp)
        (:Is%20Valid
          (if (> (Variables|/Script/TargetRunner.TR_ActorAttributeComponent|GetCurrentValue (Variables|/Game/TargetRunner/Blueprints/Player/TR_PlayerState.TR_PlayerState_C|GetAnimusAttrComponent (Variables|/Game/TargetRunner/Blueprints/Player/TR_PlayerController_Base_BP.TR_PlayerController_Base_BP_C|GetMyPlayerState _astr_player_controller_base_bp))) 0.0)
            (LocalVariables|SettmpAllDead false)
            (goto _label Break)))))
    (:Completed
      (Development|PrintString (Utilities|String|Append "Check All dead: " (Utilities|String|ToString(Boolean) (LocalVariables|GettmpAllDead))))
      (if (LocalVariables|GettmpAllDead)
        (bind _astr_player_controller_base_bp_2 (Utilities|Casting|CastToTR_PlayerController_Base_BP (Game|GetPlayerController 0)))
        (Default|ServeronRunFailed _astr_player_controller_base_bp_2)))))

(fn ShowLevelCompleteSummary
  (params (PlayerController :type TR%20Player%20Controller%20Base%20BP%20Object%20Reference))
  (bind (_hasnewstats _levelstats) (CallFunction|NewLevelStatsforPlayer PlayerController))
  (if _hasnewstats
    (Utilities|Struct|SetmembersinLevelRunStats _levelstats true)
    (Default|ShowNewLevelSummary PlayerController _levelstats)
    (return true)
    (else
      (return false))))

(fn NewLevelStatsforPlayer
  (params (PlayerController :type TR%20Player%20Controller%20Base%20BP%20Object%20Reference))
  (Utilities|IsValid PlayerController
    (:Is%20Valid
      (bind (_array_element _array_index) (Utilities|Array|ForEachLoopwithBreak (Variables|/Script/Engine.GameStateBase|GetPlayerArray (Variables|Default|GetMyGameState)) :!label _label)
        (:LoopBody
          (if (== _array_element (Variables|/Game/TargetRunner/Blueprints/Player/TR_PlayerController_Base_BP.TR_PlayerController_Base_BP_C|GetMyPlayerState PlayerController))
            (Development|PrintString (Utilities|String|Append "Player ID: " (Utilities|String|ToString(Integer) _array_index)))
            (LocalVariables|SettmpFound (.ReturnValue (Utilities|Map|Find (Variables|Default|GetLevelCompleteStats) _array_index)))
            (LocalVariables|SettmpLevelStats (.Value (Utilities|Map|Find (Variables|Default|GetLevelCompleteStats) _array_index)))
            (goto _label Break)))
        (:Completed
          (return (LocalVariables|GettmpFound) (LocalVariables|GettmpLevelStats)))))
    (:Is%20Not%20Valid
      (return (LocalVariables|GettmpFound) (LocalVariables|GettmpLevelStats)))))
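; Game mode for TargetRunner's platform levels that sets up a grid with key and exit markers and supplies scenery for each platform.
; Seeded random streams drive key placement, per-platform seeds and scenery item picks from data tables.
; Scene templates follow cell role: exit, key or a weighted default.
; Current level from the game instance scales grid extents and, with distance from grid center, shortens dynamic platforms' launcher delays through an exponential difficulty curve.
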(event EventBeginPlay
  ;[1 1 1] BeginPlay
  (|CallParentFunction)
  (bind _astr_game_instance_bp (Utilities|Casting|CastToTR_GameInstance_BP (Game|GetGameInstance)))
  (Default|OnNewGameMode _astr_game_instance_bp)
  (Variables|TRGameMode|SetCurrentGameLevel (Variables|/Game/TargetRunner/Blueprints/Game/TR_GameInstance_BP.TR_GameInstance_BP_C|GetCurrentGameLevel _astr_game_instance_bp)))

(fn ConstructionScript
  (|CallParentFunction)
  (Variables|TRGameMode|SetScenerySeedStream (Math|Random|MakeRandomStream (* (Math|Random|RandomIntegerinRangefromStream -20000 20000 (Variables|TRGameMode|GetGeneratorStream)) 10000))))

(fn InitDynamicPlatform
  (params (Platform :type Dynamic%20Platform%20Object%20Reference))
  (Variables|/Game/TargetRunner/Blueprints/Platform/DynamicPlatform.DynamicPlatform_C|SetDelayBetweenLaunchers Platform (/ (Variables|/Game/TargetRunner/Blueprints/Platform/DynamicPlatform.DynamicPlatform_C|GetDelayBetweenLaunchers Platform) (CallFunction|DifficultyMultiplierforPlatform Platform))))

(fn DifficultyMultiplierforPlatform
  (params (Platform :type Platform%20Base%20BP%20Object%20Reference))
  (bind _gridditance (Default|GetDistancefromGridCenter Platform))
  (bind _difficultycurveexponent (Variables|TRGameMode|GetDifficultyCurveExponent))
  (bind _currentgamelevel (Variables|TRGameMode|GetCurrentGameLevel))
  (bind _returnvalue (* _gridditance 0.25))
  (bind _returnvalue_2 (Math|Float|Truncate _returnvalue))
  (bind _returnvalue_3 (Math|Conversions|ToFloat(Integer) _returnvalue_2))
  (bind _returnvalue_4 (+ _currentgamelevel _returnvalue_3))
  (bind _returnvalue_5 (Math|Float|Power _returnvalue_4 _difficultycurveexponent))
  (return (select (== _returnvalue_5 0.0) 1.0 _returnvalue_5)))

(fn GetSceneLayerItemTemplates
  (params (Platform :type Platform%20Base%20Object%20Reference) (DynSceneLayer :type Dyn%20Scene%20Layer%20Structure) (PicksMultiplier :type Float%20%28single-precision%29) (EnemyPicksMultiplier :type Float%20%28single-precision%29))
  (bind _asdynamic_platform (Utilities|Casting|CastToDynamicPlatform Platform) ; If dynamic platform, use it's seed.
    (:then
      (LocalVariables|SettmpRandStream (Variables|/Game/TargetRunner/Blueprints/Platform/DynamicPlatform.DynamicPlatform_C|GetSceneryStream _asdynamic_platform)))
    (:CastFailed
      (LocalVariables|SettmpRandStream (Variables|TRGameMode|GetGeneratorStream))))
  (bind _returnvalue (Class|TRBPFunctionLibrary|EvaluateDynSceneLayertoItemNames (LocalVariables|GettmpRandStream) DynSceneLayer PicksMultiplier EnemyPicksMultiplier))
  (for _array_element _returnvalue
    (bind _returnvalue_2 (Class|DataTableFunctionLibrary|DoesDataTableRowExist (Variables|TR_DataTables|GetSceneryItemTemplates) _array_element))
    (if _returnvalue_2
      (bind _returnvalue_3 (Utilities|GetDataTableRow (Variables|TR_DataTables|GetSceneryItemTemplates) _array_element)
        (:then
          (Utilities|Array|Add (LocalVariables|GettmpItemTemplates) _returnvalue_3)))))
  (return (LocalVariables|GettmpItemTemplates)))

(fn GetSceneTemplate
  (params (Platform :type Platform%20Base%20Object%20Reference))
  (LocalVariables|SettmpCoords (Class|PlatformBase|GetGridCoordinates Platform))
  (Utilities|FlowControl|Sequence
    (:then_0
      (bind _astr_game_state_bp (Utilities|Casting|CastToTR_GameState_BP (Game|GetGameState)))
      (LocalVariables|SettmpGridManager (Variables|/Game/TargetRunner/Blueprints/Game/TR_GameState_BP.TR_GameState_BP_C|GetCurrentGridManager _astr_game_state_bp)))
    (:then_1
      (if (Default|IsExitCell (LocalVariables|GettmpGridManager) (LocalVariables|GettmpCoords))
        (LocalVariables|SettmpTemplateName "Exit_01") ; Name of exit scene template
        (elif (.Found (Default|GetKeyMarkerinCell (LocalVariables|GettmpGridManager) (LocalVariables|GettmpCoords)))
          (LocalVariables|SettmpTemplateName (Variables|/Game/TargetRunner/Blueprints/World/ExitKeys/ExitKeyMarker_Base_BP.ExitKeyMarker_Base_BP_C|GetKeyName (.KeyMarkerActor (Default|GetKeyMarkerinCell (LocalVariables|GettmpGridManager) (LocalVariables|GettmpCoords))))) ; Name of key scene template
          (else
            (LocalVariables|SettmpTemplateName (select (<= (Math|Random|RandomFloatinRangefromStream 0.0 1.0 (Variables|TRGameMode|GetGeneratorStream)) 0.2) "Pillars_01" "Basic_01")) ; Default scene template.  TODO: pick from random list
          ))))
    (:then_2
      (bind _returnvalue (Utilities|GetDataTableRow (Variables|TR_DataTables|GetSceneTemplates) (LocalVariables|GettmpTemplateName))
        (:then
          (return _returnvalue))
        (:RowNotFound
          (return ""))))))

(fn GetSeedforPlatform
  (params (Platform :type Platform%20Base%20BP%20Object%20Reference))
  (bind _sceneryseedstream (Variables|TRGameMode|GetScenerySeedStream))
  (bind _initialseed (Class|KismetMathLibrary|BreakRandomStream _sceneryseedstream))
  (bind _astr_game_state_bp (Utilities|Casting|CastToTR_GameState_BP (Game|GetGameState)))
  (return (+ _initialseed (* (Class|KismetMathLibrary|SignOfInteger _initialseed) (Class|PlatformGridMgr|GridCoordstoCellNumber (Variables|/Game/TargetRunner/Blueprints/Game/TR_GameState_BP.TR_GameState_BP_C|GetCurrentGridManager _astr_game_state_bp) (Class|PlatformBase|GetGridCoordinates Platform))))))

(fn InitGridManagerBP
  (params (GridManager :type Platform%20Grid%20Manager%20BP%20Object%20Reference))
  (bind (_minextents _maxextents) (Class|TRGameMode|GetGridExtents))
  (bind _returnvalue (Class|KismetMathLibrary|ToIntPoint(Vector2D) _minextents))
  (bind _returnvalue_2 (Class|KismetMathLibrary|ToIntPoint(Vector2D) _maxextents))
  (bind (_x _y) (Utilities|Struct|BreakIntPoint _returnvalue))
  (bind (_x_2 _y_2) (Utilities|Struct|BreakIntPoint _returnvalue_2))
  (LocalVariables|SettmpGridManager GridManager)
  (Utilities|FlowControl|Sequence
    (:then_0
      (Variables|/Game/TargetRunner/Blueprints/Platform/PlatformGridManager_BP.PlatformGridManager_BP_C|SetGridCellSize (LocalVariables|GettmpGridManager) (Variables|Default|GetGridCellSize)))
    (:then_1
      (Variables|/Script/TargetRunner.PlatformGridMgr|SetGridExtentMinX (LocalVariables|GettmpGridManager) _x)
      (Variables|/Script/TargetRunner.PlatformGridMgr|SetGridExtentMinY (LocalVariables|GettmpGridManager) _y)
      (Variables|/Script/TargetRunner.PlatformGridMgr|SetGridExtentMaxX (LocalVariables|GettmpGridManager) _x_2)
      (Variables|/Script/TargetRunner.PlatformGridMgr|SetGridExtentMaxY (LocalVariables|GettmpGridManager) _y_2))
    (:then_2
      (bind (_pickedkeymarkerclasses _pickedgridcoords) (CallFunction|PickKeys (LocalVariables|GettmpGridManager))) ; Place keys first.  Exit will look for those.
      (Variables|TRGameMode|SetPickedKeyClasses _pickedkeymarkerclasses)
      (Variables|TRGameMode|SetPickedKeyCoordinates _pickedgridcoords)
      (for (_array_element _array_index) (Variables|TRGameMode|GetPickedKeyClasses)
        (Default|PlaceKeyMarker (LocalVariables|GettmpGridManager) _array_element (Utilities|Array|Get(acopy) (Variables|TRGameMode|GetPickedKeyCoordinates) _array_index))))
    (:then_3
      (Variables|TRGameMode|SetPickedExitCoordinates (Variables|/Script/TargetRunner.PlatformGridMgr|GetExitGridCoords (LocalVariables|GettmpGridManager)))
      (Default|PlaceExitMarker (LocalVariables|GettmpGridManager) (Variables|TRGameMode|GetExitMarkerClass) (Variables|TRGameMode|GetPickedExitCoordinates))
      (Development|PrintString (Utilities|String|Append "Exit: " (Utilities|String|ToString(Vector2d) (Variables|TRGameMode|GetPickedExitCoordinates))) false))))

(fn PickKeys
  (params (GridManager :type Platform%20Grid%20Manager%20BP%20Object%20Reference))
  (LocalVariables|SettmpGridManager GridManager)
  (for _index (range 1 (Math|Integer|Clamp(Integer) (Variables|TRGameMode|GetNumberOfKeysRequired) 0 (Utilities|Array|Length (Variables|TRGameMode|GetKeyMarkerClasses))))
    (bind (_found _gridcoords) (Default|RandomEmptyCellinGrid (LocalVariables|GettmpGridManager) 20 (Variables|TRGameMode|GetGeneratorStream)))
    (if _found
      (Utilities|Array|Add (LocalVariables|GettmpGridCoords) _gridcoords)
      (Utilities|Array|Add (LocalVariables|GettmpMarkerClasses) (Utilities|Array|Get(acopy) (Variables|TRGameMode|GetKeyMarkerClasses) (- _index 1)))))
  (return (LocalVariables|GettmpMarkerClasses) (LocalVariables|GettmpGridCoords)))

(fn GetGridExtentXBP
  (return (Math|Float|Truncate (Math|Float|MapRangeClamped (Variables|TRGameMode|GetCurrentGameLevel) 0.0 1e+02 2.0 1e+01))))

(fn GetGridExtentYBP
  (return (Math|Float|Truncate (Math|Float|MapRangeClamped (Variables|TRGameMode|GetCurrentGameLevel) 0.0 1e+02 2.0 1e+01))))

(fn InitGridManager
  (bind _returnvalue (|CallParentFunction))
  (if _returnvalue
    (bind _returnvalue_2 (Class|TRGameMode|GetGridManager))
    (bind _asplatform_grid_manager_bp (Utilities|Casting|CastToPlatformGridManager_BP _returnvalue_2))
    (LocalVariables|SettmpGridManager _asplatform_grid_manager_bp)
    (Utilities|FlowControl|Sequence
      (:then_0
        (bind (_pickedkeymarkerclasses _pickedgridcoords) (CallFunction|PickKeys (LocalVariables|GettmpGridManager))) ; Place keys first.  Exit will look for those.
        (Variables|TRGameMode|SetPickedKeyClasses _pickedkeymarkerclasses)
        (Variables|TRGameMode|SetPickedKeyCoordinates _pickedgridcoords)
        (for (_array_element _array_index) (Variables|TRGameMode|GetPickedKeyClasses)
          (Default|PlaceKeyMarker (LocalVariables|GettmpGridManager) _array_element (Utilities|Array|Get(acopy) (Variables|TRGameMode|GetPickedKeyCoordinates) _array_index))))
      (:then_1
        (Default|RandomEdgeCellinGrid (LocalVariables|GettmpGridManager) (Variables|TRGameMode|GetGeneratorStream))
        (Variables|TRGameMode|SetPickedExitCoordinates (Variables|/Script/TargetRunner.PlatformGridMgr|GetExitGridCoords (LocalVariables|GettmpGridManager)))
        (Default|PlaceExitMarker (LocalVariables|GettmpGridManager) (Variables|TRGameMode|GetExitMarkerClass) (Variables|TRGameMode|GetPickedExitCoordinates))
        (Development|PrintString (Utilities|String|Append "Exit: " (Utilities|String|ToString(Vector2d) (Variables|TRGameMode|GetPickedExitCoordinates)))))
      (:then_2
        (return true)))))
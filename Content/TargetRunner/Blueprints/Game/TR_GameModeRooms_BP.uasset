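; TargetRunner game mode for room-based levels, which generates and spawns the level once all players finish traveling.
; Its construction script builds a LevelForge object with name tables, a resource table from the game state or a fallback, and generation limits.
; New players have their GoodsInventory snapshot cleared before parent start handling, which may trigger respawn.
; PostLogin warns it should not normally run, since seamless travel bypasses it.
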(event EventOnAllPlayersTravelComplete
  ;[1 1 1] AllPlayersTravelComplete
  (|CallParentFunction)
  (Utilities|FlowControl|DoOnce false
    (:Completed
      (Utilities|FlowControl|Delay 1.0)
      (CallFunction|GenerateandSpawnLevel))))

(event EventPostLogin
  (params (NewPlayer :type Player%20Controller%20Object%20Reference))
  ;[1 1 1] OnPostLogin - not called in seamless travel
  (|CallParentFunction NewPlayer)
  (Development|PrintString "GameModeRooms OnPostLogin should not normally be used." true true "(R=1.000000,G=0.000000,B=0.035352,A=1.000000)" 1e+01)
  (bind _astr_player_controller_base_bp (Utilities|Casting|CastToTR_PlayerController_Base_BP NewPlayer))
  (Class|InventoryActorComponent|ServerClearSnapshotInventory (Variables|/Script/TargetRunner.TRPlayerControllerBase|GetGoodsInventory _astr_player_controller_base_bp)))

(event EventHandleStartingNewPlayer
  (params (NewPlayer :type Player%20Controller%20Object%20Reference))
  ;[1 1 1] HandleStartingNewPlayer - is called in both seamless travel & non-seamless
  (bind _astr_player_controller_base_bp (Utilities|Casting|CastToTR_PlayerController_Base_BP NewPlayer))
  (Default|ClientHandleStartingNewPlayer _astr_player_controller_base_bp)
  (Class|InventoryActorComponent|ServerClearSnapshotInventory (Variables|/Script/TargetRunner.TRPlayerControllerBase|GetGoodsInventory _astr_player_controller_base_bp))
  (|CallParentFunction NewPlayer) ; Call this last as it may trigger respawn if match is ready
)

(fn ConstructionScript
  (|CallParentFunction)
  (CallFunction|ConstructLevelForge))

(fn ConstructLevelForge
  (Utilities|FlowControl|Sequence
    (:then_0
      (Utilities|IsValid (Variables|Default|GetLevelForge)
        (:Is%20Valid
          (Variables|Default|SetLevelForge 0))))
    (:then_1
      (bind _returnvalue (Game|ConstructObjectfromClass "/Script/TargetRunner.LevelForgeBase" self))
      (Variables|Default|SetLevelForge _returnvalue)
      (Variables|/Script/TargetRunner.LevelForgeBase|SetProperNamesTable (Variables|Default|GetLevelForge) (Variables|Default|GetProperNamesTable))
      (Variables|/Script/TargetRunner.LevelForgeBase|SetDescriptiveNamesTable (Variables|Default|GetLevelForge) (Variables|Default|GetDescriptiveNamesTable))
      (bind _astr_game_state (Utilities|Casting|CastToTR_GameState (Game|GetGameState))
        (:then
          (Variables|/Script/TargetRunner.LevelForgeBase|SetResourceDataTable (Variables|Default|GetLevelForge) (Variables|/Script/TargetRunner.TR_GameState|GetResourceTypeDataTable _astr_game_state)))
        (:CastFailed
          (Variables|/Script/TargetRunner.LevelForgeBase|SetResourceDataTable (Variables|Default|GetLevelForge) "/Game/TargetRunner/Data/TR_ResourceTypeData_Base.TR_ResourceTypeData_Base")))
      (Utilities|FlowControl|Sequence
        (:then_0
          (Variables|/Script/TargetRunner.LevelForgeBase|SetMAX_TIER (Variables|Default|GetLevelForge) 10))
        (:then_1
          (Variables|/Script/TargetRunner.LevelForgeBase|SetMAX_LEVEL (Variables|Default|GetLevelForge) 20))
        (:then_2
          (Variables|/Script/TargetRunner.LevelForgeBase|SetMAX_EXTENT_X (Variables|Default|GetLevelForge) 7))
        (:then_3
          (Variables|/Script/TargetRunner.LevelForgeBase|SetMAX_EXTENT_Y (Variables|Default|GetLevelForge) 7))
        (:then_4
          (Variables|/Script/TargetRunner.LevelForgeBase|SetDefaultThumbnail (Variables|Default|GetLevelForge) "/Game/TargetRunner/Assets/Textures/Unknown_256.Unknown_256"))))))
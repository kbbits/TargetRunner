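; Base multiplayer game mode for TargetRunner, handling player login, tagged player starts, respawns and run failure.
; Level generation polls until the template and grid manager are ready, then generates the grid and spawns rooms, flagging completion.
; Respawns set each player's Animus from the template's time; when all players lack Animus or health, the run fails back to lobby.
; It also spawns goods pickups and deletes remote players' host-side profiles on logout.
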(event Custom|RespawnPlayer
  (params (PlayerController :type TR%20Player%20Controller%20Base%20BP%20Object%20Reference))
  (bind _returnvalue (Pawn|GetControlledPawn PlayerController))
  ;[1 1 1] RespawnPlayer
  (Utilities|IsValid _returnvalue
    (:Is%20Valid
      (Actor|DestroyActor _returnvalue))
    (:Is%20Not%20Valid
      _))
  (Class|GameModeBase|RestartPlayer PlayerController))

(event Custom|OnFellOutOfWorld
  (params (PlayerController :type TR%20Player%20Controller%20Base%20BP%20Object%20Reference))
  (bind _returnvalue (Pawn|GetControlledPawn PlayerController))
  ;[1 1 1] OnFellOutOfWorld
  (Utilities|IsValid _returnvalue
    (:Is%20Valid
      (bind _astr_first_person_character_bp (Utilities|Casting|CastToTR_FirstPersonCharacter_BP _returnvalue))
      (Default|TeleporttoLocation _astr_first_person_character_bp (Transformation|GetActorLocation (Utilities|PlayerStartforController PlayerController))) ; Just teleport. Restart would reload saved data.
    )))

(event Custom|GenerateAndSpawnLevel
  ;[1 1 1] Generate And Spawn Level
  (bind _returnvalue (Class|TRGameMode|InitGridManager)) ; This first call here is to make sure it is spawned.
  (if (and _returnvalue (Variables|Default|GetbLevelTemplateReady))
    (Utilities|IsValid (Variables|/Script/TargetRunner.PlatformGridMgr|GetSpawnOwner (Class|TRGameMode|GetGridManager))
      (:Is%20Valid
        (Utilities|FlowControl|DoOnce false
          (:Completed
            (bind _asroom_platform_grid_manager_bp (Utilities|Casting|CastToRoomPlatformGridManager_BP (Class|TRGameMode|GetGridManager)))
            (EventDispatchers|BindEventtoOnSpawnRoomsComplete _asroom_platform_grid_manager_bp (delegate Custom|OnSpawnRoomsComplete))
            (CallFunction|SpawnLevelfromTemplate))))
      (:Is%20Not%20Valid
        (bind _counter (Utilities|FlowControl|DoN 100 :!label _label)
          (:Exit
            (Development|PrintString (Utilities|String|Append "GameMode waiting for valid LevelTemplate " (Utilities|String|ToString(Integer) _counter)) false)
            (Utilities|FlowControl|Delay 0.2)
            (CallFunction|GenerateandSpawnLevel)))))
    (else
      (goto _label))))

(event Custom|OnSpawnRoomsComplete
  ;[1 1 1] Generate And Spawn Level
  (Variables|Default|SetbRoomMapReady true)
  (Development|PrintString "GameModeBase - Spawn rooms complete." false))

(event Custom|OnLevelFailed
  ;[1 1 1] OnLevelFailed
  (bind _returnvalue (Class|GameModeBase|GetNumPlayers))
  (for _index (range 0 (- _returnvalue 1))
    (bind _astr_player_controller_base_bp (Utilities|Casting|CastToTR_PlayerController_Base_BP (Game|GetPlayerController _index)))
    (Default|ServeronRunFailed _astr_player_controller_base_bp))
  (bind _astr_player_controller_base_bp_2 (Utilities|Casting|CastToTR_PlayerController_Base_BP (Game|GetPlayerController 0)))
  (Default|ServerTraveltoLobbyLevel _astr_player_controller_base_bp_2))

(event EventBeginPlay
  ;[1 1 1] BeginPlay
  (|CallParentFunction))

(event EventOnAllPlayersTravelComplete
  ;[1 1 1] AllPlayersTravelComplete
  (|CallParentFunction))

(event EventPostLogin
  (params (NewPlayer :type Player%20Controller%20Object%20Reference))
  ;[1 1 1] OnPostLogin - For non-seamless travel and initial player connect
  (bind _astr_player_controller_base_bp (Utilities|Casting|CastToTR_PlayerController_Base_BP NewPlayer)
    (:then
      (Variables|/Script/TargetRunner.TRPlayerControllerBase|SetbInitialPostLogin _astr_player_controller_base_bp true))
    (:CastFailed
      _))
  (bind _astrplayer_state_bp (Utilities|Casting|CastToTRPlayerState_BP (Variables|/Script/Engine.Controller|GetPlayerState NewPlayer))
    (:then
      (bind _astr_player_controller_base_bp_2 (Utilities|Casting|CastToTR_PlayerController_Base_BP NewPlayer))
      (bind _returnvalue (Class|GameModeBase|GetNumPlayers))
      (Variables|/Game/TargetRunner/Blueprints/Player/TR_PlayerController_Base_BP.TR_PlayerController_Base_BP_C|SetPlayerStartIndex _astr_player_controller_base_bp_2 _returnvalue)
      (Development|PrintString (Utilities|String|Append "GameMode PostLogin player id: " (Utilities|String|ToString(Integer) (Variables|/Script/Engine.PlayerState|GetPlayerId _astrplayer_state_bp)) "  Profile: " (Utilities|String|ToString(Name) (Variables|/Script/TargetRunner.TRPlayerState|GetProfileName _astrplayer_state_bp)) " 
GUID: " (Guid|ToString(Guid) (Variables|/Script/TargetRunner.TRPlayerState|GetPlayerGuid _astrplayer_state_bp))) false)
      (Default|ClientPostLogin _astr_player_controller_base_bp_2)
      (|CallParentFunction NewPlayer))
    (:CastFailed
      (Development|PrintString "GameMode OnPostLogin got player with null PlayerState" true true "(R=1.000000,G=0.000000,B=0.037066,A=1.000000)" 12.0))))

(event EventOnLogout
  (params (ExitingController :type Controller%20Object%20Reference))
  ;[1 1 1] OnLogout - Delete local saves for remote players
  (if (not (Pawn|IsLocalPlayerController ExitingController))
    (bind _astrplayer_state (Utilities|Casting|CastToTRPlayerState (Variables|/Script/Engine.Controller|GetPlayerState ExitingController))
      (:then
        (Development|PrintString (Utilities|String|Append "Logout Remote player: " (Guid|ToString(Guid) (Variables|/Script/TargetRunner.TRPlayerState|GetPlayerGuid _astrplayer_state))) false)
        (bind _astrplayer_controller_base (Utilities|Casting|CastToTRPlayerControllerBase (Game|GetPlayerController 0))
          (:then
            (Class|TRPersistentDataComponent|ServerDeletePlayerProfile (Variables|/Script/TargetRunner.TRPlayerControllerBase|GetPersistentDataComponent _astrplayer_controller_base) (Variables|/Script/TargetRunner.TRPlayerState|GetPlayerGuid _astrplayer_state) true))
          (:CastFailed
            _)))
      (:CastFailed
        _)))
  (|CallParentFunction ExitingController))

(event EventOnRestartPlayer
  (params (NewPlayer :type Controller%20Object%20Reference))
  ;[1 1 1] OnRestartPlayer
  (|CallParentFunction NewPlayer)
  (Development|PrintString (Utilities|String|Append "GameMode OnRestartPlayer: " (Utilities|GetDisplayName NewPlayer)) false)
  (bind _astr_player_controller_base_bp (Utilities|Casting|CastToTR_PlayerController_Base_BP NewPlayer))
  (Class|ActorAttributeComponent|SetMaxBase (Variables|/Script/TargetRunner.TRPlayerState|GetAnimusAttribute (Default|GetTRPlayerState _astr_player_controller_base_bp)) (.AvailableTime (Utilities|Struct|BreakLevelTemplate (Class|TRGameMode|GetLevelTemplate))))
  (if (Class|GameMode|IsMatchinProgress)
    (Development|PrintString "RestartPlayer: InProgress")
    (Default|ResumeAnimus (Default|GetTRPlayerState _astr_player_controller_base_bp))
    (Default|ClientonRespawn _astr_player_controller_base_bp true)
    (bind _ascharacter (Utilities|Casting|CastToCharacter (Pawn|GetControlledPawn _astr_player_controller_base_bp)))
    (Pawn|Components|CharacterMovement|SetMovementMode (Variables|/Script/Engine.Character|GetCharacterMovement _ascharacter) (Variables|/Script/Engine.CharacterMovementComponent|GetDefaultLandMovementMode (Variables|/Script/Engine.Character|GetCharacterMovement _ascharacter)) 0)
    (bind _astr_first_person_character_bp (Utilities|Casting|CastToTR_FirstPersonCharacter_BP (Pawn|GetControlledPawn _astr_player_controller_base_bp)))
    (Default|MCPlaySoundatLocation _astr_first_person_character_bp "/Game/TargetRunner/Assets/Audio/FX/PopShort_01.PopShort_01")
    (else
      (Development|PrintString "RestartPlayer: match not in progress")
      (Default|PauseAnimus (Default|GetTRPlayerState _astr_player_controller_base_bp)))))

(event EventHandleStartingNewPlayer
  (params (NewPlayer :type Player%20Controller%20Object%20Reference))
  ;[1 1 1] HandleStartingNewPlayer - For both travel types
  (Development|PrintString (Utilities|String|Append "GameModeBase_BP HandleStartingNewPlayer: " (Utilities|GetDisplayName NewPlayer)) false)
  (|CallParentFunction NewPlayer))

(event EventOnGameModeSeamlessTravelComplete
  ;[1 1 1] GameModeSeamlessTravelComplete
)

(fn ConstructionScript
  (Variables|Default|SetbRoomMapReady false))

(fn ReadytoStartMatch
  (bind _returnvalue (|CallParentFunction))
  (return _returnvalue))

(fn ChoosePlayerStart
  (params (Player :type Controller%20Object%20Reference))
  (|CallParentFunction Player))

(fn SpawnLevelfromTemplate
  (bind _returnvalue (Class|TRGameMode|InitGridManager))
  (if _returnvalue
    (bind _output_get (LocalVariables|SettmpGridManager (Class|TRGameMode|GetGridManager)))
    (Class|PlatformGridMgr|GenerateGrid _output_get)
    (Variables|Default|SetbRoomGridTemplateReady true)
    (bind _asroom_platform_grid_manager_bp (Utilities|Casting|CastToRoomPlatformGridManager_BP (LocalVariables|GettmpGridManager))
      (:then
        (Default|SpawnRoomsDelayed _asroom_platform_grid_manager_bp))
      (:CastFailed
        (Class|TRGameMode|SpawnLevel)
        (Variables|Default|SetbRoomMapReady true)))
    (return)))

(fn FindPlayerStart
  (params (Player :type Controller%20Object%20Reference) (IncomingName :type String))
  (bind _astr_player_controller_base_bp (Utilities|Casting|CastToTR_PlayerController_Base_BP Player))
  (bind _output_get (LocalVariables|SettmpStartTag (Utilities|PlayerStartTagforController _astr_player_controller_base_bp)))
  (bind _outactors (Actor|GetAllActorsOfClass "/Script/Engine.PlayerStart"))
  (bind _array_element (Utilities|Array|ForEachLoopwithBreak _outactors)
    (:LoopBody
      (if (Utilities|Name|Equal(Name) (Variables|/Script/Engine.PlayerStart|GetPlayerStartTag _array_element) (LocalVariables|GettmpStartTag))
        (return _array_element)))
    (:Completed
      (return 0))))

(fn CheckAllDead
  (LocalVariables|SettmpAllDead true)
  (bind _returnvalue (Class|GameModeBase|GetNumPlayers))
  (bind _index (Utilities|FlowControl|ForLoopwithBreak 0 (- _returnvalue 1) :!label _label)
    (:LoopBody
      (bind _astr_player_controller_base_bp (Utilities|Casting|CastToTR_PlayerController_Base_BP (Game|GetPlayerController _index)))
      (Utilities|IsValid (Default|GetTRPlayerState _astr_player_controller_base_bp)
        (:Is%20Valid
          (if (and (> (Class|ActorAttributeComponent|GetCurrent (Variables|/Script/TargetRunner.TRPlayerState|GetAnimusAttribute (Default|GetTRPlayerState _astr_player_controller_base_bp))) 0.0) (> (Class|ActorAttributeComponent|GetCurrent (Variables|/Script/TargetRunner.TRPlayerState|GetHealthAttribute (Default|GetTRPlayerState _astr_player_controller_base_bp))) 0.0))
            (LocalVariables|SettmpAllDead false)
            (goto _label Break)))))
    (:Completed
      (if (LocalVariables|GettmpAllDead)
        (CallFunction|OnLevelFailed))
      (return (LocalVariables|GettmpAllDead)))))

(fn RespawnPlayerasSpectator
  (params (PlayerController :type TR%20Player%20Controller%20Base%20BP%20Object%20Reference))
  (bind _output_get (LocalVariables|SettmpOldPawn (Pawn|GetControlledPawn PlayerController)))
  (bind _returnvalue (Game|SpawnActorfromClass (Variables|Default|GetSpectatorClass) (Transformation|GetActorTransform _output_get) "AdjustIfPossibleButAlwaysSpawn" 0 0))
  (Pawn|Possess PlayerController _returnvalue)
  (Actor|DestroyActor (LocalVariables|GettmpOldPawn)))

(fn SpawnPickupGoods
  (params (SpawnTransform :type Transform) (PickupGoods :type Goods%20Quantity%20Structure))
  (LocalVariables|SettmpSpawnTransform SpawnTransform)
  (LocalVariables|SettmpPickupGoods PickupGoods)
  (if (Utilities|IsValidSoftClassReference (.ActorClass (Utilities|Struct|BreakGoodsType (.GoodsData (CallFunction|GetGoodsData (.Name (Utilities|Struct|BreakGoodsQuantity (LocalVariables|GettmpPickupGoods))))))))
    (if (Utilities|IsValidClass (Utilities|ResolveSoftReference (.ActorClass (Utilities|Struct|BreakGoodsType (.GoodsData (CallFunction|GetGoodsData (.Name (Utilities|Struct|BreakGoodsQuantity (LocalVariables|GettmpPickupGoods)))))))))
      (LocalVariables|SettmpDropActorToSpawn (Utilities|ResolveSoftReference (.ActorClass (Utilities|Struct|BreakGoodsType (.GoodsData (CallFunction|GetGoodsData (.Name (Utilities|Struct|BreakGoodsQuantity (LocalVariables|GettmpPickupGoods)))))))))
      (for _index (range 1 (Math|Float|Truncate (.Quantity (Utilities|Struct|BreakGoodsQuantity (LocalVariables|GettmpPickupGoods))))) :!label _label
        (bind _returnvalue (Game|SpawnActorfromClass (LocalVariables|GettmpDropActorToSpawn) (LocalVariables|GettmpSpawnTransform) "Undefined" 0 0))
        (Utilities|Array|Add (LocalVariables|GettmpSpawnedActors) _returnvalue))
      (else
        (bind _returnvalue_2 (Utilities|LoadClassAssetBlocking (.ActorClass (Utilities|Struct|BreakGoodsType (.GoodsData (CallFunction|GetGoodsData (.Name (Utilities|Struct|BreakGoodsQuantity (LocalVariables|GettmpPickupGoods)))))))))
        (bind _asactor (Utilities|Casting|CastToActorClass _returnvalue_2)
          (:then
            (LocalVariables|SettmpDropActorToSpawn _asactor)
            (goto _label))
          (:CastFailed
            (bind _returnvalue_3 (Game|SpawnActorfromClass "/Game/TargetRunner/Blueprints/Pickups/GoodsPickup_BP.GoodsPickup_BP_C" (LocalVariables|GettmpSpawnTransform) "AdjustIfPossibleButAlwaysSpawn" 0 (Utilities|Struct|MakePickupAwards (Utilities|Array|MakeArray (Utilities|Struct|MakePickupAwardsItem (Utilities|Array|MakeArray (LocalVariables|GettmpPickupGoods)) 0.0 0.0))) 0 :!label _label_2))
            (Utilities|Array|Add (LocalVariables|GettmpSpawnedActors) _returnvalue_3)))))
    (else
      (goto _label_2)))
  (return (LocalVariables|GettmpSpawnedActors)))
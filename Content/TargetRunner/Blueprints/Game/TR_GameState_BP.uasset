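; TargetRunner's GameState, which links to the level's platform grid manager and provides goods data lookups.
; On BeginPlay the authority registers itself with the game instance, and every machine caches the first PlatformGridManager found in the level.
; ReplaceProxyPlatform forwards grid coordinates to that manager when it is valid.
; GetGoodsData returns a goods table row by name with a found flag, printing unknown names.
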(event Custom|ReplaceProxyPlatform
  (params (GridCoords :type Vector%202D%20Structure))
  (bind _currentgridmanager (Variables|Default|GetCurrentGridManager))
  (Utilities|IsValid _currentgridmanager
    (:Is%20Valid
      (Default|ReplaceProxyPlatform _currentgridmanager GridCoords))))

(event EventBeginPlay
  (Networking|SwitchHasAuthority
    (:Authority
      (bind _astr_game_instance_bp (Utilities|Casting|CastToTR_GameInstance_BP (Game|GetGameInstance))
        (:then
          (Variables|/Game/TargetRunner/Blueprints/Game/TR_GameInstance_BP.TR_GameInstance_BP_C|SetMyGameState _astr_game_instance_bp self))
        (:CastFailed
          _)))
    (:Remote
      _))
  (bind _outactors (Actor|GetAllActorsOfClass "/Game/TargetRunner/Blueprints/Platform/PlatformGridManager_BP.PlatformGridManager_BP_C")) ; Find the GridManager in the level. (if any)
  (if (Utilities|Array|IsValidIndex _outactors)
    (Variables|Default|SetCurrentGridManager (Utilities|Array|Get(acopy) _outactors))))

(fn ConstructionScript)

(fn GetGoodsData
  (params (GoodsName :type Name))
  (bind _goodsdata (Variables|Default|GetGoodsData))
  (bind _returnvalue (Class|DataTableFunctionLibrary|DoesDataTableRowExist _goodsdata GoodsName))
  (if _returnvalue
    (bind _returnvalue_2 (Utilities|GetDataTableRow _goodsdata GoodsName)
      (:then
        (LocalVariables|SetTmpGoodsData _returnvalue_2)
        (return true (|Copy (LocalVariables|GetTmpGoodsData))))
      (:RowNotFound
        _))
    (else
      (Development|PrintString (Utilities|String|Append "Unknown Goods Type: " (Utilities|String|ToString(Name) GoodsName)))))
  (return false (LocalVariables|GetTmpGoodsData)))
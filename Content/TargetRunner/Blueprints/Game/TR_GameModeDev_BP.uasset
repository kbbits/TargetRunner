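; Development game mode for TargetRunner that flags the room map ready at construction and drops starting players straight in with a test loadout.
; SetupPlayer raises the equipped-weapon limit and, if the tool inventory is empty, adds and equips every StartingTools entry with 100 shots' worth of ammo goods.
; Setup completion gates ReadyToStartMatch.
; Restarting a player pauses Animus and hides the lobby wait screen.
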(event EventOnRestartPlayer
  (params (NewPlayer :type Controller%20Object%20Reference))
  ;[1 1 1] On Restart Player
  (|CallParentFunction NewPlayer)
  (bind _astr_player_controller_base_bp (Utilities|Casting|CastToTR_PlayerController_Base_BP NewPlayer))
  (Default|PauseAnimus (Default|GetTRPlayerState _astr_player_controller_base_bp))
  (Default|HideLobbyWaitScreen _astr_player_controller_base_bp))

(event EventHandleStartingNewPlayer
  (params (NewPlayer :type Player%20Controller%20Object%20Reference))
  ;[1 1 1] Handle New Starting Player
  (|CallParentFunction NewPlayer)
  (CallFunction|SetupPlayer NewPlayer)
  (Class|GameModeBase|RestartPlayer NewPlayer))

(fn ConstructionScript
  (|CallParentFunction)
  (Variables|Default|SetbRoomMapReady true))

(fn ReadytoStartMatch
  (|CallParentFunction)
  (return (Variables|Default|GetbPlayerIsSetup)))

(fn SetupPlayer
  (params (Object :type Object%20Object%20Reference))
  (bind _astr_player_controller_base_bp (Utilities|Casting|CastToTR_PlayerController_Base_BP Object))
  (LocalVariables|SettmpPlayerController _astr_player_controller_base_bp)
  (Utilities|FlowControl|Sequence
    (:then_0
      (Variables|/Script/TargetRunner.TRPlayerControllerBase|SetMaxEquippedWeapons (LocalVariables|GettmpPlayerController) 20)
      (Variables|/Script/TargetRunner.TRPlayerControllerBase|SetMaxEquippedWeapons (LocalVariables|GettmpPlayerController) 20))
    (:then_1
      (if (== (Utilities|Map|Length (Variables|/Script/TargetRunner.TRPlayerControllerBase|GetToolInventory _astr_player_controller_base_bp)) 0)
        (for _array_element (Variables|Default|GetStartingTools)
          (bind _returnvalue (Game|ConstructObjectfromClass _array_element self))
          (bind _output_get (LocalVariables|SettmpTool _returnvalue))
          (Variables|/Script/TargetRunner.ToolBase|SetItemGuid _output_get (Guid|NewGuid))
          (bind _tooldata (Class|ToolBase|ToToolData _output_get))
          (bind _output_get_2 (LocalVariables|SettmpToolData _tooldata))
          (Class|TRPlayerControllerBase|ServerAddTooltoInventory (LocalVariables|GettmpPlayerController) _output_get_2)
          (Class|TRPlayerControllerBase|ServerEquipTool (LocalVariables|GettmpPlayerController) (.ItemGuid (Utilities|Struct|BreakAttributeDataSet (.AttributeData (Utilities|Struct|BreakToolData _output_get_2)))))
          (if (> (Utilities|Array|Length (Utilities|Struct|BreakGoodsQuantitySet (.GoodsQuantitySet (Utilities|Struct|BreakNamedGoodsQuantitySet (.AmmoPerShot (Utilities|GetClassDefaults _array_element)))))) 0)
            (Class|InventoryActorComponent|AddSubtractGoodsArray (Variables|/Script/TargetRunner.TRPlayerControllerBase|GetGoodsInventory (LocalVariables|GettmpPlayerController)) (Class|GoodsFunctionLibrary|MultiplyGoodsQuantities (Utilities|Struct|BreakGoodsQuantitySet (.GoodsQuantitySet (Utilities|Struct|BreakNamedGoodsQuantitySet (.AmmoPerShot (Utilities|GetClassDefaults _array_element))))) 1e+02 true) false false)))))
    (:then_2
      (Variables|Default|SetbPlayerIsSetup true))))
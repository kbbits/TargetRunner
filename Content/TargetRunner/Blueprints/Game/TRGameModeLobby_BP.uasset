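; Lobby game mode for TargetRunner that handles players joining, spawning and leaving a multiplayer lobby.
; Post-login stores the player count as each controller's start index, and login, start and respawn events notify that player's client.
; ChoosePlayerStart seeks a PlayerStart with the player's tag, falling back to the parent's choice.
; It flags when all clients report ready, and on remote logout has the host delete that player's profile data.
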(event Custom|Server_OnClientReady
  (params (ReadyController :type TR%20Player%20Controller%20Base%20Object%20Reference))
  (bind _output (Utilities|ResolveSoftReference ReadyController))
  ;[1 1 1] Server_OnClientReady
  (Utilities|Map|Add (Variables|Default|GetReadyClients) _output true)
  (Development|PrintString (Utilities|String|Append "OnClientReady " (Utilities|ToString(SoftObjectReference) _output) " Player " (Utilities|String|ToString(Integer) (Utilities|Map|Length (Variables|Default|GetReadyClients))) " of " (Utilities|String|ToString(Integer) (Variables|Default|GetNumPlayers))))
  (if (>= (Utilities|Map|Length (Variables|Default|GetReadyClients)) (Variables|Default|GetNumPlayers))
    (Variables|Default|SetbAllClientsReady true)))

(event EventOnRestartPlayer
  (params (NewPlayer :type Controller%20Object%20Reference))
  ;[1 1 1] OnRestartPlayer
  (|CallParentFunction NewPlayer)
  (bind _astr_player_controller_base_bp (Utilities|Casting|CastToTR_PlayerController_Base_BP NewPlayer))
  (Default|ClientonRespawn _astr_player_controller_base_bp (Class|GameMode|IsMatchinProgress)))

(event EventPostLogin
  (params (NewPlayer :type Player%20Controller%20Object%20Reference))
  ;[1 1 1] OnPostLogin
  (bind _astr_player_controller_base_bp (Utilities|Casting|CastToTR_PlayerController_Base_BP NewPlayer)
    (:then
      (Variables|/Script/TargetRunner.TRPlayerControllerBase|SetbInitialPostLogin _astr_player_controller_base_bp true))
    (:CastFailed
      _))
  (bind _astrplayer_state (Utilities|Casting|CastToTRPlayerState (Variables|/Script/Engine.Controller|GetPlayerState NewPlayer))
    (:then
      (Development|PrintString (Utilities|String|Append "GameModeLobby PostLogin player id: " (Utilities|String|ToString(Integer) (Variables|/Script/Engine.PlayerState|GetPlayerId _astrplayer_state)) "  Profile: " (Utilities|String|ToString(Name) (Variables|/Script/TargetRunner.TRPlayerState|GetProfileName _astrplayer_state)) " 
GUID: " (Guid|ToString(Guid) (Variables|/Script/TargetRunner.TRPlayerState|GetPlayerGuid _astrplayer_state))) false))
    (:CastFailed
      _))
  (bind _astr_player_controller_base_bp_2 (Utilities|Casting|CastToTR_PlayerController_Base_BP NewPlayer))
  (bind _returnvalue (Class|GameModeBase|GetNumPlayers))
  (Variables|/Game/TargetRunner/Blueprints/Player/TR_PlayerController_Base_BP.TR_PlayerController_Base_BP_C|SetPlayerStartIndex _astr_player_controller_base_bp_2 _returnvalue)
  (Default|ClientPostLogin _astr_player_controller_base_bp_2)
  (|CallParentFunction NewPlayer))

(event EventOnLogout
  (params (ExitingController :type Controller%20Object%20Reference))
  ;[1 1 1] OnLogout
  (if (not (Pawn|IsLocalPlayerController ExitingController))
    (bind _astrplayer_state (Utilities|Casting|CastToTRPlayerState (Variables|/Script/Engine.Controller|GetPlayerState ExitingController))
      (:then
        (Development|PrintString (Utilities|String|Append "Logout Remote player: " (Guid|ToString(Guid) (Variables|/Script/TargetRunner.TRPlayerState|GetPlayerGuid _astrplayer_state))) false)
        (bind _astrplayer_controller_base (Utilities|Casting|CastToTRPlayerControllerBase (Game|GetPlayerController 0))
          (:then
            (Class|TRPersistentDataComponent|ServerDeletePlayerProfile (Variables|/Script/TargetRunner.TRPlayerControllerBase|GetPersistentDataComponent _astrplayer_controller_base) (Variables|/Script/TargetRunner.TRPlayerState|GetPlayerGuid _astrplayer_state) true))
          (:CastFailed
            _)))
      (:CastFailed
        _)))
  (|CallParentFunction ExitingController))

(event EventOnAllPlayersTravelComplete
  ;[1 1 1] On All Players Travel Complete
  (|CallParentFunction))

(event EventHandleStartingNewPlayer
  (params (NewPlayer :type Player%20Controller%20Object%20Reference))
  ;[1 1 1] Handle Starting New Player
  (Development|PrintString (Utilities|String|Append "GameModeLobby - handle starting new player: " (Utilities|GetDisplayName NewPlayer) " player id: " (Utilities|String|ToString(Integer) (Variables|/Script/Engine.PlayerState|GetPlayerId (Variables|/Script/Engine.Controller|GetPlayerState NewPlayer)))))
  (bind _astr_player_controller_base_bp (Utilities|Casting|CastToTR_PlayerController_Base_BP NewPlayer))
  (Default|ClientHandleStartingNewPlayer _astr_player_controller_base_bp)
  (|CallParentFunction NewPlayer))

(fn ConstructionScript)

(fn ChoosePlayerStart
  (params (Player :type Controller%20Object%20Reference))
  (LocalVariables|SetbFound false)
  (bind _astr_player_controller_base_bp (Utilities|Casting|CastToTR_PlayerController_Base_BP Player)
    (:then
      (LocalVariables|SettmpStartTag (Utilities|String|StringToName (Utilities|PlayerStartTag _astr_player_controller_base_bp)))
      (bind _outactors (Actor|GetAllActorsOfClass "/Script/Engine.PlayerStart"))
      (bind _array_element (Utilities|Array|ForEachLoopwithBreak _outactors)
        (:LoopBody
          (if (Utilities|Name|Equal(Name) (Variables|/Script/Engine.PlayerStart|GetPlayerStartTag _array_element) (LocalVariables|GettmpStartTag))
            (return _array_element)))
        (:Completed
          (bind _returnvalue (|CallParentFunction Player :!label _label))
          (return _returnvalue))))
    (:CastFailed
      (goto _label))))
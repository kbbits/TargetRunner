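; Player state for TargetRunner that tracks score, target hits and kills, shards, unlocked tools and ammo per type.
; Energy lives in an attribute component, with helpers to deduct, add up to max and report percentage.
; Shard and ammo changes reject negative totals, and tool ammo checks resolve the tool class through the game mode.
; GetPlayerSaveData packs the persistent stats, but UpdateFromSaveData is empty, leaving its restore logic disconnected.
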(event Custom|OnTargetHit
  (params (Score :type Float%20%28single-precision%29) (TargetDestroyed :type Boolean))
  ;[1 1 1] Handles targets hit and score.
  (Utilities|FlowControl|Sequence
    (:then_0
      (Math|Integer|IncrementInt (Variables|Default|GetTargetsHit)
        (:%20%20
          (Math|Integer|IncrementInt (Variables|Default|GetTotalTargetsHit)))))
    (:then_1
      (if TargetDestroyed
        (Math|Integer|IncrementInt (Variables|Default|GetTargetsDestroyed)
          (:%20%20
            (Math|Integer|IncrementInt (Variables|Default|GetTotalTargetsDestroyed))))))
    (:then_2
      (bind _output_get (Variables|Default|SetCurrentScore (+ Score (Variables|Default|GetCurrentScore))))
      (if (> _output_get (Variables|Default|GetHighScore))
        (Variables|Default|SetHighScore (Variables|Default|GetCurrentScore))))))

(event Custom|UpdateFromSaveData
  (params (PlayerSaveData :type Player%20Save%20Data%20Structure)))

(event Custom|UnlockTool
  (params (ToolName :type Name))
  (Utilities|Array|AddUnique (Variables|Default|GetToolsUnlocked) ToolName))

(fn ConstructionScript)

(fn GetCurrentEnergyPercent
  (bind _energyattrcomponent (Variables|Default|GetEnergyAttrComponent))
  (return (/ (Variables|/Game/TargetRunner/Blueprints/Player/TR_ActorAttributeComponent.TR_ActorAttributeComponent_C|GetCurrentValue _energyattrcomponent) (Variables|/Game/TargetRunner/Blueprints/Player/TR_ActorAttributeComponent.TR_ActorAttributeComponent_C|GetMaxValue _energyattrcomponent))))

(fn DeductEnergy
  (params (ToDeduct :type Float%20%28single-precision%29))
  (if (<= ToDeduct (Variables|/Game/TargetRunner/Blueprints/Player/TR_ActorAttributeComponent.TR_ActorAttributeComponent_C|GetCurrentValue (Variables|Default|GetEnergyAttrComponent)))
    (bind _output_get (Variables|/Game/TargetRunner/Blueprints/Player/TR_ActorAttributeComponent.TR_ActorAttributeComponent_C|SetCurrentValue (Variables|Default|GetEnergyAttrComponent) (- (Variables|/Game/TargetRunner/Blueprints/Player/TR_ActorAttributeComponent.TR_ActorAttributeComponent_C|GetCurrentValue (Variables|Default|GetEnergyAttrComponent)) ToDeduct)))
    (return true _output_get)
    (else
      (return false (Variables|/Game/TargetRunner/Blueprints/Player/TR_ActorAttributeComponent.TR_ActorAttributeComponent_C|GetCurrentValue (Variables|Default|GetEnergyAttrComponent))))))

(fn GetPlayerSaveData
  (bind _playername (Variables|Default|GetPlayerName))
  (return (Utilities|Struct|MakePlayerSaveData (Utilities|String|StringToName _playername) (Utilities|Text|ToText(String) _playername) 0.0 0.0 (Math|Conversions|ToFloat(Integer) (Variables|Default|GetShardsCollected)) 0.0 (Math|Conversions|ToFloat(Integer) (Variables|Default|GetTargetsHit)) (Variables|Default|GetCurrentScore) (Math|Conversions|ToFloat(Integer) (Variables|Default|GetTotalTargetsHit)) (Variables|Default|GetHighScore) (Variables|Default|GetMaxHealth) (Variables|/Game/TargetRunner/Blueprints/Player/TR_ActorAttributeComponent.TR_ActorAttributeComponent_C|GetMaxValue (Variables|Default|GetEnergyAttrComponent)) (Math|Conversions|ToFloat(Integer) (Variables|Default|GetTargetsDestroyed)) (Math|Conversions|ToFloat(Integer) (Variables|Default|GetTotalTargetsDestroyed)) (Variables|/Game/TargetRunner/Blueprints/Player/TR_ActorAttributeComponent.TR_ActorAttributeComponent_C|GetRechargeRate (Variables|Default|GetEnergyAttrComponent)) 0.0 0.0 (Variables|Default|GetToolsUnlocked) (Utilities|Map|MakeMap) (Variables|Default|GetGoodsInventory))))

(fn AddEnergy
  (params (ToAdd :type Float%20%28single-precision%29))
  (bind _energyattrcomponent (Variables|Default|GetEnergyAttrComponent))
  (if (< (Variables|/Game/TargetRunner/Blueprints/Player/TR_ActorAttributeComponent.TR_ActorAttributeComponent_C|GetMaxValue _energyattrcomponent) (+ ToAdd (Variables|/Game/TargetRunner/Blueprints/Player/TR_ActorAttributeComponent.TR_ActorAttributeComponent_C|GetCurrentValue _energyattrcomponent)))
    (bind _output_get (Variables|/Game/TargetRunner/Blueprints/Player/TR_ActorAttributeComponent.TR_ActorAttributeComponent_C|SetCurrentValue (Variables|Default|GetEnergyAttrComponent) (Variables|/Game/TargetRunner/Blueprints/Player/TR_ActorAttributeComponent.TR_ActorAttributeComponent_C|GetMaxValue (Variables|Default|GetEnergyAttrComponent))))
    (return _output_get)
    (else
      (bind _output_get_2 (Variables|/Game/TargetRunner/Blueprints/Player/TR_ActorAttributeComponent.TR_ActorAttributeComponent_C|SetCurrentValue (Variables|Default|GetEnergyAttrComponent) (+ ToAdd (Variables|/Game/TargetRunner/Blueprints/Player/TR_ActorAttributeComponent.TR_ActorAttributeComponent_C|GetCurrentValue _energyattrcomponent))))
      (return _output_get_2))))

(fn AddSubtractShards
  (params (Shards :type Float%20%28single-precision%29))
  (bind _output_get (LocalVariables|SettmpShardDelta (Math|Float|Truncate Shards)))
  (if (>= _output_get 0)
    _
    (elif (>= (+ (LocalVariables|GettmpShardDelta) (Variables|Default|GetShardsCollected)) 0)
      _
      (else
        (return false))))
  (Variables|Default|SetShardsCollected (+ (Variables|Default|GetShardsCollected) (LocalVariables|GettmpShardDelta)))
  (return true))

(fn HasAmmoforTool
  (params (ToolName :type Name))
  (bind _astr_game_mode_base_bp (Utilities|Casting|CastToTR_GameMode_Base_BP (Game|GetGameMode))
    (:then
      (if (.Valid (Default|GetToolClassbyName _astr_game_mode_base_bp ToolName))
        (return (> (.Value (Utilities|Map|Find (Variables|Default|GetAmmo) (.AmmoType (Utilities|GetClassDefaults (.ToolClass (Default|GetToolClassbyName _astr_game_mode_base_bp ToolName)))))) 0.0))
        (else
          _)))
    (:CastFailed
      _))
  (return false))

(fn AddSubtractAmmo
  (params (AmmoType :type AmmoTypes%20Enum :default "NewEnumerator2") (Quantity :type Float%20%28single-precision%29))
  (if (Utilities|Enum|Equal(Enum) AmmoType "NewEnumerator2")
    (return true 0.0)
    (else
      (LocalVariables|SettmpOldTotal (.Value (Utilities|Map|Find (Variables|Default|GetAmmo) AmmoType)))
      (if (== Quantity 0.0)
        (return true (LocalVariables|GettmpOldTotal))
        (else
          (bind _output_get (LocalVariables|SettmpNewTotal (+ (LocalVariables|GettmpOldTotal) Quantity)))
          (if (>= _output_get 0.0)
            (Utilities|Map|Add (Variables|Default|GetAmmo) AmmoType (LocalVariables|GettmpNewTotal))
            (return true (LocalVariables|GettmpNewTotal))
            (else
              (return false (LocalVariables|GettmpOldTotal)))))))))
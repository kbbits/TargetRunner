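; TR_ActorAttributeComponent is a component holding a clamped attribute value for an actor, with optional regeneration over time.
; Each tick, while the recharge rate is positive and the value is below maximum, it adds rate times delta seconds and clamps the result between minimum and maximum.
; A server-only check exists but is disconnected, so the recharge runs without an authority gate.
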(event EventBeginPlay)

(event EventTick
  (params (DeltaSeconds :type Float%20%28single-precision%29))
  (if (and (> (Variables|Default|GetRechargeRate) 0.0) (< (Variables|Default|GetCurrentValue) (Variables|Default|GetMaxValue)))
    (Variables|Default|SetCurrentValue (Math|Float|Clamp(Float) (+ (* (Variables|Default|GetRechargeRate) DeltaSeconds) (Variables|Default|GetCurrentValue)) (Variables|Default|GetMinValue) (Variables|Default|GetMaxValue)))))
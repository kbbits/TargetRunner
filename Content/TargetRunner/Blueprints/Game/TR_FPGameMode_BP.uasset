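; TR_FPGameMode_BP is a TargetRunner game mode Blueprint that supplies scene and scenery item templates from data tables for a given platform.
; GetSceneTemplate returns the hardcoded "Basic_01" row, with random selection left unwired and the Platform input unused.
; GetSceneLayerItemTemplates evaluates a dynamic scene layer into item names and collects the matching scenery rows, skipping missing names.
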(fn ConstructionScript)

(fn GetSceneTemplate
  (params (Platform :type Platform%20Base%20Object%20Reference))
  (Utilities|FlowControl|Sequence
    (:then_0
      (LocalVariables|SettmpTemplateName "Basic_01"))
    (:then_1
      (bind _returnvalue (Utilities|GetDataTableRow (Variables|Default|GetSceneTemplates) (LocalVariables|GettmpTemplateName))
        (:then
          (return _returnvalue))
        (:RowNotFound
          (return ""))))))

(fn GetSceneLayerItemTemplates
  (params (Platform :type Platform%20Base%20Object%20Reference) (DynSceneLayer :type Dyn%20Scene%20Layer%20Structure))
  (bind _returnvalue (Class|TRBPFunctionLibrary|EvaluateDynSceneLayertoItemNames DynSceneLayer 1.0))
  (for _array_element _returnvalue
    (bind _returnvalue_2 (Class|DataTableFunctionLibrary|DoesDataTableRowExist (Variables|Default|GetSceneryItemTemplates) _array_element))
    (if _returnvalue_2
      (bind _returnvalue_3 (Utilities|GetDataTableRow (Variables|Default|GetSceneryItemTemplates) _array_element)
        (:then
          (Utilities|Array|Add (LocalVariables|GettmpItemTemplates) _returnvalue_3)))))
  (return (LocalVariables|GettmpItemTemplates)))
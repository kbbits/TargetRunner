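; LauncherScenery is a dynamic scenery Blueprint that hosts a Launcher_Base in a child actor component, with helpers to fetch it and set its target box.
; On construction, if it has a valid DynamicPlatform and a positive difficulty modifier, it tunes the launcher from its class defaults.
; Higher difficulty shortens the delay between launches and scales up aim speed and base targets to spawn.
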(event EventTick
  (params (DeltaSeconds :type Float%20%28single-precision%29)))

(fn ConstructionScript
  (|CallParentFunction)
  (CallFunction|InitfromPlatform))

(fn SetLaucherTarget
  (params (TargetBox :type Launcher%20Target%20Box%20Object%20Reference))
  (bind _aslauncher_base (Utilities|Casting|CastToLauncher_Base (Variables|/Script/Engine.ChildActorComponent|GetChildActor (Variables|Default|GetLauncher_CAC))))
  (Variables|/Game/TargetRunner/Blueprints/Launcher/Launcher_Base.Launcher_Base_C|SetTargetBox _aslauncher_base TargetBox))

(fn GetLauncher
  (bind _aslauncher_base (Utilities|Casting|CastToLauncher_Base (Variables|/Script/Engine.ChildActorComponent|GetChildActor (Variables|Default|GetLauncher_CAC)))
    (:then
      (return _aslauncher_base))
    (:CastFailed
      (return 0))))

(fn InitfromPlatform
  (Utilities|IsValid (Variables|Default|GetMyPlatform)
    (:Is%20Valid
      (if (> (Variables|Default|GetDifficultyModifier) 0.0)
        (bind _asdynamic_platform (Utilities|Casting|CastToDynamicPlatform (Variables|Default|GetMyPlatform)))
        (LocalVariables|SettmpPlatform _asdynamic_platform)
        (LocalVariables|SettmpLauncher (CallFunction|GetLauncher))
        (Utilities|FlowControl|Sequence
          (:then_0
            (Variables|/Game/TargetRunner/Blueprints/Launcher/Launcher_Base.Launcher_Base_C|SetDelayBetweenLaunches (LocalVariables|GettmpLauncher) (/ (.DelayBetweenLaunches (Utilities|GetClassDefaults (Utilities|GetClass (LocalVariables|GettmpLauncher)))) (Variables|Default|GetDifficultyModifier))))
          (:then_1
            (Variables|/Game/TargetRunner/Blueprints/Launcher/Launcher_Base.Launcher_Base_C|SetAimSpeed (LocalVariables|GettmpLauncher) (* (Variables|Default|GetDifficultyModifier) (.AimSpeed (Utilities|GetClassDefaults (Utilities|GetClass (LocalVariables|GettmpLauncher)))))))
          (:then_2
            (Variables|/Game/TargetRunner/Blueprints/Launcher/Launcher_Base.Launcher_Base_C|SetBaseTargetsToSpawn (LocalVariables|GettmpLauncher) (Math|Float|Round (* (.BaseTargetsToSpawn (Utilities|GetClassDefaults (Utilities|GetClass (LocalVariables|GettmpLauncher)))) (Variables|Default|GetDifficultyModifier))))))))))
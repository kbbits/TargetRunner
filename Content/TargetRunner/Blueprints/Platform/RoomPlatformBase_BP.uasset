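; Base Blueprint for a room platform that spawns its wall segments from prefabs and links itself to the level's platform grid manager during construction.
; SpawnWalls runs the parent logic, then clears old walls, calls CalculateWalls and places a prefab at each section transform relative to the room.
; The wall template picks a blank or open-center prefab per section, with random entries split evenly.
; Spawned walls are tracked and destroyed with the platform.
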(event EventBeginPlay)

(event Collision|EventActorBeginOverlap
  (params (OtherActor :type Actor%20Object%20Reference)))

(event EventTick
  (params (DeltaSeconds :type Float%20%28single-precision%29)))

(event EventDestroyed
  (CallFunction|DestroySpawnedWalls))

(fn ConstructionScript
  (Utilities|IsValid (Variables|Default|GetMyGridManager)
    (:Is%20Not%20Valid
      (bind _outactors (Actor|GetAllActorsOfClass "/Game/TargetRunner/Blueprints/Platform/PlatformGridManager_BP.PlatformGridManager_BP_C"))
      (if (Utilities|Array|IsValidIndex _outactors)
        (Variables|Default|SetMyGridManager (Utilities|Array|Get(acopy) _outactors))))))

(fn SpawnWallsBP
  (CallFunction|DestroySpawnedWalls)
  (bind _returnvalue (Class|RoomPlatformBase|CalculateWalls))
  (if _returnvalue
    (for (_array_element _array_index) (Variables|Default|GetWallSectionTransforms)
      (LocalVariables|SettmpPrefabTransform (Math|Transform|ComposeTransforms _array_element (Transformation|GetWorldTransform (Variables|Default|GetRoomSceneComponent))))
      (switch Utilities|FlowControl|Switch|SwitchonETRWallState (Utilities|Array|Get(acopy) (Variables|Default|GetWallTemplate) _array_index)
        (:WallState_Blocked
          (bind _returnvalue_2 (Class|PrefabricatorBlueprintLibrary|SpawnPrefab self "/Game/TargetRunner/Assets/Meshes/WallSeg-Blank_PF.WallSeg-Blank_PF" (LocalVariables|GettmpPrefabTransform) :!label _label))
          (LocalVariables|SettmpPrefab _returnvalue_2))
        (:WallState_Open
          (bind _returnvalue_3 (Class|PrefabricatorBlueprintLibrary|SpawnPrefab self "/Game/TargetRunner/Assets/Meshes/WallSeg_OpenCenter_PF.WallSeg_OpenCenter_PF" (LocalVariables|GettmpPrefabTransform) :!label _label_2))
          (LocalVariables|SettmpPrefab _returnvalue_3))
        (:WallState_Random
          (if (> (Math|Random|RandomFloatinRange 0.0 1.0) 0.5)
            (goto _label)
            (else
              (goto _label_2)))))
      (Utilities|Array|Add (Variables|Default|GetSpawnedWalls_BP) (LocalVariables|GettmpPrefab)))))

(fn DestroySpawnedWalls
  (for _array_element (Variables|Default|GetSpawnedWalls_BP)
    (Actor|DestroyActor _array_element))
  (Utilities|Array|Clear (Variables|Default|GetSpawnedWalls_BP)))

(fn SpawnWalls
  (bind _returnvalue (|CallParentFunction))
  (CallFunction|SpawnWallsBP)
  (return _returnvalue))
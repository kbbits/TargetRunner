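; Manages the grid of platforms in TargetRunner, spawning, finding and removing proxy, static and dynamic platforms by cell coordinates.
; Adding runs only on authority, rejects cells beyond the maximum extent, and lets non-proxy types replace proxies.
; New dynamic platforms are initialized by the game mode, then generated.
; It also pools mesh instances into replicated instanced static mesh components, one per mesh, created on demand.
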(event Custom|ReplaceProxyPlatform
  (params (GridCoords :type Vector%202D%20Structure))
  ;[1 1 1] ReplaceProxyPlatform
  (bind (_found_ _foundplatform) (CallFunction|GetPlatformonGrid GridCoords))
  (if _found_
    (Utilities|Casting|CastToPlatformProxy_Base _foundplatform)
    (CallFunction|RemovePlatformfromGrid GridCoords)
    (CallFunction|AddPlatformtoGrid "NewEnumerator2" GridCoords)))

(event Custom|OnAddISM
  (params (Mesh :type Static%20Mesh%20Object%20Reference) (WorldTransform :type Transform) (Material :type Material%20Interface%20Object%20Reference))
  ;[1 1 1] Add ISM
  (Variables|Default|SettmpISMComp 0)
  (bind _array_element (Utilities|Array|ForEachLoopwithBreak (Variables|Default|GetISM_Components) :!label _label)
    (:LoopBody
      (if (== (Variables|/Script/Engine.StaticMeshComponent|GetStaticMesh _array_element) Mesh)
        (Variables|Default|SettmpISMComp _array_element)
        (goto _label Break)))
    (:Completed
      (Utilities|IsValid (Variables|Default|GettmpISMComp)
        (:Is%20Valid
          _)
        (:Is%20Not%20Valid
          (bind _returnvalue (AddComponent|AddInstancedStaticMeshComponent false (Math|Transform|MakeTransform "0, 0, 0")))
          (bind _output_get (Variables|Default|SettmpISMComp _returnvalue))
          (Utilities|Array|Add (Variables|Default|GetISM_Components) _output_get)
          (Class|ActorComponent|SetIsReplicated (Variables|Default|GettmpISMComp) true)
          (Components|StaticMesh|SetStaticMesh (Variables|Default|GettmpISMComp) Mesh)
          (Rendering|Material|SetMaterial (Variables|Default|GettmpISMComp) 0 Material)
          (Class|PrimitiveComponent|SetCullDistance (Variables|Default|GettmpISMComp) 0.0)
          (Collision|SetCollisionObjectType (Variables|Default|GettmpISMComp) "ECC_WorldDynamic")))
      (Class|InstancedStaticMeshComponent|AddInstanceWorldSpace (Variables|Default|GettmpISMComp) WorldTransform))))

(event EventBeginPlay
  ;[1 1 1] Begin Play
  (Class|PlatformGridMgr|Setup)
  (bind _astr_game_mode_base_bp (Utilities|Casting|CastToTR_GameMode_Base_BP (Game|GetGameMode)))
  (Variables|Default|SetGridCellSize (Variables|/Game/TargetRunner/Blueprints/Game/TR_GameMode_Base_BP.TR_GameMode_Base_BP_C|GetGridCellSize _astr_game_mode_base_bp)))

(fn ConstructionScript)

(fn AddPlatformtoGrid
  (params (PlatformType :type PlatformTypes_Enum%20Enum :default "NewEnumerator0") (GridCoords :type Vector%202D%20Structure))
  (bind (_x _y) (Math|Vector2D|BreakVector2D GridCoords))
  (bind _worldlocation (CallFunction|GetGridCellWorldLocation GridCoords))
  (bind (_x_2 _y_2) (Math|Vector2D|BreakVector2D GridCoords))
  (bind _self self)
  (bind _returnvalue (Math|Float|Truncate _x))
  (bind _returnvalue_2 (Math|Float|Truncate _y))
  (bind _returnvalue_3 (Math|Transform|MakeTransform _worldlocation))
  (Networking|SwitchHasAuthority
    (:Authority
      (Utilities|FlowControl|Sequence
        (:then_0
          (bind _astr_game_mode_base_bp (Utilities|Casting|CastToTR_GameMode_Base_BP (Game|GetGameMode))
            (:then
              (if (or (> _x_2 (Math|Conversions|ToFloat(Integer) (Variables|/Game/TargetRunner/Blueprints/Game/TR_GameMode_Base_BP.TR_GameMode_Base_BP_C|GetMaxGridExtent _astr_game_mode_base_bp))) (> _y_2 (Math|Conversions|ToFloat(Integer) (Variables|/Game/TargetRunner/Blueprints/Game/TR_GameMode_Base_BP.TR_GameMode_Base_BP_C|GetMaxGridExtent _astr_game_mode_base_bp))))
                (return false 0) ; Do nothing if out of GridExtent
              ))
            (:CastFailed
              (return false 0) ; Do nothing if out of GridExtent
            )))
        (:then_1
          (bind (_found_ _foundplatform) (CallFunction|GetPlatformonGrid GridCoords))
          (if _found_
            (bind _asplatform_proxy_base (Utilities|Casting|CastToPlatformProxy_Base _foundplatform)
              (:then
                (if (Utilities|Enum|NotEqual(Enum) PlatformType "NewEnumerator0")
                  (CallFunction|RemovePlatformfromGrid (Class|PlatformBase|GetGridCoordinates _asplatform_proxy_base))
                  (else
                    (return false 0) ; Return nothing if there is already a non-proxy platform there.
                  )))
              (:CastFailed
                (return false 0) ; Return nothing if there is already a non-proxy platform there.
              ))))
        (:then_2
          (switch Utilities|FlowControl|Switch|SwitchonPlatformTypes_Enum PlatformType
            (:NewEnumerator0
              (bind _returnvalue_4 (Game|SpawnActorfromClass "/Game/TargetRunner/Blueprints/Platform/PlatformProxy_Base.PlatformProxy_Base_C" _returnvalue_3 "Undefined" _self _returnvalue _returnvalue_2 0))
              (LocalVariables|SettmpNewPlatform _returnvalue_4))
            (:NewEnumerator1
              (bind _returnvalue_5 (Game|SpawnActorfromClass "/Game/TargetRunner/Blueprints/Platform/StaticPlatform.StaticPlatform_C" _returnvalue_3 "Undefined" _self _returnvalue _returnvalue_2 0))
              (LocalVariables|SettmpNewPlatform _returnvalue_5))
            (:NewEnumerator2
              (bind _returnvalue_6 (Game|SpawnActorfromClass "/Game/TargetRunner/Blueprints/Platform/DynamicPlatform.DynamicPlatform_C" _returnvalue_3 "Undefined" _self _returnvalue _returnvalue_2 0))
              (LocalVariables|SettmpNewPlatform _returnvalue_6)))
          (Utilities|Array|Add (Variables|Default|GetMyPlatforms) (LocalVariables|GettmpNewPlatform))
          (bind _asdynamic_platform (Utilities|Casting|CastToDynamicPlatform (LocalVariables|GettmpNewPlatform))
            (:then
              ;[1 1 1] If it's a dynamic platform, set it up and generate.
              (bind _astr_game_mode_base_bp_2 (Utilities|Casting|CastToTR_GameMode_Base_BP (Game|GetGameMode)))
              (Default|InitDynamicPlatform _astr_game_mode_base_bp_2 _asdynamic_platform)
              (Default|OnGenerate _asdynamic_platform))
            (:CastFailed
              _))
          (return true (LocalVariables|GettmpNewPlatform)))))))

(fn GetPlatformonGrid
  (params (GridCoords :type Vector%202D%20Structure))
  (bind (_x _y) (Math|Vector2D|BreakVector2D GridCoords))
  (LocalVariables|SettmpX (Math|Float|Truncate _x))
  (LocalVariables|SettmpY (Math|Float|Truncate _y))
  (bind _array_element (Utilities|Array|ForEachLoopwithBreak (Variables|Default|GetMyPlatforms) :!label _label)
    (:LoopBody
      (if (== (Variables|/Script/TargetRunner.PlatformBase|GetGridX _array_element) (LocalVariables|GettmpX))
        (if (== (Variables|/Script/TargetRunner.PlatformBase|GetGridY _array_element) (LocalVariables|GettmpY))
          (LocalVariables|SettmpFoundPlatform _array_element)
          (goto _label Break))))
    (:Completed
      (return (Utilities|IsValid (LocalVariables|GettmpFoundPlatform)) (LocalVariables|GettmpFoundPlatform)))))

(fn GetGridCellWorldLocation
  (params (GridCoords :type Vector%202D%20Structure))
  (bind _gridcellsize (Variables|Default|GetGridCellSize))
  (bind _billboard (Variables|Default|GetBillboard))
  (bind _returnvalue (Transformation|GetWorldLocation _billboard))
  (bind _returnvalue_2 (* GridCoords _gridcellsize))
  (bind (_x _y) (Math|Vector|BreakVector _returnvalue))
  (bind (_x_2 _y_2) (Math|Vector2D|BreakVector2D _returnvalue_2))
  (return (Math|Vector|MakeVector (+ _x_2 _x) (+ _y_2 _y) (Variables|Default|GetDefaultPlatformZ))))

(fn GetNeighborsonGrid
  (params (GridCoords :type Vector%202D%20Structure))
  (bind _foundplatforms (CallFunction|GetPlatformsonGrid (Utilities|Array|MakeArray (+ GridCoords "(X=1.000000,Y=0.000000)") (+ GridCoords "(X=-1.000000,Y=0.000000)") (+ GridCoords "(X=0.000000,Y=1.000000)") (+ GridCoords "(X=0.000000,Y=-1.000000)"))))
  (return _foundplatforms))

(fn GetPlatformsonGrid
  (params (GridCoords :type Array%20of%20Vector%202D%20Structures))
  (LocalVariables|SettmpFoundPlatforms (Utilities|Array|MakeArray))
  (Utilities|FlowControl|Sequence
    (:then_0
      (for _array_element GridCoords
        (Utilities|Set|Add (LocalVariables|GettmpCoords) (Utilities|Struct|MakeIntPoint (Math|Float|Truncate (.X (Math|Vector2D|BreakVector2D _array_element))) (Math|Float|Truncate (.Y (Math|Vector2D|BreakVector2D _array_element)))))))
    (:then_1
      (bind _array_element_2 (Utilities|Array|ForEachLoopwithBreak (Variables|Default|GetMyPlatforms) :!label _label)
        (:LoopBody
          (bind _returnvalue (Utilities|Set|Remove (LocalVariables|GettmpCoords) (Utilities|Struct|MakeIntPoint (Variables|/Script/TargetRunner.PlatformBase|GetGridX _array_element_2) (Variables|/Script/TargetRunner.PlatformBase|GetGridY _array_element_2))))
          (if _returnvalue
            (Utilities|Array|AddUnique (LocalVariables|GettmpFoundPlatforms) _array_element_2)
            (if (== (Utilities|Set|Length (LocalVariables|GettmpCoords)) 0)
              (goto _label Break))))
        (:Completed
          (return (Utilities|Array|IsValidIndex (LocalVariables|GettmpFoundPlatforms)) (LocalVariables|GettmpFoundPlatforms)))))))

(fn RemovePlatformfromGrid
  (params (GridCoords :type Vector%202D%20Structure))
  (bind (_found_ _foundplatform) (CallFunction|GetPlatformonGrid GridCoords))
  (if _found_
    (bind _output_get (LocalVariables|SettmpRemovedPlatform _foundplatform))
    (if (Variables|/Script/TargetRunner.PlatformBase|GetbCanRemoveDynamic _output_get)
      (Utilities|Array|RemoveItem (Variables|Default|GetMyPlatforms) _output_get)
      (Actor|DestroyActor (LocalVariables|GettmpRemovedPlatform))
      (return true)
      (else
        (return false)))
    (else
      (return true))))
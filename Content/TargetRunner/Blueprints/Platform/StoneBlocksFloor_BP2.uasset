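; Stone block floor platform that randomly shows damage by swapping some blocks for alternate meshes.
; On BeginPlay the authority rolls each instance of two block-type ISMs against DamagePercent, moving hits to the matching Alt ISM.
; It then removes instances from all four components and respawns them at world transforms through the game mode's GridManager SpawnISM.
; Both the swap and the handoff run only when DamagePercent is above zero.
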(event EventBeginPlay
  (Networking|SwitchHasAuthority
    (:Authority
      (CallFunction|ApplyAltMeshes))))

(fn ConstructionScript)

(fn ApplyAltMeshes
  (if (> (Variables|Default|GetDamagePercent) 0.0)
    (Utilities|FlowControl|Sequence
      (:then_0
        (for _index (range 0 (- (Components|InstancedStaticMesh|GetInstanceCount (Variables|Default|GetBlockType_1_ISM)) 1))
          (if (<= (Math|Random|RandomFloat) (Variables|Default|GetDamagePercent))
            (LocalVariables|SettmpTransform (.OutInstanceTransform (Components|InstancedStaticMesh|GetInstanceTransform (Variables|Default|GetBlockType_1_ISM) _index false)))
            (if (.ReturnValue (Components|InstancedStaticMesh|GetInstanceTransform (Variables|Default|GetBlockType_1_ISM) _index false))
              (bind _returnvalue (Class|InstancedStaticMeshComponent|RemoveInstance (Variables|Default|GetBlockType_1_ISM) _index))
              (if _returnvalue
                (Components|InstancedStaticMesh|AddInstance (Variables|Default|GetBlockType_1Alt_ISM) (LocalVariables|GettmpTransform)))))))
      (:then_1
        (for _index_2 (range 0 (- (Components|InstancedStaticMesh|GetInstanceCount (Variables|Default|GetBlockType_2_ISM)) 1))
          (if (<= (Math|Random|RandomFloat) (Variables|Default|GetDamagePercent))
            (LocalVariables|SettmpTransform (.OutInstanceTransform (Components|InstancedStaticMesh|GetInstanceTransform (Variables|Default|GetBlockType_2_ISM) _index_2 false)))
            (if (.ReturnValue (Components|InstancedStaticMesh|GetInstanceTransform (Variables|Default|GetBlockType_2_ISM) _index_2 false))
              (bind _returnvalue_2 (Class|InstancedStaticMeshComponent|RemoveInstance (Variables|Default|GetBlockType_2_ISM) _index_2))
              (if _returnvalue_2
                (Components|InstancedStaticMesh|AddInstance (Variables|Default|GetBlockType_2Alt_ISM) (LocalVariables|GettmpTransform)))))))
      (:then_2
        (Networking|SwitchHasAuthority
          (:Authority
            (bind _astr_game_mode_base_bp (Utilities|Casting|CastToTR_GameModeBase_BP (Game|GetGameMode)))
            (LocalVariables|SettmpGameMode _astr_game_mode_base_bp)
            (bind _returnvalue_3 (Class|TRGameMode|GetGridManager (LocalVariables|GettmpGameMode)))
            (LocalVariables|SettmpGridManager _returnvalue_3)
            (Utilities|FlowControl|Sequence
              (:then_0
                (LocalVariables|SettmpISMComp (Variables|Default|GetBlockType_1_ISM)))
              (:then_1
                (LocalVariables|SettmpISMComp (Variables|Default|GetBlockType_1Alt_ISM)))
              (:then_2
                (LocalVariables|SettmpISMComp (Variables|Default|GetBlockType_2_ISM)))
              (:then_3
                (LocalVariables|SettmpISMComp (Variables|Default|GetBlockType_2Alt_ISM))))
            (Utilities|IsValid (LocalVariables|GettmpISMComp)
              (:Is%20Valid
                (for _index_3 (range 0 (- (Components|InstancedStaticMesh|GetInstanceCount (LocalVariables|GettmpISMComp)) 1))
                  (LocalVariables|SettmpTransform (.OutInstanceTransform (Components|InstancedStaticMesh|GetInstanceTransform (LocalVariables|GettmpISMComp) _index_3 true)))
                  (Class|InstancedStaticMeshComponent|RemoveInstance (LocalVariables|GettmpISMComp) _index_3)
                  (Class|PlatformGridMgr|SpawnISM (LocalVariables|GettmpGridManager) (Utilities|ResolveSoftReference (Variables|/Script/Engine.StaticMeshComponent|GetStaticMesh (LocalVariables|GettmpISMComp))) (Rendering|Material|GetMaterial (LocalVariables|GettmpISMComp) 0) (LocalVariables|GettmpTransform)))))))))))
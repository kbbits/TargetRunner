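; Room component actor for TargetRunner that hands its instanced static meshes over to the GridManager on the server.
; On BeginPlay it applies alt meshes, waits a random delay within GridManager-defined bounds, then gathers each ISM's world-space transforms into mesh contexts.
; It clears the local instances and passes the contexts to the GridManager to respawn.
; Helpers move alt-mesh instances back to original components and create ISM components copying a static mesh's mesh and materials.
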(event EventBeginPlay
  ;[1 1 1] Begin Play
  (Variables|Default|SetbBeginPlayCalled true)
  (Networking|SwitchHasAuthority
    (:Authority
      (Class|RoomComponentActor|ApplyAltMeshes)
      (bind _astr_game_mode (Utilities|Casting|CastToTR_GameMode (Game|GetGameMode)))
      (Utilities|FlowControl|Delay (Math|Random|RandomFloatinRange (Class|PlatformGridMgr|GetRCAMinISMMoveDelay (Class|TRGameMode|GetGridManager _astr_game_mode)) (Class|PlatformGridMgr|GetRCAMaxISMMoveDelay (Class|TRGameMode|GetGridManager _astr_game_mode))))
      (Internal|MoveISMstoGridManagerBP))
    (:Remote
      (Development|PrintString "Error - BeginPlay called for RCA with NO Authority" false))))

(fn ConstructionScript)

(fn MoveISMstoGridManagerBP
  (Networking|SwitchHasAuthority
    (:Authority
      (bind _astr_game_mode_base_bp (Utilities|Casting|CastToTR_GameModeBase_BP (Game|GetGameMode))
        (:then
          (LocalVariables|SettmpGameMode _astr_game_mode_base_bp)
          (bind _output_get (LocalVariables|SettmpGridManager (Class|TRGameMode|GetGridManager (LocalVariables|GettmpGameMode))))
          (Utilities|IsValid _output_get
            (:Is%20Valid
              (Utilities|Array|Clear (LocalVariables|GetTmpISMContexts))
              (LocalVariables|SettmpAllISMComps (Actor|GetComponentsByClass "/Script/Engine.InstancedStaticMeshComponent"))
              (for _array_element (LocalVariables|GettmpAllISMComps)
                (LocalVariables|SettmpISMComp _array_element)
                (Utilities|IsValid (LocalVariables|GettmpISMComp)
                  (:Is%20Valid
                    (Utilities|Array|Clear (LocalVariables|GettmpAllTransforms))
                    (for _index (range 0 (- (Components|InstancedStaticMesh|GetInstanceCount (LocalVariables|GettmpISMComp)) 1))
                      (if (.ReturnValue (Components|InstancedStaticMesh|GetInstanceTransform (LocalVariables|GettmpISMComp) _index true))
                        (Utilities|Array|Add (LocalVariables|GettmpAllTransforms) (.OutInstanceTransform (Components|InstancedStaticMesh|GetInstanceTransform (LocalVariables|GettmpISMComp) _index true)))
                        (else
                          (Development|PrintString "MoveISMsToGridManager - Error getting instance transform" true true "(R=1.000000,G=0.000000,B=0.007402,A=1.000000)"))))
                    (if (> (Utilities|Array|Length (LocalVariables|GettmpAllTransforms)) 0)
                      (Utilities|Array|Add (LocalVariables|GetTmpISMContexts) (Utilities|Struct|MakeISMContext (Utilities|ResolveSoftReference (Variables|/Script/Engine.StaticMeshComponent|GetStaticMesh (LocalVariables|GettmpISMComp))) (Utilities|MakeSoftObjectPath (Class|KismetSystemLibrary|GetPathName (Variables|/Script/Engine.StaticMeshComponent|GetStaticMesh (LocalVariables|GettmpISMComp)))) (LocalVariables|GettmpAllTransforms))))
                    (Components|InstancedStaticMesh|ClearInstances (LocalVariables|GettmpISMComp)))
                  (:Is%20Not%20Valid
                    (Development|PrintString "MoveISMsToGridManager RCA ISM Comp not valid"))))
              (if (> (Utilities|Array|Length (LocalVariables|GetTmpISMContexts)) 0)
                (Class|PlatformGridMgr|SpawnISMs (LocalVariables|GettmpGridManager) (LocalVariables|GetTmpISMContexts)))
              (Variables|Default|SetbMyISMsCopiedOut true))
            (:Is%20Not%20Valid
              (Development|PrintString "RoomComponentActor_BP - MoveISMsToGridManager  cannot get GridManager" true true "(R=1.000000,G=0.016751,B=0.000000,A=1.000000)" 1e+01))))
        (:CastFailed
          (Development|PrintString "RCA move ISMs could not get game mode" false))))
    (:Remote
      (Development|PrintString "RCA move ISMs, RCA has no authority" false))))

(fn SwaptoOriginalISMComponentBP
  (params (OriginalISMComponent :type Instanced%20Static%20Mesh%20Component%20Object%20Reference) (AltISMComponent :type Instanced%20Static%20Mesh%20Component%20Object%20Reference))
  (LocalVariables|SettmpOriginalISMComponent OriginalISMComponent)
  (LocalVariables|SettmpAltISMComponent AltISMComponent)
  (Utilities|Array|Clear (LocalVariables|GettmpAllTransforms))
  (for _index (range 0 (- (Components|InstancedStaticMesh|GetInstanceCount (LocalVariables|GettmpAltISMComponent)) 1))
    (Utilities|Array|Add (LocalVariables|GettmpAllTransforms) (.OutInstanceTransform (Components|InstancedStaticMesh|GetInstanceTransform (LocalVariables|GettmpAltISMComponent) _index false))))
  (Components|InstancedStaticMesh|ClearInstances (LocalVariables|GettmpAltISMComponent))
  (for _array_element (LocalVariables|GettmpAllTransforms)
    (Components|InstancedStaticMesh|AddInstance (LocalVariables|GettmpOriginalISMComponent) _array_element)))

(fn AddISMCforStaticMeshComponentBP
  (params (StaticMeshComponent :type Static%20Mesh%20Component%20Object%20Reference))
  (Utilities|IsValid StaticMeshComponent
    (:Is%20Valid
      (Utilities|FlowControl|Sequence
        (:then_0
          (bind _returnvalue (AddComponent|AddInstancedStaticMeshComponent false))
          (bind _output_get (LocalVariables|SettmpNewISMC _returnvalue))
          (Components|StaticMesh|SetStaticMesh _output_get (Variables|/Script/Engine.StaticMeshComponent|GetStaticMesh StaticMeshComponent))
          (for (_array_element _array_index) (Rendering|Material|GetMaterials StaticMeshComponent)
            (Rendering|Material|SetMaterial (LocalVariables|GettmpNewISMC) _array_index _array_element)))
        (:then_1
          (return (LocalVariables|GettmpNewISMC)))))))
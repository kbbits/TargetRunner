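; Base grid platform for TargetRunner that sizes itself to the game mode's grid cell and can snap to its grid coordinates on construction.
; Its control zone notifies the local player controller on enter and leave, and locates exit and exit key markers on the platform.
; A replicated platform state drives server-side completion events, with full completion awarding overlapping pickup boxes once, or after a short delay if set to complete immediately.
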(event OnComponentBeginOverlap(PlatformControlZone)
  (params (OverlappedComponent :type Primitive%20Component%20Object%20Reference) (OtherActor :type Actor%20Object%20Reference) (OtherComp :type Primitive%20Component%20Object%20Reference) (OtherBodyIndex :type Integer) (bFromSweep :type Boolean) (SweepResult :type Hit%20Result%20Structure%20%28by%20ref%29))
  ;[1 1 1] Handle player overlap of platform control zone
  (bind _ascharacter (Utilities|Casting|CastToCharacter OtherActor))
  (if (and (Pawn|IsPlayerControlled _ascharacter) (Pawn|IsLocallyControlled _ascharacter))
    (bind _astr_player_controller_base (Utilities|Casting|CastToTR_PlayerController_Base (Pawn|GetController _ascharacter)))
    (Default|OnEnteredPlatform _astr_player_controller_base self)))

(event OnComponentEndOverlap(PlatformControlZone)
  (params (OverlappedComponent :type Primitive%20Component%20Object%20Reference) (OtherActor :type Actor%20Object%20Reference) (OtherComp :type Primitive%20Component%20Object%20Reference) (OtherBodyIndex :type Integer))
  ;[1 1 1] Handle player overlap of platform control zone
  (bind _ascharacter (Utilities|Casting|CastToCharacter OtherActor))
  (if (and (Pawn|IsPlayerControlled _ascharacter) (Pawn|IsLocallyControlled _ascharacter))
    (bind _astr_player_controller_base (Utilities|Casting|CastToTR_PlayerController_Base (Pawn|GetController _ascharacter)))
    (Default|OnLeavePlatform _astr_player_controller_base self)))

(event Custom|OnLauchersComplete
  ;[1 1 1] On Launchers Complete
  (Utilities|FlowControl|DoOnce false))

(event Custom|OnPlatformComplete
  ;[1 1 1] On Platform Complete
  (Utilities|FlowControl|DoOnce false
    (:Completed
      (for _array_element (Collision|GetOverlappingActors (Variables|Default|GetPlatformControlZone) "/Game/TargetRunner/Blueprints/PlatformScenery/PickupBox.PickupBox_C" :!class /Script/Engine.PrimitiveComponent)
        (bind _aspickup_box (Utilities|Casting|CastToPickupBox _array_element))
        (Default|GiveAwards _aspickup_box)))))

(event Custom|MC_SetPlatformWorldLocation
  (params (Location :type Vector))
  (CallFunction|InitPlatformScale)
  (Transformation|SetActorLocation Location false true))

(event EventBeginPlay
  (Networking|SwitchHasAuthority
    (:Authority
      (if (Variables|Default|GetbCompleteImmediately)
        (Utilities|FlowControl|Delay 1.0)
        (CallFunction|OnPlatformComplete)))))

(fn ConstructionScript
  (bind _returnvalue (Class|PlatformBase|GetGridCoordinates))
  (bind _platformsize (Variables|PlatformBase|GetPlatformSize))
  (bind _returnvalue_2 (* _returnvalue _platformsize))
  (bind (_x _y) (Math|Vector2D|BreakVector2D _returnvalue_2))
  (CallFunction|InitPlatformScale)
  (if (Variables|Default|GetbSetLocationOnConstruct)
    (Transformation|SetActorLocation (Math|Vector|MakeVector _x _y 0.0) false true)))

(fn InitPlatformScale
  (bind _platform (Variables|Default|GetPlatform))
  (bind (_min _max) (Components|StaticMesh|GetLocalBounds _platform))
  (bind _astr_game_mode_base_bp (Utilities|Casting|CastToTR_GameMode_Base_BP (Game|GetGameMode))
    (:then
      (Variables|PlatformBase|SetPlatformSize (Variables|/Game/TargetRunner/Blueprints/Game/TR_GameMode_Base_BP.TR_GameMode_Base_BP_C|GetGridCellSize _astr_game_mode_base_bp)))
    (:CastFailed
      _))
  (Transformation|SetWorldScale3D (Variables|Default|GetPlatformScene) (Math|Vector|MakeVector (/ (Variables|PlatformBase|GetPlatformSize) (- (.X (Math|Vector|BreakVector _max)) (.X (Math|Vector|BreakVector _min)))) (/ (Variables|PlatformBase|GetPlatformSize) (- (.X (Math|Vector|BreakVector _max)) (.X (Math|Vector|BreakVector _min)))) 1.0)))

(fn GetDistancefromGridCenter
  (return (Math|Vector|Distance2D(Vector) :V1 (Class|PlatformBase|GetGridCoordinates))))

(fn OnRepPlatformState
  (Networking|SwitchHasAuthority
    (:Authority
      (switch Utilities|FlowControl|Switch|SwitchonPlatformState (Variables|PlatformBase|GetPlatformState)
        (:NewEnumerator2
          (CallFunction|OnLauchersComplete))
        (:NewEnumerator3
          (CallFunction|OnPlatformComplete))))))

(fn GetExitMarker
  (bind _array_element (Utilities|Array|ForEachLoopwithBreak (Collision|GetOverlappingActors (Variables|Default|GetPlatformControlZone) "/Game/TargetRunner/Blueprints/World/ExitMarkerBase_BP.ExitMarkerBase_BP_C" :!class /Script/Engine.PrimitiveComponent) :!label _label)
    (:LoopBody
      (bind _asexit_marker_base_bp (Utilities|Casting|CastToExitMarkerBase_BP _array_element))
      (Utilities|IsValid _asexit_marker_base_bp
        (:Is%20Valid
          (LocalVariables|SettmpMarker _asexit_marker_base_bp)
          (goto _label Break))))
    (:Completed
      (return (Utilities|IsValid (LocalVariables|GettmpMarker)) (LocalVariables|GettmpMarker)))))

(fn GetExitKeyMarkers
  (for _array_element (Collision|GetOverlappingActors (Variables|Default|GetPlatformControlZone) "/Game/TargetRunner/Blueprints/World/ExitKeys/ExitKeyMarkerBase_BP.ExitKeyMarkerBase_BP_C" :!class /Script/Engine.PrimitiveComponent)
    (bind _asexit_key_marker_base_bp (Utilities|Casting|CastToExitKeyMarkerBase_BP _array_element))
    (Utilities|IsValid _asexit_key_marker_base_bp
      (:Is%20Valid
        (Utilities|Array|Add (LocalVariables|GettmpMarkers) _asexit_key_marker_base_bp))))
  (return (LocalVariables|GettmpMarkers)))
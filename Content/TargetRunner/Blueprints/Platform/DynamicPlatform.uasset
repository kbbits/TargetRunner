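; Grid-based platform for TargetRunner that server-generates its scenery and runs its target launchers one after another.
; Generation adds proxy platforms with shootable edge triggers on empty neighbor cells, then updates those triggers when the launchers complete.
; A grid-seeded random stream scatters scenery, with counts scaled by distance from grid center and sizes from weighted templates.
; Items drop by box trace; template items become instanced meshes on the grid manager.
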(event Custom|OnGenerate
  ;[1 1 1] Generate
  (if (Networking|IsServer)
    (Class|KismetMathLibrary|ResetRandomStream (Variables|Default|GetSceneryStream))
    (CallFunction|GenerateNeighbors)
    (CallFunction|OnGenerateScenery)))

(event Custom|OnGenerateScenery
  ;[1 1 1] Generate Scenery
  (if (Networking|IsServer)
    (CallFunction|GenerateScenery)
    (Utilities|FlowControl|Delay (Variables|Default|GetInitialLauncherStartDelay))
    (CallFunction|OnStartNextLauncher)))

(event Custom|OnStartNextLauncher
  ;[1 1 1] Start Next Launcher
  (switch Utilities|FlowControl|Switch|SwitchonPlatformState (Variables|Default|GetPlatformState)
    (:NewEnumerator0
      (CallFunction|ServerSetPlatformState "NewEnumerator1"))
    (:NewEnumerator1
      _))
  (if (< (Variables|Default|GetLauncherIndex) (Utilities|Array|Length (Variables|Default|GetLaunchers)))
    (Default|StartLaunching (Utilities|Array|Get(acopy) (Variables|Default|GetLaunchers) (Variables|Default|GetLauncherIndex)))
    (Math|Integer|IncrementInt (Variables|Default|GetLauncherIndex)
      (:%20%20
        (if (< (Variables|Default|GetDelayBetweenLaunchers) 0.0)
          (Utilities|FlowControl|Delay (Math|Float|Absolute(Float) (Variables|Default|GetDelayBetweenLaunchers)))
          (CallFunction|OnStartNextLauncher))))
    (else
      (CallFunction|ServerSetPlatformState "NewEnumerator2"))))

(event Custom|OnLauncherDone
  (params (Launcher :type Launcher%20Base%20Object%20Reference))
  ;[1 1 1] OnLauncherDone
  (if (>= (Variables|Default|GetDelayBetweenLaunchers) 0.0)
    (Utilities|FlowControl|Delay (Variables|Default|GetDelayBetweenLaunchers))
    (CallFunction|OnStartNextLauncher)))

(event Custom|SeedSceneryStreamByGrid
  (params (NewSeed :type Integer))
  (bind _scenerystream (Variables|Default|GetSceneryStream))
  ;[1 1 1] SeedSceneryStreamByGrid
  (bind _returnvalue (Class|PlatformBase|GetGridCoordinates))
  (bind _astr_game_mode_base_bp (Utilities|Casting|CastToTR_GameMode_Base_BP (Game|GetGameMode)))
  (Math|Random|SetRandomStreamSeed _scenerystream (+ NewSeed (+ (+ (Math|Float|Truncate (.X (Math|Vector2D|BreakVector2D _returnvalue))) (Variables|/Game/TargetRunner/Blueprints/Game/TR_GameMode_Base_BP.TR_GameMode_Base_BP_C|GetMaxGridExtent _astr_game_mode_base_bp)) (* (* (* (Variables|/Game/TargetRunner/Blueprints/Game/TR_GameMode_Base_BP.TR_GameMode_Base_BP_C|GetMaxGridExtent _astr_game_mode_base_bp) 2) (Math|Float|Truncate (.X (Math|Vector2D|BreakVector2D _returnvalue)))) (+ (Variables|/Game/TargetRunner/Blueprints/Game/TR_GameMode_Base_BP.TR_GameMode_Base_BP_C|GetMaxGridExtent _astr_game_mode_base_bp) (Math|Float|Truncate (.Y (Math|Vector2D|BreakVector2D _returnvalue))))))))
  (Class|KismetMathLibrary|ResetRandomStream _scenerystream))

(event EventServerSetPlatformState
  (params (NewState :type PlatformState%20Enum :default "NewEnumerator0"))
  ;[1 1 1] ServerSetPlatformState
  (|CallParentFunction NewState)
  (if (Utilities|Enum|Equal(Enum) NewState "NewEnumerator2")
    (for _array_element (Variables|Default|GetMyTriggers)
      (bind _asshootable_platform_trigger_base (Utilities|Casting|CastToShootablePlatformTrigger_Base _array_element))
      (bind _state (Default|GetShootableTriggerState _asshootable_platform_trigger_base))
      (if (Utilities|Enum|Equal(Enum) _state "NewEnumerator0")
        (Default|SetTriggerState _asshootable_platform_trigger_base "NewEnumerator1")))))

(fn ConstructionScript
  (CallFunction|InitPlatformScale)
  (Transformation|AddLocalOffset (Variables|Default|GetLauncherTargetBox_CAC) "0, 0,1000.000000" false true))

(fn GenerateNeighbors
  (if (Networking|IsServer)
    (Utilities|FlowControl|Sequence
      (:then_0
        (bind _astr_game_state_base (Utilities|Casting|CastToTR_GameState_Base (Game|GetGameState)))
        (LocalVariables|SettmpGridManager (Variables|/Game/TargetRunner/Blueprints/Game/TR_GameState_Base.TR_GameState_Base_C|GetCurrentGridManager _astr_game_state_base)))
      (:then_1
        (bind _returnvalue (Class|PlatformBase|GetGridCoordinates))
        ;[1 1 1] Place platform proxies on empty neighbor spots
        (for (_array_element _array_index) (Utilities|Array|MakeArray (+ _returnvalue "(X=1.000000,Y=0.000000)") (+ _returnvalue "(X=-1.000000,Y=0.000000)") (+ _returnvalue "(X=0.000000,Y=1.000000)") (+ _returnvalue "(X=0.000000,Y=-1.000000)"))
          (LocalVariables|SettmpAllowProxy true)
          (bind _neighbors (Default|GetNeighborsonGrid (LocalVariables|GettmpGridManager) _array_element))
          (bind _array_element_2 (Utilities|Array|ForEachLoopwithBreak _neighbors :!label _label)
            (:LoopBody
              (if (!= _array_element_2 self)
                (LocalVariables|SettmpAllowProxy false)
                (goto _label Break)))
            (:Completed
              (if (LocalVariables|GettmpAllowProxy)
                (bind (_successful_ _newplatform) (Default|AddPlatformtoGrid (LocalVariables|GettmpGridManager) "NewEnumerator0" _array_element))
                (if _successful_
                  (bind _returnvalue_2 (Game|SpawnActorfromClass "/Game/TargetRunner/Blueprints/Shootables/Triggers/ShootablePlatformTrigger_Base.ShootablePlatformTrigger_Base_C" (Math|Transform|MakeTransform (.Location (Math|Transform|BreakTransform (Utilities|Select :Index _array_index :Option%200 (Transformation|GetWorldTransform (Variables|Default|GetNorthEdgeAnchor)) :Option%201 (Transformation|GetWorldTransform (Variables|Default|GetSouthEdgeAnchor)) :Option%202 (Transformation|GetWorldTransform (Variables|Default|GetEastEdgeAnchor)) :Option%203 (Transformation|GetWorldTransform (Variables|Default|GetWestEdgeAnchor))))) (.Rotation (Math|Transform|BreakTransform (Utilities|Select :Index _array_index :Option%200 (Transformation|GetWorldTransform (Variables|Default|GetNorthEdgeAnchor)) :Option%201 (Transformation|GetWorldTransform (Variables|Default|GetSouthEdgeAnchor)) :Option%202 (Transformation|GetWorldTransform (Variables|Default|GetEastEdgeAnchor)) :Option%203 (Transformation|GetWorldTransform (Variables|Default|GetWestEdgeAnchor)))))) "AdjustIfPossibleButAlwaysSpawn" self _newplatform 0))
                  (Utilities|Array|Add (Variables|Default|GetMyTriggers) _returnvalue_2))))))))))

(fn GenerateScenery
  (if (Networking|IsServer)
    (bind _keys (Utilities|Map|Keys (Variables|Default|GetSceneryTemplate)))
    (for _array_element _keys
      (Utilities|FlowControl|Sequence
        (:then_0
          (if (Utilities|ClassIsChildOf _array_element "/Game/TargetRunner/Blueprints/DynamicScenery/LauncherScenery.LauncherScenery_C")
            (LocalVariables|SettmpQuantityModifier (* (CallFunction|GetDistancefromGridCenter) 0.25))
            (else
              (LocalVariables|SettmpQuantityModifier (* (CallFunction|GetDistancefromGridCenter) 0.85))))
          (if (not (> (LocalVariables|GettmpQuantityModifier) 0.0))
            (LocalVariables|SettmpQuantityModifier 1.0)))
        (:then_1
          (bind _sizetemplates (CallFunction|GetSizeTemplates _array_element))
          (LocalVariables|SettmpSizeTemplates _sizetemplates)
          (bind _output_get (LocalVariables|SettmpNumSceneItems (Math|Random|RandomIntegerinRangefromStream (select (>= (Math|Float|Round (* (.X (Utilities|Struct|BreakIntPoint (.Value (Utilities|Map|Find (Variables|Default|GetSceneryTemplate) _array_element)))) (LocalVariables|GettmpQuantityModifier))) 1) (Math|Float|Round (* (.X (Utilities|Struct|BreakIntPoint (.Value (Utilities|Map|Find (Variables|Default|GetSceneryTemplate) _array_element)))) (LocalVariables|GettmpQuantityModifier))) 1) (Math|Float|Round (* (.Y (Utilities|Struct|BreakIntPoint (.Value (Utilities|Map|Find (Variables|Default|GetSceneryTemplate) _array_element)))) (LocalVariables|GettmpQuantityModifier))) (Variables|Default|GetSceneryStream))))
          (LocalVariables|SettmpMaxTemplateIndex (- (Utilities|Array|Length (LocalVariables|GettmpSizeTemplates)) 1))
          (for _index (range 1 _output_get)
            (CallFunction|SpawnSceneryItem _array_element (Math|Transform|MakeTransform (CallFunction|GetScenerySpawnLocation _array_element)) (.Min (Utilities|Struct|BreakBox (Utilities|Array|Get(acopy) (LocalVariables|GettmpSizeTemplates) (Math|Float|Round (Math|Float|MapRangeClamped (Math|Conversions|ToFloat(Integer) _index) 1.0 (Math|Conversions|ToFloat(Integer) (LocalVariables|GettmpNumSceneItems)) 0.0 (Math|Conversions|ToFloat(Integer) (LocalVariables|GettmpMaxTemplateIndex))))))) (.Max (Utilities|Struct|BreakBox (Utilities|Array|Get(acopy) (LocalVariables|GettmpSizeTemplates) (Math|Float|Round (Math|Float|MapRangeClamped (Math|Conversions|ToFloat(Integer) _index) 1.0 (Math|Conversions|ToFloat(Integer) (LocalVariables|GettmpNumSceneItems)) 0.0 (Math|Conversions|ToFloat(Integer) (LocalVariables|GettmpMaxTemplateIndex))))))) true)))))))

(fn GetScenerySpawnLocation
  (params (SceneryClass :type Dynamic%20Scenery%20Base%20Class%20Reference))
  (bind _platform (Variables|Default|GetPlatform))
  (bind (_origin _boxextent) (Collision|GetComponentBounds _platform))
  (bind (_x _y) (Math|Vector|BreakVector _boxextent))
  (return (+ _origin (Math|Vector|MakeVector (Math|Random|RandomFloatinRangefromStream (* _x -0.9) (* _x 0.9) (Variables|Default|GetSceneryStream)) (Math|Random|RandomFloatinRangefromStream (* _y -0.9) (* _y 0.9) (Variables|Default|GetSceneryStream)) (+ (.Z (Math|Vector|BreakVector (Transformation|GetWorldLocation (Variables|Default|GetPlatformScene)))) 6e+03)))))

(fn SpawnSceneryItem
  (params (ClassToSpawn :type Dynamic%20Scenery%20Base%20Class%20Reference) (SpawnTransform :type Transform) (MinSizes :type Vector) (MaxSizes :type Vector) (PlaceByDrop :type Boolean))
  (bind _self self)
  (if (Networking|IsServer)
    (Utilities|FlowControl|Sequence
      (:then_0
        (bind _returnvalue (Game|SpawnActorfromClass ClassToSpawn SpawnTransform "AdjustIfPossibleButAlwaysSpawn" _self _self MinSizes MaxSizes 0))
        (bind _output_get (LocalVariables|SettmpNewScenery _returnvalue))
        (Utilities|Array|Add (Variables|Default|GetAllScenery) _output_get)
        (CallFunction|InitializeNewScenery (LocalVariables|GettmpNewScenery)))
      (:then_2
        ;[1 1 1] Drop the box using box trace.  Place it on top of where it collides.
        (if PlaceByDrop
          (bind (_outhit _returnvalue_2) (Collision|BoxTraceByChannel (+ (Transformation|GetActorLocation (LocalVariables|GettmpNewScenery)) "0, 0, 0") (+ (Transformation|GetActorLocation (LocalVariables|GettmpNewScenery)) "0, 0,-10000.000000") (.BoxExtent (Collision|GetActorBounds (LocalVariables|GettmpNewScenery) true)) (Transformation|GetActorRotation (LocalVariables|GettmpNewScenery)) "TraceTypeQuery1" false (Utilities|Array|MakeArray (LocalVariables|GettmpNewScenery)) "None" false "(R=1.000000,G=0.000000,B=0.000000,A=1.000000)" "(R=0.000000,G=1.000000,B=0.000000,A=1.000000)" 3e+01))
          (if _returnvalue_2
            (if (.bBlockingHit (Collision|BreakHitResult _outhit))
              (Transformation|SetActorLocation (LocalVariables|GettmpNewScenery) (.ImpactPoint (Collision|BreakHitResult _outhit)) false true)))))
      (:then_3
        ;[1 1 1] Convert the scenery's mesh to an ISM on the GridManager
        (if (Variables|/Game/TargetRunner/Blueprints/DynamicScenery/DynamicScenery_Base.DynamicScenery_Base_C|GetTemplateForISM? (LocalVariables|GettmpNewScenery))
          (LocalVariables|SettmpTransform (Math|Transform|MakeTransform (Transformation|GetWorldLocation (Variables|/Game/TargetRunner/Blueprints/DynamicScenery/DynamicScenery_Base.DynamicScenery_Base_C|GetSceneObject (LocalVariables|GettmpNewScenery))) (Transformation|GetWorldRotation (Variables|/Game/TargetRunner/Blueprints/DynamicScenery/DynamicScenery_Base.DynamicScenery_Base_C|GetObjectsScene (LocalVariables|GettmpNewScenery))) (Transformation|GetWorldScale (Variables|/Game/TargetRunner/Blueprints/DynamicScenery/DynamicScenery_Base.DynamicScenery_Base_C|GetObjectsScene (LocalVariables|GettmpNewScenery)))))
          (bind _astr_game_state_base (Utilities|Casting|CastToTR_GameState_Base (Game|GetGameState)))
          (Default|OnAddISM (Variables|/Game/TargetRunner/Blueprints/Game/TR_GameState_Base.TR_GameState_Base_C|GetCurrentGridManager _astr_game_state_base) (Variables|/Script/Engine.StaticMeshComponent|GetStaticMesh (Variables|/Game/TargetRunner/Blueprints/DynamicScenery/DynamicScenery_Base.DynamicScenery_Base_C|GetSceneObject (LocalVariables|GettmpNewScenery))) (LocalVariables|GettmpTransform) (Rendering|Material|GetMaterial (Variables|/Game/TargetRunner/Blueprints/DynamicScenery/DynamicScenery_Base.DynamicScenery_Base_C|GetSceneObject (LocalVariables|GettmpNewScenery)) 0))
          (Actor|DestroyActor (LocalVariables|GettmpNewScenery)))))))

(fn GetSizeTemplates
  (params (DynamicSceneryClass :type Dynamic%20Scenery%20Base%20Class%20Reference))
  (LocalVariables|SettmpSizeTemplates (Utilities|Array|MakeArray))
  (Utilities|FlowControl|Sequence
    (:then_0
      ;[1 1 1] Make default template list
      (LocalVariables|SettmpSizeInfo (Math|Box|MakeBox "500.000000,500.000000,50.000000" "1000.000000,1000.000000,100.000000"))
      (LocalVariables|SettmpWeight 1)
      (for _index (range 1 (LocalVariables|GettmpWeight)) :!label _label
        (Utilities|Array|Add (LocalVariables|GettmpSizeTemplates) (LocalVariables|GettmpSizeInfo))))
    (:then_1
      (LocalVariables|SettmpSizeInfo (Math|Box|MakeBox "500.000000,50.000000,200.000000" "1000.000000,100.000000,300.000000"))
      (LocalVariables|SettmpWeight 2)
      (goto _label))
    (:then_2
      (LocalVariables|SettmpSizeInfo (Math|Box|MakeBox "50.000000,500.000000,200.000000" "100.000000,1000.000000,300.000000"))
      (LocalVariables|SettmpWeight 2)
      (goto _label))
    (:then_3
      (LocalVariables|SettmpSizeInfo (Math|Box|MakeBox "50.000000,50.000000,200.000000" "150.000000,150.000000,400.000000"))
      (LocalVariables|SettmpWeight 4)
      (goto _label))
    (:then_4
      (LocalVariables|SettmpSizeInfo (Math|Box|MakeBox "25.000000,25.000000,50.000000" "150.000000,150.000000,100.000000"))
      (LocalVariables|SettmpWeight 10)
      (goto _label))
    (:then_5
      (LocalVariables|SettmpSizeInfo (Math|Box|MakeBox "25.000000,25.000000,25.000000" "100.000000,100.000000,75.000000"))
      (LocalVariables|SettmpWeight 15))
    (:then_6
      (return (LocalVariables|GettmpSizeTemplates)))))

(fn InitializeNewScenery
  (params (Object :type Object%20Object%20Reference))
  (bind _aslauncher_scenery (Utilities|Casting|CastToLauncherScenery Object))
  (LocalVariables|SettmpNewScenery _aslauncher_scenery)
  (Utilities|FlowControl|Sequence
    (:then_0
      (bind _aslauncher_target_box (Utilities|Casting|CastToLauncherTargetBox (Variables|/Script/Engine.ChildActorComponent|GetChildActor (Variables|Default|GetLauncherTargetBox_CAC))))
      (Default|SetLaucherTarget (LocalVariables|GettmpNewScenery) _aslauncher_target_box))
    (:then_1
      (bind _astr_game_mode_base_bp (Utilities|Casting|CastToTR_GameMode_Base_BP (Game|GetGameMode)))
      (Variables|/Game/TargetRunner/Blueprints/DynamicScenery/LauncherScenery.LauncherScenery_C|SetDifficultyModifier (LocalVariables|GettmpNewScenery) (Default|DifficultyMultiplierforPlatform _astr_game_mode_base_bp self))
      (Default|InitfromPlatform (LocalVariables|GettmpNewScenery)))
    (:then_2
      (Utilities|Array|Add (Variables|Default|GetLaunchers) (Default|GetLauncher (LocalVariables|GettmpNewScenery)))
      (EventDispatchers|BindEventtoOnLauncherDone (Default|GetLauncher (LocalVariables|GettmpNewScenery)) (EventDispatchers|CreateEvent :!event Custom|OnLauncherDone)))))
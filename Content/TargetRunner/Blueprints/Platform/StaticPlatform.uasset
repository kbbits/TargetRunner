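; StaticPlatform is a grid platform that can place shootable triggers on its edges for neighboring proxy platforms.
; Shortly after BeginPlay, on authority only and if enabled, it queries the game state's grid manager for the four cardinal neighbors.
; For proxy neighbors, it spawns a trigger with that proxy as receiver, attaches it to the matching edge anchor and stores it.
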(event EventBeginPlay
  (|CallParentFunction)
  (Networking|SwitchHasAuthority
    (:Authority
      (Utilities|FlowControl|Delay 0.3)
      (if (Variables|Default|GetAddTriggersForProxyNeighbors)
        (CallFunction|AddTriggersforNeighbors)))))

(fn ConstructionScript
  (|CallParentFunction))

(fn AddTriggersforNeighbors
  (bind _returnvalue (Class|PlatformBase|GetGridCoordinates))
  (bind _astr_game_state_base (Utilities|Casting|CastToTR_GameState_Base (Game|GetGameState)))
  (for (_array_element _array_index) (Utilities|Array|MakeArray (+ _returnvalue "(X=1.000000,Y=0.000000)") (+ _returnvalue "(X=-1.000000,Y=0.000000)") (+ _returnvalue "(X=0.000000,Y=1.000000)") (+ _returnvalue "(X=0.000000,Y=-1.000000)"))
    (bind (_found_ _foundplatform) (Default|GetPlatformonGrid (Variables|/Game/TargetRunner/Blueprints/Game/TR_GameState_Base.TR_GameState_Base_C|GetCurrentGridManager _astr_game_state_base) _array_element))
    (if _found_
      (bind _asplatform_proxy_base (Utilities|Casting|CastToPlatformProxy_Base _foundplatform))
      (bind _returnvalue_2 (Game|SpawnActorfromClass "/Game/TargetRunner/Blueprints/Shootables/Triggers/ShootablePlatformTrigger_Base.ShootablePlatformTrigger_Base_C" (Math|Transform|MakeTransform (.Location (Math|Transform|BreakTransform (Transformation|GetWorldTransform (Utilities|Select :Index _array_index :Option%200 (Variables|Default|GetNorthEdgeAnchor) :Option%201 (Variables|Default|GetSouthEdgeAnchor) :Option%202 (Variables|Default|GetEastEdgeAnchor) :Option%203 (Variables|Default|GetWestEdgeAnchor))))) (.Rotation (Math|Transform|BreakTransform (Transformation|GetWorldTransform (Utilities|Select :Index _array_index :Option%200 (Variables|Default|GetNorthEdgeAnchor) :Option%201 (Variables|Default|GetSouthEdgeAnchor) :Option%202 (Variables|Default|GetEastEdgeAnchor) :Option%203 (Variables|Default|GetWestEdgeAnchor)))))) "AdjustIfPossibleButAlwaysSpawn" self _asplatform_proxy_base 0)) ; Spawn trigger for this neighbor.
      (Utilities|Array|Add (Variables|Default|GetMyTriggers) _returnvalue_2)
      (Variables|/Game/TargetRunner/Blueprints/Shootables/Triggers/ShootablePlatformTrigger_Base.ShootablePlatformTrigger_Base_C|SetTriggerState _returnvalue_2 "NewEnumerator1")
      (Transformation|AttachComponentToComponent _returnvalue_2 (Utilities|Select :Index _array_index :Option%200 (Variables|Default|GetNorthEdgeAnchor) :Option%201 (Variables|Default|GetSouthEdgeAnchor) :Option%202 (Variables|Default|GetEastEdgeAnchor) :Option%203 (Variables|Default|GetWestEdgeAnchor)) "None" "SnapToTarget" "SnapToTarget" "KeepWorld" true))))
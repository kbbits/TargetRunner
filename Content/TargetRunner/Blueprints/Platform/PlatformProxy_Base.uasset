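; PlatformProxy_Base is a base platform proxy that stands in at a grid position until it is triggered and replaced.
; On ActivateTriggerable, the server casts the instigator to Character and gets its TR_PlayerController_Base.
; It passes the proxy's grid coordinates to that controller's ReplaceProxyPlatform.
; An unconnected path that would call the game state's CurrentGridManager directly remains in the graph but never runs.
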(event EventActivateTriggerable
  (params (Instigator :type Actor%20Object%20Reference))
  (if (Networking|IsServer)
    (bind _ascharacter (Utilities|Casting|CastToCharacter Instigator))
    (bind _astr_player_controller_base (Utilities|Casting|CastToTR_PlayerController_Base (Pawn|GetController _ascharacter)))
    (bind _returnvalue (Class|PlatformBase|GetGridCoordinates))
    (Default|ReplaceProxyPlatform _astr_player_controller_base _returnvalue)))

(fn ConstructionScript)
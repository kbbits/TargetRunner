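; Room platform grid manager that populates a level from its room grid template with rooms, contents and enemies.
; Self-calling delayed events stagger each phase, handling the start room first for rooms and contents, then notify platforms on completion.
; Enemies spawn at random navigable points, skipping start, end and blackout rooms.
; Level template tier drives enemy count and randomized class, difficulty sets enemy level, and rooms beside the exit are tougher.
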(event Custom|SpawnContentsDelayed
  (bind _roomgridtemplate (Variables|Default|GetRoomGridTemplate))
  (bind _startcells (Utilities|Struct|BreakRoomGridTemplate _roomgridtemplate))
  (bind _output (Utilities|Array|Get(acopy) _startcells))
  ;[1 1 1] Spawn Contents Delayed
  (if (>= (Utilities|Array|LastIndex (Variables|Default|GetRoomSpawnCoords)) 0)
    (bind _returnvalue (Class|PlatformGridMgr|GetPlatforminGrid (Utilities|Array|Get(acopy) (Variables|Default|GetRoomSpawnCoords) (Utilities|Array|LastIndex (Variables|Default|GetRoomSpawnCoords)))))
    (bind _asroom_platform_base (Utilities|Casting|CastToRoomPlatformBase _returnvalue))
    (Class|RoomPlatformBase|SpawnContents _asroom_platform_base)
    (Utilities|Array|RemoveIndex (Variables|Default|GetRoomSpawnCoords) (Utilities|Array|LastIndex (Variables|Default|GetRoomSpawnCoords)))
    (if (> (Utilities|Array|Length (Variables|Default|GetRoomSpawnCoords)) 0)
      (Utilities|FlowControl|Delay 0.05)
      (CallFunction|SpawnContentsDelayed)
      (else
        (CallFunction|SpawnEnemiesDelayed) ; Move on to spawning enemies
      ))
    (else
      (Utilities|FlowControl|DoOnce false
        (:Completed
          (if (== (Utilities|Array|Length (Variables|Default|GetRoomSpawnCoords)) 0)
            (Variables|Default|SetRoomSpawnCoords (.RoomCoords (Class|RoomFunctionLibrary|GetAllRoomTemplateCoords (Variables|Default|GetRoomGridTemplate) true)))
            (if (> (Utilities|Array|Length (Variables|Default|GetRoomSpawnCoords)) 0)
              (Utilities|FlowControl|Sequence
                (:then_0
                  (if (Utilities|Array|IsValidIndex _startcells) ; Put start room at end of array
                    (bind _returnvalue_2 (Utilities|Array|RemoveItem (Variables|Default|GetRoomSpawnCoords) _output))
                    (if _returnvalue_2
                      (Utilities|Array|Insert (Variables|Default|GetRoomSpawnCoords) _output (+ (Utilities|Array|LastIndex (Variables|Default|GetRoomSpawnCoords)) 1)))))
                (:then_1
                  (Utilities|FlowControl|Delay 0.05)
                  (CallFunction|SpawnContentsDelayed))))))))))

(event Custom|SpawnEnemiesDelayed
  (bind _roomgridtemplate (Variables|Default|GetRoomGridTemplate))
  (bind (_roomcoords _roomtemplates) (Class|RoomFunctionLibrary|GetRoomTemplateGridasArrays _roomgridtemplate true))
  ;[1 1 1] Spawn Enemies Delayed
  (Variables|Default|SetEnemyRoomSpawnIndex 0)
  (Variables|Default|SetEnemyRoomSpawnCoords _roomcoords)
  (Variables|Default|SetEnemyRoomTemplates _roomtemplates)
  (Utilities|FlowControl|Delay 0.0625)
  (CallFunction|SpawnEnemyDelayed))

(event Custom|SpawnRoomsDelayed
  (bind _roomgridtemplate (Variables|Default|GetRoomGridTemplate))
  (bind _startcells (Utilities|Struct|BreakRoomGridTemplate _roomgridtemplate))
  (bind _output (Utilities|Array|Get(acopy) _startcells))
  ;[1 1 1] Spawn Rooms Delayed
  (if (>= (Utilities|Array|LastIndex (Variables|Default|GetRoomSpawnCoords)) 0)
    (Class|RoomPlatformGridMgr|SpawnRoom (Utilities|Array|Get(acopy) (Variables|Default|GetRoomSpawnCoords) (Utilities|Array|LastIndex (Variables|Default|GetRoomSpawnCoords))))
    (Utilities|Array|RemoveIndex (Variables|Default|GetRoomSpawnCoords) (Utilities|Array|LastIndex (Variables|Default|GetRoomSpawnCoords)))
    (if (> (Utilities|Array|Length (Variables|Default|GetRoomSpawnCoords)) 0)
      (Utilities|FlowControl|Delay 0.0625)
      (CallFunction|SpawnRoomsDelayed)
      (else
        (Utilities|FlowControl|Delay 1.0)
        (CallFunction|SpawnContentsDelayed)))
    (else
      (Utilities|FlowControl|DoOnce false
        (:Completed
          (if (== (Utilities|Array|Length (Variables|Default|GetRoomSpawnCoords)) 0)
            (Variables|Default|SetRoomSpawnCoords (.RoomCoords (Class|RoomFunctionLibrary|GetAllRoomTemplateCoords (Variables|Default|GetRoomGridTemplate) true)))
            (if (> (Utilities|Array|Length (Variables|Default|GetRoomSpawnCoords)) 0)
              (Utilities|FlowControl|Sequence
                (:then_0
                  (if (Utilities|Array|IsValidIndex _startcells) ; Put start room at end of array
                    (bind _returnvalue (Utilities|Array|RemoveItem (Variables|Default|GetRoomSpawnCoords) _output))
                    (if _returnvalue
                      (Utilities|Array|Insert (Variables|Default|GetRoomSpawnCoords) _output (+ (Utilities|Array|LastIndex (Variables|Default|GetRoomSpawnCoords)) 1)))))
                (:then_1
                  (Utilities|FlowControl|Delay 0.05)
                  (CallFunction|SpawnRoomsDelayed))))))))))

(event Custom|SpawnEnemyDelayed
  (bind _enemyroomtemplates (Variables|Default|GetEnemyRoomTemplates))
  (bind _enemyroomspawnindex (Variables|Default|GetEnemyRoomSpawnIndex))
  (bind _enemyroomspawncoords (Variables|Default|GetEnemyRoomSpawnCoords))
  (bind _enemyroomspawnindex_2 (Variables|Default|GetEnemyRoomSpawnIndex))
  (bind _enemyroomspawnindex_3 (Variables|Default|GetEnemyRoomSpawnIndex))
  (bind _gridcellworldsize (Variables|Default|GetGridCellWorldSize))
  (bind _returnvalue (* _gridcellworldsize 0.45))
  (bind _returnvalue_2 (* _gridcellworldsize -0.45))
  (bind _output (Utilities|Array|Get(acopy) _enemyroomtemplates _enemyroomspawnindex_2))
  (bind _output_2 (Utilities|Array|Get(acopy) _enemyroomspawncoords _enemyroomspawnindex_3))
  (bind (_northwall _eastwall _southwall _westwall _group _bisblackout _bisinterior _distancetostart _distancetoend _distancetoshortestpath _resources) (Utilities|Struct|BreakRoomTemplate _output))
  (bind _returnvalue_3 (Class|PlatformGridMgr|GetGridCellWorldTransform _output_2))
  (bind _returnvalue_4 (Math|Random|RandomFloatinRange _returnvalue_2 _returnvalue))
  (bind _location (Math|Transform|BreakTransform _returnvalue_3))
  (bind _returnvalue_5 (Math|Vector|MakeVector _returnvalue_4 _returnvalue_4 1e+01))
  (bind _returnvalue_6 (+ _location _returnvalue_5))
  (bind (_randomlocation _returnvalue_7) (Class|NavigationSystemV1|GetRandomPointinNavigableRadius _returnvalue_6 2e+02 0 0))
  ;[1 1 1] Spawn Enemies Delayed
  (if (and (> (Utilities|Array|Length _enemyroomtemplates) _enemyroomspawnindex) (Utilities|Array|IsValidIndex _enemyroomtemplates _enemyroomspawnindex))
    (if (Math|Boolean|ANDBoolean (not _bisblackout) (> _distancetostart 0) (> _distancetoend 0))
      (if (> (Variables|Default|GetEnemySpawnCount) 0)
        _
        (else
          (bind _astr_game_mode_rooms_bp (Utilities|Casting|CastToTR_GameModeRooms_BP (Game|GetGameMode))
            (:then
              (Variables|Default|SetEnemySpawnCount (Math|Integer|SelectInt (Math|Float|Truncate (+ (.Tier (Utilities|Struct|BreakLevelTemplate (Class|TRGameMode|GetLevelTemplate _astr_game_mode_rooms_bp))) 2.0)) (Math|Random|RandomIntegerinRange 1 (Math|Float|Truncate (+ (.Tier (Utilities|Struct|BreakLevelTemplate (Class|TRGameMode|GetLevelTemplate _astr_game_mode_rooms_bp))) 1.0))) (== _distancetoend 1))))
            (:CastFailed
              _))))
      (if _returnvalue_7
        (bind _returnvalue_8 (Game|SpawnActorfromClass (CallFunction|GetEnemyTypeforRoom _output_2) (Math|Transform|MakeTransform _randomlocation (Math|Rotator|MakeRotator 0.0 0.0 (Math|Random|RandomFloatinRange -1.8e+02 1.8e+02))) "AdjustIfPossibleButAlwaysSpawn" 0 (CallFunction|GetEnemyLevelforRoom _output_2) (Class|ResourceFunctionLibrary|MultiplyResourceQuantity _resources 0.1 true) 0 0)))
      (bind _result (Math|Integer|DecrementInt (Variables|Default|GetEnemySpawnCount))
        (:%20%20
          (if (<= _result 0)
            (Math|Integer|IncrementInt (Variables|Default|GetEnemyRoomSpawnIndex)
              (:%20%20
                _)))
          (if (< (Variables|Default|GetEnemyRoomSpawnIndex) (Utilities|Array|Length (Variables|Default|GetEnemyRoomTemplates)))
            (Utilities|FlowControl|Delay (Math|Random|RandomFloatinRange 0.0625 0.125))
            (CallFunction|SpawnEnemyDelayed)
            (else
              ;;[1 1 1] Spawns Finished
              (Class|RoomPlatformGridMgr|SpawnsFinished)))))
      (else
        (Math|Integer|IncrementInt (Variables|Default|GetEnemyRoomSpawnIndex)
          (:%20%20
            (CallFunction|SpawnEnemyDelayed)))))
    (else
      ;;[1 1 1] Spawns Finished
      (Class|RoomPlatformGridMgr|SpawnsFinished))))

(event EventBeginPlay
  ;[1 1 1] BeginPlay
)

(event EventSpawnsFinished
  ;[1 1 1] Spawns Finished
  (|CallParentFunction)
  (Utilities|Array|Clear (Variables|Default|GetRoomSpawnCoords))
  (Utilities|Array|Clear (Variables|Default|GetEnemyRoomSpawnCoords))
  (Utilities|Array|Clear (Variables|Default|GetEnemyRoomTemplates))
  (Utilities|FlowControl|Sequence
    (:then_0
      (for _array_element (.RoomCoords (Class|RoomFunctionLibrary|GetAllRoomTemplateCoords (Variables|Default|GetRoomGridTemplate) true))
        (bind _returnvalue (Class|PlatformGridMgr|GetPlatforminGrid _array_element))
        (bind _asroom_platform_base_bp (Utilities|Casting|CastToRoomPlatformBase_BP _returnvalue))
        (Default|SpawnsFinishedBP _asroom_platform_base_bp)))
    (:then_1
      (Default|CallOnSpawnRoomComplete))))

(fn ConstructionScript)

(fn GetEnemyTypeforRoom
  (params (RoomCoords :type Vector%202D%20Structure))
  (bind _astr_game_mode_rooms_bp (Utilities|Casting|CastToTR_GameModeRooms_BP (Game|GetGameMode))
    (:then
      (bind _output_get (LocalVariables|SettmpSelectedTier (Math|Integer|Max(Integer) 1 (Math|Integer|SelectInt (- (Math|Float|Truncate (.Tier (Utilities|Struct|BreakLevelTemplate (Class|TRGameMode|GetLevelTemplate _astr_game_mode_rooms_bp)))) 1) (Math|Integer|SelectInt (+ (Math|Float|Truncate (.Tier (Utilities|Struct|BreakLevelTemplate (Class|TRGameMode|GetLevelTemplate _astr_game_mode_rooms_bp)))) 1) (Math|Float|Truncate (.Tier (Utilities|Struct|BreakLevelTemplate (Class|TRGameMode|GetLevelTemplate _astr_game_mode_rooms_bp)))) (< (Math|Random|RandomFloat) 0.1)) (< (Math|Random|RandomFloat) 0.25)))))
      (bind _enemyclasses (Class|TRGameMode|GetEnemyMobsforTier _astr_game_mode_rooms_bp _output_get))
      (bind _output_get_2 (LocalVariables|SettmpMobClasses _enemyclasses))
      (if (> (Utilities|Array|Length _output_get_2) 0)
        (bind _output_get_3 (LocalVariables|SettmpSelectedClass (Utilities|Array|Get(acopy) (LocalVariables|GettmpMobClasses) (Math|Random|RandomIntegerinRange 0 (Utilities|Array|LastIndex (LocalVariables|GettmpMobClasses))))))
        (bind _astrenemy_character_base_bp (Utilities|Casting|CastToTREnemyCharacterBase_BPClass _output_get_3)
          (:then
            (return _astrenemy_character_base_bp))
          (:CastFailed
            (Development|PrintString (Utilities|String|Append "Enemy is not TREnemyCharacterBase_BP" (Utilities|GetClassDisplayName (LocalVariables|GettmpSelectedClass))) true true "(R=1.000000,G=0.000000,B=0.024068,A=1.000000)" 1e+01)
            (return (LocalVariables|GetDefaultMobClass))))
        (else
          (Development|PrintString (Utilities|String|Append "No enemy mob found in tier " (Utilities|String|ToString(Integer) (LocalVariables|GettmpSelectedTier))) true true "(R=1.000000,G=0.000000,B=0.024068,A=1.000000)" 1e+01)
          (return (LocalVariables|GetDefaultMobClass)))))
    (:CastFailed
      (return (LocalVariables|GetDefaultMobClass)))))

(fn GetEnemyLevelforRoom
  (params (RoomCoords :type Vector%202D%20Structure))
  (LocalVariables|SettmpRoomRef (Class|RoomPlatformGridMgr|GetRoominGrid RoomCoords))
  (Utilities|FlowControl|Sequence
    (:then_0
      (bind _astr_game_mode_rooms_bp (Utilities|Casting|CastToTR_GameModeRooms_BP (Game|GetGameMode))
        (:then
          (LocalVariables|SettmpLevel (.DifficultyLevel (Utilities|Struct|BreakLevelTemplate (Class|TRGameMode|GetLevelTemplate _astr_game_mode_rooms_bp)))))
        (:CastFailed
          (LocalVariables|SettmpLevel 1))))
    (:then_1
      (Utilities|IsValid (LocalVariables|GettmpRoomRef)
        (:Is%20Valid
          (if (== (.DistanceToEnd (Utilities|Struct|BreakRoomTemplate (Variables|/Script/TargetRunner.RoomPlatformBase|GetRoomTemplate (LocalVariables|GettmpRoomRef)))) 1) ; Rooms near exit
            (LocalVariables|SettmpLevel (+ (LocalVariables|GettmpLevel) (Math|Integer|SelectInt 2 (Math|Integer|SelectInt 1 0 (< (Math|Random|RandomFloat) 0.5)) (< (Math|Random|RandomFloat) 0.25))))))))
    (:then_2
      (return (LocalVariables|GettmpLevel)))))
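; RoomComponentActor_BP is a short-lived room piece whose instanced static meshes are handed to the grid manager at BeginPlay on the server.
; It first randomly swaps a percentage of two block types to alt-mesh components, removing instances in reverse index order.
; It then clears every ISM component and respawns each instance at its world transform through the game mode's GridManager, using the mesh and first material.
; The actor destroys itself after a short delay.
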(event EventBeginPlay
  (Networking|SwitchHasAuthority
    (:Authority
      (CallFunction|ApplyAltMeshes)
      (CallFunction|MoveISMstoGridManager)
      (Utilities|FlowControl|Delay 0.2)
      (Actor|DestroyActor))))

(fn ConstructionScript)

(fn ApplyAltMeshes
  (if (> (Variables|Default|GetAltMeshPercent) 0.0)
    (Utilities|FlowControl|Sequence
      (:then_0
        (CallFunction|TrySwaptoAltISMComponent (Variables|Default|GetBlockType_1_ISM) (Variables|Default|GetBlockType_1Alt_ISM)))
      (:then_1
        (CallFunction|TrySwaptoAltISMComponent (Variables|Default|GetBlockType_2_ISM) (Variables|Default|GetBlockType_2Alt_ISM))))))

(fn MoveISMstoGridManager
  (Networking|SwitchHasAuthority
    (:Authority
      (bind _astr_game_mode_base_bp (Utilities|Casting|CastToTR_GameModeBase_BP (Game|GetGameMode)))
      (LocalVariables|SettmpGameMode _astr_game_mode_base_bp)
      (bind _returnvalue (Class|TRGameMode|GetGridManager (LocalVariables|GettmpGameMode)))
      (LocalVariables|SettmpGridManager _returnvalue)
      (bind _output_get (LocalVariables|SettmpAllISMComps (Actor|GetComponentsByClass "/Script/Engine.InstancedStaticMeshComponent")))
      (for _array_element _output_get
        (LocalVariables|SettmpISMComp _array_element)
        (Utilities|IsValid (LocalVariables|GettmpISMComp)
          (:Is%20Valid
            (Utilities|Array|Clear (LocalVariables|GettmpAllTransforms))
            (Development|PrintString (Utilities|String|Append "Moving " (Utilities|String|ToString(Integer) (Components|InstancedStaticMesh|GetInstanceCount (LocalVariables|GettmpISMComp))) " ISMs"))
            (for _index (range 0 (- (Components|InstancedStaticMesh|GetInstanceCount (LocalVariables|GettmpISMComp)) 1))
              (if (.ReturnValue (Components|InstancedStaticMesh|GetInstanceTransform (LocalVariables|GettmpISMComp) _index true))
                (Utilities|Array|Add (LocalVariables|GettmpAllTransforms) (.OutInstanceTransform (Components|InstancedStaticMesh|GetInstanceTransform (LocalVariables|GettmpISMComp) _index true)))
                (else
                  (Development|PrintString "MoveISMsToGridManager - Error getting instance transform" true true "(R=1.000000,G=0.000000,B=0.007402,A=1.000000)"))))
            (Components|InstancedStaticMesh|ClearInstances (LocalVariables|GettmpISMComp))
            (Development|PrintString (Utilities|String|Append "Transforms to move: " (Utilities|String|ToString(Integer) (Utilities|Array|Length (LocalVariables|GettmpAllTransforms)))))
            (for _array_element_2 (LocalVariables|GettmpAllTransforms)
              (LocalVariables|SettmpTransform _array_element_2)
              (bind _returnvalue_2 (Class|PlatformGridMgr|SpawnISM (LocalVariables|GettmpGridManager) (Utilities|ResolveSoftReference (Variables|/Script/Engine.StaticMeshComponent|GetStaticMesh (LocalVariables|GettmpISMComp))) (Rendering|Material|GetMaterial (LocalVariables|GettmpISMComp) 0) (LocalVariables|GettmpTransform)))
              (if (< _returnvalue_2 0)
                (Development|PrintString "Error moving ISM to grid" true true "(R=1.000000,G=0.013641,B=0.000000,A=1.000000)")))))))))

(fn TrySwaptoAltISMComponent
  (params (OriginalISMComponent :type Instanced%20Static%20Mesh%20Component%20Object%20Reference) (AltISMComponent :type Instanced%20Static%20Mesh%20Component%20Object%20Reference))
  (LocalVariables|SettmpOriginalISMComponent OriginalISMComponent)
  (LocalVariables|SettmpAltISMComponent AltISMComponent)
  (Utilities|Array|Clear (LocalVariables|GettmpRemovedIndexes))
  (Utilities|Array|Clear (LocalVariables|GettmpAltTransforms))
  (for _index (range 0 (- (Components|InstancedStaticMesh|GetInstanceCount (LocalVariables|GettmpOriginalISMComponent)) 1))
    (if (<= (Math|Random|RandomFloat) (Variables|Default|GetAltMeshPercent))
      (Utilities|Array|Add (LocalVariables|GettmpRemovedIndexes) _index)
      (Utilities|Array|Add (LocalVariables|GettmpAltTransforms) (.OutInstanceTransform (Components|InstancedStaticMesh|GetInstanceTransform (LocalVariables|GettmpOriginalISMComponent) _index false)))))
  (bind _arrayelement (Utilities|Array|ReverseforEachLoop (LocalVariables|GettmpRemovedIndexes))
    (:LoopBody
      (Class|InstancedStaticMeshComponent|RemoveInstance (LocalVariables|GettmpOriginalISMComponent) _arrayelement))
    (:Completed
      (for _array_element (LocalVariables|GettmpAltTransforms)
        (Components|InstancedStaticMesh|AddInstance (LocalVariables|GettmpAltISMComponent) _array_element)))))
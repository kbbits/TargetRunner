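; Manages the Target Runner platform grid, registering existing platforms at BeginPlay and then itself with the game mode.
; On authority, spawns proxy, static or dynamic platforms within grid extents, replacing removable occupants and initializing and generating dynamic ones.
; Places key markers and an exit marker requiring them, and provides neighbor, marker and seeded random-cell queries.
; Pools meshes into replicated instanced static mesh components, one per mesh.
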(event Custom|ReplaceProxyPlatform
  (params (GridCoords :type Vector%202D%20Structure))
  ;[1 1 1] ReplaceProxyPlatform
  (bind (_found _returnvalue) (Class|PlatformGridMgr|GetPlatforminGrid GridCoords))
  (if _found
    (Utilities|Casting|CastToPlatformProxy_Base _returnvalue)
    (bind _success (Class|PlatformGridMgr|RemovePlatformfromGrid GridCoords))
    (if _success
      (CallFunction|AddPlatform "NewEnumerator2" GridCoords))))

(event Custom|OnAddISM
  (params (Mesh :type Static%20Mesh%20Object%20Reference) (WorldTransform :type Transform) (Material :type Material%20Interface%20Object%20Reference))
  ;[1 1 1] Add ISM
  (Variables|Default|SettmpISMComp 0)
  (bind _array_element (Utilities|Array|ForEachLoopwithBreak (Variables|Default|GetISM_Components) :!label _label)
    (:LoopBody
      (if (== (Variables|/Script/Engine.StaticMeshComponent|GetStaticMesh _array_element) Mesh)
        (Variables|Default|SettmpISMComp _array_element)
        (goto _label Break)))
    (:Completed
      (Utilities|IsValid (Variables|Default|GettmpISMComp)
        (:Is%20Valid
          _)
        (:Is%20Not%20Valid
          (bind _returnvalue (AddComponent|AddInstancedStaticMeshComponent false (Math|Transform|MakeTransform "0, 0, 0")))
          (bind _output_get (Variables|Default|SettmpISMComp _returnvalue))
          (Utilities|Array|Add (Variables|Default|GetISM_Components) _output_get)
          (Class|ActorComponent|SetIsReplicated (Variables|Default|GettmpISMComp) true)
          (Components|StaticMesh|SetStaticMesh (Variables|Default|GettmpISMComp) Mesh)
          (Rendering|Material|SetMaterial (Variables|Default|GettmpISMComp) 0 Material)
          (Class|PrimitiveComponent|SetCullDistance (Variables|Default|GettmpISMComp) 0.0)
          (Collision|SetCollisionObjectType (Variables|Default|GettmpISMComp) "ECC_WorldDynamic")))
      (Class|InstancedStaticMeshComponent|AddInstanceWorldSpace (Variables|Default|GettmpISMComp) WorldTransform))))

(event Custom|PlaceExitMarker
  (params (ExitMarkerActorClass :type Exit%20Marker%20Base%20BP%20Class%20Reference) (GridCoords :type Vector%202D%20Structure))
  ;[1 1 1] Place Exit and Key Markers
  (bind _returnvalue (Game|SpawnActorfromClass ExitMarkerActorClass (Math|Transform|MakeTransform (CallFunction|GetGridCellWorldLocationBP GridCoords)) "AdjustIfPossibleButAlwaysSpawn" self (Variables|Default|GetExitKeyMarkerActors) GridCoords 0))
  (Variables|Default|SetExitMarkerActor _returnvalue))

(event Custom|PlaceKeyMarker
  (params (KeyMarkerClass :type Exit%20Key%20Marker%20Base%20BP%20Class%20Reference) (GridCoords :type Vector%202D%20Structure))
  ;[1 1 1] Place Exit and Key Markers
  (bind _returnvalue (Game|SpawnActorfromClass KeyMarkerClass (Math|Transform|MakeTransform (CallFunction|GetGridCellWorldLocationBP GridCoords)) "AdjustIfPossibleButAlwaysSpawn" self GridCoords 0))
  (Utilities|Array|Add (Variables|Default|GetExitKeyMarkerActors) _returnvalue))

(event EventBeginPlay
  ;[1 1 1] Begin Play
  (Class|PlatformGridMgr|FillGridfromExistingPlatforms)
  (Utilities|FlowControl|Delay 0.2)
  (bind _astr_game_mode (Utilities|Casting|CastToTR_GameMode (Game|GetGameMode)))
  (Class|TRGameMode|InitGridManager _astr_game_mode self))

(fn ConstructionScript)

(fn AddPlatform
  (params (PlatformType :type PlatformTypes_Enum%20Enum :default "NewEnumerator0") (GridCoords :type Vector%202D%20Structure))
  (bind (_x _y) (Math|Vector2D|BreakVector2D GridCoords))
  (bind _worldlocation (CallFunction|GetGridCellWorldLocationBP GridCoords))
  (bind (_x_2 _y_2) (Math|Vector2D|BreakVector2D GridCoords))
  (bind _self self)
  (bind _gridcellworldsize (Variables|Default|GetGridCellWorldSize))
  (bind _returnvalue (Math|Float|Truncate _x))
  (bind _returnvalue_2 (Math|Float|Truncate _y))
  (bind _returnvalue_3 (Math|Transform|MakeTransform _worldlocation))
  (Networking|SwitchHasAuthority
    (:Authority
      (Utilities|FlowControl|Sequence
        (:then_0
          (if (not (and (Math|Float|InRange(Float) _x_2 (Math|Conversions|ToFloat(Integer) (Variables|Default|GetGridExtentMinX)) (Math|Conversions|ToFloat(Integer) (Variables|Default|GetGridExtentMaxX))) (Math|Float|InRange(Float) _y_2 (Math|Conversions|ToFloat(Integer) (Variables|Default|GetGridExtentMinY)) (Math|Conversions|ToFloat(Integer) (Variables|Default|GetGridExtentMaxY)))))
            (return false 0) ; Do nothing if out of GridExtent
          ))
        (:then_1
          (bind (_found _returnvalue_4) (Class|PlatformGridMgr|GetPlatforminGrid GridCoords))
          (if _found
            (Utilities|IsValid _returnvalue_4
              (:Is%20Valid
                (bind _success (Class|PlatformGridMgr|RemovePlatformfromGrid (Class|PlatformBase|GetGridCoordinates _returnvalue_4)))
                (if (not _success)
                  (return false 0) ; Do nothing and return false if the existing platform cannot be removed
                )))))
        (:then_2
          (switch Utilities|FlowControl|Switch|SwitchonPlatformTypes_Enum PlatformType
            (:NewEnumerator0
              (bind _returnvalue_5 (Game|SpawnActorfromClass "/Game/TargetRunner/Blueprints/Platform/PlatformProxy_Base.PlatformProxy_Base_C" _returnvalue_3 "Undefined" _self _gridcellworldsize _returnvalue _returnvalue_2 0))
              (LocalVariables|SettmpNewPlatform _returnvalue_5))
            (:NewEnumerator1
              (bind _returnvalue_6 (Game|SpawnActorfromClass "/Game/TargetRunner/Blueprints/Platform/StaticPlatform.StaticPlatform_C" _returnvalue_3 "Undefined" _self _gridcellworldsize _returnvalue _returnvalue_2 0))
              (LocalVariables|SettmpNewPlatform _returnvalue_6))
            (:NewEnumerator2
              (bind _returnvalue_7 (Game|SpawnActorfromClass "/Game/TargetRunner/Blueprints/Platform/DynamicPlatform.DynamicPlatform_C" _returnvalue_3 "Undefined" _self _gridcellworldsize _returnvalue _returnvalue_2 0))
              (LocalVariables|SettmpNewPlatform _returnvalue_7)))
          (Class|PlatformGridMgr|AddPlatformtoGridMap (LocalVariables|GettmpNewPlatform))
          (bind _asdynamic_platform (Utilities|Casting|CastToDynamicPlatform (LocalVariables|GettmpNewPlatform))
            (:then
              ;[1 1 1] If it's a dynamic platform, set it up and generate.
              (bind _astr_game_mode_platforms_bp (Utilities|Casting|CastToTR_GameModePlatforms_BP (Game|GetGameMode)))
              (Default|InitDynamicPlatform _astr_game_mode_platforms_bp _asdynamic_platform)
              (Default|OnGenerate _asdynamic_platform))
            (:CastFailed
              _))
          (return true (LocalVariables|GettmpNewPlatform)))))))

(fn GetGridCellWorldLocationBP
  (params (GridCoords :type Vector%202D%20Structure))
  (bind _returnvalue (Transformation|GetActorLocation))
  (bind _gridcellworldsize (Variables|Default|GetGridCellWorldSize))
  (bind (_x _y) (Math|Vector|BreakVector _returnvalue))
  (bind _returnvalue_2 (* GridCoords _gridcellworldsize))
  (bind (_x_2 _y_2) (Math|Vector2D|BreakVector2D _returnvalue_2))
  (return (Math|Vector|MakeVector (+ _x_2 _x) (+ _y_2 _y) (Variables|Default|GetDefaultPlatformZ))))

(fn GetNeighborsonGrid
  (params (GridCoords :type Vector%202D%20Structure))
  (bind _foundplatforms (CallFunction|GetPlatformsonGrid (Utilities|Array|MakeArray (+ GridCoords "(X=1.000000,Y=0.000000)") (+ GridCoords "(X=-1.000000,Y=0.000000)") (+ GridCoords "(X=0.000000,Y=1.000000)") (+ GridCoords "(X=0.000000,Y=-1.000000)"))))
  (return _foundplatforms))

(fn GetPlatformsonGrid
  (params (GridCoords :type Array%20of%20Vector%202D%20Structures))
  (LocalVariables|SettmpCoords GridCoords)
  (LocalVariables|SettmpFoundPlatforms (Utilities|Array|MakeArray))
  (Utilities|FlowControl|Sequence
    (:then_0
      (for _array_element (LocalVariables|GettmpCoords)
        (bind (_found _returnvalue) (Class|PlatformGridMgr|GetPlatforminGrid _array_element))
        (if _found
          (Utilities|Array|Add (LocalVariables|GettmpFoundPlatforms) _returnvalue))))
    (:then_1
      (return (> (Utilities|Array|Length (LocalVariables|GettmpFoundPlatforms)) 0) (LocalVariables|GettmpFoundPlatforms)))))

(fn RemovePlatformfromGridBP
  (params (GridCoords :type Vector%202D%20Structure))
  (bind (_found _returnvalue) (Class|PlatformGridMgr|GetPlatforminGrid GridCoords))
  (if _found
    (bind _output_get (LocalVariables|SettmpRemovedPlatform _returnvalue))
    (if (Variables|/Script/TargetRunner.PlatformBase|GetbCanRemoveDynamic _output_get)
      (if (.ReturnValue (Utilities|Map|Find (Variables|Default|GetPlatformGridMap) (Variables|/Script/TargetRunner.PlatformBase|GetGridX (LocalVariables|GettmpRemovedPlatform))))
        (Utilities|Map|Remove (Utilities|Struct|BreakPlatformGridRow (.Value (Utilities|Map|Find (Variables|Default|GetPlatformGridMap) (Variables|/Script/TargetRunner.PlatformBase|GetGridX (LocalVariables|GettmpRemovedPlatform))))) (Variables|/Script/TargetRunner.PlatformBase|GetGridY (LocalVariables|GettmpRemovedPlatform))))
      (Actor|DestroyActor (LocalVariables|GettmpRemovedPlatform))
      (return true)
      (else
        (return false)))
    (else
      (return true))))

(fn RandomCellinGrid
  (params (RandStream :type Random%20Stream%20Structure%20%28by%20ref%29))
  (bind _output_get (LocalVariables|SettmpCoords (Math|Vector2D|MakeVector2D (Math|Conversions|ToFloat(Integer) (Math|Random|RandomIntegerinRangefromStream (Variables|Default|GetGridExtentMinX) (Variables|Default|GetGridExtentMaxX) RandStream)) (Math|Conversions|ToFloat(Integer) (Math|Random|RandomIntegerinRangefromStream (Variables|Default|GetGridExtentMinY) (Variables|Default|GetGridExtentMaxY) RandStream)))))
  (return _output_get))

(fn RandomEmptyCellinGrid
  (params (MaxTries :type Integer) (RandStream :type Random%20Stream%20Structure%20%28by%20ref%29))
  (Utilities|FlowControl|ForLoopwithBreak 1 MaxTries :!label _label
    (:LoopBody
      (bind _gridcoords (CallFunction|RandomCellinGrid RandStream))
      (bind _output_get (LocalVariables|SettmpGridCoords _gridcoords))
      (bind _found (Class|PlatformGridMgr|GetPlatforminGrid _output_get))
      (if (not _found)
        (LocalVariables|SettmpFoundEmptyCell true)
        (bind _array_element (Utilities|Array|ForEachLoopwithBreak (Variables|Default|GetExitKeyMarkerActors) :!label _label_2)
          (:LoopBody
            (if (Class|KismetMathLibrary|EqualExactlyVector2DVector2D (LocalVariables|GettmpGridCoords) (Variables|/Game/TargetRunner/Blueprints/World/ExitKeys/ExitKeyMarker_Base_BP.ExitKeyMarker_Base_BP_C|GetGridCoordinates _array_element))
              (LocalVariables|SettmpFoundEmptyCell false)
              (goto _label_2 Break)))
          (:Completed
            (if (LocalVariables|GettmpFoundEmptyCell)
              (goto _label Break)
              (else
                (LocalVariables|SettmpGridCoords "")))))
        (else
          (LocalVariables|SettmpGridCoords ""))))
    (:Completed
      (return (LocalVariables|GettmpFoundEmptyCell) (LocalVariables|GettmpGridCoords)))))

(fn RandomEdgeCellinGrid
  (params (RandStream :type Random%20Stream%20Structure%20%28by%20ref%29))
  (bind _output_get (LocalVariables|SettmpRandStream RandStream))
  (if (Math|Random|RandomBoolfromStream _output_get) ; X edge or Y edge
    (LocalVariables|SettmpCoords (Utilities|Struct|MakeIntPoint (select (Math|Random|RandomBoolfromStream (LocalVariables|GettmpRandStream)) (Variables|Default|GetGridExtentMaxX) (Variables|Default|GetGridExtentMinX)) (Math|Random|RandomIntegerinRangefromStream (Variables|Default|GetGridExtentMinY) (Variables|Default|GetGridExtentMaxY) (LocalVariables|GettmpRandStream))))
    (else
      (LocalVariables|SettmpCoords (Utilities|Struct|MakeIntPoint (select (Math|Random|RandomBoolfromStream (LocalVariables|GettmpRandStream)) (Variables|Default|GetGridExtentMaxY) (Variables|Default|GetGridExtentMinY)) (Math|Random|RandomIntegerinRangefromStream (Variables|Default|GetGridExtentMinX) (Variables|Default|GetGridExtentMaxX) (LocalVariables|GettmpRandStream))))))
  (return (Math|Vector2D|MakeVector2D (Math|Conversions|ToFloat(Integer) (.X (Utilities|Struct|BreakIntPoint (LocalVariables|GettmpCoords)))) (Math|Conversions|ToFloat(Integer) (.Y (Utilities|Struct|BreakIntPoint (LocalVariables|GettmpCoords)))))))

(fn IsExitCell
  (params (GridCoords :type Vector%202D%20Structure))
  (return (Math|Vector|Equal(Vector) (Variables|/Game/TargetRunner/Blueprints/World/ExitMarkerBase_BP.ExitMarkerBase_BP_C|GetGridCoordinates (Variables|Default|GetExitMarkerActor)) GridCoords 0.001)))

(fn IsKeyCell
  (params (GridCoords :type Vector%202D%20Structure))
  (return (.Found (CallFunction|GetKeyMarkerinCell GridCoords))))

(fn GetKeyMarkerinCell
  (params (GridCoords :type Vector%202D%20Structure))
  (bind _array_element (Utilities|Array|ForEachLoopwithBreak (Variables|Default|GetExitKeyMarkerActors) :!label _label)
    (:LoopBody
      (if (Math|Vector|Equal(Vector) (Variables|/Game/TargetRunner/Blueprints/World/ExitKeys/ExitKeyMarker_Base_BP.ExitKeyMarker_Base_BP_C|GetGridCoordinates _array_element) GridCoords 0.0001)
        (LocalVariables|SettmpKeyMarker _array_element)
        (goto _label Break)))
    (:Completed
      (return (Utilities|IsValid (LocalVariables|GettmpKeyMarker)) (LocalVariables|GettmpKeyMarker)))))
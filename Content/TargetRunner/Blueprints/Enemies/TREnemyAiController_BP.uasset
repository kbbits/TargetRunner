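; AI controller for shooter enemies that runs the EnemyShooter behavior tree and picks its player target through perception.
; On each perception update it scans perceived hostile player characters and writes the nearest one closer than the current target to the blackboard Target key, or clears the key if none is closer.
; A helper computing a move-to point offset from the target by attack range exists but is never run.
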(event OnTargetPerceptionUpdated(PerceptionComponent)
  (params (Actor :type Actor%20Object%20Reference) (Stimulus :type AI%20Stimulus%20Structure))
  (CallFunction|HandlePerceptionUpdated))

(event EventBeginPlay
  (AI|RunBehaviorTree "/Game/TargetRunner/Blueprints/Enemies/EnemyShooter_BT.EnemyShooter_BT"))

(event EventTick
  (params (DeltaSeconds :type Float%20%28single-precision%29)))

(fn ConstructionScript)

(fn HandlePerceptionUpdated
  (bind (_target _isvalid) (CallFunction|GetCurrentTargetBP))
  (LocalVariables|SettmpTarget _target)
  (if _isvalid
    (LocalVariables|SettmpCurrentTargetDistance (Transformation|GetDistanceTo (LocalVariables|GettmpTarget)))
    (else
      (LocalVariables|SettmpCurrentTargetDistance 1e+08)))
  (LocalVariables|SettmpTarget 0)
  (for _array_element (Class|AIPerceptionComponent|GetPerceivedHostileActors (Class|AIController|GetAIPerceptionComponent))
    (bind _astr_first_person_character_bp (Utilities|Casting|CastToTR_FirstPersonCharacter_BP _array_element))
    (if (< (Transformation|GetDistanceTo _astr_first_person_character_bp) (LocalVariables|GettmpCurrentTargetDistance))
      (LocalVariables|SettmpTarget _array_element)
      (LocalVariables|SettmpCurrentTargetDistance (Transformation|GetDistanceTo _astr_first_person_character_bp))))
  (AI|Components|Blackboard|SetValueasObject (AI|GetBlackboard 0) (Utilities|Name|MakeLiteralName "Target") (LocalVariables|GettmpTarget)))

(fn GetCurrentTargetBP
  (bind _returnvalue (AI|GetBlackboard 0))
  (bind _returnvalue_2 (Utilities|Name|MakeLiteralName "Target"))
  (bind _returnvalue_3 (AI|Components|Blackboard|GetValueasObject _returnvalue _returnvalue_2))
  (Utilities|IsValid _returnvalue_3
    (:Is%20Valid
      (bind _asactor (Utilities|Casting|CastToActor _returnvalue_3)
        (:then
          (return _asactor true))
        (:CastFailed
          _)))
    (:Is%20Not%20Valid
      _))
  (return 0 false))

(fn TrackTargetLocation
  (bind (_target _isvalid) (CallFunction|GetCurrentTargetBP))
  (if _isvalid
    (LocalVariables|SettmpCurrentTarget _target)
    (bind _astrenemy_character_base_bp (Utilities|Casting|CastToTREnemyCharacterBase_BP (Pawn|GetControlledPawn)))
    (AI|Components|Blackboard|SetValueasVector (AI|GetBlackboard 0) (Utilities|Name|MakeLiteralName "TargetMoveToLocation") (+ (Transformation|GetActorLocation (LocalVariables|GettmpCurrentTarget)) (* (Math|Vector|Normalize (- (Transformation|GetActorLocation _astrenemy_character_base_bp) (Transformation|GetActorLocation (LocalVariables|GettmpCurrentTarget)))) (/ (- (Class|TREnemyCharacter|GetMaxAttackRange _astrenemy_character_base_bp) (Class|TREnemyCharacter|GetMinAttackRange _astrenemy_character_base_bp)) 2.0))))))

(fn GetCurrentTarget
  (bind _returnvalue (AI|GetBlackboard 0))
  (bind _returnvalue_2 (Utilities|Name|MakeLiteralName "Target"))
  (bind _returnvalue_3 (AI|Components|Blackboard|GetValueasObject _returnvalue _returnvalue_2))
  (Utilities|IsValid _returnvalue_3
    (:Is%20Valid
      (bind _asactor (Utilities|Casting|CastToActor _returnvalue_3)
        (:then
          (return _asactor))
        (:CastFailed
          _)))
    (:Is%20Not%20Valid
      _))
  (return 0))
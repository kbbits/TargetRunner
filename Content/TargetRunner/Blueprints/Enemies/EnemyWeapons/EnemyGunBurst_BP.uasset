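; Enemy burst gun weapon that adds gun mesh animation syncing on top of its parent weapon class.
; On fire start, it copies the tool's auto-fire delay into the CSC_Gun1 anim blueprint as the shot delay, then runs the parent firing logic.
; Animation state updates call the parent, then push the current weapon state to that same anim blueprint.
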(event EventBeginPlay
  (|CallParentFunction))

(event EventBeginFire
  (bind _ascsc_gun_1_anim_blueprint (Utilities|Casting|CastToCSC_Gun1_AnimBlueprint (Components|SkeletalMesh|GetAnimInstance (Variables|Default|GetGunMesh))))
  (Variables|/Game/CSC/Demo/Blueprints/Anomations/CSC_Gun1_AnimBlueprint.CSC_Gun1_AnimBlueprint_C|SetShotDelaySeconds _ascsc_gun_1_anim_blueprint (Class|ToolBase|GetAutoFireDelay (Variables|Default|GetTool)))
  (|CallParentFunction))

(fn ConstructionScript
  (|CallParentFunction))

(fn UpdateAnimState
  (|CallParentFunction)
  (bind _ascsc_gun_1_anim_blueprint (Utilities|Casting|CastToCSC_Gun1_AnimBlueprint (Components|SkeletalMesh|GetAnimInstance (Variables|Default|GetGunMesh))))
  (Variables|/Game/CSC/Demo/Blueprints/Anomations/CSC_Gun1_AnimBlueprint.CSC_Gun1_AnimBlueprint_C|SetState _ascsc_gun_1_anim_blueprint (Variables|Default|GetWeaponState)))
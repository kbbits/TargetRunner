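; Base Blueprint for enemy tool weapons that scales the weapon's attribute stats to its Level.
; ScaleToLevel skips scaling at level 1 or once ScaleUpApplied is set, but always calls the parent.
; Projectile speed rises linearly, damage follows a power curve, and activation delay shrinks linearly to a clamped factor.
; Auto weapons also scale fire delay exponentially and extend burst limit, with all results floored at each attribute's MinValue.
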(event EventScaletoLevel
  (bind _projectilespeed (Variables|Default|GetProjectileSpeed))
  (bind _level (Variables|Default|GetLevel))
  (bind _damagescaleexponent_bp (Variables|Default|GetDamageScaleExponent_BP))
  (bind _activationdelay (Variables|Default|GetActivationDelay))
  (bind _level_2 (Variables|Default|GetLevel))
  (bind _level_3 (Variables|Default|GetLevel))
  (bind _autofiredelayscalebase (Variables|Default|GetAutoFireDelayScaleBase))
  (bind _autofireburstlimit (Variables|Default|GetAutoFireBurstLimit))
  (bind _level_4 (Variables|Default|GetLevel))
  (bind _level_5 (Variables|Default|GetLevel))
  (bind _basedamage (Variables|Default|GetBaseDamage))
  (bind _autofiredelay (Variables|Default|GetAutoFireDelay))
  (bind (_name _minvalue _maxvalue _currentvalue) (Utilities|Struct|BreakAttributeData _autofireburstlimit))
  (bind (_name_2 _minvalue_2 _maxvalue_2 _currentvalue_2) (Utilities|Struct|BreakAttributeData _projectilespeed))
  (bind (_name_3 _minvalue_3 _maxvalue_3 _currentvalue_3) (Utilities|Struct|BreakAttributeData _basedamage))
  (bind (_name_4 _minvalue_4 _maxvalue_4 _currentvalue_4) (Utilities|Struct|BreakAttributeData _activationdelay))
  (bind (_name_5 _minvalue_5 _maxvalue_5 _currentvalue_5) (Utilities|Struct|BreakAttributeData _autofiredelay))
  (bind _returnvalue (Math|Conversions|ToFloat(Integer) _level))
  (bind _returnvalue_2 (- _level_2 1))
  (bind _returnvalue_3 (/ _level_4 2))
  (bind _returnvalue_4 (- _level_3 1))
  (bind _returnvalue_5 (- _level_5 1))
  (bind _returnvalue_6 (* _returnvalue_2 0.1))
  (bind _returnvalue_7 (Math|Conversions|ToFloat(Integer) _returnvalue_3))
  (bind _returnvalue_8 (Math|Float|Power _returnvalue _damagescaleexponent_bp))
  (bind _returnvalue_9 (* _returnvalue_5 0.075))
  (bind _returnvalue_10 (Math|Conversions|ToFloat(Integer) _returnvalue_4))
  (bind _returnvalue_11 (Math|Float|Power _autofiredelayscalebase _returnvalue_10))
  (bind _returnvalue_12 (- 1.0 _returnvalue_9))
  (bind _returnvalue_13 (* _currentvalue_3 _returnvalue_8))
  (bind _returnvalue_14 (+ _returnvalue_6 1.0))
  (bind _returnvalue_15 (+ _currentvalue _returnvalue_7))
  (bind _returnvalue_16 (Math|Float|Clamp(Float) _returnvalue_12 0.2))
  (bind _returnvalue_17 (* _currentvalue_2 _returnvalue_14))
  (bind _returnvalue_18 (Math|Float|Max(Float) _minvalue _returnvalue_15))
  (bind _returnvalue_19 (Math|Float|Max(Float) _minvalue_3 _returnvalue_13))
  (bind _returnvalue_20 (* _currentvalue_5 _returnvalue_11))
  (bind _returnvalue_21 (Math|Float|Max(Float) _minvalue_2 _returnvalue_17))
  (bind _returnvalue_22 (Math|Float|Max(Float) _minvalue_5 _returnvalue_20))
  (bind _returnvalue_23 (* _currentvalue_4 _returnvalue_16))
  (bind _returnvalue_24 (Math|Float|Max(Float) _minvalue_4 _returnvalue_23))
  ;[1 1 1] Scale To Level - Update this actor's stats according to it's Level.
  (if (not (Variables|Default|GetbScaleUpApplied)) ; Only apply scale up once.
    (if (> (Variables|Default|GetLevel) 1) ; Don't need to do anything unless level > 1
      (Utilities|FlowControl|Sequence
        (:then_0
          ;[1 1 1] Projectile Speed
          (Utilities|Struct|SetmembersinAttributeData (Variables|Default|GetProjectileSpeed) _returnvalue_21 _returnvalue_21))
        (:then_1
          ;[1 1 1] Damage
          (Utilities|Struct|SetmembersinAttributeData (Variables|Default|GetBaseDamage) _returnvalue_19 _returnvalue_19))
        (:then_2
          ;[1 1 1] Activation Delay == shot interval speed
          (Utilities|Struct|SetmembersinAttributeData (Variables|Default|GetActivationDelay) _returnvalue_24 _returnvalue_24))
        (:then_3
          ;[1 1 1] Auto-Fire Delay
          (if (and (Utilities|Enum|Equal(Enum) (Variables|Default|GetActivationType) "Auto") (> (Class|ToolBase|GetAutoFireDelay) 0.0))
            (Utilities|Struct|SetmembersinAttributeData (Variables|Default|GetAutoFireDelay) _returnvalue_22 _returnvalue_22)))
        (:then_4
          ;[1 1 1] Auto-Fire Burst Limit
          (if (and (Utilities|Enum|Equal(Enum) (Variables|Default|GetActivationType) "Auto") (> (Class|ToolBase|GetAutoFireBurstLimit) 0.0))
            (Utilities|Struct|SetmembersinAttributeData (Variables|Default|GetAutoFireBurstLimit) _returnvalue_18 _returnvalue_18)))
        (:then_5
          ;[1 1 1] Call parent
          (|CallParentFunction :!label _label)))
      (else
        (goto _label)))
    (else
      (goto _label))))
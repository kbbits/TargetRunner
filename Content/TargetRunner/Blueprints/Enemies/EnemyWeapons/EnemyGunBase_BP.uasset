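; Base Blueprint for enemy guns in TargetRunner that fire projectiles at the AI controller's current target.
; A server-authoritative Tick state machine fires when the owning enemy has a target in range and aimed, handling single shots, auto bursts and activation delay.
; Bursts advance by timer or anim notify, and projectiles spawn from the muzzle with tool stats, aimed high on character capsules.
; A multicast event plays muzzle flash and sound, while WeaponState replication calls an animation hook left empty here.
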(event Custom|AnimNotifyFire
  ;[1 1 1] AnimNotify Fire - When animation notify drives projectile spawning. (ex: EnemyGunBurst)
  (if (Variables|Default|GetbSpawnProjectileByAnimNotify)
    (Networking|SwitchHasAuthority
      (:Authority
        (Utilities|IsValid (Variables|Default|GetTool)
          (:Is%20Valid
            (if (Utilities|Enum|Equal(Enum) (Variables|Default|GetWeaponState) "Firing")
              (if (< (Variables|Default|GetBurstFireCount) (Class|ToolBase|GetAutoFireBurstLimit (Variables|Default|GetTool)))
                (Math|Float|IncrementFloat (Variables|Default|GetBurstFireCount)
                  (:%20%20
                    (CallFunction|SpawnProjectile))))
              (else
                (CallFunction|UpdateAnimState)))))))))

(event Custom|MC_ProjectileSpawned
  (params (Transform :type Transform%20%28by%20ref%29))
  (bind (_location _rotation) (Math|Transform|BreakTransform Transform))
  ;[1 1 1] MC Projectile Spawned
  (Effects|SpawnEmitteratLocation "/Game/SciFiWeapLight/FX/Particles/P_Pistol_MuzzleFlash_Light.P_Pistol_MuzzleFlash_Light" _location _rotation "1.000000,1.000000,1.000000" true "AutoRelease")
  (Audio|PlaySoundatLocation (Utilities|ResolveSoftReference (Class|ToolActorBase|GetFireSound)) _location "0, 0, 0" 1.0 1.0 0.0 0 0 self) ; Play firing sound
)

(event EventBeginPlay
  ;[1 1 1] Begin Play
  (|CallParentFunction)
  ;[1 1 1] Load some assets. (should do this differently)
  (if (Utilities|IsValidSoftObjectReference (Class|ToolActorBase|GetFireSound))
    (bind _object (Utilities|AsyncLoadAsset (Variables|Default|GetFireSound))
      (:Completed
        (Utilities|Array|Add (Variables|Default|GetSoundCache) _object))))
  (if (Utilities|IsValidSoftObjectReference (Variables|Default|GetFireBusySound))
    (bind _object_2 (Utilities|AsyncLoadAsset (Variables|Default|GetFireBusySound))
      (:Completed
        (Utilities|Array|Add (Variables|Default|GetSoundCache) _object_2))))
  (if (Utilities|IsValidSoftObjectReference (Variables|Default|GetReloadSound))
    (bind _object_3 (Utilities|AsyncLoadAsset (Variables|Default|GetReloadSound))
      (:Completed
        (Utilities|Array|Add (Variables|Default|GetSoundCache) _object_3)))))

(event EventBeginFire
  ;[1 1 1] Begin Fire
  (Networking|SwitchHasAuthority
    (:Authority
      (if (not (Class|TREnemyCharacter|IsDead (CallFunction|GetAttachedCharacterBP)))
        (switch Utilities|FlowControl|Switch|SwitchonETRWeaponState (Variables|Default|GetWeaponState)
          (:Idle
            _)
          (:ReadyToFire
            _))
        (Variables|Default|SetWeaponState "Firing")
        (Variables|Default|SetFireDelaySum 0.0)
        (Variables|Default|SetBurstFireCount 0.0)
        (switch Utilities|FlowControl|Switch|SwitchonEToolEmitType (Variables|/Script/TargetRunner.ToolBase|GetEmitType (Variables|Default|GetTool))
          (:Projectile
            (switch Utilities|FlowControl|Switch|SwitchonEToolActivationType (Variables|/Script/TargetRunner.ToolBase|GetActivationType (Variables|Default|GetTool))
              (:Single
                (CallFunction|SpawnProjectile))
              (:Auto
                (if (Variables|Default|GetbSpawnProjectileByAnimNotify)
                  (CallFunction|UpdateAnimState)
                  (else
                    (Variables|Default|SetAutoFireDelaySum 0.0)
                    (Math|Float|IncrementFloat (Variables|Default|GetBurstFireCount)
                      (:%20%20
                        (CallFunction|SpawnProjectile)))))))))))))

(event EventTick
  (params (DeltaSeconds :type Float%20%28single-precision%29))
  ;[1 1 1] Tick
  (CallFunction|UpdateWeaponState DeltaSeconds)
  (CallFunction|UpdateDebugVis))

(event EventOnRepWeaponState
  ;[1 1 1] OnRep WeaponState
  (CallFunction|UpdateAnimState))

(event EventEndFire
  ;[1 1 1] End Fire
  (|CallParentFunction)
  (Networking|SwitchHasAuthority
    (:Authority
      (if (<= (Class|ToolActorBase|GetActivationDelay) 0.0)
        (Variables|Default|SetFireDelaySum 0.0)
        (Variables|Default|SetWeaponState "Idle")
        (CallFunction|UpdateAnimState :!label _label)
        (elif (Utilities|Enum|Equal(Enum) (Variables|Default|GetWeaponState) "Firing")
          (Variables|Default|SetWeaponState "FireBusy")
          (goto _label))))))

(fn ConstructionScript
  (Utilities|FlowControl|Sequence
    (:then_0
      (Transformation|AttachComponentToComponent (Variables|Default|GetMuzzleSphere) (Variables|Default|GetGunMesh) "Gun_EndSocket" "KeepRelative" "SnapToTarget" "KeepRelative" true))
    (:then_1
      (Class|ToolActorBase|InitToolObject)
      (CallFunction|UpdateDebugVis))))

(fn UpdateWeaponState
  (params (DeltaSeconds :type Float%20%28single-precision%29))
  (LocalVariables|SettmpDeltaSeconds DeltaSeconds)
  (if (not (Class|TREnemyCharacter|IsDead (CallFunction|GetAttachedCharacterBP)))
    (Networking|SwitchHasAuthority
      (:Authority
        (Utilities|IsValid (Variables|Default|GetTool)
          (:Is%20Valid
            (LocalVariables|SettmpOwnerCharacter (CallFunction|GetAttachedCharacterBP))
            (Utilities|FlowControl|Sequence
              (:then_0
                (switch Utilities|FlowControl|Switch|SwitchonETRWeaponState (Variables|Default|GetWeaponState)
                  (:Idle
                    (if (Variables|/Script/TargetRunner.TREnemyCharacter|GetbTargetInRange (LocalVariables|GettmpOwnerCharacter)) :!label _label
                      (if (Variables|/Script/TargetRunner.TREnemyCharacter|GetbAimOnTarget (LocalVariables|GettmpOwnerCharacter))
                        (Variables|Default|SetWeaponState "ReadyToFire")
                        (Class|ToolActorBase|BeginFire)
                        (else
                          (Variables|Default|SetWeaponState "Aiming")))
                      (else
                        (Variables|Default|SetWeaponState "Idle"))))
                  (:Aiming
                    (goto _label))
                  (:ReadyToFire
                    (Class|ToolActorBase|BeginFire))
                  (:Firing
                    (Utilities|FlowControl|Sequence
                      (:then_0
                        ;[1 1 1] Auto-Fire Burst Shot when not driven by AnimNotify
                        (if (and (Utilities|Enum|Equal(Enum) (Variables|/Script/TargetRunner.ToolBase|GetActivationType (Variables|Default|GetTool)) "Auto") (not (Variables|Default|GetbSpawnProjectileByAnimNotify)))
                          (if (< (Variables|Default|GetBurstFireCount) (Class|ToolBase|GetAutoFireBurstLimit (Variables|Default|GetTool)))
                            (bind _output_get (Variables|Default|SetAutoFireDelaySum (+ (Variables|Default|GetAutoFireDelaySum) (LocalVariables|GettmpDeltaSeconds))))
                            (if (>= _output_get (Class|ToolBase|GetAutoFireDelay (Variables|Default|GetTool)))
                              (Variables|Default|SetAutoFireDelaySum 0.0)
                              (Math|Float|IncrementFloat (Variables|Default|GetBurstFireCount)
                                (:%20%20
                                  (CallFunction|SpawnProjectile)))))))
                      (:then_1
                        ;[1 1 1] Update Activation delay
                        (if (<= (Class|ToolActorBase|GetActivationDelay) 0.0) :!label _label_2
                          (switch Utilities|FlowControl|Switch|SwitchonEToolActivationType (Variables|/Script/TargetRunner.ToolBase|GetActivationType (Variables|Default|GetTool)) :!label _label_3
                            (:Single
                              (Variables|Default|SetFireDelaySum 0.0 :!label _label_4)
                              (Variables|Default|SetWeaponState "Idle"))
                            (:Auto
                              (if (>= (Variables|Default|GetBurstFireCount) (Class|ToolBase|GetAutoFireBurstLimit (Variables|Default|GetTool)))
                                (goto _label_4)
                                (else
                                  (Variables|Default|SetFireDelaySum (+ (LocalVariables|GettmpDeltaSeconds) (Variables|Default|GetFireDelaySum)))))))
                          (elif (>= (+ (LocalVariables|GettmpDeltaSeconds) (Variables|Default|GetFireDelaySum)) (Class|ToolActorBase|GetActivationDelay))
                            (goto _label_3)
                            (else
                              (Variables|Default|SetFireDelaySum (+ (LocalVariables|GettmpDeltaSeconds) (Variables|Default|GetFireDelaySum)))
                              (switch Utilities|FlowControl|Switch|SwitchonEToolActivationType (Variables|/Script/TargetRunner.ToolBase|GetActivationType (Variables|Default|GetTool))
                                (:Single
                                  (Variables|Default|SetWeaponState "FireBusy" :!label _label_5))
                                (:Auto
                                  (if (>= (Variables|Default|GetBurstFireCount) (Class|ToolBase|GetAutoFireBurstLimit (Variables|Default|GetTool)))
                                    (goto _label_5))))))))))
                  (:FireBusy
                    (goto _label_2))))
              (:then_1
                (CallFunction|UpdateAnimState)))))))
    (else
      (Variables|Default|SetWeaponState "Idle")
      (Actor|Tick|SetActorTickEnabled false))))

(fn GetAttachedCharacterBP
  (bind _astrenemy_character_base_bp (Utilities|Casting|CastToTREnemyCharacterBase_BP (Class|EnemyToolActorBase|GetAttachedCharacter))
    (:then
      _)
    (:CastFailed
      _))
  (return _astrenemy_character_base_bp))

(fn SpawnProjectile
  (bind _tool (Variables|Default|GetTool))
  (bind _tool_2 (Variables|Default|GetTool))
  (bind _muzzlesphere (Variables|Default|GetMuzzleSphere))
  (bind _gunmesh (Variables|Default|GetGunMesh))
  (bind _returnvalue (Transformation|GetWorldLocation _muzzlesphere))
  (Networking|SwitchHasAuthority
    (:Authority
      (Utilities|FlowControl|Sequence
        (:then_0
          (bind _astrenemy_aicontroller_bp (Utilities|Casting|CastToTREnemyAIController_BP (Class|TREnemyCharacter|GetTRAIController (CallFunction|GetAttachedCharacterBP))))
          (bind _returnvalue_2 (Class|TREnemyAIController|GetCurrentTarget _astrenemy_aicontroller_bp))
          (bind _output_get (LocalVariables|SettmpTarget _returnvalue_2))
          (Utilities|IsValid _output_get
            (:Is%20Valid
              (Utilities|FlowControl|Sequence
                (:then_0
                  (switch Utilities|FlowControl|Switch|SwitchonEToolActivationType (Variables|/Script/TargetRunner.ToolBase|GetActivationType (Variables|Default|GetTool))
                    (:Single
                      (Components|Animation|SetPosition _gunmesh 0.0 false :!label _label)
                      (Audio|Components|Audio|Play _gunmesh false) ; Play firing anim
                    )
                    (:Auto
                      (if (not (Variables|Default|GetbSpawnProjectileByAnimNotify))
                        (goto _label)))))
                (:then_1
                  (LocalVariables|SettmpSpawnTransform (Math|Transform|MakeTransform _returnvalue (Math|Rotator|FindLookatRotation _returnvalue (+ (Transformation|GetActorLocation (LocalVariables|GettmpTarget)) (Math|Vector|SelectVector (* "0, 0,0.650000" (Class|CapsuleComponent|GetScaledCapsuleHalfHeightWithoutHemisphere (Variables|/Script/Engine.Character|GetCapsuleComponent (.AsCharacter (Utilities|Casting|CastToCharacter (LocalVariables|GettmpTarget)))))) "0, 0, 0" (.bSuccess (Utilities|Casting|CastToCharacter (LocalVariables|GettmpTarget))))))))
                  (bind _astrprojectile_extractor_base (Utilities|Casting|CastToTRProjectileExtractorBaseClass (Class|ToolActorBase|GetProjectileClass))
                    (:then
                      (bind _returnvalue_3 (Game|SpawnActorfromClass _astrprojectile_extractor_base (LocalVariables|GettmpSpawnTransform) "AlwaysSpawn" 0 (Class|ToolActorBase|GetResourceExtractionRates) (Class|ToolActorBase|GetDamagePerShot) (Class|ToolActorBase|GetDamageRates) (Class|ToolBase|GetMaximumBounces _tool) (Class|ToolBase|GetProjectileSpeed _tool) (CallFunction|GetAttachedCharacterBP)))
                      (bind _output_get_2 (LocalVariables|SettmpSpawnedProjectile _returnvalue_3))
                      (bind _asenemy_projectile_base_bp (Utilities|Casting|CastToEnemyProjectile_Base_BP _output_get_2)
                        (:then
                          (LocalVariables|SettmpIgnoreComponent (Variables|/Game/TargetRunner/Blueprints/Enemies/EnemyWeapons/EnemyProjectile_Base_BP.EnemyProjectile_Base_BP_C|GetCollisionComponent _asenemy_projectile_base_bp)))
                        (:CastFailed
                          (bind _astrenemy_projectile_base_bp (Utilities|Casting|CastToTREnemyProjectile_Base_BP _output_get_2))
                          (LocalVariables|SettmpIgnoreComponent (Variables|/Game/TargetRunner/Blueprints/Enemies/EnemyWeapons/TREnemyProjectile_Base_BP.TREnemyProjectile_Base_BP_C|GetCollisionComponent _astrenemy_projectile_base_bp)))))
                    (:CastFailed
                      (bind _returnvalue_4 (Game|SpawnActorfromClass (Class|ToolActorBase|GetProjectileClass) (LocalVariables|GettmpSpawnTransform) "AlwaysSpawn" 0 (Class|ToolActorBase|GetDamagePerShot) (Class|ToolActorBase|GetDamageRates) (Class|ToolBase|GetMaximumBounces _tool_2) (Class|ToolBase|GetProjectileSpeed _tool_2) (CallFunction|GetAttachedCharacterBP)))
                      (bind _output_get_3 (LocalVariables|SettmpSpawnedProjectile _returnvalue_4))
                      (bind _asenemy_projectile_base_bp_2 (Utilities|Casting|CastToEnemyProjectile_Base_BP _output_get_3)
                        (:then
                          (LocalVariables|SettmpIgnoreComponent (Variables|/Game/TargetRunner/Blueprints/Enemies/EnemyWeapons/EnemyProjectile_Base_BP.EnemyProjectile_Base_BP_C|GetCollisionComponent _asenemy_projectile_base_bp_2)))
                        (:CastFailed
                          (bind _astrenemy_projectile_base_bp_2 (Utilities|Casting|CastToTREnemyProjectile_Base_BP _output_get_3))
                          (LocalVariables|SettmpIgnoreComponent (Variables|/Game/TargetRunner/Blueprints/Enemies/EnemyWeapons/TREnemyProjectile_Base_BP.TREnemyProjectile_Base_BP_C|GetCollisionComponent _astrenemy_projectile_base_bp_2))))))
                  (Collision|IgnoreActorwhenMoving (LocalVariables|GettmpIgnoreComponent) self true)
                  (Collision|IgnoreActorwhenMoving (LocalVariables|GettmpIgnoreComponent) (CallFunction|GetAttachedCharacterBP) true)
                  (Collision|IgnoreActorwhenMoving (Variables|/Script/Engine.Character|GetCapsuleComponent (CallFunction|GetAttachedCharacterBP)) (LocalVariables|GettmpSpawnedProjectile) true))))))
        (:then_1
          (CallFunction|MCProjectileSpawned (LocalVariables|GettmpSpawnTransform)))))))

(fn UpdateDebugVis)

(fn UpdateAnimState)
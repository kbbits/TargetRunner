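; Base enemy character Blueprint for TargetRunner, handling level scaling, damage, health display, death and loot.
; Construction scales health and walk speed by level; a colour-coded health bar shows only while partially depleted.
; Damage is adjusted through the causer's interface, and lethal hits spawn homing resource pickups from its extraction rates, plus goods drops.
; Health depletion triggers multicast effects that stop the AI, then the server destroys the actor after a random delay.
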(event Custom|MC_OnDeathEffects
  (Effects|SpawnEmitterAttached "/Game/SciFiWeapLight/FX/Particles/P_Grenade_Explosion_Light.P_Grenade_Explosion_Light" (Variables|Character|GetMesh) "None" (* (.BoxExtent (Collision|GetComponentBounds (Variables|Default|GetCapsuleComponent))) "0, 0,0.500000") "0, 0, 0" "1.000000,1.000000,1.000000" "KeepRelativeOffset" true "AutoRelease")
  (Audio|PlaySoundatLocation (Utilities|ResolveSoftReference (Variables|Default|GetDeathSound)) (Transformation|GetActorLocation) "0, 0, 0" 0.8 1.0 0.0 "/Game/TargetRunner/Assets/Audio/TR_DefaultAttenuation.TR_DefaultAttenuation" 0 0)
  (Actor|Tick|SetActorTickEnabled false)
  (bind _astrenemy_aicontroller_bp (Utilities|Casting|CastToTREnemyAIController_BP (Class|TREnemyCharacter|GetTRAIController)))
  (AI|Components|Blackboard|SetValueasBool (AI|GetBlackboard _astrenemy_aicontroller_bp) (Utilities|Name|MakeLiteralName "IsDead") true)
  (Actor|Tick|SetActorTickEnabled _astrenemy_aicontroller_bp)
  (AI|Logic|StopLogic (Variables|/Script/AIModule.AIController|GetBrainComponent _astrenemy_aicontroller_bp) "Dead"))

(event Custom|OnHealthDelta
  (params (NewCurrent :type Float%20%28single-precision%29))
  (CallFunction|UpdateVis))

(event EventTick
  (params (DeltaSeconds :type Float%20%28single-precision%29))
  (|CallParentFunction DeltaSeconds))

(event EventOnHealthDepleted
  (Networking|SwitchHasAuthority
    (:Authority
      (Utilities|FlowControl|Sequence
        (:then_0
          (CallFunction|MConDeathEffects))
        (:then_1
          (Utilities|FlowControl|Delay (Math|Random|RandomFloatinRange 1e+01 25.0))
          (Actor|DestroyActor))))))

(event Game|Damage|EventAnyDamage
  (params (Damage :type Float%20%28single-precision%29) (DamageType :type Damage%20Type%20Object%20Reference) (InstigatedBy :type Controller%20Object%20Reference) (DamageCauser :type Actor%20Object%20Reference))
  (CallFunction|HandleDamage Damage "0, 0, 0" InstigatedBy DamageCauser))

(event EventBeginPlay
  (bind _deathsound (Variables|Default|GetDeathSound))
  (CallFunction|UpdateVis)
  (EventDispatchers|BindEventtoOnDeltaCurrent (Variables|Default|GetHealthAttribute) (delegate Custom|OnHealthDelta))
  (if (Utilities|IsValidSoftObjectReference _deathsound)
    (bind _object (Utilities|AsyncLoadAsset _deathsound)
      (:Completed
        (Utilities|Array|AddUnique (Variables|Default|GetAssetRefCache) _object)))))

(event EventDestroyed
  (Utilities|Array|Clear (Variables|Default|GetAssetRefCache)))

(event EventScaletoLevel
  (bind _healthattribute (Variables|Default|GetHealthAttribute))
  ;[1 1 1] ScaleToLevel
  (if (not (Variables|Default|GetbScaleUpApplied))
    (if (> (Variables|Default|GetLevel) 1)
      (Utilities|FlowControl|Sequence
        (:then_0
          ;[1 1 1] Health
          (Class|ActorAttributeComponent|SetMaxBase _healthattribute (* (Class|ActorAttributeComponent|GetMaxBase (Variables|Default|GetHealthAttribute)) (Math|Float|Power (Math|Conversions|ToFloat(Integer) (Variables|Default|GetLevel)) (Variables|Default|GetHealthScaleExponent))))
          (Class|ActorAttributeComponent|ResettoMax _healthattribute))
        (:then_1
          ;[1 1 1] Walk Speed
          (Variables|/Script/Engine.CharacterMovementComponent|SetMaxWalkSpeed (Variables|Character|GetCharacterMovement) (+ (Variables|/Script/Engine.CharacterMovementComponent|GetMaxWalkSpeed (Variables|Character|GetCharacterMovement)) (* (Math|Conversions|ToFloat(Integer) (- (Variables|Default|GetLevel) 1)) (Variables|Default|GetWalkSpeedScaleIncrement)))))
        (:then_2
          (|CallParentFunction :!label _label)))
      (else
        (goto _label)))
    (else
      (goto _label))))

(fn ConstructionScript
  (|CallParentFunction)
  (Class|TREnemyCharacter|ScaletoLevel))

(fn GetMinAttackRange
  (return (|CallParentFunction)))

(fn GetMaxAttackRange
  (return (|CallParentFunction)))

(fn HandleDamage
  (params (DamageDealt :type Float%20%28single-precision%29) (HitLocation :type Vector) (Instigator :type Controller%20Object%20Reference) (DamageCauser :type Actor%20Object%20Reference))
  (LocalVariables|SettmpDamageDealt DamageDealt)
  (LocalVariables|SettmpHitLocation HitLocation)
  (LocalVariables|SettmpInstigator Instigator)
  (LocalVariables|SettmpDamageCauser DamageCauser)
  (if (> (LocalVariables|GettmpDamageDealt) 0.0)
    (Utilities|FlowControl|Sequence
      (:then_0
        (if (Class|ResourceFunctionLibrary|IsResourceTypeValid (Variables|Default|GetTakesDamageAs))
          (bind _asdoes_damage_by_type (Utilities|Casting|CastToDoesDamageByType (LocalVariables|GettmpDamageCauser)))
          (bind _calculateddamage (Class|DoesDamagebyType|CalculateDamagebyType _asdoes_damage_by_type (LocalVariables|GettmpDamageDealt) (Variables|Default|GetTakesDamageAs)))
          (LocalVariables|SettmpDamageDealt _calculateddamage)))
      (:then_1
        (if (<= (- (Class|ActorAttributeComponent|GetCurrent (Variables|Default|GetHealthAttribute)) (LocalVariables|GettmpDamageDealt)) 0.0)
          (Utilities|FlowControl|Sequence
            (:then_0
              (bind _asextracts_resources (Utilities|Casting|CastToExtractsResources (LocalVariables|GettmpDamageCauser)))
              (bind _returnvalue (Class|ExtractsResources|GetExtractionRates _asextracts_resources))
              (LocalVariables|SettmpExtractionRates _returnvalue)
              (Utilities|FlowControl|DoOnce false
                (:Completed
                  (bind (_extractedquantities _returnvalue_2) (Class|TREnemyCharacter|GetExtractedResourcesonDestroy (LocalVariables|GettmpExtractionRates)))
                  (LocalVariables|SettmpExtractedResources _extractedquantities)
                  (Utilities|Array|Clear (Variables|Default|GetResourcesOnDestroy))
                  (if _returnvalue_2
                    (CallFunction|SpawnExtractedResources (LocalVariables|GettmpExtractedResources))))))
            (:then_1
              (CallFunction|SpawnonDestroyGoods)
              (Utilities|Array|Clear (Variables|Default|GetGoodsOnDestroy))))))
      (:then_3
        (Class|ActorAttributeComponent|DeltaValue (Variables|Default|GetHealthAttribute) (* (LocalVariables|GettmpDamageDealt) -1.0) true)))))

(fn SpawnExtractedResources
  (params (ExtractedResources :type Array%20of%20Resource%20Quantity%20Structures))
  (bind _mesh (Variables|Character|GetMesh))
  (LocalVariables|SettmpExtractedResources ExtractedResources)
  (bind _astr_game_state (Utilities|Casting|CastToTR_GameState (Game|GetGameState)))
  (LocalVariables|SettmpGameState _astr_game_state)
  (for _array_element (LocalVariables|GettmpExtractedResources)
    (if (> (.Quantity (Utilities|Struct|BreakResourceQuantity _array_element)) 0.0)
      (LocalVariables|SettmpExtractedGoods (Utilities|Struct|MakeGoodsQuantity (Class|ResourceFunctionLibrary|GoodsNameforResource (.ResourceType (Utilities|Struct|BreakResourceQuantity _array_element))) (.Quantity (Utilities|Struct|BreakResourceQuantity _array_element))))
      (bind (_resourcedata _returnvalue) (Class|TRGameState|GetResourceTypeData (LocalVariables|GettmpGameState) (.ResourceType (Utilities|Struct|BreakResourceQuantity _array_element))))
      (if _returnvalue
        (LocalVariables|SettmpExtactedResourceData _resourcedata)
        (Game|SpawnActorfromClass "/Game/TargetRunner/Blueprints/Pickups/PickupResourcesHomingBase_BP.PickupResourcesHomingBase_BP_C" (Math|Transform|MakeTransform (Transformation|GetWorldLocation _mesh) (Transformation|GetWorldRotation _mesh)) "AlwaysSpawn" 0 0 (Utilities|ResolveSoftReference (.DefaultMaterial (Utilities|Struct|BreakResourceTypeData (LocalVariables|GettmpExtactedResourceData)))) "0.000000,0.000000,0.000000" (Utilities|Struct|MakePickupAwards (Utilities|Array|MakeArray (Utilities|Struct|MakePickupAwardsItem (Utilities|Array|MakeArray (LocalVariables|GettmpExtractedGoods)) 0.0 0.0))) (Utilities|Array|MakeArray) 0)))))

(fn UpdateVis
  (bind _healthwidget (Variables|Default|GetHealthWidget))
  (bind _healthattribute (Variables|Default|GetHealthAttribute))
  (bind _returnvalue (Class|ActorAttributeComponent|GetCurrentPercent _healthattribute))
  (if (Math|Float|InRange(Float) (Class|ActorAttributeComponent|GetCurrentPercent (Variables|Default|GetHealthAttribute)) 0.0 1.0 false false)
    (Rendering|SetVisibility (Variables|Default|GetHealthWidget) true true)
    (bind _returnvalue_2 (Rendering|Material|CreateDynamicMaterialInstance _healthwidget 0 (Rendering|Material|GetMaterial _healthwidget 0) "None" :!class /Script/Engine.PrimitiveComponent))
    (Rendering|Material|SetScalarParameterValue _returnvalue_2 "Progress" _returnvalue :!class /Script/Engine.MaterialInstanceDynamic)
    (Rendering|Material|SetVectorParameterValue _returnvalue_2 "ProgressColor1" (Math|Color|SelectColor (Math|Color|SelectColor "(R=1.000000,G=0.000000,B=0.000000,A=1.000000)" "(R=1.000000,G=0.640717,B=0.000000,A=1.000000)" (<= _returnvalue 0.2)) "(R=0.000000,G=1.000000,B=0.000000,A=1.000000)" (<= _returnvalue 0.5)) :!class /Script/Engine.MaterialInstanceDynamic)
    (else
      (Rendering|SetVisibility (Variables|Default|GetHealthWidget) false false))))

(fn SpawnonDestroyGoods
  (for _array_element (Variables|Default|GetGoodsOnDestroy)
    (if (> (.Quantity (Utilities|Struct|BreakGoodsQuantity _array_element)) 0.0)
      (bind _goodsdata (Utilities|GetGoodsDatafromGameState? (CallFunction|GetTRGameState) (.Name (Utilities|Struct|BreakGoodsQuantity _array_element)))
        (:Found
          (LocalVariables|SettmpGoodsData _goodsdata)
          (if (Utilities|IsValidSoftClassReference (.ActorClass (Utilities|Struct|BreakGoodsType (LocalVariables|GettmpGoodsData))))
            (LocalVariables|SettmpActorSpawnClass (Utilities|ResolveSoftReference (.ActorClass (Utilities|Struct|BreakGoodsType (LocalVariables|GettmpGoodsData)))))
            (if (Utilities|IsValidClass (LocalVariables|GettmpActorSpawnClass))
              _
              (else
                (bind _returnvalue (Utilities|LoadClassAssetBlocking (.ActorClass (Utilities|Struct|BreakGoodsType (LocalVariables|GettmpGoodsData)))))
                (bind _asactor (Utilities|Casting|CastToActorClass _returnvalue))
                (LocalVariables|SettmpActorSpawnClass _asactor)))
            (if (Utilities|IsValidClass (LocalVariables|GettmpActorSpawnClass))
              (for _index (range 1 (Math|Float|Truncate (.Quantity (Utilities|Struct|BreakGoodsQuantity _array_element))))
                (Game|SpawnActorfromClass (LocalVariables|GettmpActorSpawnClass) (Math|Transform|MakeTransform (+ (Transformation|GetActorLocation) (Math|Vector|MakeVector 0.0 0.0 (+ (.Z (Math|Vector|BreakVector (.BoxExtent (Collision|GetActorBounds true true)))) 3.0))) (Math|Conversions|RotationFromXVector (Math|Vector|GetRightVector (Math|Rotator|MakeRotator 0.0 0.0 (Math|Random|RandomFloatinRange 0.0 3.6e+02))))) "AdjustIfPossibleButAlwaysSpawn" 0 0)))))))))
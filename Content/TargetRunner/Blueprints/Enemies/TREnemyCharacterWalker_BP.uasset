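; Walker enemy character with a turret that tracks the AI controller's current target and scales its rotation speed with level.
; Each tick on authority, it interpolates toward an in-range target, biased to the head of Characters, with a downward-angle limit.
; It exchanges blend and rotation state with the BP_Anim_Base1 instance and variables, flagging AimOnTarget once aligned and fully blended.
; Death sets the dead animation state and disables collision.
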(event EventScaletoLevel
  ;[1 1 1] Scale to Level
  (if (not (Variables|Default|GetbScaleUpApplied))
    (Variables|Default|SetTurretRotationSpeed (* (Variables|Default|GetTurretRotationSpeed) (+ (* (- (Variables|Default|GetLevel) 1) 0.1) 1.0)))
    (|CallParentFunction)))

(event EventTick
  (params (DeltaSeconds :type Float%20%28single-precision%29))
  ;[1 1 1] Tick
  (|CallParentFunction DeltaSeconds)
  (CallFunction|HandleTurretRotation DeltaSeconds))

(event EventMConDeathEffects
  ;[1 1 1] OnDeath effects
  (bind _asbp_anim_base_1 (Utilities|Casting|CastToBP_Anim_Base1 (Components|SkeletalMesh|GetAnimInstance (Variables|Character|GetMesh))))
  (Variables|/Game/CSC/Demo/Blueprints/Anomations/BP_Anim_Base1.BP_Anim_Base1_C|SetST_State _asbp_anim_base_1 "dead")
  (Collision|SetCollisionEnabled (Variables|Character|GetMesh) "NoCollision")
  (|CallParentFunction))

(fn ConstructionScript
  (|CallParentFunction)
  (Transformation|AttachComponentToComponent (Variables|Default|GetTurretHeading) (Variables|Character|GetMesh) "ADD_Parts_Here_Socket" "SnapToTarget" "SnapToTarget" "KeepRelative" true))

(fn HandleTurretRotation
  (params (DeltaSeconds :type Float%20%28single-precision%29))
  (bind _tmpdownangletolerance (LocalVariables|GettmpDownAngleTolerance))
  (Networking|SwitchHasAuthority
    (:Authority
      (LocalVariables|SettmpDeltaTime DeltaSeconds)
      (bind _asbp_anim_base_1 (Utilities|Casting|CastToBP_Anim_Base1 (Components|SkeletalMesh|GetAnimInstance (Variables|Character|GetMesh))))
      (LocalVariables|SettmpAnimInstance _asbp_anim_base_1)
      (Variables|/Game/CSC/Demo/Blueprints/Anomations/BP_Anim_Base1.BP_Anim_Base1_C|SetSt_DoBlend _asbp_anim_base_1 (Variables|Default|GetbTargetInRange))
      (Variables|Default|SetAnimBlendControlRotate (Variables|/Game/CSC/Demo/Blueprints/Anomations/BP_Anim_Base1.BP_Anim_Base1_C|GetST_BlendControlRotate (LocalVariables|GettmpAnimInstance)))
      (bind _astrenemy_aicontroller_bp (Utilities|Casting|CastToTREnemyAIController_BP (Class|TREnemyCharacter|GetTRAIController)))
      (bind _returnvalue (Class|TREnemyAIController|GetCurrentTarget _astrenemy_aicontroller_bp))
      (bind _output_get (LocalVariables|SettmpCurrentTarget _returnvalue))
      (Utilities|IsValid _output_get
        (:Is%20Valid
          (LocalVariables|SettmpTurretRotation (Variables|/Game/CSC/Demo/Blueprints/Anomations/BP_Anim_Base1.BP_Anim_Base1_C|GetSt_ToRotate (LocalVariables|GettmpAnimInstance)))
          (if (Variables|Default|GetbTargetInRange)
            (LocalVariables|SettmpOnTargetRotation (Math|Transform|InverseTransformRotation (Transformation|GetActorTransform) (Math|Rotator|FindLookatRotation (Transformation|GetSocketLocation (Variables|Character|GetMesh) "ADD_Parts_Here_Socket") (+ (Transformation|GetActorLocation (LocalVariables|GettmpCurrentTarget)) (Math|Vector|SelectVector (* "0, 0,0.650000" (Class|CapsuleComponent|GetScaledCapsuleHalfHeightWithoutHemisphere (Variables|/Script/Engine.Character|GetCapsuleComponent (.AsCharacter (Utilities|Casting|CastToCharacter (LocalVariables|GettmpCurrentTarget)))))) "0, 0, 0" (.bSuccess (Utilities|Casting|CastToCharacter (LocalVariables|GettmpCurrentTarget))))))))
            (if (and (>= (.Pitch (Math|Rotator|BreakRotator (LocalVariables|GettmpOnTargetRotation))) (- 0.0 _tmpdownangletolerance)) (<= (.Pitch (Math|Rotator|BreakRotator (LocalVariables|GettmpOnTargetRotation))) (+ 1.8e+02 _tmpdownangletolerance))) ; Don't aim below us
              (bind _output_get_2 (LocalVariables|SettmpTurretRotation (Math|Interpolation|RInterpTo (LocalVariables|GettmpTurretRotation) (LocalVariables|GettmpOnTargetRotation) (LocalVariables|GettmpDeltaTime) (Variables|Default|GetTurretRotationSpeed))))
              (Variables|Default|SetAnimTurrentRotation _output_get_2)
              (Variables|Default|SetbAimOnTarget (and (Math|Rotator|Equal(Rotator) (LocalVariables|GettmpTurretRotation) (LocalVariables|GettmpOnTargetRotation) 3.0) (>= (Variables|/Game/CSC/Demo/Blueprints/Anomations/BP_Anim_Base1.BP_Anim_Base1_C|GetST_BlendControlRotate (LocalVariables|GettmpAnimInstance)) 1.0)))
              (else
                (Variables|Default|SetbAimOnTarget false :!label _label)))
            (else
              (goto _label))))))))
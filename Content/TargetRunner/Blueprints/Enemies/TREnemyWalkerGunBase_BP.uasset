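; Base Blueprint for a walker enemy that carries a gun and can drop energy when destroyed.
; The construction script snaps the gun child actor component to a mesh socket and scales the gun to the enemy's Level, printing errors if it is missing or mistyped.
; On BeginPlay, the server usually assigns a random, Level-based amount of small energy as destroy loot.
; Logic to set the gun class from a tool instance is present but disconnected.
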(event EventBeginPlay
  (|CallParentFunction)
  (Networking|SwitchHasAuthority
    (:Authority
      (if (<= (Math|Random|RandomFloat) 0.75)
        (bind _returnvalue (Class|GoodsFunctionLibrary|GoodsQuantitiesfromRanges (Math|Random|MakeRandomStream (Math|Random|RandomInteger 99999)) (Utilities|Array|MakeArray (Utilities|Struct|MakeGoodsQuantityRange "Energy.Small.Normal" 1.0 (+ (Math|Conversions|ToFloat(Integer) (Variables|Default|GetLevel)) 1.0))) -1.0))
        (Variables|Default|SetGoodsOnDestroy _returnvalue)))))

(fn ConstructionScript
  (bind _gun_cac (Variables|Default|GetGun_CAC))
  (bind _childactor (Variables|/Script/Engine.ChildActorComponent|GetChildActor _gun_cac))
  (|CallParentFunction)
  (Transformation|AttachComponentToComponent (Variables|Default|GetGun_CAC) (Variables|Character|GetMesh) "ADD_Parts_Here_Socket" "SnapToTarget" "SnapToTarget" "KeepRelative" true)
  (Utilities|IsValid _childactor
    (:Is%20Valid
      (bind _asenemy_gun_base_bp (Utilities|Casting|CastToEnemyGunBase_BP _childactor)
        (:then
          (Default|ScaletoLevel _asenemy_gun_base_bp (Variables|Default|GetLevel)))
        (:CastFailed
          (Development|PrintString (Utilities|String|Append "Enemy weapon actor invalid class" (Utilities|GetDisplayName self)) true true "(R=1.000000,G=0.000000,B=0.000000,A=1.000000)" 5.0))))
    (:Is%20Not%20Valid
      (Development|PrintString (Utilities|String|Append "Enemy weapon child acter is null" (Utilities|GetDisplayName self)) true true "(R=1.000000,G=0.000000,B=0.000000,A=1.000000)" 5.0))))
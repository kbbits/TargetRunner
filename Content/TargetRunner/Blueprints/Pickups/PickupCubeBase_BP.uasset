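; Base Blueprint for physics-driven goods pickups that pop out with a random impulse and optional spin on spawn.
; The construction script sizes the overlap sphere from the pickup mesh's bounds, within clamped limits.
; Collection triggers an MC FX event that plays the pickup sound at the mesh before calling the parent.
; Display name comes from the first goods entry, and inspect info lists every goods type with its quantity.
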(event Custom|MC_OnPickupFX
  (bind _pickupsound (Variables|Default|GetPickupSound))
  (Utilities|IsValid _pickupsound
    (:Is%20Valid
      (Audio|PlaySoundatLocation _pickupsound (Transformation|GetWorldLocation (Variables|Default|GetPickupMesh)) "0, 0, 0" 1.0 1.0 0.0 0 0 0))))

(event EventBeginPlay
  (bind _returnvalue (Math|Random|RandomFloatinRange 1e+01 5e+01))
  (bind _returnvalue_2 (Math|Random|RandomFloat))
  (bind _initialrotationmax (Variables|Default|GetInitialRotationMax))
  (bind _returnvalue_3 (<= _returnvalue_2 0.5))
  (bind _returnvalue_4 (* _returnvalue -1.0))
  (bind _returnvalue_5 (Math|Float|SelectFloat _returnvalue _returnvalue_4 _returnvalue_3))
  (|CallParentFunction)
  (Physics|AddImpulse (Variables|Default|GetPhsxCollision) (Math|Vector|MakeVector _returnvalue_5 _returnvalue_5 (Math|Random|RandomFloatinRange (Variables|Default|GetInitialZImpulseMin) (Variables|Default|GetInitialZImpulseMax))) "None" false)
  (if (> (Variables|Default|GetInitialRotationMax) 0.0)
    (Class|PrimitiveComponent|AddAngularImpulseinDegrees (Variables|Default|GetPhsxCollision) (Math|Vector|MakeVector 0.0 0.0 (Math|Random|RandomFloatinRange (/ _initialrotationmax 2.0) _initialrotationmax)) "None" false)))

(event EventNotifyPickupCollected
  (CallFunction|MConPickupFX)
  (|CallParentFunction))

(fn ConstructionScript
  (CallFunction|AdjustOverlapBounds))

(fn AdjustOverlapBounds
  (Components|Sphere|SetSphereRadius (Variables|Default|GetPickupOverlap) (Math|Conversions|ToFloat(Integer) (Math|Float|Ceil (Math|Float|Clamp(Float) (* (.SphereRadius (Collision|GetComponentBounds (Variables|Default|GetPickupMesh))) 1.5) 3e+01 1e+02))) false))

(fn GetItemDisplayName
  (bind _pickupgoods (Class|TRPickupBase|GetPickupGoods))
  (bind _output_get (LocalVariables|SettmpPickupGoods _pickupgoods))
  (if (Utilities|Array|IsValidIndex _output_get)
    (if (.Found (CallFunction|GetGoodsQuantityData (Utilities|Array|Get(acopy) (LocalVariables|GettmpPickupGoods))))
      (return (.DisplayName (Utilities|Struct|BreakGoodsType (.GoodsData (Utilities|Struct|BreakGoodsTypeQuantity (.GoodsQuantityData (CallFunction|GetGoodsQuantityData (Utilities|Array|Get(acopy) (LocalVariables|GettmpPickupGoods)))))))))
      (else
        _)))
  (return ""))

(fn GetInspectInfo
  (bind _pickupgoods (Class|TRPickupBase|GetPickupGoods))
  (LocalVariables|SettmpPickupGoods _pickupgoods)
  (bind _returnvalue (CallFunction|GetItemDisplayName))
  (Utilities|Struct|SetmembersinInspectInfo (LocalVariables|GettmpInspectInfo) _returnvalue)
  (for _array_element (.GoodsTypeQuantities (CallFunction|GetAllGoodsQuantitiesData (LocalVariables|GettmpPickupGoods)))
    (Utilities|Array|Add (.DetailInfo (Utilities|Struct|BreakInspectInfo (LocalVariables|GettmpInspectInfo))) (Utilities|Struct|MakeInspectInfoItem (.DisplayName (Utilities|Struct|BreakGoodsType (.GoodsData (Utilities|Struct|BreakGoodsTypeQuantity _array_element)))) (Utilities|Text|ToText(Float) (.Quantity (Utilities|Struct|BreakGoodsTypeQuantity _array_element)) "HalfToEven"))))
  (return (LocalVariables|GettmpInspectInfo)))
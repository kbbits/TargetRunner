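; Base Blueprint for Target Runner weapon mods, providing automatic and burst-limited fire for the first-person character that is its parent actor.
; BeginAutoFire resets the counters and fires immediately, and EndAutoFire stops firing.
; Tick accumulates time, carrying over the remainder, and calls the character's ClientSpawnProjetile after each delay until the burst limit, where zero means unlimited.
; The construction script tints the mesh with BaseColor.
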(event Custom|BeginAutoFire
  (Variables|Default|SetIsAutoFiring true)
  (Variables|Default|SetAutoFireBurstCount 0.0)
  (Variables|Default|SetAutoFireDelaySum 0.0)
  (bind _astr_first_person_character (Utilities|Casting|CastToTR_FirstPersonCharacter (Actor|GetParentActor)))
  (Default|ClientSpawnProjetile _astr_first_person_character)
  (Math|Float|IncrementFloat (Variables|Default|GetAutoFireBurstCount)))

(event Custom|EndAutoFire
  (Variables|Default|SetIsAutoFiring false)
  (Variables|Default|SetAutoFireBurstCount 0.0)
  (Variables|Default|SetAutoFireDelaySum 0.0))

(event EventTick
  (params (DeltaSeconds :type Float%20%28single-precision%29))
  (if (Variables|Default|GetIsAutoFiring)
    (if (or (== (Variables|Default|GetAutoFireBurstLimit) 0.0) (< (Variables|Default|GetAutoFireBurstCount) (Variables|Default|GetAutoFireBurstLimit)))
      (if (>= (+ DeltaSeconds (Variables|Default|GetAutoFireDelaySum)) (Variables|Default|GetAutoFireDelay))
        (Variables|Default|SetAutoFireDelaySum (- (+ DeltaSeconds (Variables|Default|GetAutoFireDelaySum)) (Variables|Default|GetAutoFireDelay)))
        (bind _astr_first_person_character (Utilities|Casting|CastToTR_FirstPersonCharacter (Actor|GetParentActor)))
        (Default|ClientSpawnProjetile _astr_first_person_character)
        (Math|Float|IncrementFloat (Variables|Default|GetAutoFireBurstCount))
        (else
          (Variables|Default|SetAutoFireDelaySum (+ DeltaSeconds (Variables|Default|GetAutoFireDelaySum))))))))

(fn ConstructionScript
  (Rendering|Material|SetVectorParameterValueonMaterials (Variables|Default|GetStaticMesh) "DiffuseColor" (Math|Conversions|ToVector(LinearColor) (Math|Color|SelectColor :A (Variables|Default|GetBaseColor) :bPickA true))))
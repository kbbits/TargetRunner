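; Base pickup projectile that homes in on a target and awards Energy or Shards to the player character it touches, then destroys itself.
; Tick eases its scale up while Expanding, then starts the homing component and raises homing agility once a quarter of its lifespan passes.
; Hit events award only on authority while Flying, whereas box overlap awards directly.
; UpdateMesh tints materials by award type.
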(event OnStartHoming(HomingMovementManagerComponent)
  ;[1 1 1] Homing
  (Variables|Default|SetProjectileState "NewEnumerator1"))

(event OnStopHoming(HomingMovementManagerComponent)
  ;[1 1 1] Homing
  (Variables|Default|SetProjectileState (Variables|Default|GetProjectileState)))

(event OnComponentHit(BoxCollision)
  (params (HitComponent :type Primitive%20Component%20Object%20Reference) (OtherActor :type Actor%20Object%20Reference) (OtherComp :type Primitive%20Component%20Object%20Reference) (NormalImpulse :type Vector :default "0, 0, 0") (Hit :type Hit%20Result%20Structure%20%28by%20ref%29))
  (CallFunction|HandleHitBase HitComponent OtherActor OtherComp NormalImpulse Hit))

(event OnComponentHit(ProjectileMesh)
  (params (HitComponent :type Primitive%20Component%20Object%20Reference) (OtherActor :type Actor%20Object%20Reference) (OtherComp :type Primitive%20Component%20Object%20Reference) (NormalImpulse :type Vector :default "0, 0, 0") (Hit :type Hit%20Result%20Structure%20%28by%20ref%29))
  (CallFunction|HandleHitBase HitComponent OtherActor OtherComp NormalImpulse Hit))

(event OnTargetAquired(HomingMovementManagerComponent)
  ;[1 1 1] Homing
  (Variables|Default|SetProjectileState "NewEnumerator1"))

(event OnComponentBeginOverlap(BoxCollision)
  (params (OverlappedComponent :type Primitive%20Component%20Object%20Reference) (OtherActor :type Actor%20Object%20Reference) (OtherComp :type Primitive%20Component%20Object%20Reference) (OtherBodyIndex :type Integer) (bFromSweep :type Boolean) (SweepResult :type Hit%20Result%20Structure%20%28by%20ref%29))
  (bind _ascharacter (Utilities|Casting|CastToCharacter OtherActor))
  (CallFunction|OnHitPlayer _ascharacter))

(event OnTargetLost(HomingMovementManagerComponent)
  ;[1 1 1] Homing
  (Variables|Default|SetProjectileState (Variables|Default|GetProjectileState)))

(event Custom|HandleHit_Base
  (params (HitComponent :type Primitive%20Component%20Object%20Reference) (OtherActor :type Actor%20Object%20Reference) (OtherComponent :type Primitive%20Component%20Object%20Reference) (NormalImpulse :type Vector) (Hit :type Hit%20Result%20Structure))
  ;[1 1 1] Target hit something while it is flying around
  (Networking|SwitchHasAuthority
    (:Authority
      (if (Utilities|Enum|Equal(Enum) (Variables|Default|GetProjectileState) "NewEnumerator1")
        (bind _ascharacter (Utilities|Casting|CastToCharacter OtherActor))
        (CallFunction|OnHitPlayer _ascharacter)))))

(event Custom|OnHitPlayer
  (params (PlayerCharacter :type Character%20Object%20Reference))
  (bind _astr_first_person_character (Utilities|Casting|CastToTR_FirstPersonCharacter PlayerCharacter))
  (Utilities|IsValid (Pawn|GetController _astr_first_person_character)
    (:Is%20Valid
      (if (> (Variables|Default|GetAwardAmount) 0.0)
        (bind _astr_player_state (Utilities|Casting|CastToTR_PlayerState (Variables|/Script/Engine.Controller|GetPlayerState (Pawn|GetController _astr_first_person_character))))
        (switch Utilities|FlowControl|Switch|SwitchonPickupAwards (Variables|Default|GetAwardType)
          (:NewEnumerator0
            (Default|AddEnergy _astr_player_state (Variables|Default|GetAwardAmount)))
          (:NewEnumerator1
            (Default|AddSubtractShards _astr_player_state (Variables|Default|GetAwardAmount))))
        (Variables|Default|SetAwardAmount 0.0)
        (Actor|DestroyActor)))))

(event Custom|MC_HitTarget
  (params (Instigator :type Pawn%20Object%20Reference) (Hit :type Hit%20Result%20Structure) (Destroyed :type Boolean) (ScoreValue :type Float%20%28single-precision%29))
  ;[1 1 1] MC Hit target - Client side hit FX
  (Audio|PlaySoundatLocation (select Destroyed "/Game/TargetRunner/Assets/Audio/PopShort_01.PopShort_01" 0) (.ImpactPoint (Collision|BreakHitResult Hit)) "0, 0, 0" 3.0 1.0 0.0 0 0 0)
  (if Destroyed
    (Effects|SpawnEmitteratLocation "/Game/TargetRunner/Assets/FX/Particles/TR_TargetExplode_01.TR_TargetExplode_01" (Transformation|GetActorLocation))
    (else
      (CallFunction|UpdateMesh))))

(event EventBeginPlay
  ;[1 1 1] BeginPlay
  (if (Variables|Default|GetRotateToHorizonalOnLaunch)
    (Transformation|SetWorldRotation (Variables|Transformation|GetRootComponent) (Math|Rotator|MakeRotator 0.0 0.0 (.Yaw (Math|Rotator|BreakRotator (Transformation|GetActorRotation)))) false true)))

(event EventTick
  (params (DeltaSeconds :type Float%20%28single-precision%29))
  ;[1 1 1] Tick
  (switch Utilities|FlowControl|Switch|SwitchonLauncherProjectileState (Variables|Default|GetProjectileState)
    (:NewEnumerator0
      (CallFunction|ExpandMesh DeltaSeconds))
    (:NewEnumerator1
      (Utilities|FlowControl|DoOnce false :!label _label
        (:Completed
          (if (<= (/ (Actor|GetLifeSpan) (Variables|Actor|GetInitialLifeSpan)) 0.75)
            (Variables|/Game/TargetRunner/Blueprints/General/HomingMovementManagerComponent.HomingMovementManagerComponent_C|SetHomingAgility (Variables|Default|GetHomingMovementManagerComponent) 1.25)
            (else
              (goto _label Reset))))))
    (:NewEnumerator3
      (goto _label))))

(fn ConstructionScript
  (Variables|Default|SetBaseRotationRate (Variables|/Script/Engine.RotatingMovementComponent|GetRotationRate (Variables|Default|GetRotatingMovement)))
  (CallFunction|UpdateMesh))

(fn ExpandMesh
  (params (DeltaSeconds :type Float%20%28single-precision%29))
  (switch Utilities|FlowControl|Switch|SwitchonLauncherProjectileState (Variables|Default|GetProjectileState)
    (:NewEnumerator0
      (Variables|Default|SetExpandTimeSum (+ DeltaSeconds (Variables|Default|GetExpandTimeSum)))
      (if (== (Class|KismetMathLibrary|FInterpEaseinOut (.X (Math|Vector|BreakVector (Transformation|GetActorScale3D))) (Variables|Default|GetFinalScale) (/ (Variables|Default|GetExpandTimeSum) (Variables|Default|GetExpandTime)) 1.5) (Variables|Default|GetFinalScale))
        (Transformation|SetActorScale3D (* "1.000000,1.000000,1.000000" (Variables|Default|GetFinalScale)))
        (Variables|Default|SetProjectileState "NewEnumerator1")
        (Default|StartHoming (Variables|Default|GetHomingMovementManagerComponent))
        (else
          (Transformation|SetActorScale3D (* "1.000000,1.000000,1.000000" (Class|KismetMathLibrary|FInterpEaseinOut (.X (Math|Vector|BreakVector (Transformation|GetActorScale3D))) (Variables|Default|GetFinalScale) (/ (Variables|Default|GetExpandTimeSum) (Variables|Default|GetExpandTime)) 1.5))))))))

(fn OnRepProjectileState
  (CallFunction|UpdateMesh))

(fn UpdateMesh
  (bind _output_get (LocalVariables|SettmpMesh (Variables|Default|GetProjectileMesh)))
  (Utilities|IsValid _output_get
    (:Is%20Valid
      (Rendering|Material|SetVectorParameterValueonMaterials (LocalVariables|GettmpMesh) "BaseColor" (Math|Conversions|ToVector(LinearColor) (Utilities|Select :Index (Variables|Default|GetAwardType) :NewEnumerator0 "(R=0.019608,G=0.180392,B=0.749020,A=1.000000)" :NewEnumerator1 "(R=1.000000,G=0.738211,B=0.000000,A=1.000000)")))
      (Rendering|Material|SetVectorParameterValueonMaterials (LocalVariables|GettmpMesh) "EmissiveColor" (Math|Conversions|ToVector(LinearColor) (Utilities|Select :Index (Variables|Default|GetAwardType) :NewEnumerator0 "(R=0.121569,G=0.749020,B=0.729412,A=1.000000)" :NewEnumerator1 "(R=1.000000,G=0.824724,B=0.270759,A=1.000000)"))))))

(fn EdGraph51
  (if (Variables|Default|GetStopped)
    (return (Variables|Default|GetBaseDestroyScoreValue) 0.0)
    (else
      (return (/ (Variables|Default|GetBaseDestroyScoreValue) 3.0) 0.0))))
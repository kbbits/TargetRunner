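; Base Blueprint for homing pickups that reacts to events from its HomingMovementManagerComponent.
; Target acquired and lost events flip the User.AttractorAnimDirection parameter between forward and reverse on every effect system in MyChunkSystems.
; Homing start and stop only print debug messages, as the nodes that toggle collision physics simulation are disconnected.
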(event OnStartHoming(HomingMovementManagerComponent)
  (Development|PrintString (Utilities|String|Append (Utilities|GetDisplayName self) " is Homing")))

(event OnTargetAquired(HomingMovementManagerComponent)
  (for _array_element (Variables|Default|GetMyChunkSystems)
    (Niagara|SetNiagaraVariable(Float) _array_element "User.AttractorAnimDirection" 1.0)))

(event OnTargetLost(HomingMovementManagerComponent)
  (for _array_element (Variables|Default|GetMyChunkSystems)
    (Niagara|SetNiagaraVariable(Float) _array_element "User.AttractorAnimDirection" -1.0)))

(event OnStopHoming(HomingMovementManagerComponent)
  (Development|PrintString (Utilities|String|Append (Utilities|GetDisplayName self) " stopped Homing")))

(fn ConstructionScript
  (|CallParentFunction))
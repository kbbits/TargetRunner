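; PickupPillar is a glowing pillar actor that spawns pickup rewards around itself.
; A timeline pulses the pillar material's emissive factor and its point light intensity together.
; GiveAwards spawns each class in the Awards map by its count at random angles around the pillar, applying radial impulses to physics-simulated pickups.
; Capsule overlap only casts to the player character and controller; nothing here calls GiveAwards.
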(event OnComponentBeginOverlap(Capsule)
  (params (OverlappedComponent :type Primitive%20Component%20Object%20Reference) (OtherActor :type Actor%20Object%20Reference) (OtherComp :type Primitive%20Component%20Object%20Reference) (OtherBodyIndex :type Integer) (bFromSweep :type Boolean) (SweepResult :type Hit%20Result%20Structure%20%28by%20ref%29))
  (bind _astr_first_person_character (Utilities|Casting|CastToTR_FirstPersonCharacter OtherActor))
  (bind _astr_player_controller_base (Utilities|Casting|CastToTR_PlayerController_Base (Pawn|GetController _astr_first_person_character))))

(event Custom|GiveAwards
  (bind _keys (Utilities|Map|Keys (Variables|Default|GetAwards)))
  (for _array_element _keys
    (for _index (range 1 (.Value (Utilities|Map|Find (Variables|Default|GetAwards) _array_element)))
      (CallFunction|SpawnSingleAward _array_element))))

(event EventBeginPlay
  (bind _pulsevalue (Timeline|PulseTimeline PlayFromStart)
    (:Update
      (Rendering|Material|SetScalarParameterValueonMaterials (Variables|Default|GetPillar) "EmissiveFactor" _pulsevalue)
      (Rendering|Components|Light|SetIntensity (Variables|Default|GetPointLight) (* _pulsevalue 3.2e+03)))))

(fn ConstructionScript)

(fn SpawnSingleAward
  (params (PickupClass :type Pickup%20Base%20BP%20Class%20Reference))
  (LocalVariables|SettmpPickupClass PickupClass)
  (LocalVariables|SettmpSpawnDirection (Math|Rotator|MakeRotator 0.0 0.0 (Math|Random|RandomFloatinRange 0.0 3.6e+02)))
  (bind _returnvalue (Game|SpawnActorfromClass (LocalVariables|GettmpPickupClass) (Math|Transform|MakeTransform (+ (Transformation|GetWorldLocation (Variables|Default|GetPickupSpawnPoint)) (* (Math|Vector|GetForwardVector (LocalVariables|GettmpSpawnDirection)) (* (.X (Math|Vector|BreakVector (.BoxExtent (Collision|GetComponentBounds (Variables|Default|GetPillar))))) 1.2))) (LocalVariables|GettmpSpawnDirection)) "AdjustIfPossibleButAlwaysSpawn" 0 0))
  (bind _aspickup_base_bp (Utilities|Casting|CastToPickup_BaseBP _returnvalue))
  (if (Physics|IsSimulatingPhysics (Variables|/Game/TargetRunner/Blueprints/Pickups/Pickup_BaseBP.Pickup_BaseBP_C|GetPickupMesh _aspickup_base_bp) "None")
    (Physics|AddRadialImpulse (Variables|/Game/TargetRunner/Blueprints/Pickups/Pickup_BaseBP.Pickup_BaseBP_C|GetPickupMesh _aspickup_base_bp) (+ (Transformation|GetWorldLocation (Variables|Default|GetPickupSpawnPoint)) "0, 0,-50.000000") 1e+02 3e+02 "RIF_Constant" false)))
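; Goods pickup actor that sets its appearance from the first entry in PickupGoods.
; InitFromGoods, run at construction and BeginPlay, applies the goods' default mesh, or without one puts its thumbnail on material slot 1 via a dynamic instance.
; Soft references are async-loaded when not in memory, then AdjustOverlapBounds runs.
; Disconnected leftover nodes hold an unused resource-type path with random mesh and default material.
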(event Custom|InitFromGoods
  (bind _pickupgoods (Variables|Default|GetPickupGoods))
  (bind _output (Utilities|Array|Get(acopy) _pickupgoods))
  (bind (_found _goodsquantitydata) (CallFunction|GetGoodsQuantityData _output))
  (if (Utilities|Array|IsValidIndex (Variables|Default|GetPickupGoods))
    (if _found
      (Variables|Default|SetTmpGoodsQuantityData _goodsquantitydata)
      (bind _output_get (Variables|Default|SetTmpPickupMeshRef (.DefaultMesh (Utilities|Struct|BreakGoodsType (.GoodsData (Utilities|Struct|BreakGoodsTypeQuantity (Variables|Default|GetTmpGoodsQuantityData)))))))
      (if (Utilities|IsValidSoftObjectReference _output_get)
        (Utilities|IsValid (Utilities|ResolveSoftReference (Variables|Default|GetTmpPickupMeshRef))
          (:Is%20Valid
            (Components|StaticMesh|SetStaticMesh (Variables|Default|GetPickupMesh) (Utilities|ResolveSoftReference (Variables|Default|GetTmpPickupMeshRef))))
          (:Is%20Not%20Valid
            (bind _object (Utilities|AsyncLoadAsset (Variables|Default|GetTmpPickupMeshRef))
              (:Completed
                (bind _asstatic_mesh (Utilities|Casting|CastToStaticMesh _object))
                (Components|StaticMesh|SetStaticMesh (Variables|Default|GetPickupMesh) _asstatic_mesh)))))
        (CallFunction|AdjustOverlapBounds :!label _label)
        (Variables|Default|SetTmpGoodsImageTexture 0)
        (elif (Utilities|IsValidSoftObjectReference (.Thumbnail (Utilities|Struct|BreakGoodsType (.GoodsData (Utilities|Struct|BreakGoodsTypeQuantity (Variables|Default|GetTmpGoodsQuantityData))))))
          (Utilities|IsValid (Utilities|ResolveSoftReference (.Thumbnail (Utilities|Struct|BreakGoodsType (.GoodsData (Utilities|Struct|BreakGoodsTypeQuantity (Variables|Default|GetTmpGoodsQuantityData))))))
            (:Is%20Valid
              (Variables|Default|SetTmpGoodsImageTexture (Utilities|ResolveSoftReference (.Thumbnail (Utilities|Struct|BreakGoodsType (.GoodsData (Utilities|Struct|BreakGoodsTypeQuantity (Variables|Default|GetTmpGoodsQuantityData))))))))
            (:Is%20Not%20Valid
              (bind _object_2 (Utilities|AsyncLoadAsset (.Thumbnail (Utilities|Struct|BreakGoodsType (.GoodsData (Utilities|Struct|BreakGoodsTypeQuantity (Variables|Default|GetTmpGoodsQuantityData))))))
                (:Completed
                  (bind _astexture_2d (Utilities|Casting|CastToTexture2D _object_2))
                  (Variables|Default|SetTmpGoodsImageTexture _astexture_2d)))))
          (bind _returnvalue (Rendering|Material|CreateDynamicMaterialInstance (Variables|Default|GetPickupMesh) 1 0 "None" :!class /Script/Engine.PrimitiveComponent))
          (Rendering|Material|SetTextureParameterValue _returnvalue "Image" (Variables|Default|GetTmpGoodsImageTexture))
          (Rendering|Material|SetMaterial (Variables|Default|GetPickupMesh) 1 _returnvalue)
          (goto _label))))))

(event EventBeginPlay
  (CallFunction|InitfromGoods))

(fn ConstructionScript
  (CallFunction|InitfromGoods))
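; Base pickup actor for TargetRunner that displays its goods as Niagara chunk particle effects.
; Construction rebuilds one system per PickupGoods entry, scaling spawn count by quantity and attaching it to Sphere1.
; A valid ExplodingMesh feeds a mesh-based system; otherwise a point explosion is oriented along the initiating impact normal.
; All systems currently share ResourceMaterial, pending per-goods materials, and are destroyed with the actor.
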(event EventDestroyed
  (CallFunction|KillGoodsParticleSystems))

(event EventTick
  (params (DeltaSeconds :type Float%20%28single-precision%29)))

(fn ConstructionScript
  (CallFunction|SpawnGoodsParticleSystems))

(fn SpawnGoodsParticleSystems
  (CallFunction|KillGoodsParticleSystems)
  (for _array_element (Variables|Default|GetPickupGoods)
    (Utilities|IsValid (Variables|Default|GetExplodingMesh)
      (:Is%20Valid
        (bind _returnvalue (AddComponent|AddNiagaraComponent true)) ; Exploding Mesh System
        (bind _output_get (LocalVariables|SettmpNewPS _returnvalue))
        (Utilities|Array|Add (Variables|Default|GetMyChunkSystems) _output_get)
        (Class|NiagaraComponent|SetVariableInt (LocalVariables|GettmpNewPS) "User.SpawnCount" (Math|Float|Truncate (Math|Float|MapRangeClamped (.Quantity (Utilities|Struct|BreakGoodsQuantity _array_element)) 1.0 1e+03 1.0 2e+02)))
        (Class|NiagaraFunctionLibrary|OverrideSystemUserVariableStaticMesh (LocalVariables|GettmpNewPS) "User.NodeMesh" (Variables|Default|GetExplodingMesh))
        ;[1 1 1] TODO: Set material based on goods type
        (Class|NiagaraComponent|SetVariableMaterial (LocalVariables|GettmpNewPS) "User.ParticleMaterial" (Variables|Default|GetResourceMaterial))
        (Niagara|SetNiagaraVariable(Float) (LocalVariables|GettmpNewPS) "User.AttractorAnimDirection" 0.0)
        (Transformation|AttachComponentToComponent (LocalVariables|GettmpNewPS) (Variables|Default|GetSphere1) "None" "KeepRelative" "KeepRelative" "KeepRelative" true))
      (:Is%20Not%20Valid
        (bind _returnvalue_2 (AddComponent|AddNiagaraComponent true)) ; Point Explostion System
        (bind _output_get_2 (LocalVariables|SettmpNewPS _returnvalue_2))
        (Utilities|Array|Add (Variables|Default|GetMyChunkSystems) _output_get_2)
        (Class|NiagaraComponent|SetVariableInt (LocalVariables|GettmpNewPS) "User.SpawnCount" (Math|Float|Truncate (Math|Float|MapRangeClamped (.Quantity (Utilities|Struct|BreakGoodsQuantity _array_element)) 1.0 1e+03 1.0 2e+02)))
        ;[1 1 1] TODO: Set material based on goods type
        (Class|NiagaraComponent|SetVariableMaterial (LocalVariables|GettmpNewPS) "User.ParticleMaterial" (Variables|Default|GetResourceMaterial))
        (Niagara|SetNiagaraVariable(Float) (LocalVariables|GettmpNewPS) "User.AttractorAnimDirection" 0.0)
        (Transformation|AttachComponentToComponent (LocalVariables|GettmpNewPS) (Variables|Default|GetSphere1) "None" "KeepRelative" "KeepRelative" "KeepRelative" true)
        (Transformation|SetRelativeRotation (LocalVariables|GettmpNewPS) (Math|Rotator|MakeRotfromZ (Math|Vector|Normalize (Variables|Default|GetInitiatingImpactNormal))) false true)))))

(fn KillGoodsParticleSystems
  (for _array_element (Variables|Default|GetMyChunkSystems)
    (Class|NiagaraComponent|SetRenderingEnabled _array_element false)
    (Components|Activation|Deactivate _array_element)
    (Components|DestroyComponent _array_element))
  (Utilities|Array|Clear (Variables|Default|GetMyChunkSystems)))
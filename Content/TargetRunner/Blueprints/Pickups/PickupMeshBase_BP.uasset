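; Base Blueprint for mesh-based pickups in TargetRunner that carry resource goods and can report inspect info.
; The construction script centers the overlap sphere on the mesh bounds and scales its radius from those bounds within a clamped range.
; The display name comes from the first goods entry, or is empty if none is found.
; Inspect info combines that name with a detail line for each goods type and quantity.
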(event EventBeginPlay
  (|CallParentFunction))

(fn ConstructionScript
  (CallFunction|AdjustOverlapBounds))

(fn AdjustOverlapBounds
  (bind _pickupmesh (Variables|Default|GetPickupMesh))
  (bind _pickupoverlap (Variables|Default|GetPickupOverlap))
  (bind (_origin _boxextent _sphereradius) (Collision|GetComponentBounds _pickupmesh))
  (Transformation|SetRelativeLocation _pickupoverlap (- _origin (Transformation|GetActorLocation)) false true)
  (Components|Sphere|SetSphereRadius _pickupoverlap (Math|Conversions|ToFloat(Integer) (Math|Float|Ceil (Math|Float|Clamp(Float) (* _sphereradius 1.5) 3e+01 1e+02))) false))

(fn GetItemDisplayName
  (bind _collectedgoods (Class|TRPickupBase|GetResourceGoods))
  (bind _output_get (LocalVariables|SettmpPickupGoods _collectedgoods))
  (if (Utilities|Array|IsValidIndex _output_get)
    (if (.Found (CallFunction|GetGoodsQuantityData (Utilities|Array|Get(acopy) (LocalVariables|GettmpPickupGoods))))
      (return (.DisplayName (Utilities|Struct|BreakGoodsType (.GoodsData (Utilities|Struct|BreakGoodsTypeQuantity (.GoodsQuantityData (CallFunction|GetGoodsQuantityData (Utilities|Array|Get(acopy) (LocalVariables|GettmpPickupGoods)))))))))
      (else
        _)))
  (return ""))

(fn GetInspectInfo
  (bind _collectedgoods (Class|TRPickupBase|GetResourceGoods))
  (LocalVariables|SettmpPickupGoods _collectedgoods)
  (bind _returnvalue (CallFunction|GetItemDisplayName))
  (Utilities|Struct|SetmembersinInspectInfo (LocalVariables|GettmpInspectInfo) _returnvalue)
  (for _array_element (.GoodsTypeQuantities (CallFunction|GetAllGoodsQuantitiesData (LocalVariables|GettmpPickupGoods)))
    (Utilities|Array|Add (.DetailInfo (Utilities|Struct|BreakInspectInfo (LocalVariables|GettmpInspectInfo))) (Utilities|Struct|MakeInspectInfoItem (.DisplayName (Utilities|Struct|BreakGoodsType (.GoodsData (Utilities|Struct|BreakGoodsTypeQuantity _array_element)))) (Utilities|Text|ToText(Float) (.Quantity (Utilities|Struct|BreakGoodsTypeQuantity _array_element)) "HalfToEven"))))
  (return (LocalVariables|GettmpInspectInfo)))
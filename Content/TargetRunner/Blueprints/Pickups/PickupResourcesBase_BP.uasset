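; Base resource pickup that shows its goods as Niagara chunk particle systems.
; BeginPlay and the OnRep handlers resolve the soft mesh and material references, async loading when needed, and spawn particles once both initialize.
; Each goods entry gets a component with spawn count scaled by quantity, using either the exploding mesh or a point burst aligned to the impact normal.
; Systems are cleared before respawning and on Destroyed.
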(event Custom|SetParticleResourceMaterial
  (bind _resourcematerialtype (Variables|Default|GetResourceMaterialType))
  (bind _output (Utilities|ResolveSoftReference _resourcematerialtype))
  (Utilities|IsValid (Variables|Default|GetResourceMaterial)
    (:Is%20Valid
      (Variables|Default|SetbMaterialInitialized true :!label _label)
      (CallFunction|TrySpawnParticleSystem))
    (:Is%20Not%20Valid
      (if (Utilities|IsValidSoftObjectReference _resourcematerialtype)
        (Utilities|IsValid _output
          (:Is%20Valid
            (Variables|Default|SetResourceMaterial _output)
            (goto _label))
          (:Is%20Not%20Valid
            (bind _object (Utilities|AsyncLoadAsset (Variables|Default|GetResourceMaterialType))
              (:Completed
                (bind _asmaterial_interface (Utilities|Casting|CastToMaterialInterface _object))
                (Variables|Default|SetResourceMaterial _asmaterial_interface)
                (goto _label)))))))))

(event Custom|SetParticleExplodingMesh
  (bind _explodingmeshtype (Variables|Default|GetExplodingMeshType))
  (bind _output (Utilities|ResolveSoftReference _explodingmeshtype))
  (if (Utilities|IsValidSoftClassReference (Variables|Default|GetExplodingMeshType))
    (Utilities|IsValid (Variables|Default|GetExplodingMesh)
      (:Is%20Valid
        _)
      (:Is%20Not%20Valid
        (if (Utilities|IsValidClass _output)
          (bind _returnvalue (Game|ConstructObjectfromClass _output self))
          (Variables|Default|SetExplodingMesh _returnvalue)
          (else
            (bind _class (Utilities|AsyncLoadClassAsset (Variables|Default|GetExplodingMeshType))
              (:Completed
                (bind _asstatic_mesh (Utilities|Casting|CastToStaticMeshClass _class))
                (bind _returnvalue_2 (Game|ConstructObjectfromClass _asstatic_mesh self))
                (Variables|Default|SetExplodingMesh _returnvalue_2)))))))
    (Variables|Default|SetbMeshInitialized true)
    (CallFunction|TrySpawnParticleSystem)
    (else
      (Variables|Default|SetbMeshInitialized true))))

(event Custom|TrySpawnParticleSystem
  (if (and (Variables|Default|GetbMeshInitialized) (Variables|Default|GetbMaterialInitialized)) ; If we have all replicated info, spawn the system
    (CallFunction|SpawnGoodsParticleSystems) ; Spawn on client and server
    (else
      (Development|PrintString (Utilities|String|Append "TrySpawnParticles MeshInit: " (Utilities|String|ToString(Boolean) (Variables|Default|GetbMeshInitialized)) " MaterialInit: " (Utilities|String|ToString(Boolean) (Variables|Default|GetbMaterialInitialized)))))))

(event EventDestroyed
  (CallFunction|KillGoodsParticleSystems))

(event EventBeginPlay
  ;[1 1 1] Wait for replicated info.
  (CallFunction|SetParticleExplodingMesh)
  (CallFunction|SetParticleResourceMaterial))

(fn ConstructionScript)

(fn SpawnGoodsParticleSystems
  (CallFunction|KillGoodsParticleSystems)
  (bind _pickupgoods (Class|TRPickupBase|GetPickupGoods))
  (bind _output_get (LocalVariables|SettmpPickupGoods _pickupgoods))
  (for _array_element _output_get
    (Utilities|IsValid (Variables|Default|GetExplodingMesh)
      (:Is%20Valid
        (bind _returnvalue (AddComponent|AddNiagaraComponent true)) ; Exploding Mesh System
        (bind _output_get_2 (LocalVariables|SettmpNewPS _returnvalue))
        (Utilities|Array|Add (Variables|Default|GetMyChunkSystems) _output_get_2)
        (Class|NiagaraComponent|SetVariableInt (LocalVariables|GettmpNewPS) "User.SpawnCount" (Math|Float|Truncate (Math|Float|MapRangeClamped (.Quantity (Utilities|Struct|BreakGoodsQuantity _array_element)) 1.0 1e+03 1.0 2e+02)))
        (Class|NiagaraFunctionLibrary|OverrideSystemUserVariableStaticMesh (LocalVariables|GettmpNewPS) "User.NodeMesh" (Variables|Default|GetExplodingMesh))
        (Class|NiagaraComponent|SetVariableMaterial (LocalVariables|GettmpNewPS) "User.ParticleMaterial" (Variables|Default|GetResourceMaterial))
        (Niagara|SetNiagaraVariable(Float) (LocalVariables|GettmpNewPS) "User.AttractorAnimDirection" 0.0)
        (Transformation|AttachComponentToComponent (LocalVariables|GettmpNewPS) (Variables|Default|GetPickupCollision) "None" "KeepRelative" "KeepRelative" "KeepRelative" true))
      (:Is%20Not%20Valid
        (bind _returnvalue_2 (AddComponent|AddNiagaraComponent true)) ; Point Explosion System
        (bind _output_get_3 (LocalVariables|SettmpNewPS _returnvalue_2))
        (Utilities|Array|Add (Variables|Default|GetMyChunkSystems) _output_get_3)
        (Class|NiagaraComponent|SetVariableInt (LocalVariables|GettmpNewPS) "User.SpawnCount" (Math|Float|Truncate (Math|Float|MapRangeClamped (.Quantity (Utilities|Struct|BreakGoodsQuantity _array_element)) 1.0 1e+03 1.0 2e+02)))
        (Class|NiagaraComponent|SetVariableMaterial (LocalVariables|GettmpNewPS) "User.ParticleMaterial" (Variables|Default|GetResourceMaterial))
        (Niagara|SetNiagaraVariable(Float) (LocalVariables|GettmpNewPS) "User.AttractorAnimDirection" 0.0)
        (Transformation|AttachComponentToComponent (LocalVariables|GettmpNewPS) (Variables|Default|GetPickupCollision) "None" "SnapToTarget" "KeepRelative" "KeepRelative" true)
        (Transformation|SetRelativeRotation (LocalVariables|GettmpNewPS) (Math|Rotator|MakeRotfromZ (Math|Vector|Normalize (Variables|Default|GetInitiatingImpactNormal))) false true)
        (Components|Activation|Activate (LocalVariables|GettmpNewPS) false))))
  (Variables|Default|SetbParticleSystemSpawned true))

(fn KillGoodsParticleSystems
  (for _array_element (Variables|Default|GetMyChunkSystems)
    (Class|NiagaraComponent|SetRenderingEnabled _array_element false)
    (Components|Activation|Deactivate _array_element)
    (Components|DestroyComponent _array_element))
  (Utilities|Array|Clear (Variables|Default|GetMyChunkSystems)))

(fn OnRepResourceMaterialType
  (CallFunction|SetParticleResourceMaterial))

(fn OnRepExplodingMeshType
  (CallFunction|SetParticleExplodingMesh))
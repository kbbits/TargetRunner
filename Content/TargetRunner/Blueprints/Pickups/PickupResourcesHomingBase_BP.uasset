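; Base Blueprint for homing resource pickups, adding visual feedback as the pickup gains or loses a homing target.
; HomingMovementManagerComponent's target acquired and lost events loop over MyChunkSystems, flipping the User.AttractorAnimDirection effect parameter between forward and reverse.
; Start and stop homing events are empty; debug prints and collision physics toggles are left disconnected.
; The construction script only calls the parent.
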(event OnStartHoming(HomingMovementManagerComponent))

(event OnTargetAquired(HomingMovementManagerComponent)
  (for _array_element (Variables|Default|GetMyChunkSystems)
    (Niagara|SetNiagaraVariable(Float) _array_element "User.AttractorAnimDirection" 1.0)))

(event OnTargetLost(HomingMovementManagerComponent)
  (for _array_element (Variables|Default|GetMyChunkSystems)
    (Niagara|SetNiagaraVariable(Float) _array_element "User.AttractorAnimDirection" -1.0)))

(event OnStopHoming(HomingMovementManagerComponent))

(fn ConstructionScript
  (|CallParentFunction))
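; Base pickup actor that awards energy, goods, ammo or a weapon to a character that overlaps it.
; On spawn it eases up to final scale, then the server switches its projectile state from Expanding to Flying.
; The server checks capacity (energy needs room for 75% of the amount), passes awards to the player controller, then destroys the actor.
; Energy and goods pickups get type-based material colors, refreshed in the state's OnRep.
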(event OnComponentBeginOverlap(PickupCollision)
  (params (OverlappedComponent :type Primitive%20Component%20Object%20Reference) (OtherActor :type Actor%20Object%20Reference) (OtherComp :type Primitive%20Component%20Object%20Reference) (OtherBodyIndex :type Integer) (bFromSweep :type Boolean) (SweepResult :type Hit%20Result%20Structure%20%28by%20ref%29))
  (bind _returnvalue (Actor|GetParentActor OtherActor))
  (bind _ascharacter (Utilities|Casting|CastToCharacter OtherActor)
    (:then
      (CallFunction|OnHitPlayer _ascharacter))
    (:CastFailed
      (Utilities|IsValid _returnvalue
        (:Is%20Valid
          (bind _ascharacter_2 (Utilities|Casting|CastToCharacter _returnvalue))
          (CallFunction|OnHitPlayer _ascharacter_2))))))

(event OnComponentHit(BoxCollision)
  (params (HitComponent :type Primitive%20Component%20Object%20Reference) (OtherActor :type Actor%20Object%20Reference) (OtherComp :type Primitive%20Component%20Object%20Reference) (NormalImpulse :type Vector :default "0, 0, 0") (Hit :type Hit%20Result%20Structure%20%28by%20ref%29)))

(event OnComponentHit(PickupMesh)
  (params (HitComponent :type Primitive%20Component%20Object%20Reference) (OtherActor :type Actor%20Object%20Reference) (OtherComp :type Primitive%20Component%20Object%20Reference) (NormalImpulse :type Vector :default "0, 0, 0") (Hit :type Hit%20Result%20Structure%20%28by%20ref%29)))

(event OnComponentBeginOverlap(BoxCollision)
  (params (OverlappedComponent :type Primitive%20Component%20Object%20Reference) (OtherActor :type Actor%20Object%20Reference) (OtherComp :type Primitive%20Component%20Object%20Reference) (OtherBodyIndex :type Integer) (bFromSweep :type Boolean) (SweepResult :type Hit%20Result%20Structure%20%28by%20ref%29)))

(event Custom|HandleHit_Base
  (params (HitComponent :type Primitive%20Component%20Object%20Reference) (OtherActor :type Actor%20Object%20Reference) (OtherComponent :type Primitive%20Component%20Object%20Reference) (NormalImpulse :type Vector) (Hit :type Hit%20Result%20Structure))
  (bind _returnvalue (Actor|GetParentActor OtherActor))
  ;[1 1 1] UNUSED  Target hit something while it is flying around
  (bind _ascharacter (Utilities|Casting|CastToCharacter OtherActor)
    (:then
      (CallFunction|OnHitPlayer _ascharacter))
    (:CastFailed
      (Utilities|IsValid _returnvalue
        (:Is%20Valid
          (bind _ascharacter_2 (Utilities|Casting|CastToCharacter _returnvalue))
          (CallFunction|OnHitPlayer _ascharacter_2))))))

(event Custom|OnHitPlayer
  (params (PlayerCharacter :type Character%20Object%20Reference))
  ;[1 1 1] OnHitPlayer
  (Networking|SwitchHasAuthority
    (:Authority
      (if (not (Variables|Default|GetisPickedUp))
        (Utilities|HasCapacityforAwards PlayerCharacter
          (:HasCapacity
            (Variables|Default|SetisPickedUp true)
            (CallFunction|GiveAwards PlayerCharacter)
            (Utilities|FlowControl|Delay 0.2)
            (Actor|DestroyActor)))))))

(event EventBeginPlay
  ;[1 1 1] BeginPlay
  (if (Variables|Default|GetRotateToHorizonalOnLaunch)
    (Transformation|SetWorldRotation (Variables|Transformation|GetRootComponent) (Math|Rotator|MakeRotator 0.0 0.0 (.Yaw (Math|Rotator|BreakRotator (Transformation|GetActorRotation)))) false true)))

(event EventTick
  (params (DeltaSeconds :type Float%20%28single-precision%29))
  ;[1 1 1] Tick
  (switch Utilities|FlowControl|Switch|SwitchonLauncherProjectileState (Variables|Default|GetProjectileState)
    (:NewEnumerator0
      (CallFunction|ExpandMesh DeltaSeconds))))

(fn ConstructionScript
  (CallFunction|UpdateMesh))

(fn ExpandMesh
  (params (DeltaSeconds :type Float%20%28single-precision%29))
  (switch Utilities|FlowControl|Switch|SwitchonLauncherProjectileState (Variables|Default|GetProjectileState)
    (:NewEnumerator0
      (Variables|Default|SetExpandTimeSum (+ DeltaSeconds (Variables|Default|GetExpandTimeSum)))
      (if (== (Class|KismetMathLibrary|FInterpEaseinOut (.X (Math|Vector|BreakVector (Transformation|GetActorScale3D))) (Variables|Default|GetFinalScale) (/ (Variables|Default|GetExpandTimeSum) (Variables|Default|GetExpandTime)) 1.5) (Variables|Default|GetFinalScale))
        (Transformation|SetActorScale3D (* "1.000000,1.000000,1.000000" (Variables|Default|GetFinalScale)))
        (Networking|SwitchHasAuthority
          (:Authority
            (Variables|Default|SetProjectileState "NewEnumerator1")))
        (else
          (Transformation|SetActorScale3D (* "1.000000,1.000000,1.000000" (Class|KismetMathLibrary|FInterpEaseinOut (.X (Math|Vector|BreakVector (Transformation|GetActorScale3D))) (Variables|Default|GetFinalScale) (/ (Variables|Default|GetExpandTimeSum) (Variables|Default|GetExpandTime)) 1.5))))))))

(fn OnRepProjectileState
  (CallFunction|UpdateMesh))

(fn UpdateMesh
  (bind _awardtype (Variables|Default|GetAwardType))
  (bind _output_get (LocalVariables|SettmpMesh (Variables|Default|GetPickupMesh)))
  (Utilities|IsValid _output_get
    (:Is%20Valid
      (switch Utilities|FlowControl|Switch|SwitchonPickupAwards _awardtype
        (:NewEnumerator0
          _)
        (:NewEnumerator1
          _))
      (Rendering|Material|SetVectorParameterValueonMaterials (LocalVariables|GettmpMesh) "BaseColor" (Math|Conversions|ToVector(LinearColor) (Utilities|Select :Index _awardtype :NewEnumerator0 "(R=0.019608,G=0.180392,B=0.749020,A=1.000000)" :NewEnumerator1 "(R=1.000000,G=0.738211,B=0.000000,A=1.000000)" :NewEnumerator2 "" :NewEnumerator3 "")))
      (Rendering|Material|SetVectorParameterValueonMaterials (LocalVariables|GettmpMesh) "EmissiveColor" (Math|Conversions|ToVector(LinearColor) (Utilities|Select :Index (Variables|Default|GetAwardType) :NewEnumerator0 "(R=0.121569,G=0.749020,B=0.729412,A=1.000000)" :NewEnumerator1 "(R=1.000000,G=0.824724,B=0.270759,A=1.000000)" :NewEnumerator2 "" :NewEnumerator3 "")))
      (Networking|SwitchHasAuthority
        (:Remote
          (if (Utilities|Enum|NotEqual(Enum) (Variables|Default|GetProjectileState) "NewEnumerator0")
            (Utilities|FlowControl|DoOnce false
              (:Completed
                (Transformation|SetActorScale3D (* "1.000000,1.000000,1.000000" (Variables|Default|GetFinalScale)))))))))))

(fn GiveAwards
  (params (PlayerCharacter :type Character%20Object%20Reference))
  (bind _astr_first_person_character (Utilities|Casting|CastToTR_FirstPersonCharacter PlayerCharacter))
  (bind _astr_player_controller_base_bp (Utilities|Casting|CastToTR_PlayerController_Base_BP (Pawn|GetController _astr_first_person_character)))
  (LocalVariables|SettmpPlayerController _astr_player_controller_base_bp)
  (if (> (Variables|Default|GetAwardAmount) 0.0)
    (Utilities|Array|Add (LocalVariables|GettmpGoodsAwarded) (Utilities|Struct|MakeGoodsQuantity (Variables|Default|GetGoodsTypeName) (Variables|Default|GetAwardAmount)))
    (Default|AddAwards (LocalVariables|GettmpPlayerController) (Variables|Default|GetAwardType) (Variables|Default|GetAwardAmount) (Variables|Default|GetAwardAmmoType) (Variables|Default|GetAwardWeaponName) (LocalVariables|GettmpGoodsAwarded))))

(fn EdGraph51
  (if (Variables|Default|GetStopped)
    (return (Variables|Default|GetBaseDestroyScoreValue) 0.0)
    (else
      (return (/ (Variables|Default|GetBaseDestroyScoreValue) 3.0) 0.0))))
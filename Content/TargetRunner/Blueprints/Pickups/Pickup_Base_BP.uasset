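; Base pickup actor for TargetRunner that awards energy, goods, ammo, weapons or animus to characters overlapping it.
; Construction picks a random alternate mesh; Tick eases scale up while Expanding, then the server switches to Flying and OnRep snaps final scale.
; On overlap, the server checks capacity for energy and animus only, grants awards through the player controller, then destroys the pickup.
; Hit-based pickup and material tinting logic are unused.
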(event OnComponentBeginOverlap(PickupCollision)
  (params (OverlappedComponent :type Primitive%20Component%20Object%20Reference) (OtherActor :type Actor%20Object%20Reference) (OtherComp :type Primitive%20Component%20Object%20Reference) (OtherBodyIndex :type Integer) (bFromSweep :type Boolean) (SweepResult :type Hit%20Result%20Structure%20%28by%20ref%29))
  (bind _returnvalue (Actor|GetAttachParentActor OtherActor))
  (bind _returnvalue_2 (Actor|GetParentActor OtherActor))
  (bind _ascharacter (Utilities|Casting|CastToCharacter OtherActor)
    (:then
      (CallFunction|OnHitPlayer _ascharacter))
    (:CastFailed
      (Utilities|IsValid _returnvalue
        (:Is%20Valid
          (bind _ascharacter_2 (Utilities|Casting|CastToCharacter _returnvalue))
          (CallFunction|OnHitPlayer _ascharacter_2))
        (:Is%20Not%20Valid
          (Utilities|IsValid _returnvalue_2
            (:Is%20Valid
              (bind _ascharacter_3 (Utilities|Casting|CastToCharacter _returnvalue_2))
              (CallFunction|OnHitPlayer _ascharacter_3))))))))

(event OnComponentHit(BoxCollision)
  (params (HitComponent :type Primitive%20Component%20Object%20Reference) (OtherActor :type Actor%20Object%20Reference) (OtherComp :type Primitive%20Component%20Object%20Reference) (NormalImpulse :type Vector :default "0, 0, 0") (Hit :type Hit%20Result%20Structure%20%28by%20ref%29)))

(event OnComponentHit(PickupMesh)
  (params (HitComponent :type Primitive%20Component%20Object%20Reference) (OtherActor :type Actor%20Object%20Reference) (OtherComp :type Primitive%20Component%20Object%20Reference) (NormalImpulse :type Vector :default "0, 0, 0") (Hit :type Hit%20Result%20Structure%20%28by%20ref%29)))

(event OnComponentBeginOverlap(BoxCollision)
  (params (OverlappedComponent :type Primitive%20Component%20Object%20Reference) (OtherActor :type Actor%20Object%20Reference) (OtherComp :type Primitive%20Component%20Object%20Reference) (OtherBodyIndex :type Integer) (bFromSweep :type Boolean) (SweepResult :type Hit%20Result%20Structure%20%28by%20ref%29)))

(event Custom|HandleHit_Base
  (params (HitComponent :type Primitive%20Component%20Object%20Reference) (OtherActor :type Actor%20Object%20Reference) (OtherComponent :type Primitive%20Component%20Object%20Reference) (NormalImpulse :type Vector) (Hit :type Hit%20Result%20Structure))
  (bind _returnvalue (Actor|GetAttachParentActor OtherActor))
  (bind _returnvalue_2 (Actor|GetParentActor OtherActor))
  ;[1 1 1] UNUSED  Target hit something while it is flying around
  (bind _ascharacter (Utilities|Casting|CastToCharacter OtherActor)
    (:then
      (CallFunction|OnHitPlayer _ascharacter))
    (:CastFailed
      (Utilities|IsValid _returnvalue
        (:Is%20Valid
          (bind _ascharacter_2 (Utilities|Casting|CastToCharacter _returnvalue))
          (CallFunction|OnHitPlayer _ascharacter_2))
        (:Is%20Not%20Valid
          (Utilities|IsValid _returnvalue_2
            (:Is%20Valid
              (bind _ascharacter_3 (Utilities|Casting|CastToCharacter _returnvalue_2))
              (CallFunction|OnHitPlayer _ascharacter_3))))))))

(event Custom|OnHitPlayer
  (params (PlayerCharacter :type Character%20Object%20Reference))
  ;[1 1 1] OnHitPlayer
  (Networking|SwitchHasAuthority
    (:Authority
      (if (not (Variables|Default|GetisPickedUp))
        (Utilities|HasCapacityforAwards PlayerCharacter
          (:HasCapacity
            (Variables|Default|SetisPickedUp true)
            (CallFunction|GiveAwards PlayerCharacter)
            (Utilities|FlowControl|Delay 0.1)
            (Actor|DestroyActor)))))))

(event EventBeginPlay
  ;[1 1 1] BeginPlay
  (if (Variables|Default|GetRotateToHorizonalOnLaunch)
    (Transformation|SetWorldRotation (Variables|Transformation|GetRootComponent) (Math|Rotator|MakeRotator 0.0 0.0 (.Yaw (Math|Rotator|BreakRotator (Transformation|GetActorRotation)))) false true)))

(event EventTick
  (params (DeltaSeconds :type Float%20%28single-precision%29))
  ;[1 1 1] Tick
  (switch Utilities|FlowControl|Switch|SwitchonLauncherProjectileState (Variables|Default|GetProjectileState)
    (:NewEnumerator0
      (CallFunction|ExpandMesh DeltaSeconds))))

(fn ConstructionScript
  (bind _altmeshes (Variables|Default|GetAltMeshes))
  (if (> (Utilities|Array|Length (Variables|Default|GetAltMeshes)) 0)
    (bind _returnvalue (Utilities|LoadAssetBlocking (Utilities|Array|Get(acopy) _altmeshes (Math|Random|RandomIntegerinRange 0 (Utilities|Array|LastIndex _altmeshes))))) ; Should not block - asset should be loaded.
    (bind _asstatic_mesh (Utilities|Casting|CastToStaticMesh _returnvalue))
    (Components|StaticMesh|SetStaticMesh (Variables|Default|GetPickupMesh) _asstatic_mesh))
  (CallFunction|UpdateMesh))

(fn ExpandMesh
  (params (DeltaSeconds :type Float%20%28single-precision%29))
  (switch Utilities|FlowControl|Switch|SwitchonLauncherProjectileState (Variables|Default|GetProjectileState)
    (:NewEnumerator0
      (Variables|Default|SetExpandTimeSum (+ DeltaSeconds (Variables|Default|GetExpandTimeSum)))
      (if (== (Class|KismetMathLibrary|FInterpEaseinOut (.X (Math|Vector|BreakVector (Transformation|GetActorScale3D))) (Variables|Default|GetFinalScale) (/ (Variables|Default|GetExpandTimeSum) (Variables|Default|GetExpandTime)) 1.5) (Variables|Default|GetFinalScale))
        (Transformation|SetActorScale3D (* "1.000000,1.000000,1.000000" (Variables|Default|GetFinalScale)))
        (Networking|SwitchHasAuthority
          (:Authority
            (Variables|Default|SetProjectileState "NewEnumerator1")))
        (else
          (Transformation|SetActorScale3D (* "1.000000,1.000000,1.000000" (Class|KismetMathLibrary|FInterpEaseinOut (.X (Math|Vector|BreakVector (Transformation|GetActorScale3D))) (Variables|Default|GetFinalScale) (/ (Variables|Default|GetExpandTimeSum) (Variables|Default|GetExpandTime)) 1.5))))))))

(fn OnRepProjectileState
  (CallFunction|UpdateMesh))

(fn UpdateMesh
  (if (Utilities|Enum|NotEqual(Enum) (Variables|Default|GetProjectileState) "NewEnumerator0")
    (Utilities|FlowControl|DoOnce false
      (:Completed
        (Transformation|SetActorScale3D (* "1.000000,1.000000,1.000000" (Variables|Default|GetFinalScale)))))))

(fn GiveAwards
  (params (PlayerCharacter :type Character%20Object%20Reference))
  (bind _astr_first_person_character (Utilities|Casting|CastToTR_FirstPersonCharacter PlayerCharacter))
  (bind _astr_player_controller_base_bp (Utilities|Casting|CastToTR_PlayerController_Base_BP (Pawn|GetController _astr_first_person_character)))
  (LocalVariables|SettmpPlayerController _astr_player_controller_base_bp)
  (if (> (Variables|Default|GetAwardAmount) 0.0)
    (Utilities|Array|Add (LocalVariables|GettmpGoodsAwarded) (Utilities|Struct|MakeGoodsQuantity (Variables|Default|GetGoodsTypeName) (Variables|Default|GetAwardAmount)))
    (Default|AddAwards (LocalVariables|GettmpPlayerController) (Variables|Default|GetAwardType) (Variables|Default|GetAwardAmount) (Variables|Default|GetAwardWeaponName) (LocalVariables|GettmpGoodsAwarded))))

(fn EdGraph51
  (if (Variables|Default|GetStopped)
    (return (Variables|Default|GetBaseDestroyScoreValue) 0.0)
    (else
      (return (/ (Variables|Default|GetBaseDestroyScoreValue) 3.0) 0.0))))
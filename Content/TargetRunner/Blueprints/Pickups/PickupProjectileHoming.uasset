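; Homing variant of a pickup projectile that begins seeking a target through HomingMovementManagerComponent once flying, triggered from the mesh expansion step.
; While flying, it doubles homing agility once its remaining lifespan falls to three quarters.
; A DisableHoming flag, handled on BeginPlay and RepNotify, stops homing and movement and restores gravity.
; Its destroy score is the full base value when stopped, otherwise a third.
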(event OnStartHoming(HomingMovementManagerComponent)
  ;[1 1 1] Homing
  (Variables|Default|SetProjectileState "NewEnumerator1"))

(event OnStopHoming(HomingMovementManagerComponent)
  ;[1 1 1] Homing
  (Variables|Default|SetProjectileState (Variables|Default|GetProjectileState)))

(event OnTargetAquired(HomingMovementManagerComponent)
  ;[1 1 1] Homing
  (Variables|Default|SetProjectileState "NewEnumerator1"))

(event OnTargetLost(HomingMovementManagerComponent)
  ;[1 1 1] Homing
  (Variables|Default|SetProjectileState (Variables|Default|GetProjectileState)))

(event Custom|OnDisableHoming
  (bind _projectilemovement (Variables|Default|GetProjectileMovement))
  (if (Variables|Default|GetDisableHoming)
    _
    (else
      (Variables|Default|SetDisableHoming true)))
  (Default|StopHoming (Variables|Default|GetHomingMovementManagerComponent))
  (Variables|/Script/Engine.ProjectileMovementComponent|SetMaxSpeed _projectilemovement 0.0)
  (Components|Movement|StopMovementImmediately _projectilemovement)
  (Variables|/Script/Engine.ProjectileMovementComponent|SetProjectileGravityScale _projectilemovement 1.0))

(event EventBeginPlay
  ;[1 1 1] BeginPlay
  (if (Variables|Default|GetDisableHoming)
    (CallFunction|OnDisableHoming)))

(event EventExpandMesh
  (params (DeltaSeconds :type Float%20%28single-precision%29))
  ;[1 1 1] Override ExpandMesh
  (|CallParentFunction DeltaSeconds)
  (if (and (Utilities|Enum|Equal(Enum) (Variables|Default|GetProjectileState) "NewEnumerator1") (not (Variables|Default|GetDisableHoming)))
    (Utilities|FlowControl|DoOnce false
      (:Completed
        (Default|StartHoming (Variables|Default|GetHomingMovementManagerComponent))))))

(event EventTick
  (params (DeltaSeconds :type Float%20%28single-precision%29))
  (bind _homingmovementmanagercomponent (Variables|Default|GetHomingMovementManagerComponent))
  ;[1 1 1] Tick
  (|CallParentFunction DeltaSeconds)
  (switch Utilities|FlowControl|Switch|SwitchonLauncherProjectileState (Variables|Default|GetProjectileState)
    (:NewEnumerator1
      _)
    (:NewEnumerator3
      _))
  (Utilities|FlowControl|DoOnce false :!label _label
    (:Completed
      (if (<= (/ (Actor|GetLifeSpan) (Variables|Default|GetInitialLifeSpan)) 0.75)
        (Variables|/Game/TargetRunner/Blueprints/General/HomingMovementManagerComponent.HomingMovementManagerComponent_C|SetHomingAgility _homingmovementmanagercomponent (* (Variables|/Game/TargetRunner/Blueprints/General/HomingMovementManagerComponent.HomingMovementManagerComponent_C|GetHomingAgility _homingmovementmanagercomponent) 2.0))
        (else
          (goto _label Reset))))))

(event EventUpdateMesh
  (|CallParentFunction))

(fn ConstructionScript)

(fn OnRepDisableHoming
  (if (Variables|Default|GetDisableHoming)
    (CallFunction|OnDisableHoming)))

(fn EdGraph51
  (if (Variables|Default|GetStopped)
    (return (Variables|Default|GetBaseDestroyScoreValue) 0.0)
    (else
      (return (/ (Variables|Default|GetBaseDestroyScoreValue) 3.0) 0.0))))
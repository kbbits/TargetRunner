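; NextLevelTrigger_BP is an interactable world trigger that lets a player start the next game level.
; On BeginPlay it caches the current level plus one and the current game seed from TR_GameInstance_BP.
; On interaction it passes both values to ServerStartNewGameLevel on the interacting player's TR_PlayerController_Base_BP.
; GetInteractText builds the prompt from the truncated next level number.
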(event EventBeginPlay
  (bind _astr_game_instance_bp (Utilities|Casting|CastToTR_GameInstance_BP (Game|GetGameInstance)))
  (Variables|Default|SetNextLevel (+ (Variables|/Game/TargetRunner/Blueprints/Game/TR_GameInstance_BP.TR_GameInstance_BP_C|GetCurrentGameLevel _astr_game_instance_bp) 1.0))
  (Variables|Default|SetNextGameSeed (Variables|/Game/TargetRunner/Blueprints/Game/TR_GameInstance_BP.TR_GameInstance_BP_C|GetGameSeed _astr_game_instance_bp)))

(event EventOnPlayerInteract
  (params (PlayerCharacter :type TR%20Character%20Object%20Reference))
  ;[1 1 1] On Player Interact
  (bind _astr_player_controller_base_bp (Utilities|Casting|CastToTR_PlayerController_Base_BP (Pawn|GetController PlayerCharacter)))
  (Default|ServerStartNewGameLevel _astr_player_controller_base_bp (Variables|Default|GetNextLevel) (Variables|Default|GetNextGameSeed)))

(fn ConstructionScript)

(fn GetInteractText
  (return (Utilities|Text|ToText(String) (Utilities|String|Append "Start level " (Utilities|String|ToString(Integer) (Math|Float|Truncate (Variables|Default|GetNextLevel)))))))
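; Base exit key pickup that a player collects by interacting with it rather than touching it.
; Interaction sets a non-replicated PickedUp flag and calls GiveAwards once for that player.
; It overrides the inherited hit-player and mesh-update events to do nothing.
; GoodsTypeName supplies both the key name and the interact prompt text.
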(event EventUpdateMesh)

(event EventOnHitPlayer
  (params (PlayerCharacter :type Character%20Object%20Reference)))

(event EventOnPlayerInteract
  (params (PlayerCharacter :type TR%20Character%20Object%20Reference))
  (if (not (Variables|Default|GetPickedUp))
    (Variables|Default|SetPickedUp true) ; Does not replicate
    (CallFunction|GiveAwards PlayerCharacter)))

(fn ConstructionScript)

(fn GetKeyName
  (return (Variables|Default|GetGoodsTypeName)))

(fn GetInteractText
  (return (Utilities|Text|ToText(Name) (Variables|Default|GetGoodsTypeName))))
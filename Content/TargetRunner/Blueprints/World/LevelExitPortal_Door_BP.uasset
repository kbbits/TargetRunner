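; Level exit portal behind a stone door that completes the run when every player stands in its trigger.
; On setup, the server turns child actor slots into random resource-node locks, dividing the exit resources between them.
; Destroying all locks enables trigger overlaps and fires effects that swap the base material and sink the door with sound.
; The server tracks players inside, updating a waiting count that drives the inspect name.
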(event OnComponentEndOverlap(ExitTriggerVolume)
  (params (OverlappedComponent :type Primitive%20Component%20Object%20Reference) (OtherActor :type Actor%20Object%20Reference) (OtherComp :type Primitive%20Component%20Object%20Reference) (OtherBodyIndex :type Integer))
  (Networking|SwitchHasAuthority
    (:Authority
      (bind _astr_first_person_character_bp (Utilities|Casting|CastToTR_FirstPersonCharacter_BP OtherActor))
      (bind _astr_player_controller_base_bp (Utilities|Casting|CastToTR_PlayerController_Base_BP (Pawn|GetController _astr_first_person_character_bp)))
      (Utilities|Array|RemoveItem (Variables|Default|GetPlayersInExit) (Class|GameplayStatics|GetPlayerControllerID _astr_player_controller_base_bp))
      (Utilities|UpdateWaitingonPlayers))))

(event OnComponentBeginOverlap(ExitTriggerVolume)
  (params (OverlappedComponent :type Primitive%20Component%20Object%20Reference) (OtherActor :type Actor%20Object%20Reference) (OtherComp :type Primitive%20Component%20Object%20Reference) (OtherBodyIndex :type Integer) (bFromSweep :type Boolean) (SweepResult :type Hit%20Result%20Structure%20%28by%20ref%29))
  (Networking|SwitchHasAuthority
    (:Authority
      (bind _astr_first_person_character_bp (Utilities|Casting|CastToTR_FirstPersonCharacter_BP OtherActor))
      (bind _astr_player_controller_base_bp (Utilities|Casting|CastToTR_PlayerController_Base_BP (Pawn|GetController _astr_first_person_character_bp)))
      (Utilities|Array|AddUnique (Variables|Default|GetPlayersInExit) (Class|GameplayStatics|GetPlayerControllerID _astr_player_controller_base_bp))
      (Utilities|UpdateWaitingonPlayers)
      (bind _returnvalue (Class|GameModeBase|GetNumPlayers (Game|GetGameMode)))
      (if (== _returnvalue (Utilities|Array|Length (Variables|Default|GetPlayersInExit)))
        (Default|ServeronRunComplete _astr_player_controller_base_bp)))))

(event Custom|OnNodeLockDestroyed
  (Networking|SwitchHasAuthority
    (:Authority
      (bind _result (Math|Integer|DecrementInt (Variables|Default|GetActiveNodeLocks))
        (:%20%20
          (if (<= _result 0)
            (Variables|/Script/Engine.PrimitiveComponent|SetbGenerateOverlapEvents (Variables|Default|GetExitTriggerVolume) true)
            (CallFunction|MConNodeLocksDestroyedFX)))))))

(event Custom|MC_OnNodeLocksDestroyedFX
  (bind _stoneblock_tall_2k (Variables|Default|GetStoneBlock_Tall_2k))
  (bind _stoneblock_tall_2k_2 (Variables|Default|GetStoneBlock_Tall_2k))
  (bind _returnvalue (Transformation|GetWorldLocation _stoneblock_tall_2k))
  (bind _returnvalue_2 (+ _returnvalue "0, 0,200.000000"))
  (Rendering|Material|SetMaterial (Variables|Default|GetBaseMesh) 0 "/Game/TargetRunner/Assets/Materials/MI_TR_Pickup_Reverse.MI_TR_Pickup_Reverse")
  (Utilities|FlowControl|DoOnce false
    (:Completed
      (Audio|PlaySoundatLocation "/Game/TargetRunner/Assets/Audio/FX/RockBurst_2_Cue.RockBurst_2_Cue" _returnvalue_2 "0, 0, 0" 1.0 1.0 0.0 0 0 0)
      (Utilities|FlowControl|Delay 0.1)
      (Audio|PlaySoundatLocation "/Game/TargetRunner/Assets/Audio/FX/RockBurst_1_Cue.RockBurst_1_Cue" _returnvalue_2 "0, 0, 0" 1.0 0.8 0.0 0 0 0)
      (Class|GameplayStatics|PrimeSound (Variables|Default|GetDoorSound))
      (Utilities|FlowControl|Delay 0.3)
      (bind _returnvalue_3 (Audio|SpawnSoundatLocation (Variables|Default|GetDoorSound) _returnvalue_2 "0, 0, 0" 1.6 0.6 0.0 0 0))
      (Variables|Default|SetDoorSoundComponent _returnvalue_3)
      (Components|MoveComponentTo (Variables|Default|GetStoneBlock_Tall_2k) (+ (Variables|/Script/Engine.SceneComponent|GetRelativeLocation _stoneblock_tall_2k_2) "0, 0,-388.000000") (Variables|/Script/Engine.SceneComponent|GetRelativeRotation _stoneblock_tall_2k_2) false false 3.0 false)
      (Audio|Components|Audio|Stop (Variables|Default|GetDoorSoundComponent))
      (Variables|Default|SetDoorSoundComponent 0))))

(event EventBeginPlay
  (|CallParentFunction)
  (Class|LevelExitBase|SetupNodes))

(event EventSetupNodes
  (|CallParentFunction)
  (Networking|SwitchHasAuthority
    (:Authority
      (CallFunction|SetupNodeLocks))))

(fn ConstructionScript)

(fn SetupNodeLocks
  (bind _returnvalue (Actor|GetComponentsByClass "/Script/Engine.ChildActorComponent"))
  (Networking|SwitchHasAuthority
    (:Authority
      (LocalVariables|SettmpNodeResources (Class|ResourceFunctionLibrary|MultiplyResourceQuantity (Variables|Default|GetExitResourceTypes) (/ 1.0 (Math|Conversions|ToFloat(Integer) (Utilities|Array|Length _returnvalue))) true))
      (for _array_element _returnvalue
        (ChildActorComponent|SetChildActorClass _array_element (Utilities|Array|Get(acopy) (Variables|Default|GetNodeClasses) (Math|Random|RandomIntegerinRange 0 (Utilities|Array|LastIndex (Variables|Default|GetNodeClasses)))))
        (bind _asresource_node_base_bp (Utilities|Casting|CastToResourceNodeBase_BP (Variables|/Script/Engine.ChildActorComponent|GetChildActor _array_element)))
        (Class|ResourceNodeBase|SetResources _asresource_node_base_bp (.ResourceType (Utilities|Struct|BreakResourceQuantity (Utilities|Array|Get(acopy) (LocalVariables|GettmpNodeResources)))) (LocalVariables|GettmpNodeResources) 0.1)
        (bind _output_get (Variables|/Script/TargetRunner.ResourceNodeBase|SetBaseHealth _asresource_node_base_bp (Variables|Default|GetNodeLockHealth)))
        (Class|ResourceNodeBase|ServerSetCurrentHealth _asresource_node_base_bp _output_get)
        (EventDispatchers|BindEventtoOnNodeDestroyed _asresource_node_base_bp (EventDispatchers|CreateEvent :!event Custom|OnNodeLockDestroyed))
        (Utilities|Array|Add (LocalVariables|GettmpNewResourceNodes) _asresource_node_base_bp))
      (Variables|Default|SetActiveNodeLocks (Utilities|Array|Length (LocalVariables|GettmpNewResourceNodes)))
      (return (LocalVariables|GettmpNewResourceNodes)))))

(fn GetInspectInfo
  (bind _returnvalue (CallFunction|GetItemDisplayName))
  (return (Utilities|Struct|MakeInspectInfo _returnvalue)))

(fn GetItemDisplayName
  (if (>= (Variables|Default|GetWaitingOnPlayers_Rep) 0)
    (if (> (Variables|Default|GetWaitingOnPlayers_Rep) 1)
      (return (Utilities|Text|FormatText "Waiting on {0} players" (Variables|Default|GetWaitingOnPlayers_Rep)))
      (else
        (return (Utilities|Text|FormatText "Waiting on {0} player" (Variables|Default|GetWaitingOnPlayers_Rep)))))
    (else
      (return "Exit Portal"))))
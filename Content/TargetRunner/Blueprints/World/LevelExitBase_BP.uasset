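; Base level exit for TargetRunner that ends a player's run, gated by a destructible resource-node door.
; SetupDoors spawns the node as a child actor, configures its exit resources and health, and binds its destruction event.
; Destroying the node turns the exit volume into an active trigger and tints the main mesh green.
; On authority, a player character overlapping that volume calls ServerOnRunComplete on its controller.
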(event OnComponentBeginOverlap(ExitVolume)
  (params (OverlappedComponent :type Primitive%20Component%20Object%20Reference) (OtherActor :type Actor%20Object%20Reference) (OtherComp :type Primitive%20Component%20Object%20Reference) (OtherBodyIndex :type Integer) (bFromSweep :type Boolean) (SweepResult :type Hit%20Result%20Structure%20%28by%20ref%29))
  (Networking|SwitchHasAuthority
    (:Authority
      (bind _astr_first_person_character_bp (Utilities|Casting|CastToTR_FirstPersonCharacter_BP OtherActor))
      (bind _astr_player_controller_base_bp (Utilities|Casting|CastToTR_PlayerController_Base_BP (Pawn|GetController _astr_first_person_character_bp)))
      (Default|ServeronRunComplete _astr_player_controller_base_bp))))

(event Custom|OnDoorDestroyed
  (bind _exitvolume (Variables|Default|GetExitVolume))
  (Variables|/Script/Engine.PrimitiveComponent|SetbGenerateOverlapEvents _exitvolume true)
  (Collision|SetCollisionProfileName _exitvolume "Trigger" true :!class /Script/Engine.PrimitiveComponent)
  (Rendering|Material|SetVectorParameterValueonMaterials (Variables|Default|GetMainMesh) "DiffuseColor" (Math|Conversions|ToVector(LinearColor) "(R=0.024161,G=0.609375,B=0.000000,A=1.000000)"))
  (bind _asresource_node_base_bp (Utilities|Casting|CastToResourceNodeBase_BP (Variables|/Script/Engine.ChildActorComponent|GetChildActor (Variables|Default|GetDoorNode))))
  (Utilities|IsValid _asresource_node_base_bp
    (:Is%20Valid
      (EventDispatchers|UnbindEventfromOnNodeDestroyed _asresource_node_base_bp (delegate Custom|OnDoorDestroyed)))))

(event EventBeginPlay)

(event EventSetupDoors
  (|CallParentFunction)
  (ChildActorComponent|SetChildActorClass (Variables|Default|GetDoorNode) (Variables|Default|GetNodeClass))
  (bind _asresource_node_base_bp (Utilities|Casting|CastToResourceNodeBase_BP (Variables|/Script/Engine.ChildActorComponent|GetChildActor (Variables|Default|GetDoorNode))))
  (Default|SetResourcesBP _asresource_node_base_bp (.ResourceType (Utilities|Struct|BreakResourceQuantity (Utilities|Array|Get(acopy) (Variables|Default|GetExitResourceTypes)))) (Variables|Default|GetExitResourceTypes) 0.1)
  (Variables|/Script/TargetRunner.ResourceNodeBase|SetBaseHealth _asresource_node_base_bp 6.0)
  (EventDispatchers|BindEventtoOnNodeDestroyed _asresource_node_base_bp (delegate Custom|OnDoorDestroyed)))

(fn ConstructionScript)
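; FollowerController is a controller that makes its pawn follow a TR_FirstPersonCharacter, with all logic running on the server.
; Shortly after BeginPlay it stores the first such character found in the world as its target.
; While that target is valid, Tick issues MoveToActor toward it through a DoOnce that resets after a delay, throttling path requests to every couple of seconds.
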(event EventBeginPlay
  (Networking|SwitchHasAuthority
    (:Authority
      (Utilities|FlowControl|Delay 0.5)
      (bind _outactors (Actor|GetAllActorsOfClass "/Game/TargetRunner/Blueprints/Player/TR_FirstPersonCharacter.TR_FirstPersonCharacter_C"))
      (Variables|Default|SetFollowingCharacter (Utilities|Array|Get(acopy) _outactors)))))

(event EventTick
  (params (DeltaSeconds :type Float%20%28single-precision%29))
  (Networking|SwitchHasAuthority
    (:Authority
      (Utilities|IsValid (Variables|Default|GetFollowingCharacter)
        (:Is%20Valid
          (Utilities|FlowControl|DoOnce false :!label _label
            (:Completed
              (AI|Navigation|MovetoActor (Variables|Default|GetFollowingCharacter) 1e+02 true true true 0)
              (Utilities|FlowControl|Delay 2.0)
              (goto _label Reset))))))))

(fn ConstructionScript)
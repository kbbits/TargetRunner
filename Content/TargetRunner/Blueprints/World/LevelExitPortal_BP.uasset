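; Level exit portal that completes a player's run once its resource-node locks are destroyed.
; On the server, SetupNodeLocks fills each child actor slot with a random node class, dividing the exit resources between them and setting their health.
; Node destruction decrements a lock counter; at zero, the trigger volume activates and the base mesh material changes.
; A character overlapping the trigger calls ServerOnRunComplete on its controller, under authority.
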(event OnComponentBeginOverlap(ExitTriggerVolume)
  (params (OverlappedComponent :type Primitive%20Component%20Object%20Reference) (OtherActor :type Actor%20Object%20Reference) (OtherComp :type Primitive%20Component%20Object%20Reference) (OtherBodyIndex :type Integer) (bFromSweep :type Boolean) (SweepResult :type Hit%20Result%20Structure%20%28by%20ref%29))
  (Networking|SwitchHasAuthority
    (:Authority
      (bind _astr_first_person_character_bp (Utilities|Casting|CastToTR_FirstPersonCharacter_BP OtherActor))
      (bind _astr_player_controller_base_bp (Utilities|Casting|CastToTR_PlayerController_Base_BP (Pawn|GetController _astr_first_person_character_bp)))
      (Default|ServeronRunComplete _astr_player_controller_base_bp))))

(event Custom|OnNodeLockDestroyed
  (bind _exittriggervolume (Variables|Default|GetExitTriggerVolume))
  (bind _result (Math|Integer|DecrementInt (Variables|Default|GetActiveNodeLocks))
    (:%20%20
      (if (<= _result 0)
        (Variables|/Script/Engine.PrimitiveComponent|SetbGenerateOverlapEvents _exittriggervolume true)
        (Collision|SetCollisionProfileName _exittriggervolume "Trigger" true :!class /Script/Engine.PrimitiveComponent)
        (Rendering|Material|SetMaterial (Variables|Default|GetBaseMesh) 0 "/Game/TargetRunner/Assets/Materials/MI_TR_Pickup_Reverse.MI_TR_Pickup_Reverse")))))

(event EventBeginPlay
  (|CallParentFunction)
  (Class|LevelExitBase|SetupNodes))

(event EventSetupNodes
  (|CallParentFunction)
  (Networking|SwitchHasAuthority
    (:Authority
      (CallFunction|SetupNodeLocks))))

(fn ConstructionScript)

(fn SetupNodeLocks
  (bind _returnvalue (Actor|GetComponentsByClass "/Script/Engine.ChildActorComponent"))
  (LocalVariables|SettmpNodeResources (Class|ResourceFunctionLibrary|MultiplyResourceQuantity (Variables|Default|GetExitResourceTypes) (/ 1.0 (Math|Conversions|ToFloat(Integer) (Utilities|Array|Length _returnvalue))) true))
  (for _array_element _returnvalue
    (ChildActorComponent|SetChildActorClass _array_element (Utilities|Array|Get(acopy) (Variables|Default|GetNodeClasses) (Math|Random|RandomIntegerinRange 0 (Utilities|Array|LastIndex (Variables|Default|GetNodeClasses)))))
    (bind _asresource_node_base_bp (Utilities|Casting|CastToResourceNodeBase_BP (Variables|/Script/Engine.ChildActorComponent|GetChildActor _array_element)))
    (Class|ResourceNodeBase|SetResources _asresource_node_base_bp (.ResourceType (Utilities|Struct|BreakResourceQuantity (Utilities|Array|Get(acopy) (LocalVariables|GettmpNodeResources)))) (LocalVariables|GettmpNodeResources) 0.1)
    (Variables|/Script/TargetRunner.ResourceNodeBase|SetBaseHealth _asresource_node_base_bp (Variables|Default|GetNodeLockHealth))
    (EventDispatchers|BindEventtoOnNodeDestroyed _asresource_node_base_bp (EventDispatchers|CreateEvent :!event Custom|OnNodeLockDestroyed))
    (Utilities|Array|Add (LocalVariables|GettmpNewResourceNodes) _asresource_node_base_bp))
  (Variables|Default|SetActiveNodeLocks (Utilities|Array|Length (LocalVariables|GettmpNewResourceNodes)))
  (return (LocalVariables|GettmpNewResourceNodes)))
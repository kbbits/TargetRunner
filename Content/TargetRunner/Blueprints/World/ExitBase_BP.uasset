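; Base Blueprint for a run exit that players interact with to finish the run, locked until required keys are acquired.
; Shortly after BeginPlay, the server reads required keys from the exit marker on its parent actor's platform, unlocking immediately if none exist.
; Interaction calls the player controller to complete the run when unlocked, otherwise to attempt an unlock.
; Interact text reflects the lock state; the Unlocked RepNotify is empty.
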(event Custom|SetupFromMarkers
  (bind _returnvalue (Actor|GetParentActor))
  ;[1 1 1] Determine required keys from exit marker in same platform
  (Utilities|IsValid _returnvalue
    (:Is%20Valid
      (bind _asiplatform_placeable (Utilities|Casting|CastToIPlatformPlaceable _returnvalue))
      (bind _platform (Default|GetMyPlatform _asiplatform_placeable))
      (bind (_found _exitmarker) (Default|GetExitMarker _platform))
      (if _found
        (for _array_element (Variables|/Game/TargetRunner/Blueprints/World/ExitMarkerBase_BP.ExitMarkerBase_BP_C|GetRequiredKeys _exitmarker)
          (Utilities|Array|Add (Variables|Default|GetRequiredKeys) (Utilities|Struct|MakeGoodsQuantity _array_element 1.0)))
        (if (== (Utilities|Array|Length (Variables|Default|GetRequiredKeys)) 0)
          (Variables|Default|SetUnlocked true))
        (else
          (Development|PrintString "Warning: No exit marker found on exit platform" true true "(R=1.000000,G=0.687076,B=0.000000,A=1.000000)" 5.0))))))

(event EventBeginPlay
  ;[1 1 1] Begin Play
  (Networking|SwitchHasAuthority
    (:Authority
      (Utilities|FlowControl|Delay 0.75)
      (CallFunction|SetupfromMarkers))))

(event EventOnPlayerInteract
  (params (PlayerCharacter :type TR%20First%20Person%20Character%20Object%20Reference))
  ;[1 1 1] On Player Interact
  (bind _astr_player_controller_base (Utilities|Casting|CastToTR_PlayerController_Base (Pawn|GetController PlayerCharacter)))
  (if (Variables|Default|GetUnlocked)
    (Default|OnRunComplete _astr_player_controller_base)
    (else
      (Default|AttemptExitUnlock _astr_player_controller_base self))))

(fn ConstructionScript)

(fn OnRepUnlocked)

(fn GetInteractText
  (return (select (Variables|Default|GetUnlocked) "Sync and exit this run" (Utilities|Text|ToText(String) (Utilities|String|MakeLiteralString (Utilities|String|Append "You must acquire all " (Utilities|String|ToString(Integer) (Utilities|Array|Length (Variables|Default|GetRequiredKeys))) " keys to unlock this exit sync"))))))
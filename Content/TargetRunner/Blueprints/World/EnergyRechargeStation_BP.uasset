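; Energy recharge station that periodically awards a charge amount to the player controllers of characters standing in its collect volume.
; The server tracks overlapping characters, starting a looping timer for the first arrival and pausing it when the last leaves.
; A retriggerable delay clears the timer if it stays paused.
; Multicast events start a hum sound at the beacon pillar and fade it out on stop.
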(event OnComponentBeginOverlap(CollectVolume)
  (params (OverlappedComponent :type Primitive%20Component%20Object%20Reference) (OtherActor :type Actor%20Object%20Reference) (OtherComp :type Primitive%20Component%20Object%20Reference) (OtherBodyIndex :type Integer) (bFromSweep :type Boolean) (SweepResult :type Hit%20Result%20Structure%20%28by%20ref%29))
  (Networking|SwitchHasAuthority
    (:Authority
      (bind _astr_first_person_character_bp (Utilities|Casting|CastToTR_FirstPersonCharacter_BP OtherActor))
      (Utilities|Array|AddUnique (Variables|Default|GetCurrentChargingCharacters) _astr_first_person_character_bp)
      (if (== (Utilities|Array|Length (Variables|Default|GetCurrentChargingCharacters)) 1)
        (CallFunction|StartCharging)))))

(event OnComponentEndOverlap(CollectVolume)
  (params (OverlappedComponent :type Primitive%20Component%20Object%20Reference) (OtherActor :type Actor%20Object%20Reference) (OtherComp :type Primitive%20Component%20Object%20Reference) (OtherBodyIndex :type Integer))
  (Networking|SwitchHasAuthority
    (:Authority
      (bind _astr_first_person_character_bp (Utilities|Casting|CastToTR_FirstPersonCharacter_BP OtherActor))
      (Utilities|Array|RemoveItem (Variables|Default|GetCurrentChargingCharacters) _astr_first_person_character_bp)
      (if (== (Utilities|Array|Length (Variables|Default|GetCurrentChargingCharacters)) 0)
        (CallFunction|StopCharging)))))

(event Custom|OnChargeFire
  (for _array_element (Variables|Default|GetCurrentChargingCharacters)
    (Utilities|IsValid _array_element
      (:Is%20Valid
        (Default|AddAwards (Default|GetTRPlayerControllerBP _array_element) "NewEnumerator0" (Variables|Default|GetChargePerFire) "None" (Utilities|Array|MakeArray) false)))))

(event Custom|StartCharging
  (Networking|SwitchHasAuthority
    (:Authority
      (if (Utilities|Time|IsValidTimerHandle (Variables|Default|GetChargeTimer))
        (if (Class|KismetSystemLibrary|IsTimerPausedHandle (Variables|Default|GetChargeTimer))
          (Utilities|Time|UnpauseTimerbyHandle (Variables|Default|GetChargeTimer))
          (CallFunction|MCStartChargeFX :!label _label))
        (else
          (bind _returnvalue (Utilities|Time|SetTimerbyEvent (delegate Custom|OnChargeFire) (Variables|Default|GetChargeFireDelay) true))
          (Variables|Default|SetChargeTimer _returnvalue)
          (goto _label))))))

(event Custom|StopCharging
  (Networking|SwitchHasAuthority
    (:Authority
      (Utilities|Time|PauseTimerbyHandle (Variables|Default|GetChargeTimer))
      (CallFunction|MCStopChargeFX)
      (Utilities|FlowControl|RetriggerableDelay 5.0)
      (if (Utilities|Time|IsValidTimerHandle (Variables|Default|GetChargeTimer))
        (if (Class|KismetSystemLibrary|IsTimerPausedHandle (Variables|Default|GetChargeTimer))
          (Utilities|Time|ClearandInvalidateTimerbyHandle (Variables|Default|GetChargeTimer)))))))

(event Custom|MC_StartChargeFX
  (Utilities|IsValid (Variables|Default|GetChargingSoundRef)
    (:Is%20Valid
      (if (not (Audio|Components|Audio|IsPlaying (Variables|Default|GetChargingSoundRef)))
        (Audio|Components|Audio|SetVolumeMultiplier (Variables|Default|GetChargingSoundRef) 1.0 :!class /Script/Engine.AudioComponent)
        (Audio|Components|Audio|Play (Variables|Default|GetChargingSoundRef) 0.0)))
    (:Is%20Not%20Valid
      (bind _returnvalue (Audio|SpawnSoundatLocation "/Game/TargetRunner/Assets/Audio/FX/EnergyHumLoop_1_Cue.EnergyHumLoop_1_Cue" (Transformation|GetWorldLocation (Variables|Default|GetBeaconPillar)) "0, 0, 0" 1.0 1.0 0.0 0 0))
      (Variables|Default|SetChargingSoundRef _returnvalue))))

(event Custom|MC_StopChargeFX
  (Utilities|IsValid (Variables|Default|GetChargingSoundRef)
    (:Is%20Valid
      (Audio|Components|Audio|FadeOut (Variables|Default|GetChargingSoundRef) 0.5 0.0 "Linear" :!class /Script/Engine.AudioComponent))))

(fn ConstructionScript)
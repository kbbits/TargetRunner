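; Player inventory that stores named goods and quantities in a map and answers count, requirement and tool ammo checks.
; Add/subtract applies a multiplier, rejects results below zero and broadcasts the new totals through an inventory delta event.
; Batch changes are not atomic: they apply what succeeds, return failed entries and send one combined event.
; The saveable copy omits goods whose names contain "Key.", so keys do not persist.
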(event EventBeginPlay)

(event EventTick
  (params (DeltaSeconds :type Float%20%28single-precision%29)))

(fn HasAmmoforTool
  (params (ToolName :type Name))
  (bind (_bvalid _toolclass) (CallFunction|GetToolClassbyName ToolName))
  (if _bvalid
    (return (CallFunction|HasGoods (Utilities|GetClassDefaults _toolclass)))
    (else
      (return false))))

(fn AddSubtractGoods
  (params (GoodsQuantity :type Goods%20Quantity%20Structure) (SkipDeltaEvent :type Boolean) (QuantityMultiple :type Float%20%28single-precision%29))
  (bind (_name _quantity) (Utilities|Struct|BreakGoodsQuantity GoodsQuantity))
  (LocalVariables|SettmpGoodsName _name)
  (if (Utilities|Name|NotEqual(Name) (LocalVariables|GettmpGoodsName) "None")
    (if (>= (+ (* _quantity QuantityMultiple) (.Value (Utilities|Map|Find (Variables|Default|GetGoodsInventory) (LocalVariables|GettmpGoodsName)))) 0.0)
      (Utilities|Map|Add (Variables|Default|GetGoodsInventory) (LocalVariables|GettmpGoodsName) (+ (* _quantity QuantityMultiple) (.Value (Utilities|Map|Find (Variables|Default|GetGoodsInventory) (LocalVariables|GettmpGoodsName)))))
      (if SkipDeltaEvent
        _
        (else
          (Default|CallOnInventoryDelta (Utilities|Array|MakeArray (Utilities|Struct|MakeGoodsQuantity (LocalVariables|GettmpGoodsName) (.Value (Utilities|Map|Find (Variables|Default|GetGoodsInventory) (LocalVariables|GettmpGoodsName))))))))
      (return true (.Value (Utilities|Map|Find (Variables|Default|GetGoodsInventory) (LocalVariables|GettmpGoodsName))))
      (else
        (return false (.Value (Utilities|Map|Find (Variables|Default|GetGoodsInventory) (LocalVariables|GettmpGoodsName))))))
    (else
      (return false 0.0))))

(fn GetGoodsCount
  (params (GoodsName :type Name))
  (bind _goodsinventory (Variables|Default|GetGoodsInventory))
  (bind (_value _returnvalue) (Utilities|Map|Find _goodsinventory GoodsName))
  (LocalVariables|SettmpCurrentCount _value)
  (if _returnvalue
    (return (LocalVariables|GettmpCurrentCount))
    (else
      (return 0.0))))

(fn AddSubtractGoodsBatch
  (params (Goods :type Array%20of%20Goods%20Quantity%20Structures) (QuantityMultiple :type Float%20%28single-precision%29))
  (LocalVariables|SettmpSuccessful true)
  (for _array_element Goods
    (bind (_successful _currentquantity) (CallFunction|AddSubtractGoods _array_element true QuantityMultiple))
    (if _successful
      (Utilities|Array|Add (LocalVariables|GettmpNewGoodsQuantities) (Utilities|Struct|MakeGoodsQuantity (.Name (Utilities|Struct|BreakGoodsQuantity _array_element)) _currentquantity))
      (else
        (LocalVariables|SettmpSuccessful false)
        (Utilities|Array|Add (LocalVariables|GettmpGoodsNotProcessed) _array_element))))
  (Default|CallOnInventoryDelta (LocalVariables|GettmpNewGoodsQuantities))
  (return (LocalVariables|GettmpSuccessful) (LocalVariables|GettmpGoodsNotProcessed)))

(fn HasAllGoods
  (params (RequiredGoods :type Array%20of%20Goods%20Quantity%20Structures))
  (LocalVariables|SettmpHasAllGoods true)
  (bind _array_element (Utilities|Array|ForEachLoopwithBreak RequiredGoods :!label _label)
    (:LoopBody
      (if (not (CallFunction|HasGoods _array_element))
        (LocalVariables|SettmpHasAllGoods false)
        (goto _label Break)))
    (:Completed
      (return (LocalVariables|GettmpHasAllGoods)))))

(fn GetSaveableGoodsInventory
  (bind _keys (Utilities|Map|Keys (Variables|Default|GetGoodsInventory)))
  (for _array_element _keys
    (if (not (Utilities|String|Contains (Utilities|String|ToString(Name) _array_element) "Key."))
      (Utilities|Map|Add (LocalVariables|GettmpSaveable) _array_element (.Value (Utilities|Map|Find (Variables|Default|GetGoodsInventory) _array_element)))))
  (return (LocalVariables|GettmpSaveable)))

(fn HasGoods
  (params (GoodsQuantity :type Goods%20Quantity%20Structure%20%28by%20ref%29))
  (bind (_name _quantity) (Utilities|Struct|BreakGoodsQuantity GoodsQuantity))
  (if (Utilities|Name|Equal(Name) _name "None")
    (return true)
    (else
      (return (>= (.Value (Utilities|Map|Find (Variables|Default|GetGoodsInventory) _name)) _quantity)))))

(fn GetAllGoodsInventory
  (bind _keys (Utilities|Map|Keys (Variables|Default|GetGoodsInventory)))
  (for _array_element _keys
    (Utilities|Array|Add (LocalVariables|GettmpAllGoods) (Utilities|Struct|MakeGoodsQuantity _array_element (.Value (Utilities|Map|Find (Variables|Default|GetGoodsInventory) _array_element)))))
  (return (LocalVariables|GettmpAllGoods)))
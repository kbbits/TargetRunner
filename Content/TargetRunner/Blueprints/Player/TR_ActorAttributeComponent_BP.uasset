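; Actor attribute component for TargetRunner that holds a bounded value which changes over time at a recharge rate.
; While active, Tick applies the rate and clamps the value between minimum and maximum.
; DoOnce gates fire hit-maximum and hit-minimum dispatchers once per arrival at each limit.
; Helpers return remaining capacity and current percent; all members carry an "Old" suffix, and debug prints are disconnected.
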(event EventTick
  (params (DeltaSeconds :type Float%20%28single-precision%29))
  (if (Components|Activation|IsActive)
    (if (and (!= (Variables|Default|GetRechargeRate_Old) 0.0) (Math|Float|InRange(Float) (Variables|Default|GetCurrentValue_Old) (Variables|Default|GetMinValue_Old) (Variables|Default|GetMaxValue_Old)))
      (Variables|Default|SetCurrentValue_Old (Math|Float|Clamp(Float) (+ (* (Variables|Default|GetRechargeRate_Old) DeltaSeconds) (Variables|Default|GetCurrentValue_Old)) (Variables|Default|GetMinValue_Old) (Variables|Default|GetMaxValue_Old)))
      (if (== (Variables|Default|GetCurrentValue_Old) (Variables|Default|GetMaxValue_Old))
        (Utilities|FlowControl|DoOnce true :!label _label
          (:Completed
            (Default|CallOnHitMaximumOld)))
        (else
          (Utilities|FlowControl|Sequence
            (:then_0
              (goto _label Reset))
            (:then_1
              (if (== (Variables|Default|GetCurrentValue_Old) (Variables|Default|GetMinValue_Old))
                (Utilities|FlowControl|DoOnce true :!label _label_2
                  (:Completed
                    (Default|CallOnHitMinimumOld)))
                (else
                  (goto _label_2 Reset))))))))))

(fn GetRemainingCapacityOld
  (return (- (Variables|Default|GetMaxValue_Old) (Variables|Default|GetCurrentValue_Old))))

(fn GetCurrentPercentOld
  (return (select (== (Variables|Default|GetMaxValue_Old) 0.0) 0.0 (/ (Variables|Default|GetCurrentValue_Old) (Variables|Default|GetMaxValue_Old)))))
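; Base player controller for TargetRunner, handling menus, awards, inventory costs, exit unlocks and run flow.
; Menus route through ShowMenuOnDevice/HideMenuOnDevice, which choose between VR widgets and viewport.
; Awards and energy/ammo deductions apply locally and are mirrored by RPC to PlayerState and PlayerInventory.
; Run completion saves and animus depletion reloads or checks all dead in multiplayer, with GameInstance handling save slots, sessions and travel.
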(event Custom|OnStartGame
  (params (GameLevel :type Float%20%28single-precision%29) (Seed :type Integer))
  ;[1 1 1] Start local game
  (Variables|Default|SetGameOptionsMenu 0) ; Clear refs to these widgets.  They won't be needed until next new game.
  (Variables|Default|SetGameSlotMenu 0)
  (Variables|Default|SetGameSelectMenu 0)
  (bind _astr_game_instance_bp (Utilities|Casting|CastToTR_GameInstance_BP (Game|GetGameInstance)))
  (Default|LocalTraveltoGameStart _astr_game_instance_bp GameLevel Seed))

(event Custom|_ServerAddAwards
  (params (PickupType :type PickupAwards%20Enum :default "NewEnumerator0") (Quantity :type Float%20%28single-precision%29) (WeaponName :type Name) (GoodsAwarded :type Array%20of%20Goods%20Quantity%20Structures))
  ;[1 1 1] Add Awards
  (CallFunction|AddAwardsImpl PickupType Quantity WeaponName GoodsAwarded))

(event Custom|ShowGameMenu
  ;[1 1 1] Game Menu
  (CallFunction|StartfromGameSelectMenu))

(event Custom|HideGameMenu
  ;[1 1 1] Game Menu
  (CallFunction|HideMenuonDevice (Variables|Default|GetGameSelectMenu)))

(event Custom|ClientPostLogin
  ;[1 1 1] Post Login
  (CallFunction|CreateWaitHUD)
  (CallFunction|ShowWaitHUD)
  (Utilities|FlowControl|Delay 0.2)
  (CallFunction|ServerPostLogin))

(event Custom|ServerPostLogin
  ;[1 1 1] Post Login
  (bind _astr_game_mode_base_bp (Utilities|Casting|CastToTR_GameMode_Base_BP (Game|GetGameMode))))

(event Custom|ServerRespawnAfterDeath
  ;[1 1 1] ServerRespawnAfterDeath
  (CallFunction|MCPlaySoundatLoation "/Game/TargetRunner/Assets/Audio/PopShort_01.PopShort_01")
  (bind _astr_game_mode_base_bp (Utilities|Casting|CastToTR_GameMode_Base_BP (Game|GetGameMode)))
  (Default|RespawnPlayer _astr_game_mode_base_bp self))

(event Custom|MC_PlaySoundAtLoation
  (params (Sound :type Sound%20Base%20Object%20Reference))
  (bind _returnvalue (Game|Player|GetPlayerPawn 0))
  ;[1 1 1] MC_PlaySoundAtLocation
  (Utilities|IsValid _returnvalue
    (:Is%20Valid
      (Audio|PlaySoundatLocation Sound (Transformation|GetActorLocation _returnvalue) "0, 0, 0" 1.0 1.0 0.0 0 0 0))))

(event Custom|Server_DeductEnergyAmmo
  (params (Energy :type Float%20%28single-precision%29) (AmmoGoods :type Goods%20Quantity%20Structure))
  ;[1 1 1] Deduct Energy & Ammo Goods
  (CallFunction|DeductEnergyAmmoClient-Server Energy AmmoGoods))

(event Custom|Client_DeductEnergyAmmo
  (params (EnergyToDeduct :type Float%20%28single-precision%29) (AmmoGoods :type Goods%20Quantity%20Structure))
  ;[1 1 1] Deduct Energy & Ammo Goods
  (CallFunction|DeductEnergyAmmoImpl EnergyToDeduct AmmoGoods))

(event Custom|StartFromGameSlotMenu
  ;[1 1 1] Start From GameSlot Menu
  (Utilities|IsValid (Variables|Default|GetGameSlotMenu)
    (:Is%20Valid
      _)
    (:Is%20Not%20Valid
      (bind _returnvalue (UserInterface|CreateWidget "/Game/TargetRunner/Blueprints/UI/TR_GameSlotMenu.TR_GameSlotMenu_C" self))
      (bind _output_get (Variables|Default|SetGameSlotMenu _returnvalue))
      (EventDispatchers|BindEventtoOnSlotSelected _output_get (delegate Custom|OnSlotSelected))))
  (CallFunction|ShowMenuonDevice (Variables|Default|GetGameSlotMenu) false))

(event Custom|OnSlotSelected
  (params (SelectedSlotNumber :type Integer))
  ;[1 1 1] Start From GameSlot Menu
  (bind _astr_game_instance_bp (Utilities|Casting|CastToTR_GameInstance_BP (Game|GetGameInstance)))
  (Variables|/Game/TargetRunner/Blueprints/Game/TR_GameInstance_BP.TR_GameInstance_BP_C|SetSaveSlot _astr_game_instance_bp SelectedSlotNumber)
  (CallFunction|LoadfromCurrentSaveSlot)
  (CallFunction|HideMenuonDevice (Variables|Default|GetGameSlotMenu))
  (CallFunction|StartfromGameSelectMenu))

(event Custom|StartFromGameOptions
  (params (Multiplayer :type Boolean))
  ;[1 1 1] Start From GameOptions Menu
  (Utilities|IsValid (Variables|Default|GetGameOptionsMenu)
    (:Is%20Valid
      (Default|InitforDisplay (Variables|Default|GetGameOptionsMenu)))
    (:Is%20Not%20Valid
      (bind _returnvalue (UserInterface|CreateWidget "/Game/TargetRunner/Blueprints/UI/TR_GameOptions.TR_GameOptions_C" self 1.0 0))
      (Variables|Default|SetGameOptionsMenu _returnvalue)
      (if Multiplayer
        (EventDispatchers|BindEventtoOnStartGameClicked (Variables|Default|GetGameOptionsMenu) (delegate Custom|HostMultiplayerGame_delegate))
        (else
          (EventDispatchers|BindEventtoOnStartGameClicked (Variables|Default|GetGameOptionsMenu) (delegate Custom|OnStartGame))))
      (EventDispatchers|BindEventtoOnCancelClicked (Variables|Default|GetGameOptionsMenu) (delegate Custom|OnGameOpionsCanceled))))
  (CallFunction|ShowMenuonDevice (Variables|Default|GetGameOptionsMenu) false))

(event Custom|LoadFromCurrentSaveSlot
  ;[1 1 1] Save / Load Game
  (bind _astr_game_instance_bp (Utilities|Casting|CastToTR_GameInstance_BP (Game|GetGameInstance)))
  (bind (_successful _player_slot_save) (Default|LoadPlayerGameData _astr_game_instance_bp (Variables|Default|GetPlayerNumber)))
  (if _successful
    (CallFunction|UpdatefromSaveData (Variables|/Game/TargetRunner/Blueprints/Game/SaveLoad/TR_PlayerSlotSave.TR_PlayerSlotSave_C|GetPlayerSaveData _player_slot_save))))

(event Custom|SaveToCurrentSlot
  ;[1 1 1] Save / Load Game
  (bind _astr_game_instance_bp (Utilities|Casting|CastToTR_GameInstance_BP (Game|GetGameInstance)))
  (bind _playersavedata (CallFunction|GetPlayerSaveData))
  (bind _successful (Default|SavePlayerGameData _astr_game_instance_bp (Variables|Default|GetPlayerNumber) _playersavedata))
  (if (not _successful)
    (Development|PrintString "Failed to save game" true true "(R=1.000000,G=0.014578,B=0.000000,A=1.000000)")))

(event Custom|StartFromGameSelectMenu
  ;[1 1 1] StartFromGameSelectMenu
  (Utilities|IsValid (Variables|Default|GetGameSelectMenu)
    (:Is%20Valid
      _)
    (:Is%20Not%20Valid
      (bind _returnvalue (UserInterface|CreateWidget "/Game/TargetRunner/Blueprints/UI/TR_GameSelectMenu.TR_GameSelectMenu_C" self))
      (Variables|Default|SetGameSelectMenu _returnvalue)))
  (CallFunction|ShowMenuonDevice (Variables|Default|GetGameSelectMenu) false))

(event Custom|OnEnteredPlatform
  (params (Platform :type Platform%20Base%20BP%20Object%20Reference))
  ;[1 1 1] OnEnteredPlatform - called from Platform_Base overlap
  (Variables|Default|SetCurrentPlatform Platform)
  (Default|CallOnPlayerEnteredPlatform))

(event Custom|OnLeavePlatform
  (params (OldPlatform :type Platform%20Base%20BP%20Object%20Reference))
  ;[1 1 1] OnLeavePlatform
  (if (== OldPlatform (Variables|Default|GetCurrentPlatform))
    (Variables|Default|SetCurrentPlatform 0)
    (Default|CallOnPlayerLeftPlatform)))

(event Custom|OnGameOpionsCanceled
  ;[1 1 1] Start From GameOptions Menu
  (CallFunction|StartfromGameSlotMenu))

(event Custom|HostMultiplayerGame_delegate
  (params (GameLevel :type Float%20%28single-precision%29) (Seed :type Integer))
  ;[1 1 1] Start From GameOptions Menu
  (Variables|Default|SetGameOptionsMenu 0) ; Clear refs to these widgets.  They won't be needed until next new game.
  (Variables|Default|SetGameSlotMenu 0)
  (Variables|Default|SetGameSelectMenu 0)
  (CallFunction|ServerStartNewGameLevel GameLevel Seed))

(event Custom|AddGoodsBatch
  (params (GoodsToAdd :type Array%20of%20Goods%20Quantity%20Structures))
  ;[1 1 1] Add Goods
  (Default|AddSubtractGoodsBatch (Variables|Default|GetPlayerInventory) GoodsToAdd 1.0))

(event Custom|_ServerOnRunComplete
  ;[1 1 1] OnRunComplete - Player has reached the goal and triggered it.
  (bind _astr_game_mode_base_bp (Utilities|Casting|CastToTR_GameMode_Base_BP (Game|GetGameMode)))
  (Variables|/Game/TargetRunner/Blueprints/Player/TR_PlayerState.TR_PlayerState_C|SetMaxLevelCompleted (Variables|Default|GetMyPlayerState) (Math|Float|Max(Float) (Variables|/Game/TargetRunner/Blueprints/Game/TR_GameMode_Base_BP.TR_GameMode_Base_BP_C|GetCurrentGameLevel _astr_game_mode_base_bp) (Variables|/Game/TargetRunner/Blueprints/Player/TR_PlayerState.TR_PlayerState_C|GetMaxLevelCompleted (Variables|Default|GetMyPlayerState))))
  (CallFunction|SavetoCurrentSlot)
  (Development|PrintString "Successfully completed this run!")
  (bind _astr_game_instance_bp (Utilities|Casting|CastToTR_GameInstance_BP (Game|GetGameInstance)))
  (if (Variables|/Game/TargetRunner/Blueprints/Game/TR_GameInstance_BP.TR_GameInstance_BP_C|GetisMultiplayerSession _astr_game_instance_bp)
    (CallFunction|ServerSessionTraveltoLevel "LobbyMap01")
    (else
      (Default|LocalTraveltoRunComplete _astr_game_instance_bp))))

(event Custom|OnFellOutOfWorld
  ;[1 1 1] Fell Out of World
  (bind _astr_game_mode_base_bp (Utilities|Casting|CastToTR_GameMode_Base_BP (Game|GetGameMode)))
  (Default|OnFellOutOfWorld _astr_game_mode_base_bp self))

(event Custom|ServerHostSession
  (params (GameLevel :type Float%20%28single-precision%29) (Seed :type Integer))
  ;[1 1 1] Server HostSession
  (bind _astr_game_instance_bp (Utilities|Casting|CastToTR_GameInstance_BP (Game|GetGameInstance)))
  (CallFunction|HideGameMenu)
  (CallFunction|ShowWaitHUD)
  (Default|DestroyPlayerSession _astr_game_instance_bp self)
  (Default|ServerHostNewSesssion _astr_game_instance_bp self GameLevel Seed))

(event Custom|AddGoods
  (params (GoodsToAdd :type Goods%20Quantity%20Structure))
  ;[1 1 1] Add Goods
  (Default|AddSubtractGoods (Variables|Default|GetPlayerInventory) GoodsToAdd false 1.0))

(event Custom|_ServerAttemptExitUnlock
  (params (ExitActor :type Exit%20Base%20BP%20Object%20Reference))
  (bind _requiredkeys (Variables|/Game/TargetRunner/Blueprints/World/ExitBase_BP.ExitBase_BP_C|GetRequiredKeys ExitActor))
  ;[1 1 1] Exit Unlock
  (if (Default|HasAllGoods (Variables|Default|GetPlayerInventory) _requiredkeys)
    (bind _successful (Default|AddSubtractGoodsBatch (Variables|Default|GetPlayerInventory) _requiredkeys -1.0)) ; Remove the keys used to unlock
    (Variables|/Game/TargetRunner/Blueprints/World/ExitBase_BP.ExitBase_BP_C|SetUnlocked ExitActor _successful)
    (else
      (CallFunction|OCFailedExitUnlock ExitActor))))

(event Custom|_ClientAddAwards
  (params (PickupType :type PickupAwards%20Enum :default "NewEnumerator0") (Quantity :type Float%20%28single-precision%29) (WeaponName :type Name) (GoodsAwarded :type Array%20of%20Goods%20Quantity%20Structures))
  ;[1 1 1] Add Awards
  (CallFunction|AddAwardsImpl PickupType Quantity WeaponName GoodsAwarded))

(event Custom|OnRunComplete
  ;[1 1 1] OnRunComplete - Player has reached the goal and triggered it.
  (CallFunction|ServeronRunComplete))

(event Custom|AttemptExitUnlock
  (params (ExitActor :type Exit%20Base%20BP%20Object%20Reference))
  ;[1 1 1] Exit Unlock
  (CallFunction|ServerAttemptExitUnlock ExitActor))

(event Custom|OC_FailedExitUnlock
  (params (ExitActor :type Exit%20Base%20BP%20Object%20Reference))
  ;[1 1 1] Exit Unlock
  (Development|PrintString "You do not have all requird keys." true true "(R=1.000000,G=0.916800,B=0.000000,A=1.000000)" 5.0))

(event Custom|OC_NewGame
  ;[1 1 1] New Game
  (Game|OpenLevel(byName) "StartupMap"))

(event Custom|ShowNewLevelSummary
  (params (LevelStats :type Level%20Run%20Stats%20Structure))
  ;[1 1 1] Show Level Summary
  (Utilities|IsValid (Variables|Default|GetLevelSummaryMenu)
    (:Is%20Valid
      _)
    (:Is%20Not%20Valid
      (bind _returnvalue (UserInterface|CreateWidget "/Game/TargetRunner/Blueprints/UI/TR_LevelSummaryMenu.TR_LevelSummaryMenu_C" self))
      (bind _output_get (Variables|Default|SetLevelSummaryMenu _returnvalue))
      (EventDispatchers|BindEventtoOnMenuClosed _output_get (delegate Custom|OnSummaryClosed))))
  (Default|SetLevelStats (Variables|Default|GetLevelSummaryMenu) LevelStats)
  (CallFunction|ShowMenuonDevice (Variables|Default|GetLevelSummaryMenu) true))

(event Custom|OnSummaryClosed
  ;[1 1 1] Show Level Summary
  (CallFunction|HideMenuonDevice (Variables|Default|GetLevelSummaryMenu)))

(event Custom|ServerStartNewGameLevel
  (params (GameLevel :type Float%20%28single-precision%29) (GameSeed :type Integer))
  ;[1 1 1] Server Start New GameLevel
  (bind _astr_game_instance_bp (Utilities|Casting|CastToTR_GameInstance_BP (Game|GetGameInstance)))
  (CallFunction|HideGameMenu)
  (Default|ServerTraveltoGameStart _astr_game_instance_bp GameLevel GameSeed self))

(event Custom|ServerJoinSession
  ;[1 1 1] Server JoinSession - Need to rework
  (bind _astr_game_instance_bp (Utilities|Casting|CastToTR_GameInstance_BP (Game|GetGameInstance)))
  (CallFunction|HideGameMenu)
  (CallFunction|ShowWaitHUD)
  (Default|ServerJoinSession _astr_game_instance_bp self))

(event Custom|OnAnimusDepleted
  ;[1 1 1] Begin Play
  (CallFunction|AnimusDepletedImpl))

(event Custom|HidePlayerInventory
  ;[1 1 1] Debug & Testing
  (Utilities|IsValid (Variables|Default|GetPlayerInventoryMenu)
    (:Is%20Valid
      (CallFunction|HideMenuonDevice (Variables|Default|GetPlayerInventoryMenu)))))

(event Custom|Server_ShowNewLevelSummary
  ;[1 1 1] Show Level Summary
  (bind _astr_game_instance_bp (Utilities|Casting|CastToTR_GameInstance_BP (Game|GetGameInstance)))
  (Default|ShowLevelCompleteSummary _astr_game_instance_bp self))

(event Custom|AddKeyAwards
  ;[1 1 1] Debug & Testing
  (CallFunction|AddAwards "NewEnumerator1" 1.0 "None" (Utilities|Array|MakeArray (Utilities|Struct|MakeGoodsQuantity "Key.Alpha" 1.0) (Utilities|Struct|MakeGoodsQuantity "Key.Beta" 1.0))) ; Debug - Add keys
)

(event Custom|ServerOnRunFailed
  ;[1 1 1] On Run Failed
  (Development|PrintString "You ran out of animus!!")
  (CallFunction|LoadfromCurrentSaveSlot)
  (bind _astr_game_instance_bp (Utilities|Casting|CastToTR_GameInstance_BP (Game|GetGameInstance)))
  (if (Variables|/Game/TargetRunner/Blueprints/Game/TR_GameInstance_BP.TR_GameInstance_BP_C|GetisMultiplayerSession _astr_game_instance_bp)
    (CallFunction|ServerSessionTraveltoLevel "LobbyMap01")
    (else
      (Default|LocalTraveltoRunComplete _astr_game_instance_bp))))

(event Custom|ServerSessionTravelToLevel
  (params (LevelName :type String))
  ;[1 1 1] Group Travel To Level
  (bind _astr_game_instance_bp (Utilities|Casting|CastToTR_GameInstance_BP (Game|GetGameInstance)))
  (CallFunction|HideGameMenu)
  (CallFunction|ShowWaitHUD)
  (Default|ServerTraveltoLevel _astr_game_instance_bp LevelName self))

(event Custom|AddAwards
  (params (PickupType :type PickupAwards%20Enum :default "NewEnumerator0") (QuantityToAdd :type Float%20%28single-precision%29) (WeaponName :type Name) (GoodsAwarded :type Array%20of%20Goods%20Quantity%20Structures))
  ;[1 1 1] Add Awards
  (Networking|SwitchHasAuthority
    (:Authority
      (if (Pawn|IsLocalController)
        _
        (else
          (CallFunction|ClientAddAwards PickupType QuantityToAdd WeaponName GoodsAwarded)))
      (CallFunction|AddAwardsImpl PickupType QuantityToAdd WeaponName GoodsAwarded))
    (:Remote
      (CallFunction|AddAwardsImpl PickupType QuantityToAdd WeaponName GoodsAwarded)
      (CallFunction|ServerAddAwards PickupType QuantityToAdd WeaponName GoodsAwarded))))

(event Custom|ShowWaitHUD
  ;[1 1 1] Show/Hide WaitHUD
  (Utilities|IsValid (Variables|Default|GetWaitHud)
    (:Is%20Valid
      (if (not (UserInterface|Viewport|IsinViewport (Variables|Default|GetWaitHud)))
        (UserInterface|Viewport|AddtoViewport (Variables|Default|GetWaitHud) 10)))))

(event Custom|HideWaitHUD
  (bind _waithud (Variables|Default|GetWaitHud))
  ;[1 1 1] Show/Hide WaitHUD
  (Utilities|IsValid _waithud
    (:Is%20Valid
      (Widget|RemovefromParent _waithud))))

(event Custom|NewGame
  ;[1 1 1] New Game
  (CallFunction|OCNewGame)
  (Utilities|FlowControl|Delay 1.0)
  (bind _astr_game_instance_bp (Utilities|Casting|CastToTR_GameInstance_BP (Game|GetGameInstance)))
  (Default|DestroyPlayerSession _astr_game_instance_bp self))

(event EventBeginPlay
  ;[1 1 1] Begin Play
  (Utilities|FlowControl|Delay 0.2 :!label _label)
  (bind _astr_player_state (Utilities|Casting|CastToTR_PlayerState (Variables|GetPlayerState))
    (:then
      (bind _output_get (Variables|Default|SetMyPlayerState _astr_player_state))
      (EventDispatchers|BindEventtoOnHitMinimum (Variables|/Game/TargetRunner/Blueprints/Player/TR_PlayerState.TR_PlayerState_C|GetAnimusAttrComponent _output_get) (delegate Custom|OnAnimusDepleted))
      (if (and (Pawn|IsLocalController) (Class|Controller|IsPlayerController))
        (CallFunction|SetupHUDs)
        (CallFunction|HideWaitHUD)))
    (:CastFailed
      (goto _label))))

(event EventEndPlay
  (params (EndPlayReason :type EEndPlayReason%20Enum :default "Destroyed"))
  ;[1 1 1] End Play
)

(event Input|ActionEvents|InputActionGameOptions
  (params (Key :type Key%20Structure :default "None"))
  ;[1 1 1] Game Menu
  (:Pressed
    (Utilities|FlowControl|FlipFlop
      (:A
        (CallFunction|ShowGameMenu))
      (:B
        (CallFunction|HideGameMenu)))))

(event Input|ActionEvents|InputActionInventory
  (params (Key :type Key%20Structure :default "None"))
  ;[1 1 1] Debug & Testing
  (:Pressed
    (Utilities|IsValid (Variables|Default|GetPlayerInventoryMenu)
      (:Is%20Valid
        _)
      (:Is%20Not%20Valid
        (bind _returnvalue (UserInterface|CreateWidget "/Game/TargetRunner/Blueprints/UI/TR_PlayerInventory_Menu.TR_PlayerInventory_Menu_C" self))
        (bind _output_get (Variables|Default|SetPlayerInventoryMenu _returnvalue))
        (EventDispatchers|BindEventtoOnMenuClosed _output_get (delegate Custom|HidePlayerInventory))))
    (Default|RefreshInventory (Variables|Default|GetPlayerInventoryMenu))
    (CallFunction|ShowMenuonDevice (Variables|Default|GetPlayerInventoryMenu) true)))

(event Input|KeyboardEvents|0
  (params (Key :type Key%20Structure :default "None"))
  ;[1 1 1] Debug & Testing
  (:Pressed
    (CallFunction|OnRunComplete)))

(event Input|KeyboardEvents|I
  (params (Key :type Key%20Structure :default "None"))
  ;[1 1 1] Debug & Testing
)

(event Input|KeyboardEvents|V
  (params (Key :type Key%20Structure :default "None"))
  ;[1 1 1] Debug & Testing
  (:Pressed
    (bind _astr_first_person_character (Utilities|Casting|CastToTR_FirstPersonCharacter (Pawn|GetControlledPawn)))
    (Class|HeadMountedDisplayFunctionLibrary|EnableHMD true)
    (Development|ExecuteConsoleCommand "Stereo On" 0)
    (Default|InitVREvent _astr_first_person_character)))

(fn ConstructionScript)

(fn SetupHUDs
  (Utilities|IsValid (Variables|Default|GetWaitHud)
    (:Is%20Not%20Valid
      (if (and (Pawn|IsLocalController) (Class|Controller|IsPlayerController))
        (CallFunction|CreateWaitHUD)))))

(fn CreateWaitHUD
  (Utilities|IsValid (Variables|Default|GetWaitHud)
    (:Is%20Not%20Valid
      (bind _returnvalue (UserInterface|CreateWidget "/Game/TargetRunner/Blueprints/UI/TR_WaitSpinner.TR_WaitSpinner_C" self))
      (Variables|Default|SetWaitHud _returnvalue))))

(fn CreateGameMenuHUD
  (Utilities|IsValid (Variables|Default|GetGameMenu)
    (:Is%20Not%20Valid
      (bind _returnvalue (UserInterface|CreateWidget "/Game/TargetRunner/Blueprints/UI/TR_GameMenu_Widget.TR_GameMenu_Widget_C" self))
      (Variables|Default|SetGameMenu _returnvalue))))

(fn ShowMenuonDevice
  (params (Menu :type User%20Widget%20Object%20Reference) (HideHUD :type Boolean))
  (LocalVariables|SettmpMenu Menu)
  (if HideHUD
    (bind _astr_player_hud (Utilities|Casting|CastToTR_PlayerHUD (HUD|GetHUD))
      (:then
        (Default|HideAll _astr_player_hud))
      (:CastFailed
        _)))
  (bind _astr_first_person_character (Utilities|Casting|CastToTR_FirstPersonCharacter (Pawn|GetControlledPawn))
    (:then
      (if (and (Class|HeadMountedDisplayFunctionLibrary|IsHeadMountedDisplayEnabled) (Variables|/Game/TargetRunner/Blueprints/Player/TR_FirstPersonCharacter.TR_FirstPersonCharacter_C|GetUsingMotionControllers? _astr_first_person_character))
        (Default|AddWidgettoVR _astr_first_person_character (LocalVariables|GettmpMenu) true)
        (bind _astr_first_person_character_2 (Utilities|Casting|CastToTR_FirstPersonCharacter (Pawn|GetControlledPawn)))
        (Variables|/Game/TargetRunner/Blueprints/Player/TR_FirstPersonCharacter.TR_FirstPersonCharacter_C|SetPlayerInteractState _astr_first_person_character_2 "NewEnumerator1")
        (else
          (if (UserInterface|Viewport|IsinViewport (LocalVariables|GettmpMenu)) :!label _label
            _
            (else
              (UserInterface|Viewport|AddtoViewport (LocalVariables|GettmpMenu) 10)))
          (Input|SetInputModeUIOnly self (LocalVariables|GettmpMenu) "DoNotLock")
          (Variables|Default|SetbShowMouseCursor true))))
    (:CastFailed
      (goto _label))))

(fn HideMenuonDevice
  (params (Menu :type User%20Widget%20Object%20Reference))
  (LocalVariables|SettmpMenu Menu)
  (bind _astr_first_person_character (Utilities|Casting|CastToTR_FirstPersonCharacter (Pawn|GetControlledPawn))
    (:then
      (if (and (Class|HeadMountedDisplayFunctionLibrary|IsHeadMountedDisplayEnabled) (Variables|/Game/TargetRunner/Blueprints/Player/TR_FirstPersonCharacter.TR_FirstPersonCharacter_C|GetUsingMotionControllers? _astr_first_person_character))
        (Default|ClearVRWidget _astr_first_person_character)
        (bind _astr_first_person_character_2 (Utilities|Casting|CastToTR_FirstPersonCharacter (Pawn|GetControlledPawn)))
        (Default|SetDefaultInteractState _astr_first_person_character_2)
        (else
          (Utilities|IsValid (LocalVariables|GettmpMenu) :!label _label
            (:Is%20Valid
              (Widget|RemovefromParent (LocalVariables|GettmpMenu))
              (Input|SetInputModeGameOnly self)
              (Variables|Default|SetbShowMouseCursor false))))))
    (:CastFailed
      (goto _label)))
  (bind _astr_player_hud (Utilities|Casting|CastToTR_PlayerHUD (HUD|GetHUD)))
  (Default|ShowAll _astr_player_hud))

(fn SavetoCurrentSlotImpl
  (params (SaveSlotPrefix :type String)))

(fn DeductEnergyAmmoClient-Server
  (params (EnergyToDeduct :type Float%20%28single-precision%29) (AmmoGoods :type Goods%20Quantity%20Structure))
  (Utilities|FlowControl|Sequence
    (:then_0
      (bind _success (CallFunction|DeductEnergyAmmoImpl EnergyToDeduct AmmoGoods))
      (LocalVariables|SettmpSuccess _success))
    (:then_1
      (Networking|SwitchHasAuthority
        (:Remote
          (CallFunction|ServerDeductEnergyAmmo EnergyToDeduct AmmoGoods))))
    (:then_2
      (return (LocalVariables|GettmpSuccess)))))

(fn DeductEnergyAmmoImpl
  (params (EnergyToDeduct :type Float%20%28single-precision%29) (AmmoGoods :type Goods%20Quantity%20Structure))
  (LocalVariables|SettmpAmmoGoods AmmoGoods)
  (Utilities|FlowControl|Sequence
    (:then_0
      (bind _successful (Default|DeductEnergy (Variables|Default|GetMyPlayerState) EnergyToDeduct))
      (if _successful
        (if (or (Utilities|Name|Equal(Name) (.Name (Utilities|Struct|BreakGoodsQuantity (LocalVariables|GettmpAmmoGoods))) "None") (== (.Quantity (Utilities|Struct|BreakGoodsQuantity (LocalVariables|GettmpAmmoGoods))) 0.0))
          (LocalVariables|SettmpSuccess true)
          (elif (Default|HasGoods (Variables|Default|GetPlayerInventory) (LocalVariables|GettmpAmmoGoods))
            (bind _successful_2 (Default|AddSubtractGoods (Variables|Default|GetPlayerInventory) (LocalVariables|GettmpAmmoGoods) false -1.0))
            (LocalVariables|SettmpSuccess _successful_2)))))
    (:then_1
      (return (LocalVariables|GettmpSuccess)))))

(fn UpdatefromSaveData
  (params (PlayerSaveData :type Player%20Save%20Data%20Structure))
  (Variables|/Game/TargetRunner/Blueprints/Player/PlayerInventory.PlayerInventory_C|SetGoodsInventory (Variables|Default|GetPlayerInventory) (.GoodsInventory (Utilities|Struct|BreakPlayerSaveData PlayerSaveData)))
  (Default|UpdatefromSaveData (Variables|Default|GetMyPlayerState) PlayerSaveData))

(fn GetPlayerSaveData
  (bind _playersavedata (Default|GetPlayerSaveData (Variables|Default|GetMyPlayerState)))
  (bind _structout (Utilities|Struct|SetmembersinPlayerSaveData _playersavedata (Utilities|Map|MakeMap) (Default|GetSaveableGoodsInventory (Variables|Default|GetPlayerInventory))))
  (return _structout))

(fn AddAwardsImpl
  (params (PickupType :type PickupAwards%20Enum :default "NewEnumerator0") (QuantityToAdd :type Float%20%28single-precision%29) (WeaponName :type Name) (GoodsAwarded :type Array%20of%20Goods%20Quantity%20Structures))
  (switch Utilities|FlowControl|Switch|SwitchonPickupAwards PickupType
    (:NewEnumerator0
      (Default|AddEnergy (Variables|Default|GetMyPlayerState) QuantityToAdd))
    (:NewEnumerator1
      (CallFunction|AddGoodsBatch GoodsAwarded))
    (:NewEnumerator2
      (Development|PrintString "Warning: Ammo Type no longer used in awards." true true "(R=0.875000,G=0.000000,B=0.000000,A=1.000000)" 1e+01))
    (:NewEnumerator3
      (Default|UnlockTool (Variables|Default|GetMyPlayerState) WeaponName))
    (:NewEnumerator4
      (Default|AddAnimus (Variables|Default|GetMyPlayerState) QuantityToAdd))))

(fn AnimusDepletedImpl
  (Networking|SwitchHasAuthority
    (:Authority
      (LocalVariables|SettmpPawn (Pawn|GetControlledPawn))
      (bind _astr_game_instance_bp (Utilities|Casting|CastToTR_GameInstance_BP (Game|GetGameInstance)))
      (if (Variables|/Game/TargetRunner/Blueprints/Game/TR_GameInstance_BP.TR_GameInstance_BP_C|GetisMultiplayerSession _astr_game_instance_bp)
        (Default|CheckAllDead _astr_game_instance_bp)
        (else
          (CallFunction|ServeronRunFailed))))))
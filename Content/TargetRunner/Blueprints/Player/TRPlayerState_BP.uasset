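; Player state Blueprint for TargetRunner that tracks a player's score, target counts and Health, Energy and Animus attributes.
; Target hits update current and total counters plus the high score, a path noted as unused in the Rooms game mode.
; Attribute components handle resets, Animus recharge pausing and add or deduct calls, with overspill allowed only on additions.
; GetLevelRunStats packages score, time and the game mode's level template info into a run record.
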(event Custom|OnTargetHit
  (params (Score :type Float%20%28single-precision%29) (TargetDestroyed :type Boolean))
  ;[1 1 1] Handles targets hit and score.  -- Not used in Rooms gamemode
  (Utilities|FlowControl|Sequence
    (:then_0
      (Math|Integer|IncrementInt (Variables|Default|GetTargetsHit)
        (:%20%20
          (Math|Integer|IncrementInt (Variables|Default|GetTotalTargetsHit)))))
    (:then_1
      (if TargetDestroyed
        (Math|Integer|IncrementInt (Variables|Default|GetTargetsDestroyed)
          (:%20%20
            (Math|Integer|IncrementInt (Variables|Default|GetTotalTargetsDestroyed))))))
    (:then_2
      (bind _output_get (Variables|Default|SetCurrentScore (+ Score (Variables|Default|GetCurrentScore))))
      (if (> _output_get (Variables|Default|GetHighScore))
        (Variables|Default|SetHighScore (Variables|Default|GetCurrentScore))))))

(event Custom|PauseAnimus
  (Variables|/Script/TargetRunner.ActorAttributeComponent|SetbRechargePaused (Variables|Default|GetAnimusAttribute) true))

(event Custom|ResetAnimus
  (Class|ActorAttributeComponent|ResettoMax (Variables|Default|GetAnimusAttribute)))

(event Custom|ResumeAnimus
  (Variables|/Script/TargetRunner.ActorAttributeComponent|SetbRechargePaused (Variables|Default|GetAnimusAttribute) false))

(event EventCopyProperties
  (params (NewPlayerState :type Player%20State%20Object%20Reference))
  ;[1 1 1] TODO: Use this in BP?
  (|CallParentFunction NewPlayerState))

(event EventBeginPlay
  (Class|ActorAttributeComponent|ResettoMax (Variables|Default|GetHealthAttribute)))

(fn ConstructionScript)

(fn DeductEnergy
  (params (ToDeduct :type Float%20%28single-precision%29))
  (bind _energyattribute (Variables|Default|GetEnergyAttribute))
  (bind _returnvalue (Class|ActorAttributeComponent|DeltaValue _energyattribute (* ToDeduct -1.0) false))
  (return _returnvalue (Class|ActorAttributeComponent|GetCurrent _energyattribute)))

(fn AddEnergy
  (params (ToAdd :type Float%20%28single-precision%29))
  (bind _energyattribute (Variables|Default|GetEnergyAttribute))
  (Class|ActorAttributeComponent|DeltaValue _energyattribute ToAdd true)
  (return (Class|ActorAttributeComponent|GetCurrent _energyattribute)))

(fn GetLevelRunStats
  (bind _astr_game_mode_base_bp (Utilities|Casting|CastToTR_GameModeBase_BP (Game|GetGameMode)))
  (return (Utilities|Struct|MakeLevelRunStats (Variables|Default|GetPlayerGuid) (.LevelId (Utilities|Struct|BreakLevelTemplate (Class|TRGameMode|GetLevelTemplate _astr_game_mode_base_bp))) false (.Tier (Utilities|Struct|BreakLevelTemplate (Class|TRGameMode|GetLevelTemplate _astr_game_mode_base_bp))) (Variables|Default|GetCurrentScore) (Class|GameplayStatics|GetUnpausedTimeSeconds) (Utilities|Array|MakeArray))))

(fn AddAnimus
  (params (ToAdd :type Float%20%28single-precision%29))
  (bind _animusattribute (Variables|Default|GetAnimusAttribute))
  (Class|ActorAttributeComponent|DeltaValue _animusattribute ToAdd true)
  (return (Class|ActorAttributeComponent|GetCurrent _animusattribute)))

(fn GetCurrentEnergy
  (return (Class|ActorAttributeComponent|GetCurrent (Variables|Default|GetEnergyAttribute))))
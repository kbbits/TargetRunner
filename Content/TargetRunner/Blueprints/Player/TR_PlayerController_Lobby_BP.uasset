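; Player controller for the TargetRunner lobby that manages the lobby menu.
; It shows the menu after client post-login.
; The MenuToggle input action hides the menu when it is in the viewport, and otherwise shows it, including when no valid menu exists yet.
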(event EventClientPostLogin
  (|CallParentFunction)
  (CallFunction|ShowLobbyMenu))

(event EventBeginPlay
  (|CallParentFunction))

(event Input|ActionEvents|InputActionMenuToggle
  (params (Key :type Key%20Structure :default "None"))
  (:Pressed
    (Utilities|IsValid (Variables|Default|GetLobbyMenu)
      (:Is%20Valid
        (if (UserInterface|Viewport|IsinViewport (Variables|Default|GetLobbyMenu))
          (CallFunction|HideLobbyMenu)
          (else
            (CallFunction|ShowLobbyMenu :!label _label))))
      (:Is%20Not%20Valid
        (goto _label)))))

(fn ConstructionScript
  (|CallParentFunction))
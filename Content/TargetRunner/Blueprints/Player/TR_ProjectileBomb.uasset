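; TR_ProjectileBomb is a timed explosive projectile that deals area damage to shootable targets and triggers.
; The server runs the fuse timer and, on the first hit, shortens it to the after-bounce delay if longer.
; Detonation multicasts sphere scale and sound, then the server sphere-overlaps actors and calls their shootable interfaces before destroying the bomb.
; Line traces toward each actor supply hit data without checking occlusion.
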(event Custom|OnExplode
  (Networking|SwitchHasAuthority
    (:Authority
      (CallFunction|MConExplode)
      (CallFunction|HandleExplode)
      (Utilities|FlowControl|Delay 0.2)
      (Actor|DestroyActor))))

(event Custom|MC_OnExplode
  (Transformation|SetWorldScale3D (Variables|Default|GetExplosionSphere) (Math|Conversions|ToVector(Float) (/ (Variables|Default|GetExplosionRadius) 1e+02)))
  (Audio|PlaySoundatLocation "/Game/TargetRunner/Assets/Audio/PopShort.PopShort" (Transformation|GetActorLocation) "0, 0, 0" 1.0 1.0 0.0 0 0 0))

(event EventBeginPlay
  (Networking|SwitchHasAuthority
    (:Authority
      (bind _returnvalue (Utilities|Time|SetTimerbyEvent (delegate Custom|OnExplode) (Variables|Default|GetExplodeTime)))
      (Variables|Default|SetExplodeTimer _returnvalue))))

(event Collision|EventActorBeginOverlap
  (params (OtherActor :type Actor%20Object%20Reference)))

(event EventTick
  (params (DeltaSeconds :type Float%20%28single-precision%29)))

(event EventHandleEventHit
  (params (OtherActor :type Actor%20Object%20Reference) (OtherComponent :type Primitive%20Component%20Object%20Reference) (Hit :type Hit%20Result%20Structure))
  (|CallParentFunction OtherActor OtherComponent Hit)
  (Networking|SwitchHasAuthority
    (:Authority
      (Utilities|FlowControl|DoOnce false
        (:Completed
          (if (> (Utilities|Time|GetTimerRemainingTimebyHandle (Variables|Default|GetExplodeTimer)) (Variables|Default|GetAfterBounceExplodeTime))
            (Utilities|Time|ClearandInvalidateTimerbyHandle (Variables|Default|GetExplodeTimer))
            (bind _returnvalue (Utilities|Time|SetTimerbyEvent (delegate Custom|OnExplode) (Variables|Default|GetAfterBounceExplodeTime)))
            (Variables|Default|SetExplodeTimer _returnvalue)))))))

(fn ConstructionScript
  (|CallParentFunction))

(fn HandleExplode
  (bind _explosionsphere (Variables|Default|GetExplosionSphere))
  (bind (_origin _boxextent _sphereradius) (Collision|GetComponentBounds _explosionsphere))
  (Utilities|FlowControl|Sequence
    (:then_0
      (Transformation|SetWorldScale3D (Variables|Default|GetExplosionSphere) (Math|Conversions|ToVector(Float) (/ (Variables|Default|GetExplosionRadius) 1e+02))))
    (:then_1
      ;[1 1 1] AOE Damage
      (bind _outactors (Collision|SphereOverlapActors _origin _sphereradius (Utilities|Array|MakeArray "ObjectTypeQuery6" "ObjectTypeQuery2") 0 (Utilities|Array|MakeArray self)))
      (for _array_element _outactors
        (bind _output_get (LocalVariables|SettmpCurrentTarget _array_element))
        (bind _asishootable_target (Utilities|Casting|CastToIShootableTarget _output_get)
          (:then
            (bind _outhit (Class|KismetSystemLibrary|LineTraceSinglebyProfile (Transformation|GetActorLocation) (Transformation|GetActorLocation (LocalVariables|GettmpCurrentTarget)) "Projectile" false 0 "None" true))
            (Default|OnShootableTargetHit _asishootable_target (Variables|Default|GetInstigator) _outhit (CallFunction|GetCurrentDamage)))
          (:CastFailed
            (bind _asishootable_trigger (Utilities|Casting|CastToIShootableTrigger (LocalVariables|GettmpCurrentTarget)))
            (bind _outhit_2 (Class|KismetSystemLibrary|LineTraceSinglebyProfile (Transformation|GetActorLocation) (Transformation|GetActorLocation (LocalVariables|GettmpCurrentTarget)) "Projectile" false 0 "None" true))
            (Default|OnShootableTriggerHit _asishootable_trigger (Variables|Default|GetInstigator) _outhit_2)))))))
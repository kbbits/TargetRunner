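; Player controller for the TargetRunner start menu, which shows the menu on BeginPlay and handles profile selection and lobby hosting or joining.
; Selecting a profile stores its GUID on the game instance and loads that player's data through the persistent data component.
; Host and join swap in a lobby loading menu, then call the game instance's session functions.
; Show and hide helpers route menus to a VR widget when using HMD motion controllers, otherwise to the viewport.
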(event Custom|OnProfileSelected
  (params (PlayerGuid :type Guid%20Structure))
  (bind _astr_game_instance_bp (Utilities|Casting|CastToTR_GameInstance_BP (Game|GetGameInstance)))
  (bind _output_get (Variables|/Script/TargetRunner.TRGameInstance|SetHostProfileGuid _astr_game_instance_bp PlayerGuid))
  (Class|TRPersistentDataComponent|ServerLoadPlayerData (Variables|Default|GetPersistentDataComponent) _output_get))

(event Custom|HostLobby
  (CallFunction|ShowLobbyLoadingMenu)
  (bind _astr_game_instance_bp (Utilities|Casting|CastToTR_GameInstance_BP (Game|GetGameInstance)))
  (bind _astrplayer_state (Utilities|Casting|CastToTRPlayerState (Variables|Default|GetPlayerState)))
  (Development|PrintString (Utilities|String|Append "PlayerControllerStartMenu hosting new session. Player Guid: " (Guid|ToString(Guid) (Variables|/Script/TargetRunner.TRPlayerState|GetPlayerGuid _astrplayer_state))) false)
  (Default|ServerHostNewSesssion _astr_game_instance_bp))

(event Custom|JoinLobby
  (CallFunction|ShowLobbyLoadingMenu)
  (bind _astr_game_instance_bp (Utilities|Casting|CastToTR_GameInstance_BP (Game|GetGameInstance)))
  (Default|ServerJoinSession _astr_game_instance_bp self))

(event EventBeginPlay
  (Utilities|IsValid (Variables|Default|GetStartMenu)
    (:Is%20Valid
      _)
    (:Is%20Not%20Valid
      (bind _returnvalue (UserInterface|CreateWidget "/Game/TargetRunner/Blueprints/UI/StartMenu/StartMenu_Menu.StartMenu_Menu_C" self))
      (Variables|Default|SetStartMenu _returnvalue)))
  (CallFunction|ShowMenuonDevice (Variables|Default|GetStartMenu)))

(fn ConstructionScript)

(fn ShowMenuonDevice
  (params (Menu :type User%20Widget%20Object%20Reference))
  (bind _output_get (LocalVariables|SettmpMenu Menu))
  (bind _asitrstandard_menu (Utilities|Casting|CastToITRStandardMenu _output_get)
    (:then
      (Default|OnBeforeShowMenu _asitrstandard_menu))
    (:CastFailed
      _))
  (bind _astr_first_person_character (Utilities|Casting|CastToTR_FirstPersonCharacter (Pawn|GetControlledPawn))
    (:then
      (if (and (Class|HeadMountedDisplayFunctionLibrary|IsHeadMountedDisplayEnabled) (Variables|/Game/TargetRunner/Blueprints/Player/TR_FirstPersonCharacter.TR_FirstPersonCharacter_C|GetUsingMotionControllers? _astr_first_person_character))
        (Default|AddWidgettoVR _astr_first_person_character (LocalVariables|GettmpMenu) true)
        (bind _astr_first_person_character_2 (Utilities|Casting|CastToTR_FirstPersonCharacter (Pawn|GetControlledPawn)))
        (Variables|/Game/TargetRunner/Blueprints/Player/TR_FirstPersonCharacter.TR_FirstPersonCharacter_C|SetPlayerInteractState _astr_first_person_character_2 "NewEnumerator1")
        (else
          (if (UserInterface|Viewport|IsinViewport (LocalVariables|GettmpMenu)) :!label _label
            _
            (else
              (UserInterface|Viewport|AddtoViewport (LocalVariables|GettmpMenu) 10)))
          (Input|SetInputModeUIOnly self (LocalVariables|GettmpMenu) "DoNotLock")
          (Variables|Default|SetbShowMouseCursor true))))
    (:CastFailed
      (goto _label))))

(fn ShowLobbyLoadingMenu
  (CallFunction|HideMenuonDevice (Variables|Default|GetStartMenu))
  (Utilities|IsValid (Variables|Default|GetLobbyLoadingMenu)
    (:Is%20Valid
      _)
    (:Is%20Not%20Valid
      (bind _returnvalue (UserInterface|CreateWidget "/Game/TargetRunner/Blueprints/UI/StartMenu/LoadingLobby_Menu.LoadingLobby_Menu_C" self))
      (Variables|Default|SetLobbyLoadingMenu _returnvalue)))
  (CallFunction|ShowMenuonDevice (Variables|Default|GetLobbyLoadingMenu)))

(fn HideMenuonDevice
  (params (Menu :type User%20Widget%20Object%20Reference))
  (LocalVariables|SettmpMenu Menu)
  (bind _astr_first_person_character (Utilities|Casting|CastToTR_FirstPersonCharacter (Pawn|GetControlledPawn))
    (:then
      (if (and (Class|HeadMountedDisplayFunctionLibrary|IsHeadMountedDisplayEnabled) (Variables|/Game/TargetRunner/Blueprints/Player/TR_FirstPersonCharacter.TR_FirstPersonCharacter_C|GetUsingMotionControllers? _astr_first_person_character))
        (Default|ClearVRWidget _astr_first_person_character)
        (bind _astr_first_person_character_2 (Utilities|Casting|CastToTR_FirstPersonCharacter (Pawn|GetControlledPawn)))
        (Variables|/Game/TargetRunner/Blueprints/Player/TR_FirstPersonCharacter.TR_FirstPersonCharacter_C|SetPlayerInteractState _astr_first_person_character_2 "NewEnumerator1")
        (else
          (Utilities|IsValid (LocalVariables|GettmpMenu) :!label _label
            (:Is%20Valid
              (Widget|RemovefromParent (LocalVariables|GettmpMenu))
              (Input|SetInputModeGameandUI self 0 "DoNotLock" false)
              (Variables|Default|SetbShowMouseCursor false))))))
    (:CastFailed
      (goto _label)))
  (bind _astr_player_hud (Utilities|Casting|CastToTR_PlayerHUD (HUD|GetHUD)))
  (Default|ShowAll _astr_player_hud))
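; Base weapon mod actor for TargetRunner that controls firing for the first-person character it is attached to.
; BeginFire and Tick share a shot path that checks player energy and inventory ammo before having the character spawn a projectile.
; Tick accumulators time auto-fire, optional burst limits and single-shot cooldown.
; Firing while busy notifies the character via multicast or server RPC; the construction script tints the mesh.
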(event EventBeginFire
  ;[1 1 1] Begin Fire
  (if (not (Variables|Default|GetIsFiring))
    (Variables|Default|SetIsFiring true)
    (Variables|Default|SetFireDelaySum 0.0)
    (Variables|Default|SetIsAutoFiring (Variables|Default|GetAutoFire))
    (Variables|Default|SetAutoFireBurstCount 0.0)
    (Variables|Default|SetAutoFireDelaySum 0.0)
    ;[1 1 1] Try to spawn projectile
    (bind _astr_first_person_character (Utilities|Casting|CastToTR_FirstPersonCharacter (Actor|GetParentActor)))
    (bind _astr_player_controller_base_bp (Utilities|Casting|CastToTR_PlayerController_Base_BP (Pawn|GetController _astr_first_person_character)))
    (if (>= (Default|GetCurrentEnergy (Default|GetTRPlayerState _astr_player_controller_base_bp)) (Variables|Default|GetEnergyPerShot))
      (if (Default|HasGoods (Variables|/Game/TargetRunner/Blueprints/Player/TR_PlayerController_Base_BP.TR_PlayerController_Base_BP_C|GetPlayerInventory _astr_player_controller_base_bp) (Variables|Default|GetAmmoPerShot))
        (Default|SpawnProjetile _astr_first_person_character)
        (if (Variables|Default|GetIsAutoFiring)
          (Math|Float|IncrementFloat (Variables|Default|GetAutoFireBurstCount)))))
    (else
      (bind _astr_first_person_character_2 (Utilities|Casting|CastToTR_FirstPersonCharacter (Actor|GetParentActor)))
      (Networking|SwitchHasAuthority
        (:Authority
          (Default|MConWeaponFireBusy _astr_first_person_character_2))
        (:Remote
          (Default|ServeronWeaponFireBusy _astr_first_person_character_2))))))

(event EventEndFire
  ;[1 1 1] End Fire
  (Variables|Default|SetIsAutoFiring false)
  (Variables|Default|SetAutoFireBurstCount 0.0)
  (Variables|Default|SetAutoFireDelaySum 0.0)
  (if (<= (Variables|Default|GetFireDelay) 0.0)
    (Variables|Default|SetFireDelaySum 0.0)
    (Variables|Default|SetIsFiring false)))

(event EventTick
  (params (DeltaSeconds :type Float%20%28single-precision%29))
  ;[1 1 1] Tick
  (if (Variables|Default|GetIsFiring)
    (if (Variables|Default|GetIsAutoFiring)
      (if (or (== (Variables|Default|GetAutoFireBurstLimit) 0.0) (< (Variables|Default|GetAutoFireBurstCount) (Variables|Default|GetAutoFireBurstLimit)))
        (if (>= (+ DeltaSeconds (Variables|Default|GetAutoFireDelaySum)) (Variables|Default|GetAutoFireDelay))
          (Variables|Default|SetAutoFireDelaySum (- (+ DeltaSeconds (Variables|Default|GetAutoFireDelaySum)) (Variables|Default|GetAutoFireDelay)))
          ;[1 1 1] Try to spawn projectile
          (bind _astr_first_person_character (Utilities|Casting|CastToTR_FirstPersonCharacter (Actor|GetParentActor)))
          (bind _astr_player_controller_base_bp (Utilities|Casting|CastToTR_PlayerController_Base_BP (Pawn|GetController _astr_first_person_character)))
          (if (>= (Default|GetCurrentEnergy (Default|GetTRPlayerState _astr_player_controller_base_bp)) (Variables|Default|GetEnergyPerShot))
            (if (Default|HasGoods (Variables|/Game/TargetRunner/Blueprints/Player/TR_PlayerController_Base_BP.TR_PlayerController_Base_BP_C|GetPlayerInventory _astr_player_controller_base_bp) (Variables|Default|GetAmmoPerShot))
              (Default|SpawnProjetile _astr_first_person_character)
              (if (Variables|Default|GetIsAutoFiring)
                (Math|Float|IncrementFloat (Variables|Default|GetAutoFireBurstCount)))))
          (else
            (Variables|Default|SetAutoFireDelaySum (+ DeltaSeconds (Variables|Default|GetAutoFireDelaySum))))))
      (elif (> (Variables|Default|GetFireDelay) 0.0)
        (if (>= (+ DeltaSeconds (Variables|Default|GetFireDelaySum)) (Variables|Default|GetFireDelay))
          (Variables|Default|SetFireDelaySum 0.0)
          (Variables|Default|SetIsFiring false)
          (else
            (Variables|Default|SetFireDelaySum (+ DeltaSeconds (Variables|Default|GetFireDelaySum)))))))))

(fn ConstructionScript
  (Rendering|Material|SetVectorParameterValueonMaterials (Variables|Default|GetStaticMesh) "DiffuseColor" (Math|Conversions|ToVector(LinearColor) (Variables|Default|GetBaseColor))))
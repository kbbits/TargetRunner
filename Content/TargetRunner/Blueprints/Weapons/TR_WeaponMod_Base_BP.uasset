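; Base weapon mod actor for TargetRunner, attached to the first-person character, that runs server-side firing and spawns projectiles.
; A WeaponState machine driven by Begin/End Fire and authority-only Tick handles auto-fire delay, burst limits and activation cooldown.
; A Tool object, constructed from a default class if missing, supplies fire settings and projectile stats.
; Shots route through the character before spawning, with extractor projectiles also receiving resource extraction rates.
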(event Custom|ServerSpawnProjectile
  (params (SpawnTransform :type Transform))
  (bind _tool (Variables|Default|GetTool))
  (bind _tool_2 (Variables|Default|GetTool))
  ;[1 1 1] ServerSpawnProjectile
  (if (CallFunction|IsAutoFire?)
    (Math|Float|IncrementFloat (Variables|Default|GetAutoFireBurstCount)
      (:%20%20
        _)))
  (bind _astrprojectile_extractor_base (Utilities|Casting|CastToTRProjectileExtractorBaseClass (Class|ToolActorBase|GetProjectileClass))
    (:then
      (Game|SpawnActorfromClass _astrprojectile_extractor_base SpawnTransform "AlwaysSpawn" 0 (Class|ToolActorBase|GetResourceExtractionRates) (Class|ToolActorBase|GetDamagePerShot) (Class|ToolActorBase|GetDamageRates) (Class|ToolBase|GetMaximumBounces _tool) (Class|ToolBase|GetProjectileSpeed _tool) (CallFunction|GetAttachedCharacter)))
    (:CastFailed
      (Game|SpawnActorfromClass (Class|ToolActorBase|GetProjectileClass) SpawnTransform "AlwaysSpawn" 0 (Class|ToolActorBase|GetDamagePerShot) (Class|ToolActorBase|GetDamageRates) (Class|ToolBase|GetMaximumBounces _tool_2) (Class|ToolBase|GetProjectileSpeed _tool_2) (CallFunction|GetAttachedCharacter)))))

(event Custom|ServerBeginFire
  ;[1 1 1] Begin Fire
  (switch Utilities|FlowControl|Switch|SwitchonETRWeaponState (Variables|Default|GetWeaponState)
    (:Idle
      (Variables|Default|SetWeaponState "Firing" :!label _label)
      (Variables|Default|SetFireDelaySum 0.0)
      (Variables|Default|SetAutoFireBurstCount 0.0)
      (Variables|Default|SetAutoFireDelaySum 0.0)
      (if (CallFunction|EmitsProjectile?)
        (Default|ServerAttemptSpawnProjectile (CallFunction|GetAttachedCharacter))))
    (:Aiming
      (goto _label))
    (:ReadyToFire
      (goto _label))
    (:Firing
      (Default|MConWeaponFireBusy (CallFunction|GetAttachedCharacter) :!label _label_2))
    (:FireBusy
      (goto _label_2))
    (:OutOfAmmo
      (goto _label_2))))

(event Custom|ServerEndFire
  ;[1 1 1] End Fire
  (Variables|Default|SetAutoFireBurstCount 0.0)
  (Variables|Default|SetAutoFireDelaySum 0.0)
  (if (<= (Class|ToolActorBase|GetActivationDelay) 0.0)
    (Variables|Default|SetFireDelaySum 0.0)
    (Variables|Default|SetWeaponState "Idle")
    (elif (Utilities|Enum|Equal(Enum) (Variables|Default|GetWeaponState) "Firing")
      (Variables|Default|SetWeaponState "FireBusy"))))

(event EventBeginFire
  ;[1 1 1] Begin Fire
  (Networking|SwitchHasAuthority
    (:Authority
      (switch Utilities|FlowControl|Switch|SwitchonETRWeaponState (Variables|Default|GetWeaponState)
        (:Idle
          (Variables|Default|SetWeaponState "Firing" :!label _label)
          (Variables|Default|SetFireDelaySum 0.0)
          (Variables|Default|SetAutoFireBurstCount 0.0)
          (Variables|Default|SetAutoFireDelaySum 0.0)
          (if (CallFunction|EmitsProjectile?)
            (Default|ServerAttemptSpawnProjectile (CallFunction|GetAttachedCharacter))))
        (:Aiming
          (goto _label))
        (:ReadyToFire
          (goto _label))
        (:Firing
          (Default|MConWeaponFireBusy (CallFunction|GetAttachedCharacter) :!label _label_2))
        (:FireBusy
          (goto _label_2))
        (:OutOfAmmo
          (goto _label_2))))
    (:Remote
      (CallFunction|ServerBeginFire))))

(event EventEndFire
  ;[1 1 1] End Fire
  (CallFunction|ServerEndFire))

(event EventTick
  (params (DeltaSeconds :type Float%20%28single-precision%29))
  ;[1 1 1] Tick
  (Networking|SwitchHasAuthority
    (:Authority
      (if (Utilities|Enum|Equal(Enum) (Variables|Default|GetWeaponState) "Firing")
        (if (CallFunction|IsAutoFire?)
          (if (or (== (CallFunction|GetAutoFireBurstLimit) 0.0) (< (Variables|Default|GetAutoFireBurstCount) (CallFunction|GetAutoFireBurstLimit)))
            (if (>= (+ DeltaSeconds (Variables|Default|GetAutoFireDelaySum)) (CallFunction|GetAutoFireDelay))
              (Variables|Default|SetAutoFireDelaySum (- (+ DeltaSeconds (Variables|Default|GetAutoFireDelaySum)) (CallFunction|GetAutoFireDelay)))
              (if (CallFunction|EmitsProjectile?)
                (Default|ServerAttemptSpawnProjectile (CallFunction|GetAttachedCharacter)))
              (else
                (Variables|Default|SetAutoFireDelaySum (+ DeltaSeconds (Variables|Default|GetAutoFireDelaySum)))))
            (else
              (Variables|Default|SetFireDelaySum 0.0)
              (Variables|Default|SetWeaponState "FireBusy")))
          (else
            (if (<= (Class|ToolActorBase|GetActivationDelay) 0.0) :!label _label
              (Variables|Default|SetFireDelaySum 0.0 :!label _label_2)
              (Variables|Default|SetWeaponState "Idle")
              (elif (>= (+ DeltaSeconds (Variables|Default|GetFireDelaySum)) (Class|ToolActorBase|GetActivationDelay))
                (goto _label_2)
                (else
                  (Variables|Default|SetFireDelaySum (+ DeltaSeconds (Variables|Default|GetFireDelaySum)))
                  (Variables|Default|SetWeaponState "FireBusy"))))))
        (elif (Utilities|Enum|Equal(Enum) (Variables|Default|GetWeaponState) "FireBusy")
          (goto _label))))))

(event EventBeginPlay
  ;[1 1 1] Begin Play
  (if (Utilities|IsValidSoftObjectReference (Variables|Default|GetFireSound))
    (Utilities|AsyncLoadAsset (Variables|Default|GetFireSound)
      (:Completed
        _)))
  (if (Utilities|IsValidSoftObjectReference (Variables|Default|GetFireBusySound))
    (Utilities|AsyncLoadAsset (Variables|Default|GetFireBusySound)
      (:Completed
        _)))
  (if (Utilities|IsValidSoftObjectReference (Variables|Default|GetReloadSound))
    (Utilities|AsyncLoadAsset (Variables|Default|GetReloadSound))))

(fn ConstructionScript
  (Rendering|Material|SetVectorParameterValueonMaterials (Variables|Default|GetStaticMesh) "DiffuseColor" (Math|Conversions|ToVector(LinearColor) (Variables|Default|GetBaseColor)))
  (CallFunction|ConstructDefaultTool))

(fn GetAttachedCharacter
  (bind _returnvalue (Actor|GetAttachParentActor))
  (Utilities|IsValid _returnvalue
    (:Is%20Valid
      (bind _astr_first_person_character_bp (Utilities|Casting|CastToTR_FirstPersonCharacter_BP _returnvalue)
        (:then
          (return _astr_first_person_character_bp))
        (:CastFailed
          _)))
    (:Is%20Not%20Valid
      (bind _astr_first_person_character_bp_2 (Utilities|Casting|CastToTR_FirstPersonCharacter_BP (Actor|GetParentActor))
        (:then
          (return _astr_first_person_character_bp_2))
        (:CastFailed
          _))))
  (return 0))

(fn ConstructDefaultTool
  (Utilities|IsValid (Variables|Default|GetTool)
    (:Is%20Not%20Valid
      (bind _returnvalue (Game|ConstructObjectfromClass (Variables|Default|GetDefaultToolClass_BP) self))
      (Variables|Default|SetTool _returnvalue))))

(fn IsAutoFire?
  (bind _tool (Variables|Default|GetTool))
  (Utilities|IsValid _tool
    (:Is%20Valid
      (return (Utilities|Enum|Equal(Enum) (Variables|/Script/TargetRunner.ToolBase|GetActivationType _tool) "Auto")))
    (:Is%20Not%20Valid
      (return false))))

(fn GetAutoFireDelay
  (bind _tool (Variables|Default|GetTool))
  (Utilities|IsValid _tool
    (:Is%20Valid
      (return (Class|ToolBase|GetAutoFireDelay _tool)))
    (:Is%20Not%20Valid
      (return 0.0))))

(fn GetAutoFireBurstLimit
  (bind _tool (Variables|Default|GetTool))
  (Utilities|IsValid _tool
    (:Is%20Valid
      (return (Class|ToolBase|GetAutoFireBurstLimit _tool)))
    (:Is%20Not%20Valid
      (return 0.0))))

(fn EmitsProjectile?
  (bind _tool (Variables|Default|GetTool))
  (Utilities|IsValid _tool
    (:Is%20Valid
      (return (Utilities|Enum|Equal(Enum) (Variables|/Script/TargetRunner.ToolBase|GetEmitType _tool) "Projectile")))
    (:Is%20Not%20Valid
      (return true))))
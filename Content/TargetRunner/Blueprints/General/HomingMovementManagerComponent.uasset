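; Actor component that turns its owner's ProjectileMovement into a homing projectile, starting after an optional delay.
; Starting homing removes gravity, damps launch velocity by agility, and targets a specified component or the nearest overlapping Character.
; Tick scales speed and homing acceleration by how directly the owner faces the target, drops out-of-range targets, and searches again every half second.
; Start, stop, target-acquired and target-lost changes fire event dispatchers.
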(event Custom|StartHoming
  (bind _projectilemovementreference (Variables|Default|GetProjectileMovementReference))
  ;[1 1 1] StartHoming
  (Variables|Default|SetEnableHomingMaster true)
  (bind _found_ (CallFunction|FindClosestHomingTarget))
  (if _found_
    (Default|CallOnTargetAquired))
  (Variables|/Script/Engine.ProjectileMovementComponent|SetProjectileGravityScale (Variables|Default|GetProjectileMovementReference) 0.0)
  (Variables|/Script/Engine.ProjectileMovementComponent|SetMaxSpeed (Variables|Default|GetProjectileMovementReference) (Variables|Default|GetBaseSpeedWhenTargeting))
  (Variables|/Script/Engine.MovementComponent|SetVelocity (Variables|Default|GetProjectileMovementReference) (* (Variables|/Script/Engine.MovementComponent|GetVelocity (Variables|Default|GetProjectileMovementReference)) (* "1.000000,1.000000,0.700000" (- 1.0 (Math|Float|Clamp(Float) (Math|Float|Square (Variables|Default|GetHomingAgility)) 0.1)))))
  (Variables|/Script/Engine.ProjectileMovementComponent|SetHomingAccelerationMagnitude _projectilemovementreference (* (Variables|Default|GetHomingAgility) (Variables|/Script/Engine.ProjectileMovementComponent|GetMaxSpeed _projectilemovementreference))) ; Homing accel. based on agility
  (Variables|/Script/Engine.ProjectileMovementComponent|SetbIsHomingProjectile (Variables|Default|GetProjectileMovementReference) true)
  (Default|CallOnStartHoming))

(event Custom|StopHoming
  ;[1 1 1] StopHoming
  (CallFunction|ResetHomingTarget false)
  (Variables|Default|SetEnableHomingMaster false)
  (Variables|/Script/Engine.ProjectileMovementComponent|SetbIsHomingProjectile (Variables|Default|GetProjectileMovementReference) false)
  (Default|CallOnStopHoming))

(event Custom|ResetHomingTarget
  (params (ResetGravity :type Boolean))
  (bind _projectilemovementreference (Variables|Default|GetProjectileMovementReference))
  ;[1 1 1] ResetHomingTarget
  (Utilities|IsValid (Variables|Default|GetProjectileMovementReference)
    (:Is%20Valid
      (if ResetGravity
        ;;[1 1 1] reset gravity
        (if (!= (Variables|/Script/Engine.ProjectileMovementComponent|GetProjectileGravityScale _projectilemovementreference) (Variables|Default|GetOrigialGravity))
          (Variables|/Script/Engine.ProjectileMovementComponent|SetProjectileGravityScale _projectilemovementreference (Variables|Default|GetOrigialGravity))))
      (Variables|/Script/Engine.ProjectileMovementComponent|SetHomingTargetComponent (Variables|Default|GetProjectileMovementReference) 0))))

(event Custom|SetSpecificHomingTarget
  (params (SpecificHomingTarget :type Scene%20Component%20Object%20Reference))
  (Variables|Default|SetSpecificHomingTarget SpecificHomingTarget))

(event EventBeginPlay
  ;[1 1 1] BeginPlay
  (Utilities|FlowControl|Sequence
    (:then_0
      (bind _output_get (Variables|Default|SetProjectileMovementReference (Actor|GetComponentbyClass (Components|GetOwner) "/Script/Engine.ProjectileMovementComponent")))
      (Variables|Default|SetOrigialGravity (Variables|/Script/Engine.ProjectileMovementComponent|GetProjectileGravityScale _output_get)))
    (:then_1
      (if (>= (Variables|Default|GetDelayBeforeHoming) 0.0)
        (Utilities|FlowControl|Delay (Variables|Default|GetDelayBeforeHoming))
        (CallFunction|StartHoming)))))

(event EventTick
  (params (DeltaSeconds :type Float%20%28single-precision%29))
  ;[1 1 1] Tick
  (if (Variables|Default|GetEnableHomingMaster)
    (if (Utilities|IsValid (Variables|Default|GetProjectileMovementReference))
      (Utilities|SwitchonValidTargetinRange
        (:InRange
          (Utilities|FlowControl|Sequence
            (:then_0
              (Variables|/Script/Engine.ProjectileMovementComponent|SetMaxSpeed (Variables|Default|GetProjectileMovementReference) (+ (Variables|Default|GetBaseSpeedWhenTargeting) (* (Variables|Default|GetBaseSpeedWhenTargeting) (* (- (Variables|Default|GetOnTargetSpeedMultiplier) 1.0) (Math|Float|Clamp(Float) (Math|Float|Square (CallFunction|PercentonTarget))))))))
            (:then_1
              (Variables|/Script/Engine.ProjectileMovementComponent|SetHomingAccelerationMagnitude (Variables|Default|GetProjectileMovementReference) (+ (Variables|/Script/Engine.ProjectileMovementComponent|GetMaxSpeed (Variables|Default|GetProjectileMovementReference)) (* (Variables|Default|GetHomingAgility) (* (Variables|/Script/Engine.ProjectileMovementComponent|GetMaxSpeed (Variables|Default|GetProjectileMovementReference)) 1.0)))))))
        (:OutOfRange
          (CallFunction|ResetHomingTarget false)
          (Default|CallOnTargetLost))
        (:Invalid
          ;;[1 1 1 1 14] Look for target every half second if we don't have one.
          (Utilities|FlowControl|DoOnce false :!label _label
            (:Completed
              (bind _found_ (CallFunction|FindClosestHomingTarget))
              (if _found_
                (Default|CallOnTargetAquired))
              (Utilities|FlowControl|Delay 0.5)
              (goto _label Reset))))))))

(fn FindClosestHomingTarget
  (bind _returnvalue (Components|GetOwner))
  (if (Utilities|IsValid (Variables|Default|GetProjectileMovementReference))
    (Utilities|FlowControl|Sequence
      (:then_0
        (bind _specifichomingtarget (Variables|Default|GetSpecificHomingTarget)
          (:then
            (LocalVariables|SettmpNewTarget _specifichomingtarget))
          (:else
            (bind _outactors (Collision|SphereOverlapActors (Transformation|GetActorLocation _returnvalue) (Variables|Default|GetTargetingRange) (Utilities|Array|MakeArray) "/Script/Engine.Character" (Utilities|Array|MakeArray _returnvalue)))
            (bind _output_get (LocalVariables|SettmpTargets _outactors))
            (for (_array_element _array_index) _output_get
              (if (== _array_index 0)
                (LocalVariables|SettmpNewTarget (Variables|/Script/Engine.Actor|GetRootComponent _array_element) :!label _label)
                (LocalVariables|SettmpClosestDistance (Transformation|GetDistanceTo _array_element (Components|GetOwner)))
                (elif (< (Transformation|GetDistanceTo _array_element (Components|GetOwner)) (LocalVariables|GettmpClosestDistance))
                  (goto _label)))))))
      (:then_1
        (Utilities|IsValid (LocalVariables|GettmpNewTarget)
          (:Is%20Valid
            (Variables|/Script/Engine.ProjectileMovementComponent|SetHomingTargetComponent (Variables|Default|GetProjectileMovementReference) (LocalVariables|GettmpNewTarget))
            (return true))
          (:Is%20Not%20Valid
            (return false)))))))

(fn PercentonTarget
  (Utilities|IsValid (Variables|/Script/Engine.ProjectileMovementComponent|GetHomingTargetComponent (Variables|Default|GetProjectileMovementReference))
    (:Is%20Valid
      (return (Math|Float|MapRangeUnclamped (Math|Vector|DotProduct (Math|Vector|Normalize (Transformation|GetActorForwardVector (Components|GetOwner))) (Math|Vector|Normalize (- (Transformation|GetWorldLocation (Variables|/Script/Engine.ProjectileMovementComponent|GetHomingTargetComponent (Variables|Default|GetProjectileMovementReference))) (Transformation|GetActorLocation (Components|GetOwner))))) -1.0 1.0 0.0 1.0)))
    (:Is%20Not%20Valid
      (return 0.0))))

(fn HasTargetinRange
  (Utilities|SwitchonValidTargetinRange
    (:InRange
      (return true))
    (:OutOfRange
      _)
    (:Invalid
      _))
  (return false))
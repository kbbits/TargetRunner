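; Sky sphere Blueprint that runs a day-night cycle by rotating the directional light as the sun.
; On BeginPlay it sets a timeline's play rate from the cycle duration and starts it at either the real-world hour or a configured start hour.
; Each timeline update applies the rotation change to the light and refreshes the sun direction, optionally throttled to a maximum number of updates per second.
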(event EventBeginPlay
  (Components|Timeline|SetPlayRate (Variables|Default|GetDayCycleTimeline) (/ (Math|Float|MakeLiteralFloat 8.64e+04) (Variables|Default|GetCycleDurationSeconds)))
  (Components|Timeline|SetPlaybackPosition (Variables|Default|GetDayCycleTimeline) (* (Math|Float|MakeLiteralFloat 3.6e+03) (select (Variables|Default|GetStartAtRealWorldTime) (Math|Conversions|ToFloat(Integer) (Class|KismetMathLibrary|GetHour (Math|DateTime|Now))) (Variables|Default|GetStartHourOfDay))) false true)
  (bind _rotationdegrees (Timeline|DayCycleTimeline Play)
    (:Update
      (if (> (Variables|Default|GetMaxUpdatesPerSecond) 0.0)
        (Utilities|FlowControl|DoOnce false :!label _label
          (:Completed
            _)))
      (Class|Actor|AddActorWorldRotation (Variables|Default|GetDirectional%20light%20actor) (Math|Rotator|MakeRotator (- (Variables|Default|GetLastSunRotation) _rotationdegrees) 0.0 0.0))
      (CallFunction|UpdateSunDirection)
      (Variables|Default|SetLastSunRotation _rotationdegrees)
      (if (> (Variables|Default|GetMaxUpdatesPerSecond) 0.0)
        (Utilities|FlowControl|Delay (/ 1.0 (Variables|Default|GetMaxUpdatesPerSecond)))
        (goto _label Reset)))))

(fn ConstructionScript
  (|CallParentFunction))
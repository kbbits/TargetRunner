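; ResourcePoint_BP is a room scenery Blueprint that marks where something, by its name a resource, can spawn.
; GetSpawnLocation returns a random point within the SpawnBox bounds, and GetSpawnRotation returns the Scene component's world rotation.
; It has no active event or construction logic, so it only supplies transform data to callers.
; Randomized rotation within a DirectionArrow-based cone remains in the graph but is unconnected.
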(event EventBeginPlay)

(event Collision|EventActorBeginOverlap
  (params (OtherActor :type Actor%20Object%20Reference)))

(event EventTick
  (params (DeltaSeconds :type Float%20%28single-precision%29)))

(fn ConstructionScript)

(fn GetSpawnLocation
  (bind _spawnbox (Variables|Default|GetSpawnBox))
  (bind (_origin _boxextent) (Collision|GetComponentBounds _spawnbox))
  (return (Math|Random|RandomPointinBoundingBox _origin _boxextent)))

(fn GetSpawnRotation
  (return (Transformation|GetWorldRotation (Variables|Default|GetScene))))
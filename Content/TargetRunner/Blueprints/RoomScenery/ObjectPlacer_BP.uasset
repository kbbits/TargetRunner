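; Room scenery placer actor that spawns an instance of ClassToPlace on a surface found by tracing from its arrow.
; GetPlacementTransform_BP line-traces along stream-seeded random directions within a cone, retrying up to 20 times on misses or hits on the same class.
; A hit yields a transform offset along and aligned to the surface normal, with unseeded random rotation jitter, which PlaceOne_BP spawns.
; Persistent debug lines and a trace-count text visualise the search.
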(event EventBeginPlay)

(event Collision|EventActorBeginOverlap
  (params (OtherActor :type Actor%20Object%20Reference)))

(event EventTick
  (params (DeltaSeconds :type Float%20%28single-precision%29)))

(fn ConstructionScript)

(fn GetPlacementTransformBP
  (params (RandomStream :type Random%20Stream%20Structure%20%28by%20ref%29))
  (bind _returnvalue (Math|Random|RandomFloatinRange -5.0 5.0))
  (LocalVariables|SettmpEndLocation (+ (Transformation|GetWorldLocation (Variables|Default|GetFacingArrow)) (* (Math|Random|RandomUnitVectorinConeinDegreesfromStream (Math|Vector|GetForwardVector (Variables|Default|GetFacingArrow)) (Variables|Default|GetConeAngle) RandomStream) (Variables|Default|GetConeLength))) :!label _label)
  (Math|Integer|IncrementInt (Variables|Default|GettmpTracesRun)
    (:%20%20
      (bind _outhit (Collision|LineTraceByChannel (Transformation|GetWorldLocation (Variables|Default|GetFacingArrow)) (LocalVariables|GettmpEndLocation) "TraceTypeQuery1" false 0 "Persistent"))
      (LocalVariables|SettmpHit _outhit)
      (if (and (.bBlockingHit (Collision|BreakHitResult (LocalVariables|GettmpHit))) (!= (Utilities|GetClass (.HitActor (Collision|BreakHitResult (LocalVariables|GettmpHit)))) (Variables|Default|GetClassToPlace)))
        (LocalVariables|SettmpRotation (Math|Rotator|MakeRotator (Math|Random|RandomFloatinRange -9e+01 9e+01) (+ (.Pitch (Math|Rotator|BreakRotator (Math|Conversions|RotationFromXVector (.ImpactNormal (Collision|BreakHitResult (LocalVariables|GettmpHit)))))) _returnvalue) (+ (.Yaw (Math|Rotator|BreakRotator (Math|Conversions|RotationFromXVector (.ImpactNormal (Collision|BreakHitResult (LocalVariables|GettmpHit)))))) _returnvalue)))
        (LocalVariables|SettmpTransform (Math|Transform|MakeTransform (+ (.Location (Collision|BreakHitResult (LocalVariables|GettmpHit))) (* (.ImpactNormal (Collision|BreakHitResult (LocalVariables|GettmpHit))) 16.0)) (LocalVariables|GettmpRotation)))
        (Rendering|Components|TextRender|SetText (Variables|Default|GetTextRender) (Utilities|Text|ToText(Integer) (Variables|Default|GettmpTracesRun)))
        (return (LocalVariables|GettmpTransform))
        (else
          (Utilities|FlowControl|DoN 20
            (:Exit
              (goto _label))))))))

(fn PlaceOneBP
  (params (RandomStream :type Random%20Stream%20Structure%20%28by%20ref%29) (Owner :type Actor%20Object%20Reference))
  (LocalVariables|SettmpTransform (CallFunction|GetPlacementTransformBP RandomStream))
  (bind _returnvalue (Game|SpawnActorfromClass (Variables|Default|GetClassToPlace) (LocalVariables|GettmpTransform) "AlwaysSpawn" Owner 0))
  (return _returnvalue))
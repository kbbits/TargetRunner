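; Small box variant of a clutter placer proxy for room scenery, which supplies the actor class to place.
; It overrides GetClassToPlace to pick a random entry from AvailableClasses, using it directly if already loaded or blocking-loading it and casting to Actor otherwise.
; An empty list falls back to the parent's choice, and the construction script only calls the parent.
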(fn ConstructionScript
  (|CallParentFunction))

(fn GetClasstoPlace
  (if (> (Utilities|Array|Length (LocalVariables|GetAvailableClasses)) 0)
    (bind _output_get (LocalVariables|SettmpPickedClass (Utilities|Array|Get(acopy) (LocalVariables|GetAvailableClasses) (Math|Random|RandomIntegerinRange 0 (Utilities|Array|LastIndex (LocalVariables|GetAvailableClasses))))))
    (if (Utilities|IsValidClass (Utilities|ResolveSoftReference _output_get))
      (return (Utilities|ResolveSoftReference (LocalVariables|GettmpPickedClass)))
      (else
        (bind _returnvalue (Utilities|LoadClassAssetBlocking (LocalVariables|GettmpPickedClass)))
        (bind _asactor (Utilities|Casting|CastToActorClass _returnvalue))
        (return _asactor)))
    (else
      (bind _returnvalue_2 (|CallParentFunction))
      (return _returnvalue_2))))
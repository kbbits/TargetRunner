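; Base actor for a shootable scene target that awards score to the shooting player and is destroyed when hit.
; On authority, a hit reports Score to the instigator's TRPlayerState_BP and calls a multicast that plays the impact sound, spawns the destroy emitter and destroys the actor.
; It also stores its owning platform and exposes StaticMesh as both placeable and target mesh, opting out as an ISM template.
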(event Custom|MC_ShootableHit
  (params (Instigator :type Pawn%20Object%20Reference) (Hit :type Hit%20Result%20Structure) (Destroyed :type Boolean) (ScoreValue :type Float%20%28single-precision%29))
  (Audio|PlaySoundatLocation (select Destroyed (Variables|Default|GetDestroySound) (Variables|Default|GetHitSound)) (.ImpactPoint (Collision|BreakHitResult Hit)) "0, 0, 0" 1.0 1.0 0.0 0 0 0)
  (if Destroyed
    (Effects|SpawnEmitteratLocation (Variables|Default|GetDestroyEmitter) (Transformation|GetWorldLocation (Variables|Default|GetStaticMesh)))
    (Actor|DestroyActor)))

(event EventBeginPlay)

(event Collision|EventActorBeginOverlap
  (params (OtherActor :type Actor%20Object%20Reference)))

(event EventTick
  (params (DeltaSeconds :type Float%20%28single-precision%29)))

(event EventOnShootableTargetHit
  (params (Instigator :type Pawn%20Object%20Reference) (Hit :type Hit%20Result%20Structure) (Damage :type Float%20%28single-precision%29))
  (Networking|SwitchHasAuthority
    (:Authority
      (bind _astrplayer_state_bp (Utilities|Casting|CastToTRPlayerState_BP (Variables|/Script/Engine.Pawn|GetPlayerState Instigator)))
      (Default|OnTargetHit _astrplayer_state_bp (Variables|Default|GetScore) true)
      (CallFunction|MCShootableHit Instigator Hit true (Variables|Default|GetScore)))))

(event EventSetMyPlatform
  (params (Platform :type Platform%20Base%20Object%20Reference))
  (Variables|Default|SetMyPlatform Platform))

(fn ConstructionScript)

(fn GetMyPlatform
  (bind _asplatform_base_bp (Utilities|Casting|CastToPlatform_Base_BP (Variables|Default|GetMyPlatform)))
  (return _asplatform_base_bp))

(fn GetPlaceableMesh
  (return (Variables|Default|GetStaticMesh)))

(fn GetTargetMesh
  (return (Variables|Default|GetStaticMesh)))

(fn IsTemplateforISM
  (return false))
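; Base launcher projectile in TargetRunner, suffixed OLD, that adds optional homing to its parent projectile.
; Tick stops homing on expansion, then restarts it through HomingMovementManagerComponent after a delay, using paired DoOnce gates.
; Homing start sets the Flying state, and mesh updates apply a homing color.
; Helpers pick the closest overlapping character, toggling gravity, and score aim alignment, but are uncalled here; hit-impulse and bounds-setup logic is disconnected.
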(event Custom|OnHitCharacter
  (params (HitCharacter :type TR%20Character%20Object%20Reference) (Hit :type Hit%20Result%20Structure))
  ;[1 1 1] Unused
  (if false
    (Utilities|FlowControl|DoOnce false :!label _label
      (:Completed
        (Utilities|FlowControl|Delay 1.0)
        (goto _label Reset)))))

(event Custom|OnStartHoming
  ;[1 1 1] BeginPlay
  (Variables|Default|SetLauncherProjectileState "NewEnumerator1"))

(event EventBeginPlay
  ;[1 1 1] BeginPlay
  (|CallParentFunction)
  (EventDispatchers|BindEventtoOnStartHoming (Variables|Default|GetHomingMovementManagerComponent) (delegate Custom|OnStartHoming)))

(event EventTick
  (params (DeltaSeconds :type Float%20%28single-precision%29))
  (switch Utilities|FlowControl|Switch|SwitchonLauncherProjectileState (Variables|Default|GetLauncherProjectileState)
    (:NewEnumerator0
      _)
    (:NewEnumerator1
      (if (Variables|Default|GetEnableHoming) :!label _label
        (Utilities|FlowControl|DoOnce false :!label _label_2
          (:Completed
            (Utilities|FlowControl|Delay (Variables|Default|GetDelayBeforeHoming_0))
            (Default|StartHoming (Variables|Default|GetHomingMovementManagerComponent))
            (goto _label_3 Reset)))
        (else
          _)))
    (:NewEnumerator3
      (goto _label))
    (:NewEnumerator2
      (goto _label)))
  (|CallParentFunction DeltaSeconds)
  (Utilities|FlowControl|DoOnce false :!label _label_3
    (:Completed
      (Default|StopHoming (Variables|Default|GetHomingMovementManagerComponent))
      (goto _label_2 Reset))))

(event EventUpdateMeshbyState
  ;[1 1 1] Override UpdateMeshByState
  (if (Variables|Default|GetEnableHoming)
    (switch Utilities|FlowControl|Switch|SwitchonLauncherProjectileState (Variables|Default|GetLauncherProjectileState)
      (:NewEnumerator0
        _)
      (:NewEnumerator1
        (if (Variables|/Script/Engine.ProjectileMovementComponent|GetbIsHomingProjectile (Variables|Default|GetProjectileMovement)) :!label _label
          (Variables|Default|SetColor (Variables|Default|GetHomingColor_0_0))))
      (:NewEnumerator3
        (goto _label))
      (:NewEnumerator2
        _))
    (|CallParentFunction)
    (else
      (|CallParentFunction))))

(fn ConstructionScript
  (|CallParentFunction)
  (if (Variables|Default|GetEnableHoming)
    _))

(fn FindClosestHomingTarget
  (bind _output_get (LocalVariables|SettmpTargets (Collision|GetOverlappingActors (Variables|Default|GetTargetingBounds) "/Script/TargetRunner.TR_Character" :!class /Script/Engine.PrimitiveComponent)))
  (for (_array_element _array_index) _output_get
    (if (== _array_index 0)
      (LocalVariables|SettmpNewTarget _array_element :!label _label)
      (LocalVariables|SettmpClosestDistance (Transformation|GetDistanceTo _array_element self))
      (elif (< (Transformation|GetDistanceTo _array_element self) (LocalVariables|GettmpClosestDistance))
        (goto _label))))
  (Utilities|IsValid (LocalVariables|GettmpNewTarget)
    (:Is%20Valid
      (Variables|/Script/Engine.ProjectileMovementComponent|SetHomingTargetComponent (Variables|Default|GetProjectileMovement) (Variables|/Script/Engine.Actor|GetRootComponent (LocalVariables|GettmpNewTarget)))
      (if (Variables|Default|GetEnableHoming)
        (Variables|/Script/Engine.ProjectileMovementComponent|SetProjectileGravityScale (Variables|Default|GetProjectileMovement) 0.0))
      (return true))
    (:Is%20Not%20Valid
      (if (Variables|Default|GetEnableHoming)
        (Variables|/Script/Engine.ProjectileMovementComponent|SetProjectileGravityScale (Variables|Default|GetProjectileMovement) 1.0))
      (return false))))

(fn PercentonTarget
  (Utilities|IsValid (Variables|/Script/Engine.ProjectileMovementComponent|GetHomingTargetComponent (Variables|Default|GetProjectileMovement))
    (:Is%20Valid
      (return (Math|Float|MapRangeUnclamped (Math|Vector|DotProduct (Math|Vector|Normalize (Transformation|GetActorForwardVector)) (Math|Vector|Normalize (- (Transformation|GetWorldLocation (Variables|/Script/Engine.ProjectileMovementComponent|GetHomingTargetComponent (Variables|Default|GetProjectileMovement))) (Transformation|GetActorLocation)))) -1.0 1.0 0.0 1.0)))
    (:Is%20Not%20Valid
      (return 0.0))))
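; Base shootable target projectile that grows after launch, flies with optional homing, and awards score when shot.
; A replicated state (Expanding, Flying, Bounced, Stopped) drives scale-up, velocity-based stop detection, spin slowdown, score and mesh color, which desaturates as health drops.
; The server handles collisions and damage, credits the shooter's PlayerState and multicasts hit effects.
; On destruction it spawns award pickups that home in on the shooter.
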(event OnStartHoming(HomingMovementManagerComponent)
  ;[1 1 1] Homing
  (Variables|Default|SetProjectileState "NewEnumerator1"))

(event OnStopHoming(HomingMovementManagerComponent)
  ;[1 1 1] Homing
  (Variables|Default|SetProjectileState (Variables|Default|GetProjectileState)))

(event OnComponentHit(BoxCollision)
  (params (HitComponent :type Primitive%20Component%20Object%20Reference) (OtherActor :type Actor%20Object%20Reference) (OtherComp :type Primitive%20Component%20Object%20Reference) (NormalImpulse :type Vector :default "0, 0, 0") (Hit :type Hit%20Result%20Structure%20%28by%20ref%29))
  (CallFunction|HandleHitBase HitComponent OtherActor OtherComp NormalImpulse Hit))

(event OnComponentHit(ProjectileMesh)
  (params (HitComponent :type Primitive%20Component%20Object%20Reference) (OtherActor :type Actor%20Object%20Reference) (OtherComp :type Primitive%20Component%20Object%20Reference) (NormalImpulse :type Vector :default "0, 0, 0") (Hit :type Hit%20Result%20Structure%20%28by%20ref%29))
  (CallFunction|HandleHitBase HitComponent OtherActor OtherComp NormalImpulse Hit))

(event OnTargetAquired(HomingMovementManagerComponent)
  ;[1 1 1] Homing
  (Variables|Default|SetProjectileState "NewEnumerator1"))

(event OnTargetLost(HomingMovementManagerComponent)
  ;[1 1 1] Homing
  (Variables|Default|SetProjectileState (Variables|Default|GetProjectileState)))

(event Custom|HandleHit_Base
  (params (HitComponent :type Primitive%20Component%20Object%20Reference) (OtherActor :type Actor%20Object%20Reference) (OtherComponent :type Primitive%20Component%20Object%20Reference) (NormalImpulse :type Vector) (Hit :type Hit%20Result%20Structure))
  ;[1 1 1] Target hit something while it is flying around
  (Networking|SwitchHasAuthority
    (:Authority
      (if (Utilities|Enum|Equal(Enum) (Variables|Default|GetProjectileState) "NewEnumerator1")
        (Utilities|Casting|CastToPawn OtherActor
          (:then
            _)
          (:CastFailed
            (Utilities|Casting|CastToPlatform_Base_BP OtherActor
              (:then
                _)
              (:CastFailed
                (Utilities|Casting|CastToDynSceneryBPBase OtherActor)))))
        (Variables|Default|SetProjectileState "NewEnumerator3")))))

(event Custom|StartHoming
  (params (Delay :type Float%20%28single-precision%29))
  (Utilities|FlowControl|Delay Delay)
  (Default|StartHoming (Variables|Default|GetHomingMovementManagerComponent)))

(event Custom|SpawnPickups
  (params (Instigator :type Pawn%20Object%20Reference))
  (bind _returnvalue (Transformation|GetActorLocation))
  ;[1 1 1] Spawn Pickups
  (bind _keys (Utilities|Map|Keys (Variables|Default|GetAwards)))
  (for _array_element _keys
    (for _index (range 1 (.Value (Utilities|Map|Find (Variables|Default|GetAwards) _array_element)))
      (bind _returnvalue_2 (Game|SpawnActorfromClass _array_element (Math|Transform|MakeTransform _returnvalue (Math|Conversions|RotationFromXVector (Math|Vector|GetRightVector (Math|Rotator|CombineRotators (Math|Rotator|FindLookatRotation _returnvalue (Transformation|GetActorLocation Instigator)) (Math|Rotator|MakeRotator (Math|Random|RandomFloatinRange 0.0 3.6e+02) 0.0 0.0))))) "AdjustIfPossibleButAlwaysSpawn" Instigator 0))
      (bind _aspickup_projectile_homing (Utilities|Casting|CastToPickupProjectileHoming _returnvalue_2))
      (if (not (Game|IsActorBeingDestroyed _aspickup_projectile_homing))
        (bind _asihoming_targetable (Utilities|Casting|CastToIHomingTargetable Instigator)
          (:then
            (bind _targetedcomponent (Default|GetHomingTargetComponent _asihoming_targetable))
            (Default|SetSpecificHomingTarget (Variables|/Game/TargetRunner/Blueprints/Pickups/PickupProjectileHoming.PickupProjectileHoming_C|GetHomingMovementManagerComponent _aspickup_projectile_homing) _targetedcomponent))
          (:CastFailed
            (Default|SetSpecificHomingTarget (Variables|/Game/TargetRunner/Blueprints/Pickups/PickupProjectileHoming.PickupProjectileHoming_C|GetHomingMovementManagerComponent _aspickup_projectile_homing) (Variables|/Script/Engine.Actor|GetRootComponent Instigator))))))))

(event Custom|MC_HitTarget
  (params (Instigator :type Pawn%20Object%20Reference) (Hit :type Hit%20Result%20Structure) (Destroyed :type Boolean) (ScoreValue :type Float%20%28single-precision%29))
  ;[1 1 1] MC Hit target - Client side hit FX
  (Audio|PlaySoundatLocation (select Destroyed "/Game/TargetRunner/Assets/Audio/PopShort.PopShort" 0) (.ImpactPoint (Collision|BreakHitResult Hit)) "0, 0, 0" 1.0 1.0 0.0 0 0 0)
  (if Destroyed
    (Effects|SpawnEmitteratLocation "/Game/TargetRunner/Assets/FX/Particles/TR_TargetExplode_01.TR_TargetExplode_01" (Transformation|GetActorLocation))
    (else
      (CallFunction|UpdateMeshbyState))))

(event EventBeginPlay
  ;[1 1 1] BeginPlay
  (if (Variables|Default|GetRotateToHorizonalOnLaunch)
    (Transformation|SetWorldRotation (Variables|Transformation|GetRootComponent) (Math|Rotator|MakeRotator 0.0 0.0 (.Yaw (Math|Rotator|BreakRotator (Transformation|GetActorRotation)))) false true)))

(event EventOnShootableTargetHit
  (params (Instigator :type Pawn%20Object%20Reference) (Hit :type Hit%20Result%20Structure) (Damage :type Float%20%28single-precision%29))
  (bind _scorevalue (CallFunction|GetScore))
  ;[1 1 1] Shootable Target Hit
  (Networking|SwitchHasAuthority
    (:Authority
      (if (> (Variables|Default|GetCurrentHealth) 0.0)
        (Variables|Default|SetCurrentHealth (- (Variables|Default|GetCurrentHealth) Damage))
        (bind _astr_player_controller_base (Utilities|Casting|CastToTR_PlayerController_Base (Pawn|GetController Instigator)))
        (Default|OnTargetHit (Variables|/Game/TargetRunner/Blueprints/Player/TR_PlayerController_Base.TR_PlayerController_Base_C|GetMyPlayerState _astr_player_controller_base) _scorevalue true)
        (CallFunction|MCHitTarget Instigator Hit (<= (Variables|Default|GetCurrentHealth) 0.0) _scorevalue)
        (if (<= (Variables|Default|GetCurrentHealth) 0.0)
          (CallFunction|SpawnPickups Instigator)
          (Actor|DestroyActor))))))

(event EventTick
  (params (DeltaSeconds :type Float%20%28single-precision%29))
  ;[1 1 1] Tick
  (switch Utilities|FlowControl|Switch|SwitchonLauncherProjectileState (Variables|Default|GetProjectileState)
    (:NewEnumerator0
      (CallFunction|ExpandTargetMesh DeltaSeconds))
    (:NewEnumerator3
      ;;[1 1 1] Check every DelayTime to see if we've "stopped"
      (Networking|SwitchHasAuthority
        (:Authority
          (Utilities|FlowControl|DoOnce false :!label _label
            (:Completed
              (if (not (Variables|Default|GetEnableHoming))
                (if (<= (Math|Vector|VectorLength (Transformation|GetVelocity)) 125.0)
                  (Variables|Default|SetProjectileState "NewEnumerator2")
                  (else
                    (Utilities|FlowControl|Delay 0.2 :!label _label_2)
                    (goto _label Reset)))
                (else
                  (goto _label_2))))))))
    (:NewEnumerator2
      ;;[1 1 1] Slow rotation
      (if (and (Variables|Default|GetStopRotaionOnStopped) (> (Variables|Default|GetRotationMultiplier) 0.0))
        (Variables|Default|SetRotationMultiplier (Math|Interpolation|FInterpTo (Variables|Default|GetRotationMultiplier) 0.0 DeltaSeconds 2.0))
        (Variables|/Script/Engine.RotatingMovementComponent|SetRotationRate (Variables|Default|GetRotatingMovement) (* (Variables|Default|GetBaseRotationRate) (Variables|Default|GetRotationMultiplier)))))))

(fn ConstructionScript
  (Variables|Default|SetCurrentHealth (Variables|Default|GetMaxHealth))
  (Variables|Default|SetBaseRotationRate (Variables|/Script/Engine.RotatingMovementComponent|GetRotationRate (Variables|Default|GetRotatingMovement)))
  (Variables|/Game/TargetRunner/Blueprints/General/HomingMovementManagerComponent.HomingMovementManagerComponent_C|SetEnableHomingMaster (Variables|Default|GetHomingMovementManagerComponent) false) ; Start with it off.
  (CallFunction|UpdateMeshbyState))

(fn ExpandTargetMesh
  (params (DeltaSeconds :type Float%20%28single-precision%29))
  (switch Utilities|FlowControl|Switch|SwitchonLauncherProjectileState (Variables|Default|GetProjectileState)
    (:NewEnumerator0
      (Variables|Default|SetExpandTimeSum (+ DeltaSeconds (Variables|Default|GetExpandTimeSum)))
      (if (== (Class|KismetMathLibrary|FInterpEaseinOut (.X (Math|Vector|BreakVector (Transformation|GetActorScale3D))) (Variables|Default|GetFinalScale) (/ (Variables|Default|GetExpandTimeSum) (Variables|Default|GetExpandTime)) 1.5) (Variables|Default|GetFinalScale))
        (Transformation|SetActorScale3D (* "1.000000,1.000000,1.000000" (Variables|Default|GetFinalScale)))
        (Variables|Default|SetProjectileState "NewEnumerator1")
        (if (Variables|Default|GetEnableHoming)
          (CallFunction|StartHoming (Variables|Default|GetDelayBeforeHoming)))
        (else
          (Transformation|SetActorScale3D (* "1.000000,1.000000,1.000000" (Class|KismetMathLibrary|FInterpEaseinOut (.X (Math|Vector|BreakVector (Transformation|GetActorScale3D))) (Variables|Default|GetFinalScale) (/ (Variables|Default|GetExpandTimeSum) (Variables|Default|GetExpandTime)) 1.5))))))))

(fn GetScore
  (LocalVariables|SettmpScore (Utilities|Select :Index (Variables|Default|GetProjectileState) :NewEnumerator0 (* (Variables|Default|GetBaseDestroyScoreValue) 2.0) :NewEnumerator1 (Variables|Default|GetBaseDestroyScoreValue) :NewEnumerator3 0.0 :NewEnumerator2 (/ (Variables|Default|GetBaseDestroyScoreValue) 3.0)))
  (if (> (Variables|Default|GetCurrentHealth) 0.0)
    (return (/ (LocalVariables|GettmpScore) (Variables|Default|GetCurrentHealth)))
    (else
      (return (LocalVariables|GettmpScore)))))

(fn OnRepProjectileState
  (CallFunction|UpdateMeshbyState))

(fn UpdateMeshbyState
  (bind _color (Variables|Default|GetColor))
  (bind _hominghastargetcolor (Variables|Default|GetHomingHasTargetColor))
  (bind _enablehoming (Variables|Default|GetEnableHoming))
  (bind _returnvalue (select _enablehoming _hominghastargetcolor _color))
  (LocalVariables|SettmpMesh (CallFunction|GetProjectileMesh))
  (bind _tmpmesh (LocalVariables|GettmpMesh)
    (:then
      (Rendering|Material|SetVectorParameterValueonMaterials _tmpmesh "DiffuseColor" (Math|Conversions|ToVector(LinearColor) (Class|KismetMathLibrary|LinearColorDesaturated (Utilities|Select :Index (Variables|Default|GetProjectileState) :NewEnumerator0 (Variables|Default|GetColor) :NewEnumerator1 _returnvalue :NewEnumerator3 _returnvalue :NewEnumerator2 (Variables|Default|GetStoppedColor)) (- 1.0 (Math|Float|Square (/ (Variables|Default|GetCurrentHealth) (Variables|Default|GetMaxHealth)))))))
      (Networking|SwitchHasAuthority
        (:Remote
          (if (Utilities|Enum|NotEqual(Enum) (Variables|Default|GetProjectileState) "NewEnumerator0")
            (Utilities|FlowControl|DoOnce false
              (:Completed
                (Transformation|SetActorScale3D (* "1.000000,1.000000,1.000000" (Variables|Default|GetFinalScale)))))))))
    (:else)))

(fn GetProjectileMesh
  (return (Variables|Default|GetProjectileMesh)))

(fn EdGraph51
  (if (Variables|Default|GetStopped)
    (return (Variables|Default|GetBaseDestroyScoreValue) 0.0)
    (else
      (return (/ (Variables|Default|GetBaseDestroyScoreValue) 3.0) 0.0))))
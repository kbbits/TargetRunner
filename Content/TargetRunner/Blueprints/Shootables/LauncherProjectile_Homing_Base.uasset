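; Base homing launcher projectile that drains energy from a player character it hits.
; On the server, a DoOnce-gated box hit deducts energy through the player controller, mirrored to remote clients by RPC, and multicasts an electric sound.
; Replicated IsDraining clears after a delay that doubles as hit cooldown.
; Its RepNotify resets elapsed time and updates the mesh, which Tick color-interpolates from cyan while draining.
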(event OnComponentHit(BoxCollision)
  (params (HitComponent :type Primitive%20Component%20Object%20Reference) (OtherActor :type Actor%20Object%20Reference) (OtherComp :type Primitive%20Component%20Object%20Reference) (NormalImpulse :type Vector :default "0, 0, 0") (Hit :type Hit%20Result%20Structure%20%28by%20ref%29))
  (Networking|SwitchHasAuthority
    (:Authority
      (Utilities|FlowControl|DoOnce false :!label _label
        (:Completed
          (bind _hitcharacter (CallFunction|DeductEnergyforHit OtherActor))
          (if _hitcharacter
            (CallFunction|MCDrainEnergy)
            (Utilities|FlowControl|Delay (Variables|Default|GetEnergyDrainDelay))
            (Variables|Default|SetIsDraining false)
            (goto _label Reset)
            (else
              (goto _label Reset))))))))

(event Custom|MC_DrainEnergy
  (Audio|PlaySoundatLocation "/Game/TargetRunner/Assets/Audio/electriccurrent_Cue.electriccurrent_Cue" (Transformation|GetActorLocation) "0, 0, 0" 1.0 1.0 0.0 0 0 0))

(event EventBeginPlay
  (|CallParentFunction))

(event EventUpdateMeshbyState
  (|CallParentFunction)
  (if (Variables|Default|GetIsDraining)
    (bind _asmaterial_instance_dynamic (Utilities|Casting|CastToMaterialInstanceDynamic (Rendering|Material|GetMaterial (CallFunction|GetProjectileMesh) 0))
      (:then
        (bind _returnvalue (Rendering|Material|GetVectorParameterValue _asmaterial_instance_dynamic "DiffuseColor" :!class /Script/Engine.MaterialInstanceDynamic))
        (Rendering|Material|SetVectorParameterValueonMaterials (CallFunction|GetProjectileMesh) "DiffuseColor" (Math|Conversions|ToVector(LinearColor) (Class|KismetMathLibrary|CInterpto "(R=0.180392,G=0.827451,B=0.788235,A=1.000000)" _returnvalue (Variables|Default|GetEnergyDrainElapseTime) (Variables|Default|GetEnergyDrainDelay)))))
      (:CastFailed
        (Rendering|Material|SetVectorParameterValueonMaterials (CallFunction|GetProjectileMesh) "DiffuseColor" (Math|Conversions|ToVector(LinearColor) "(R=0.179716,G=0.828125,B=0.786907,A=1.000000)"))))))

(event EventTick
  (params (DeltaSeconds :type Float%20%28single-precision%29))
  (|CallParentFunction DeltaSeconds)
  (if (Variables|Default|GetIsDraining)
    (Variables|Default|SetEnergyDrainElapseTime (+ DeltaSeconds (Variables|Default|GetEnergyDrainElapseTime)))
    (CallFunction|UpdateMeshbyState)))

(fn ConstructionScript
  (|CallParentFunction))

(fn DeductEnergyforHit
  (params (Object :type Object%20Object%20Reference))
  (bind _returnvalue (Utilities|Enum|LiteralenumEAmmoType "None"))
  (bind _astr_first_person_character (Utilities|Casting|CastToTR_FirstPersonCharacter Object)
    (:then
      (bind _astr_player_controller_base_bp (Utilities|Casting|CastToTR_PlayerController_Base_BP (Pawn|GetController _astr_first_person_character))
        (:then
          (Variables|Default|SetIsDraining true)
          (if (Pawn|IsLocallyControlled _astr_first_person_character)
            _
            (else
              (Default|ClientDeductEnergyAmmo _astr_player_controller_base_bp (Variables|Default|GetEnergyDrain) _returnvalue 0.0)))
          (Default|DeductEnergyAmmo _astr_player_controller_base_bp (Variables|Default|GetEnergyDrain) _returnvalue 0.0)
          (return true))
        (:CastFailed
          _)))
    (:CastFailed
      _))
  (return false))

(fn OnRepIsDraining
  (Variables|Default|SetEnergyDrainElapseTime 0.0)
  (CallFunction|UpdateMeshbyState))
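; Base actor for a shootable resource cluster built from two child-actor resource nodes.
; Construction gives each node a 25% chance to become a cactus variant, binds its destroyed event, sets health and splits the cluster's total resources evenly.
; Node destructions decrement an active count; when none remain, the authority triggers a rock-burst sound effect and destroys the cluster after a short delay.
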(event Custom|OnNodeDestroyed
  (Math|Integer|DecrementInt (Variables|Default|GetActiveNodes)
    (:%20%20
      (Networking|SwitchHasAuthority
        (:Authority
          (if (<= (Variables|Default|GetActiveNodes) 0)
            (Utilities|FlowControl|Sequence
              (:then_0
                (CallFunction|MConDestroyedEffects))
              (:then_1
                (Utilities|FlowControl|Delay 0.075)
                (Actor|DestroyActor)))))))))

(event Custom|MC_OnDestroyedEffects
  (Audio|PlaySoundatLocation "/Game/TargetRunner/Assets/Audio/FX/RockBurst_2_Cue.RockBurst_2_Cue" (Transformation|GetActorLocation) "0, 0, 0" 1.0 1.0 0.0 0 0 0))

(event EventBeginPlay
  (|CallParentFunction))

(fn ConstructionScript
  (CallFunction|SetupNodes 3.0))

(fn SetupNodes
  (params (NodeBaseHealth :type Float%20%28single-precision%29))
  (LocalVariables|SettmpNodeHealth NodeBaseHealth)
  (Variables|Default|SetActiveNodes 0)
  (LocalVariables|SettmpAllNodCACs (CallFunction|GetNodeCACs))
  (Utilities|FlowControl|Sequence
    (:then_0
      (for _array_element (LocalVariables|GettmpAllNodCACs)
        (LocalVariables|SettmpNodeClass (select (<= (Math|Random|RandomFloatinRange 0.0 1.0) 0.25) "/Game/TargetRunner/Blueprints/Shootables/Resources/ResourceNodeCactus_BP.ResourceNodeCactus_BP_C" (Variables|Default|GetNodeClass)))
        (if (!= (Variables|/Script/Engine.ChildActorComponent|GetChildActorClass _array_element) (LocalVariables|GettmpNodeClass))
          (ChildActorComponent|SetChildActorClass _array_element (LocalVariables|GettmpNodeClass)))
        (bind _asresource_node_base_bp (Utilities|Casting|CastToResourceNodeBase_BP (Variables|/Script/Engine.ChildActorComponent|GetChildActor _array_element)))
        (EventDispatchers|BindEventtoOnNodeDestroyed _asresource_node_base_bp (EventDispatchers|CreateEvent :!event Custom|OnNodeDestroyed))))
    (:then_1
      (for _array_element_2 (LocalVariables|GettmpAllNodCACs)
        (bind _asresource_node_base_bp_2 (Utilities|Casting|CastToResourceNodeBase_BP (Variables|/Script/Engine.ChildActorComponent|GetChildActor _array_element_2))
          (:then
            (LocalVariables|SettmpCurrentNode _asresource_node_base_bp_2)
            (if (> (Utilities|Array|Length (Variables|Default|GetTotalResources)) 0)
              (Default|SetResourcesBP (LocalVariables|GettmpCurrentNode) (.ResourceType (Utilities|Struct|BreakResourceQuantity (Utilities|Array|Get(acopy) (Variables|Default|GetTotalResources)))) (Class|ResourceFunctionLibrary|MultiplyResourceQuantity (Variables|Default|GetTotalResources) (/ 1.0 (Math|Conversions|ToFloat(Integer) (Utilities|Array|Length (LocalVariables|GettmpAllNodCACs)))) true) 0.5))
            (bind _output_get (Variables|/Script/TargetRunner.ResourceNodeBase|SetBaseHealth (LocalVariables|GettmpCurrentNode) (LocalVariables|GettmpNodeHealth)))
            (Class|ResourceNodeBase|ServerSetCurrentHealth (LocalVariables|GettmpCurrentNode) _output_get)
            (Math|Integer|IncrementInt (Variables|Default|GetActiveNodes)))
          (:CastFailed
            (Development|PrintString "Incalid Node class")))))))

(fn GetNodeCACs
  (return (Utilities|Array|MakeArray (Variables|Default|GetNodePoint) (Variables|Default|GetNodePoint2))))
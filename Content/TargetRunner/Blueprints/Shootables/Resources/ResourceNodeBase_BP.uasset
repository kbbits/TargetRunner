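; Base Blueprint for a shootable resource node that yields homing goods pickups as it is damaged and destroyed.
; Point and radial damage are scaled by the causer's DoesDamageByType, reduce health, and extract resources using the causer's ExtractsResources rates.
; SetResources_BP splits totals between damage and destruction yields, and the node material comes from GameState resource data.
; Point-hit and destruction pickups spawn only on authority; radial-hit pickups lack that check.
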(event Custom|UpdateVisuals
  (bind _noderesourcetype (Variables|Default|GetNodeResourceType))
  (bind _astr_game_state (Utilities|Casting|CastToTR_GameState (Game|GetGameState)))
  (bind (_resourcedata _returnvalue) (Class|TRGameState|GetResourceTypeData _astr_game_state _noderesourcetype))
  (if _returnvalue
    (Utilities|IsValid (Utilities|ResolveSoftReference (.DefaultMaterial (Utilities|Struct|BreakResourceTypeData _resourcedata)))
      (:Is%20Valid
        (Variables|Default|SetNodeMaterial_BP (Utilities|ResolveSoftReference (.DefaultMaterial (Utilities|Struct|BreakResourceTypeData _resourcedata))))
        (Rendering|Material|SetMaterial (Variables|Default|GetNodeMesh) 0 (Variables|Default|GetNodeMaterial_BP)))
      (:Is%20Not%20Valid
        (bind _object (Utilities|AsyncLoadAsset (.DefaultMaterial (Utilities|Struct|BreakResourceTypeData _resourcedata)))
          (:Completed
            (bind _asmaterial_interface (Utilities|Casting|CastToMaterialInterface _object))
            (Variables|Default|SetNodeMaterial_BP _asmaterial_interface)
            (Rendering|Material|SetMaterial (Variables|Default|GetNodeMesh) 0 (Variables|Default|GetNodeMaterial_BP))))))
    (else
      (Development|PrintString (Utilities|String|Append "Error getting resource data " (Utilities|String|ToString(Name) (.Code (Utilities|Struct|BreakResourceType _noderesourcetype))))))))

(event EventBeginPlay
  (CallFunction|UpdateVisuals))

(event Game|Damage|EventPointDamage
  (params (Damage :type Float%20%28single-precision%29) (DamageType :type Damage%20Type%20Object%20Reference) (HitLocation :type Vector :default "0, 0, 0") (HitNormal :type Vector :default "0, 0, 0") (HitComponent :type Primitive%20Component%20Object%20Reference) (BoneName :type Name :default "None") (ShotFromDirection :type Vector :default "0, 0, 0") (InstigatedBy :type Controller%20Object%20Reference) (DamageCauser :type Actor%20Object%20Reference) (HitInfo :type Hit%20Result%20Structure%20%28by%20ref%29))
  (CallFunction|HandlePointDamage Damage HitLocation HitNormal InstigatedBy DamageCauser HitInfo))

(event Game|Damage|EventRadialDamage
  (params (DamageReceived :type Float%20%28single-precision%29) (DamageType :type Damage%20Type%20Object%20Reference) (Origin :type Vector :default "0, 0, 0") (HitInfo :type Hit%20Result%20Structure%20%28by%20ref%29) (InstigatedBy :type Controller%20Object%20Reference) (DamageCauser :type Actor%20Object%20Reference))
  (CallFunction|HandleRadialDamage DamageReceived Origin HitInfo InstigatedBy DamageCauser))

(event EventOnRepCurrentHealth
  (|CallParentFunction))

(fn ConstructionScript
  (Variables|Default|SetResourcesByDamageCurrent (Variables|Default|GetResourcesByDamage)))

(fn HandlePointDamage
  (params (BaseDamage :type Float%20%28single-precision%29) (HitLocation :type Vector) (HitNormal :type Vector) (Instigator :type Controller%20Object%20Reference) (DamageCauser :type Actor%20Object%20Reference) (HitterInfo :type Hit%20Result%20Structure))
  (LocalVariables|SettmpDamageDealt BaseDamage)
  (LocalVariables|SettmpHitLocation HitLocation)
  (LocalVariables|SettmpHitNormal HitNormal)
  (LocalVariables|SettmpInstigator Instigator)
  (LocalVariables|SettmpHitterInfo HitterInfo)
  (if (> (LocalVariables|GettmpDamageDealt) 0.0)
    (Utilities|FlowControl|Sequence
      (:then_0
        (bind _asdoes_damage_by_type (Utilities|Casting|CastToDoesDamageByType DamageCauser))
        (bind _calculateddamage (Class|DoesDamagebyType|CalculateDamagebyType _asdoes_damage_by_type (LocalVariables|GettmpDamageDealt) (Variables|Default|GetNodeResourceType)))
        (LocalVariables|SettmpDamageDealt _calculateddamage))
      (:then_1
        (Class|ResourceNodeBase|ServerSetCurrentHealth (Math|Float|Clamp(Float) (- (Variables|Default|GetCurrentHealth) (LocalVariables|GettmpDamageDealt)) 0.0 (Variables|Default|GetCurrentHealth))))
      (:then_2
        (bind _asextracts_resources (Utilities|Casting|CastToExtractsResources DamageCauser))
        (bind _returnvalue (Class|ExtractsResources|GetExtractionRates _asextracts_resources))
        (LocalVariables|SettmpExtractionRates _returnvalue)
        (Utilities|FlowControl|Sequence
          (:then_0
            (bind (_extractedquantities _returnvalue_2) (Class|ResourceNodeBase|ExtractedResourcesforDamage (LocalVariables|GettmpDamageDealt) (LocalVariables|GettmpExtractionRates)))
            (LocalVariables|SettmpExtractedResources _extractedquantities)
            (if _returnvalue_2
              (Class|ResourceNodeBase|ServerExtractResources (LocalVariables|GettmpExtractedResources))
              (CallFunction|HandleExtractedResourcesDamagePoint (LocalVariables|GettmpExtractedResources) (LocalVariables|GettmpHitLocation) (LocalVariables|GettmpHitNormal) (LocalVariables|GettmpHitterInfo))))
          (:then_1
            (if (<= (Variables|Default|GetCurrentHealth) 0.0)
              (Utilities|FlowControl|DoOnce false
                (:Completed
                  (bind (_extractedquantities_2 _returnvalue_3) (Class|ResourceNodeBase|ExtractedResourcesonDestroy (LocalVariables|GettmpExtractionRates)))
                  (LocalVariables|SettmpExtractedResources _extractedquantities_2)
                  (Utilities|Array|Clear (Variables|Default|GetResourcesOnDestroy))
                  (if _returnvalue_3
                    (CallFunction|HandleExtractedResouresDestroy (LocalVariables|GettmpExtractedResources)))))))))
      (:then_3
        (if (<= (Variables|Default|GetCurrentHealth) 0.0)
          (Actor|DestroyActor))))))

(fn HandleExtractedResourcesDamagePoint
  (params (ExtractedResources :type Array%20of%20Resource%20Quantity%20Structures) (HitLocation :type Vector) (HitNormal :type Vector) (HitterInfo :type Hit%20Result%20Structure))
  (Networking|SwitchHasAuthority
    (:Authority
      (LocalVariables|SettmpExtractedResources ExtractedResources)
      (LocalVariables|SettmpHitLocation HitLocation)
      (LocalVariables|SettmpHitNormal HitNormal)
      (LocalVariables|SettmpHitterInfo HitterInfo)
      (bind _astr_game_state (Utilities|Casting|CastToTR_GameState (Game|GetGameState)))
      (LocalVariables|SettmpGameState _astr_game_state)
      (for _array_element (LocalVariables|GettmpExtractedResources)
        (if (> (.Quantity (Utilities|Struct|BreakResourceQuantity _array_element)) 0.0)
          (LocalVariables|SettmpExtractedGoods (Utilities|Struct|MakeGoodsQuantity (Class|ResourceFunctionLibrary|GoodsNameforResource (.ResourceType (Utilities|Struct|BreakResourceQuantity _array_element))) (.Quantity (Utilities|Struct|BreakResourceQuantity _array_element))))
          (bind _returnvalue (Class|TRGameState|GetResourceTypeData (LocalVariables|GettmpGameState) (.ResourceType (Utilities|Struct|BreakResourceQuantity _array_element))))
          (if _returnvalue
            (Game|SpawnActorfromClass "/Game/TargetRunner/Blueprints/Pickups/PickupHomingBase_BP.PickupHomingBase_BP_C" (Math|Transform|MakeTransform (+ (LocalVariables|GettmpHitLocation) (* (Math|Vector|Normalize (LocalVariables|GettmpHitNormal)) 4.0))) "AlwaysSpawn" 0 (Variables|/Script/Engine.StaticMeshComponent|GetStaticMesh (Variables|Default|GetNodeMesh)) (Variables|Default|GetNodeMaterial_BP) (LocalVariables|GettmpHitNormal) (Utilities|Array|MakeArray (LocalVariables|GettmpExtractedGoods)) 0)))))))

(fn HandleExtractedResouresDestroy
  (params (ExtractedResources :type Array%20of%20Resource%20Quantity%20Structures))
  (Networking|SwitchHasAuthority
    (:Authority
      (bind _output_get (LocalVariables|SettmpExtractedResources ExtractedResources))
      (bind _astr_game_state (Utilities|Casting|CastToTR_GameState (Game|GetGameState)))
      (LocalVariables|SettmpGameState _astr_game_state)
      (for _array_element _output_get
        (if (> (.Quantity (Utilities|Struct|BreakResourceQuantity _array_element)) 0.0)
          (LocalVariables|SettmpExtractedGoods (Utilities|Struct|MakeGoodsQuantity (Class|ResourceFunctionLibrary|GoodsNameforResource (.ResourceType (Utilities|Struct|BreakResourceQuantity _array_element))) (.Quantity (Utilities|Struct|BreakResourceQuantity _array_element))))
          (bind _returnvalue (Class|TRGameState|GetResourceTypeData (LocalVariables|GettmpGameState) (.ResourceType (Utilities|Struct|BreakResourceQuantity _array_element))))
          (if _returnvalue
            (Game|SpawnActorfromClass "/Game/TargetRunner/Blueprints/Pickups/PickupHomingBase_BP.PickupHomingBase_BP_C" (Transformation|GetWorldTransform (Variables|Default|GetNodeMesh)) "AlwaysSpawn" 0 (Variables|/Script/Engine.StaticMeshComponent|GetStaticMesh (Variables|Default|GetNodeMesh)) (Variables|Default|GetNodeMaterial_BP) "0.000000,0.000000,0.000000" (Utilities|Array|MakeArray (LocalVariables|GettmpExtractedGoods)) 0)))))))

(fn HandleRadialDamage
  (params (DamageDealt :type Float%20%28single-precision%29) (DamageOrigin :type Vector) (Hit :type Hit%20Result%20Structure) (Instigator :type Controller%20Object%20Reference) (DamageDealer :type Actor%20Object%20Reference))
  (LocalVariables|SettmpDamageDealt DamageDealt)
  (LocalVariables|SettmpDamageOrigin DamageOrigin)
  (LocalVariables|SettmpHit Hit)
  (LocalVariables|SettmpInstigator Instigator)
  (LocalVariables|SettmpDamageDealer DamageDealer)
  (if (> (LocalVariables|GettmpDamageDealt) 0.0)
    (Utilities|FlowControl|Sequence
      (:then_0
        (bind _asdoes_damage_by_type (Utilities|Casting|CastToDoesDamageByType (LocalVariables|GettmpDamageDealer)))
        (bind _calculateddamage (Class|DoesDamagebyType|CalculateDamagebyType _asdoes_damage_by_type (LocalVariables|GettmpDamageDealt) (Variables|Default|GetNodeResourceType)))
        (LocalVariables|SettmpDamageDealt _calculateddamage))
      (:then_1
        (Variables|Default|SetCurrentHealth (Math|Float|Clamp(Float) (- (Variables|Default|GetCurrentHealth) (LocalVariables|GettmpDamageDealt)) 0.0 (Variables|Default|GetCurrentHealth))))
      (:then_2
        (bind _asextracts_resources (Utilities|Casting|CastToExtractsResources (LocalVariables|GettmpDamageDealer)))
        (bind _returnvalue (Class|ExtractsResources|GetExtractionRates _asextracts_resources))
        (LocalVariables|SettmpExtractionRates _returnvalue)
        (Utilities|FlowControl|Sequence
          (:then_0
            (bind (_extractedquantities _returnvalue_2) (Class|ResourceNodeBase|ExtractedResourcesforDamage (LocalVariables|GettmpDamageDealt) (LocalVariables|GettmpExtractionRates)))
            (LocalVariables|SettmpExtractedResources _extractedquantities)
            (if _returnvalue_2
              (Class|ResourceNodeBase|ServerExtractResources (LocalVariables|GettmpExtractedResources))
              (CallFunction|HandleExtractedResourcesDamageRadius (LocalVariables|GettmpExtractedResources) (LocalVariables|GettmpDamageOrigin) (LocalVariables|GettmpHit))))
          (:then_1
            (if (<= (Variables|Default|GetCurrentHealth) 0.0)
              (Utilities|FlowControl|DoOnce false
                (:Completed
                  (bind (_extractedquantities_2 _returnvalue_3) (Class|ResourceNodeBase|ExtractedResourcesonDestroy (LocalVariables|GettmpExtractionRates)))
                  (LocalVariables|SettmpExtractedResources _extractedquantities_2)
                  (Utilities|Array|Clear (Variables|Default|GetResourcesOnDestroy))
                  (if _returnvalue_3
                    (CallFunction|HandleExtractedResouresDestroy (LocalVariables|GettmpExtractedResources)))))))))
      (:then_3
        (if (<= (Variables|Default|GetCurrentHealth) 0.0)
          (Actor|DestroyActor))))))

(fn HandleExtractedResourcesDamageRadius
  (params (ExtractedResources :type Array%20of%20Resource%20Quantity%20Structures) (DamagerOrigin :type Vector) (Hit :type Hit%20Result%20Structure))
  (LocalVariables|SettmpExtractedResources ExtractedResources)
  (LocalVariables|SettmpDamagerOrigin DamagerOrigin)
  (LocalVariables|SettmpHit Hit)
  (bind _astr_game_state (Utilities|Casting|CastToTR_GameState (Game|GetGameState)))
  (LocalVariables|SettmpGameState _astr_game_state)
  (for _array_element (LocalVariables|GettmpExtractedResources)
    (if (> (.Quantity (Utilities|Struct|BreakResourceQuantity _array_element)) 0.0)
      (LocalVariables|SettmpExtractedGoods (Utilities|Struct|MakeGoodsQuantity (Class|ResourceFunctionLibrary|GoodsNameforResource (.ResourceType (Utilities|Struct|BreakResourceQuantity _array_element))) (.Quantity (Utilities|Struct|BreakResourceQuantity _array_element))))
      (bind _returnvalue (Class|TRGameState|GetResourceTypeData (LocalVariables|GettmpGameState) (.ResourceType (Utilities|Struct|BreakResourceQuantity _array_element))))
      (if _returnvalue
        (Game|SpawnActorfromClass "/Game/TargetRunner/Blueprints/Pickups/PickupHomingBase_BP.PickupHomingBase_BP_C" (Math|Transform|MakeTransform (+ (.Location (Collision|BreakHitResult (LocalVariables|GettmpHit))) (* (.ImpactNormal (Collision|BreakHitResult (LocalVariables|GettmpHit))) 4.0))) "AlwaysSpawn" 0 0 (Variables|Default|GetNodeMaterial_BP) (.ImpactNormal (Collision|BreakHitResult (LocalVariables|GettmpHit))) (Utilities|Array|MakeArray (LocalVariables|GettmpExtractedGoods)) 0)))))

(fn SetResourcesBP
  (params (NodeResourceType :type Resource%20Type%20Structure) (TotalResources :type Array%20of%20Resource%20Quantity%20Structures) (ResourcesOnDamageSplit :type Float%20%28single-precision%29))
  (Variables|Default|SetNodeResourceType NodeResourceType)
  (LocalVariables|SettmpTotalResources TotalResources)
  (LocalVariables|SettmpResourcesOnDamageSplit ResourcesOnDamageSplit)
  (for _array_element (LocalVariables|GettmpTotalResources)
    (bind _output_get (LocalVariables|SettmpDmgResourceQty (Math|Float|Round (* (.Quantity (Utilities|Struct|BreakResourceQuantity _array_element)) (LocalVariables|GettmpResourcesOnDamageSplit)))))
    (Utilities|FlowControl|Sequence
      (:then_0
        (Utilities|Array|Add (Variables|Default|GetResourcesByDamage) (Utilities|Struct|MakeResourceQuantity (.ResourceType (Utilities|Struct|BreakResourceQuantity _array_element)) (Math|Conversions|ToFloat(Integer) (LocalVariables|GettmpDmgResourceQty)))))
      (:then_1
        (Utilities|Array|Add (Variables|Default|GetResourcesOnDestroy) (Utilities|Struct|MakeResourceQuantity (.ResourceType (Utilities|Struct|BreakResourceQuantity _array_element)) (Math|Conversions|ToFloat(Integer) (Math|Float|Truncate (- (.Quantity (Utilities|Struct|BreakResourceQuantity _array_element)) (Math|Conversions|ToFloat(Integer) _output_get)))))))))
  (Variables|Default|SetResourcesByDamageCurrent (Variables|Default|GetResourcesByDamage))
  (CallFunction|UpdateVisuals))
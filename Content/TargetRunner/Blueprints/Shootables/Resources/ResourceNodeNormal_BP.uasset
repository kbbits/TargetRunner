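; Resource node Blueprint that builds its visuals from its resource type and quantity, updated from the construction script and the UpdateNodeVisuals event.
; It picks a type-specific mesh from ResourceMeshMap, falling back to a default mesh that uses the resource data's default material.
; Meshes and default materials async-load when not in memory.
; Mesh scale is multiplied by a clamped factor based on total resource quantity.
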(event Custom|LoadAndSetMesh
  (bind _nodemesh (CallFunction|GetStaticMeshforNode))
  (Utilities|IsValid (Utilities|ResolveSoftReference _nodemesh)
    (:Is%20Valid
      (if (Variables|Default|GetbUseDefaultMaterial)
        _
        (else
          (Variables|Default|SetNodeMaterial (Rendering|Material|GetMaterial (Utilities|ResolveSoftReference _nodemesh) 0))))
      (Components|StaticMesh|SetStaticMesh (Variables|Default|GetNodeMesh) (Utilities|ResolveSoftReference _nodemesh)))
    (:Is%20Not%20Valid
      (bind _object (Utilities|AsyncLoadAsset _nodemesh)
        (:Completed
          (bind _asstatic_mesh (Utilities|Casting|CastToStaticMesh _object))
          (if (Variables|Default|GetbUseDefaultMaterial)
            _
            (else
              (Variables|Default|SetNodeMaterial (Rendering|Material|GetMaterial _asstatic_mesh 0))))
          (Components|StaticMesh|SetStaticMesh (Variables|Default|GetNodeMesh) _asstatic_mesh)))))
  (CallFunction|UpdateNodeMeshScale)
  (CallFunction|LoadandSetMaterial))

(event Custom|LoadAndSetMaterial
  (bind _noderesourcetype (Variables|Default|GetNodeResourceType))
  (bind _code (Utilities|Struct|BreakResourceType _noderesourcetype))
  (bind (_found _resourcedata) (CallFunction|GetResourceTypeData _code))
  (Utilities|FlowControl|Sequence
    (:then_0
      (if (Variables|Default|GetbUseDefaultMaterial)
        (Utilities|IsValid (Game|GetGameState)
          (:Is%20Valid
            (if (Utilities|Name|NotEqual(Name) _code (.Code (Utilities|Struct|BreakResourceTypeData (Variables|Default|GetTmpResourceTypeData))))
              (if _found
                (Variables|Default|SetTmpResourceTypeData _resourcedata)
                (else
                  (Development|PrintString (Utilities|String|Append "Error getting resource data " (Utilities|String|ToString(Name) _code)) true true "(R=1.000000,G=0.000000,B=0.026276,A=1.000000)")
                  (goto _label Close))))))))
    (:then_1
      (Utilities|FlowControl|Gate false :!label _label
        (:Exit
          (if (Variables|Default|GetbUseDefaultMaterial)
            (if (Utilities|IsValidSoftObjectReference (.DefaultMaterial (Utilities|Struct|BreakResourceTypeData (Variables|Default|GetTmpResourceTypeData))))
              (Utilities|IsValid (Utilities|ResolveSoftReference (.DefaultMaterial (Utilities|Struct|BreakResourceTypeData (Variables|Default|GetTmpResourceTypeData))))
                (:Is%20Valid
                  (Variables|Default|SetNodeMaterial (Utilities|ResolveSoftReference (.DefaultMaterial (Utilities|Struct|BreakResourceTypeData (Variables|Default|GetTmpResourceTypeData)))))
                  (Rendering|Material|SetMaterial (Variables|Default|GetNodeMesh) 0 (Variables|Default|GetNodeMaterial)))
                (:Is%20Not%20Valid
                  (bind _object (Utilities|AsyncLoadAsset (.DefaultMaterial (Utilities|Struct|BreakResourceTypeData (Variables|Default|GetTmpResourceTypeData))))
                    (:Completed
                      (bind _asmaterial_interface (Utilities|Casting|CastToMaterialInterface _object))
                      (Variables|Default|SetNodeMaterial _asmaterial_interface)
                      (Rendering|Material|SetMaterial (Variables|Default|GetNodeMesh) 0 (Variables|Default|GetNodeMaterial)))))))
            (else
              (Utilities|IsValid (Variables|Default|GetNodeMaterial)
                (:Is%20Valid
                  (Rendering|Material|SetMaterial (Variables|Default|GetNodeMesh) 0 (Variables|Default|GetNodeMaterial)))
                (:Is%20Not%20Valid
                  (Variables|Default|SetNodeMaterial 0))))))))))

(event EventUpdateNodeVisuals
  (CallFunction|LoadandSetMesh))

(fn ConstructionScript
  (|CallParentFunction)
  (CallFunction|UpdateNodeVisuals))

(fn UpdateNodeMeshScale
  (for _array_element (Variables|Default|GetTotalResources)
    (LocalVariables|SettmpTotalQuantity (+ (LocalVariables|GettmpTotalQuantity) (.Quantity (Utilities|Struct|BreakResourceQuantity _array_element)))))
  (Transformation|SetWorldScale3D (Variables|Default|GetNodeMesh) (* (Transformation|GetWorldScale (Variables|Default|GetNodeMesh)) (Math|Float|MapRangeClamped (- (LocalVariables|GettmpTotalQuantity) 2e+01) 0.0 2e+03 1.0 2.0))))

(fn GetStaticMeshforNode
  (bind _noderesourcetype (Variables|Default|GetNodeResourceType))
  (bind _resourcemeshmap (LocalVariables|GetResourceMeshMap))
  (bind _code (Utilities|Struct|BreakResourceType _noderesourcetype))
  (bind (_value _returnvalue) (Utilities|Map|Find _resourcemeshmap _code))
  (if _returnvalue
    (Variables|Default|SetbUseDefaultMaterial false)
    (return _value)
    (else
      (Variables|Default|SetbUseDefaultMaterial true)
      (return (Utilities|ResolveSoftReference (Variables|Default|GetDefaultNodeMesh))))))
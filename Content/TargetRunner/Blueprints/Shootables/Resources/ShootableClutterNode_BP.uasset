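; Shootable clutter resource node that scatters goods pickups when its extracted items are destroyed.
; Shortly after BeginPlay, at a randomized delay, it pulls clutter drop resources from TR_GameMode to set its contents.
; On destruction handling, the authority gets drop goods from the game mode and spawns each item's actor class, falling back to GoodsPickup_BP.
; Drops launch from above the bounds center with random impulses in an upward cone.
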(event EventBeginPlay
  (|CallParentFunction)
  (Utilities|FlowControl|Delay (Math|Random|RandomFloatinRange 0.1 1.0))
  (CallFunction|InitClutterResources))

(fn ConstructionScript
  (|CallParentFunction))

(fn HandleExtractedItemsDestroy
  (params (ExtractedResources :type Array%20of%20Resource%20Quantity%20Structures))
  (bind (_origin _boxextent) (Collision|GetActorBounds true true))
  (|CallParentFunction ExtractedResources)
  (Networking|SwitchHasAuthority
    (:Authority
      (LocalVariables|SettmpSpawnOrigin _origin)
      (LocalVariables|SettmpActorExtent _boxextent)
      (bind _astr_game_mode (Utilities|Casting|CastToTR_GameMode (Game|GetGameMode)))
      (bind _droppedgoods (Class|TRGameMode|GetClutterDropGoods _astr_game_mode))
      (bind _output_get (LocalVariables|SettmpDroppedGoods _droppedgoods))
      (for _array_element _output_get
        (LocalVariables|SettmpSpawnDirection (Math|Random|RandomUnitVectorinConeinDegrees "0, 0,1.000000" 35.0))
        (LocalVariables|SettmpSpawnTransform (Math|Transform|MakeTransform (+ (LocalVariables|GettmpSpawnOrigin) (* (LocalVariables|GettmpSpawnDirection) (+ (Math|Vector|VectorLength (LocalVariables|GettmpActorExtent)) 5.0))) (Math|Rotator|MakeRotator 0.0 0.0 (Math|Random|RandomFloatinRange 0.0 359.0))))
        (if (Utilities|IsValidSoftClassReference (.ActorClass (Utilities|Struct|BreakGoodsType (.GoodsData (CallFunction|GetGoodsData (.Name (Utilities|Struct|BreakGoodsQuantity _array_element)))))))
          (if (Utilities|IsValidClass (Utilities|ResolveSoftReference (.ActorClass (Utilities|Struct|BreakGoodsType (.GoodsData (CallFunction|GetGoodsData (.Name (Utilities|Struct|BreakGoodsQuantity _array_element))))))))
            (bind _returnvalue (Game|SpawnActorfromClass (Utilities|ResolveSoftReference (.ActorClass (Utilities|Struct|BreakGoodsType (.GoodsData (CallFunction|GetGoodsData (.Name (Utilities|Struct|BreakGoodsQuantity _array_element))))))) (LocalVariables|GettmpSpawnTransform) "Undefined" 0 0))
            (Utilities|IsValid (Actor|GetComponentbyClass _returnvalue "/Script/Engine.PrimitiveComponent")
              (:Is%20Valid
                (Physics|AddImpulse (Actor|GetComponentbyClass _returnvalue "/Script/Engine.PrimitiveComponent") (* (LocalVariables|GettmpSpawnDirection) (Math|Random|RandomFloatinRange (Variables|Default|GetDropImpulseMin) (Variables|Default|GetDropImpulseMax))) "None" true)))
            (else
              (bind _returnvalue_2 (Game|SpawnActorfromClass "/Game/TargetRunner/Blueprints/Pickups/GoodsPickup_BP.GoodsPickup_BP_C" (LocalVariables|GettmpSpawnTransform) "AdjustIfPossibleButAlwaysSpawn" 0 (Utilities|Struct|MakePickupAwards (Utilities|Array|MakeArray (Utilities|Struct|MakePickupAwardsItem (Utilities|Array|MakeArray _array_element) 0.0 0.0))) 0 0 :!label _label))
              (Physics|AddImpulse (Variables|/Game/TargetRunner/Blueprints/Pickups/PickupMeshBase_BP.PickupMeshBase_BP_C|GetPickupMesh _returnvalue_2) (* (LocalVariables|GettmpSpawnDirection) (Math|Random|RandomFloatinRange (Variables|Default|GetDropImpulseMin) (Variables|Default|GetDropImpulseMax))) "None" true)))
          (else
            (goto _label))))
      (return))))

(fn InitClutterResources
  (bind _astr_game_mode (Utilities|Casting|CastToTR_GameMode (Game|GetGameMode)))
  (bind _droppedresources (Class|TRGameMode|GetClutterDropResources _astr_game_mode))
  (bind _output_get (LocalVariables|SettmpClutterResources _droppedresources))
  (if (Class|ResourceFunctionLibrary|ContainsAnyQuantity _output_get 0.0)
    (Class|ResourceNodeBase|SetResources (Variables|Default|GetNodeResourceType) (LocalVariables|GettmpClutterResources) 0.0)))
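; Drone variant of a homing launcher projectile that shows its homing state through the color of the ring around its eye.
; It overrides UpdateMeshbyState without calling the parent, creating a dynamic material instance on the ring's material slot of the projectile mesh.
; The ring's diffuse color switches between has-target and no-target colors based on whether the HomingMovementManagerComponent is homing.
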(event EventBeginPlay
  (|CallParentFunction) ; This node is disabled and will not be called.\nDrag off pins to build functionality.
)

(event Collision|EventActorBeginOverlap
  (params (OtherActor :type Actor%20Object%20Reference)))

(event EventTick
  (params (DeltaSeconds :type Float%20%28single-precision%29))
  (|CallParentFunction DeltaSeconds) ; This node is disabled and will not be called.\nDrag off pins to build functionality.
)

(event EventUpdateMeshbyState
  (bind _returnvalue (Rendering|Material|CreateDynamicMaterialInstance (Variables|Default|GetProjectileMesh) 1 0 "" :!class /Script/Engine.PrimitiveComponent)) ; Index 1 is the ring around the drone eye
  (Rendering|Material|SetVectorParameterValue _returnvalue "DiffuseColor" (select (Variables|/Game/TargetRunner/Blueprints/General/HomingMovementManagerComponent.HomingMovementManagerComponent_C|GetIsHoming (Variables|Default|GetHomingMovementManagerComponent)) (Variables|Default|GetHomingHasTargetColor) (Variables|Default|GetHomingNoTargetColor)) :!class /Script/Engine.MaterialInstanceDynamic))

(fn ConstructionScript
  (|CallParentFunction))
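; Base shootable target actor for TargetRunner that takes damage, awards score and releases pickups when its health runs out.
; On authority, hits reduce health, notify the shooter's player state and spawn homing pickups from the Awards map that seek the shooter.
; A multicast hit event updates the health-based material color and plays sound.
; On destruction, a Niagara harvest effect copies the mesh and attracts toward the shooter before the actor is destroyed.
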(event Custom|SpawnPickups
  (params (Instigator :type Pawn%20Object%20Reference))
  (bind _returnvalue (Transformation|GetActorLocation Instigator))
  (bind _returnvalue_2 (Transformation|GetActorLocation))
  (bind _returnvalue_3 (Math|Rotator|FindLookatRotation _returnvalue_2 _returnvalue))
  ;[1 1 1] Spawn Pickups
  (bind _keys (Utilities|Map|Keys (Variables|Default|GetAwards)))
  (for _array_element _keys
    (for _index (range 1 (.Value (Utilities|Map|Find (Variables|Default|GetAwards) _array_element)))
      (bind _returnvalue_4 (Game|SpawnActorfromClass _array_element (Math|Transform|MakeTransform (+ _returnvalue_2 (* (Math|Rotator|GetRotationXVector _returnvalue_3) 5e+01)) (Math|Conversions|RotationFromXVector (Math|Vector|GetRightVector (Math|Rotator|CombineRotators _returnvalue_3 (Math|Rotator|MakeRotator (Math|Random|RandomFloatinRange 0.0 3.6e+02) 0.0 0.0))))) "AdjustIfPossibleButAlwaysSpawn" Instigator 0))
      (bind _aspickup_projectile_homing (Utilities|Casting|CastToPickupProjectileHoming _returnvalue_4))
      (Utilities|IsValid _aspickup_projectile_homing
        (:Is%20Valid
          (bind _asihoming_targetable (Utilities|Casting|CastToIHomingTargetable Instigator)
            (:then
              (bind _targetedcomponent (Default|GetHomingTargetComponent _asihoming_targetable))
              (Default|SetSpecificHomingTarget (Variables|/Game/TargetRunner/Blueprints/Pickups/PickupProjectileHoming.PickupProjectileHoming_C|GetHomingMovementManagerComponent _aspickup_projectile_homing) _targetedcomponent))
            (:CastFailed
              (Default|SetSpecificHomingTarget (Variables|/Game/TargetRunner/Blueprints/Pickups/PickupProjectileHoming.PickupProjectileHoming_C|GetHomingMovementManagerComponent _aspickup_projectile_homing) (Variables|/Script/Engine.Actor|GetRootComponent Instigator)))))))))

(event Custom|MC_ShootableHit
  (params (Instigator :type Pawn%20Object%20Reference) (Hit :type Hit%20Result%20Structure) (Destroyed :type Boolean) (ScoreValue :type Float%20%28single-precision%29))
  (bind _staticmesh (Variables|Default|GetStaticMesh))
  (CallFunction|UpdateVisbyState)
  (Audio|PlaySoundatLocation (select Destroyed (Variables|Default|GetDestroySound) (Variables|Default|GetHitSound)) (.ImpactPoint (Collision|BreakHitResult Hit)) "0, 0, 0" 1.0 1.0 0.0 0 0 0)
  (if Destroyed
    (Utilities|Casting|CastToTR_FirstPersonCharacter Instigator)
    (bind _returnvalue (Niagara|SpawnSystematLocation "/Game/TargetRunner/Assets/FX/Particles/Niagara/TR_ResourceHarvest_NS.TR_ResourceHarvest_NS" (Transformation|GetWorldLocation _staticmesh) (Transformation|GetWorldRotation _staticmesh) "1.000000,1.000000,1.000000" true false))
    (Niagara|SetNiagaraVariable(Vector3) _returnvalue "User.AttractorPosition" (Transformation|GetActorLocation Instigator))
    (Class|NiagaraFunctionLibrary|OverrideSystemUserVariableStaticMesh _returnvalue "User.StaticMesh" (Variables|/Script/Engine.StaticMeshComponent|GetStaticMesh (Variables|Default|GetStaticMesh)))
    (Components|Activation|Activate _returnvalue false)
    (Actor|DestroyActor)))

(event EventBeginPlay)

(event EventSetRandomStream
  (params (RandomStream :type Random%20Stream%20Structure%20%28by%20ref%29))
  (Variables|Default|SetRandStream RandomStream))

(event EventOnShootableTargetHit
  (params (Instigator :type Pawn%20Object%20Reference) (Hit :type Hit%20Result%20Structure) (Damage :type Float%20%28single-precision%29))
  (Networking|SwitchHasAuthority
    (:Authority
      (if (> (Variables|Default|GetCurrentHealth) 0.0)
        (Variables|Default|SetCurrentHealth (- (Variables|Default|GetCurrentHealth) Damage))
        (bind _astr_player_state (Utilities|Casting|CastToTR_PlayerState (Variables|/Script/Engine.Pawn|GetPlayerState Instigator)))
        (Default|OnTargetHit _astr_player_state (Variables|Default|GetScore) (and (<= (Variables|Default|GetCurrentHealth) 0.0) (Variables|Default|GetDestroyAtZeroHealth)))
        (if (<= (Variables|Default|GetCurrentHealth) 0.0)
          (CallFunction|SpawnPickups Instigator))
        (CallFunction|MCShootableHit Instigator Hit (and (<= (Variables|Default|GetCurrentHealth) 0.0) (Variables|Default|GetDestroyAtZeroHealth)) (Variables|Default|GetScore))))))

(event EventSetMyPlatform
  (params (Platform :type Platform%20Base%20Object%20Reference))
  (Variables|Default|SetMyPlatform Platform))

(event EventSetDifficulty
  (params (Difficulty :type Float%20%28single-precision%29))
  (Variables|Default|SetDifficulty Difficulty))

(fn ConstructionScript
  (Variables|Default|SetCurrentHealth (Variables|Default|GetMaxHealth))
  (CallFunction|UpdateVisbyState))

(fn UpdateVisbyState
  (Rendering|Material|SetVectorParameterValueonMaterials (Variables|Default|GetStaticMesh) "DiffuseColor" (Math|Conversions|ToVector(LinearColor) (select (> (Variables|Default|GetCurrentHealth) 0.0) (Math|Color|Lerp(LinearColor) (Variables|Default|GetMidColor) (Variables|Default|GetStartColor) (/ (Variables|Default|GetCurrentHealth) (Variables|Default|GetMaxHealth))) (Variables|Default|GetEndColor)))))

(fn GetMyPlatform
  (bind _asplatform_base_bp (Utilities|Casting|CastToPlatform_Base_BP (Variables|Default|GetMyPlatform)))
  (return _asplatform_base_bp))

(fn GetPlaceableMesh
  (return (Variables|Default|GetStaticMesh)))

(fn GetTargetMesh
  (return (Variables|Default|GetStaticMesh)))

(fn IsTemplateforISM
  (return false))
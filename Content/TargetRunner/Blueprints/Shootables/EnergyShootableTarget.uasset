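; Shootable target Blueprint that grants energy to the player who hits it.
; On a hit, the server casts the instigator's PlayerState to TR_PlayerState and adds the target's Energy value to it.
; It then runs the parent hit handling on both server and clients, leaving base target behavior intact.
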(event EventBeginPlay
  (|CallParentFunction) ; This node is disabled and will not be called.\nDrag off pins to build functionality.
)

(event Collision|EventActorBeginOverlap
  (params (OtherActor :type Actor%20Object%20Reference))
  (|CallParentFunction OtherActor) ; This node is disabled and will not be called.\nDrag off pins to build functionality.
)

(event EventTick
  (params (DeltaSeconds :type Float%20%28single-precision%29))
  (|CallParentFunction DeltaSeconds) ; This node is disabled and will not be called.\nDrag off pins to build functionality.
)

(event EventOnShootableTargetHit
  (params (Instigator :type Pawn%20Object%20Reference) (Hit :type Hit%20Result%20Structure) (Damage :type Float%20%28single-precision%29))
  (Utilities|FlowControl|Sequence
    (:then_0
      (Networking|SwitchHasAuthority
        (:Authority
          (bind _astr_player_state (Utilities|Casting|CastToTR_PlayerState (Variables|/Script/Engine.Pawn|GetPlayerState Instigator)))
          (Default|AddEnergy _astr_player_state (Variables|Default|GetEnergy)))))
    (:then_1
      (|CallParentFunction Instigator Hit Damage))))

(fn ConstructionScript
  (|CallParentFunction))
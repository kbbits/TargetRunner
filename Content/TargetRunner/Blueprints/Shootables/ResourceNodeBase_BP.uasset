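; Base Blueprint for a shootable resource node that loses health and yields resources when damaged or destroyed.
; Point and radial damage handlers adjust damage by resource type and compute extraction yields through interfaces on the damage dealer.
; Extraction result handlers only store their inputs, apparently as hooks for children.
; Only point damage destroys the actor at zero health, and the radial event passes only the damage amount, leaving the dealer unset.
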(event EventBeginPlay)

(event Game|Damage|EventPointDamage
  (params (Damage :type Float%20%28single-precision%29) (DamageType :type Damage%20Type%20Object%20Reference) (HitLocation :type Vector :default "0, 0, 0") (HitNormal :type Vector :default "0, 0, 0") (HitComponent :type Primitive%20Component%20Object%20Reference) (BoneName :type Name :default "None") (ShotFromDirection :type Vector :default "0, 0, 0") (InstigatedBy :type Controller%20Object%20Reference) (DamageCauser :type Actor%20Object%20Reference) (HitInfo :type Hit%20Result%20Structure%20%28by%20ref%29))
  (CallFunction|HandlePointDamage Damage HitLocation HitNormal InstigatedBy DamageCauser))

(event Game|Damage|EventRadialDamage
  (params (DamageReceived :type Float%20%28single-precision%29) (DamageType :type Damage%20Type%20Object%20Reference) (Origin :type Vector :default "0, 0, 0") (HitInfo :type Hit%20Result%20Structure%20%28by%20ref%29) (InstigatedBy :type Controller%20Object%20Reference) (DamageCauser :type Actor%20Object%20Reference))
  (CallFunction|HandleRadialDamage DamageReceived "0, 0, 0"))

(fn ConstructionScript
  (Rendering|Material|SetMaterial (Variables|Default|GetNodeMesh) 0 (Variables|Default|GetNodeMaterial_BP))
  (Variables|Default|SetResourcesByDamageCurrent (Variables|Default|GetResourcesByDamage)))

(fn HandlePointDamage
  (params (BaseDamage :type Float%20%28single-precision%29) (HitLocation :type Vector) (HitNormal :type Vector) (Instigator :type Controller%20Object%20Reference) (DamageCauser :type Actor%20Object%20Reference))
  (LocalVariables|SettmpDamageDealt BaseDamage)
  (LocalVariables|SettmpHitLocation HitLocation)
  (LocalVariables|SettmpHitNormal HitNormal)
  (if (> (LocalVariables|GettmpDamageDealt) 0.0)
    (Utilities|FlowControl|Sequence
      (:then_0
        (bind _asdoes_damage_by_type (Utilities|Casting|CastToDoesDamageByType DamageCauser))
        (bind _calculateddamage (Class|DoesDamagebyType|CalculateDamagebyType _asdoes_damage_by_type (LocalVariables|GettmpDamageDealt) (Variables|Default|GetNodeResourceType)))
        (LocalVariables|SettmpDamageDealt _calculateddamage))
      (:then_1
        (Variables|Default|SetCurrentHealth (Math|Float|Clamp(Float) (- (Variables|Default|GetCurrentHealth) (LocalVariables|GettmpDamageDealt)) 0.0 (Variables|Default|GetCurrentHealth))))
      (:then_2
        (bind _asextracts_resources (Utilities|Casting|CastToExtractsResources DamageCauser))
        (bind _returnvalue (Class|ExtractsResources|GetExtractionRates _asextracts_resources))
        (LocalVariables|SettmpExtractionRates _returnvalue)
        (Utilities|FlowControl|Sequence
          (:then_0
            (bind (_extractedquantities _returnvalue_2) (Class|ResourceNodeBase|ExtractedResourcesforDamage (LocalVariables|GettmpDamageDealt) (LocalVariables|GettmpExtractionRates) true))
            (LocalVariables|SettmpExtractedResources _extractedquantities)
            (if _returnvalue_2
              (CallFunction|HandleExtractedResourcesDamagePoint (LocalVariables|GettmpExtractedResources) (LocalVariables|GettmpHitLocation) (LocalVariables|GettmpHitNormal))))
          (:then_1
            (if (<= (Variables|Default|GetCurrentHealth) 0.0)
              (bind (_extractedquantities_2 _returnvalue_3) (Class|ResourceNodeBase|ExtractedResourcesonDestroy (LocalVariables|GettmpExtractionRates)))
              (LocalVariables|SettmpExtractedResources _extractedquantities_2)
              (Utilities|Array|Clear (Variables|Default|GetResourcesOnDestroy))
              (if _returnvalue_3
                (CallFunction|HandleExtractedResouresDestroy (LocalVariables|GettmpExtractedResources)))))))
      (:then_3
        (if (<= (Variables|Default|GetCurrentHealth) 0.0)
          (Actor|DestroyActor))))))

(fn HandleExtractedResourcesDamagePoint
  (params (ExtractedResources :type Array%20of%20Resource%20Quantity%20Structures) (HitLocation :type Vector) (HitNormal :type Vector))
  (LocalVariables|SettmpExtractedResources ExtractedResources)
  (LocalVariables|SettmpHitLocation HitLocation)
  (LocalVariables|SettmpHitNormal HitNormal))

(fn HandleExtractedResouresDestroy
  (params (ExtractedResources :type Array%20of%20Resource%20Quantity%20Structures))
  (LocalVariables|SettmpExtractedResources ExtractedResources))

(fn HandleRadialDamage
  (params (DamageDealt :type Float%20%28single-precision%29) (DamageOrigin :type Vector) (Instigator :type Controller%20Object%20Reference) (DamageDealer :type Actor%20Object%20Reference))
  (LocalVariables|SettmpDamageDealt DamageDealt)
  (LocalVariables|SettmpDamageOrigin DamageOrigin)
  (LocalVariables|SettmpInstigator Instigator)
  (LocalVariables|SettmpDamageDealer DamageDealer)
  (if (> (LocalVariables|GettmpDamageDealt) 0.0)
    (Utilities|FlowControl|Sequence
      (:then_0
        (bind _asdoes_damage_by_type (Utilities|Casting|CastToDoesDamageByType (LocalVariables|GettmpDamageDealer)))
        (bind _calculateddamage (Class|DoesDamagebyType|CalculateDamagebyType _asdoes_damage_by_type (LocalVariables|GettmpDamageDealt) (Variables|Default|GetNodeResourceType)))
        (LocalVariables|SettmpDamageDealt _calculateddamage))
      (:then_1
        (Variables|Default|SetCurrentHealth (Math|Float|Clamp(Float) (- (Variables|Default|GetCurrentHealth) (LocalVariables|GettmpDamageDealt)) 0.0 (Variables|Default|GetCurrentHealth))))
      (:then_2
        (bind _asextracts_resources (Utilities|Casting|CastToExtractsResources (LocalVariables|GettmpDamageDealer)))
        (bind _returnvalue (Class|ExtractsResources|GetExtractionRates _asextracts_resources))
        (LocalVariables|SettmpExtractionRates _returnvalue)
        (Utilities|FlowControl|Sequence
          (:then_0
            (bind (_extractedquantities _returnvalue_2) (Class|ResourceNodeBase|ExtractedResourcesforDamage (LocalVariables|GettmpDamageDealt) (LocalVariables|GettmpExtractionRates) true))
            (LocalVariables|SettmpExtractedResources _extractedquantities)
            (if _returnvalue_2
              (CallFunction|HandleExtractedResourcesDamageRadius (LocalVariables|GettmpExtractedResources) (LocalVariables|GettmpDamageOrigin))))
          (:then_1
            (if (<= (Variables|Default|GetCurrentHealth) 0.0)
              (bind (_extractedquantities_2 _returnvalue_3) (Class|ResourceNodeBase|ExtractedResourcesonDestroy (LocalVariables|GettmpExtractionRates)))
              (LocalVariables|SettmpExtractedResources _extractedquantities_2)
              (Utilities|Array|Clear (Variables|Default|GetResourcesOnDestroy))
              (if _returnvalue_3
                (CallFunction|HandleExtractedResouresDestroy (LocalVariables|GettmpExtractedResources))))))))))

(fn HandleExtractedResourcesDamageRadius
  (params (ExtractedResources :type Array%20of%20Resource%20Quantity%20Structures) (DamagerOrigin :type Vector))
  (LocalVariables|SettmpExtractedResources ExtractedResources)
  (LocalVariables|SettmpDamagerOrigin DamagerOrigin))
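; Base shootable target projectile that moves through Expanding, Flying, Bounced and Stopped states, each with its own score value.
; It scales up, flies until it hits a pawn, platform or scenery, then stops once slow and eases out its spin.
; The server handles state changes, damage and player scoring, and multicasts hit effects.
; Material color follows the replicated state and desaturates as health drops.
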(event Custom|HandleHit_Base
  (params (HitComponent :type Primitive%20Component%20Object%20Reference) (OtherActor :type Actor%20Object%20Reference) (OtherComponent :type Primitive%20Component%20Object%20Reference) (NormalImpulse :type Vector) (Hit :type Hit%20Result%20Structure))
  ;[1 1 1] Target hit something while it is flying around
  (Networking|SwitchHasAuthority
    (:Authority
      (if (Utilities|Enum|Equal(Enum) (Variables|Default|GetLauncherProjectileState) "NewEnumerator1")
        (Utilities|Casting|CastToPawn OtherActor
          (:then
            _)
          (:CastFailed
            (Utilities|Casting|CastToPlatform_Base_BP OtherActor
              (:then
                _)
              (:CastFailed
                (Utilities|Casting|CastToDynSceneryBPBase OtherActor)))))
        (Variables|Default|SetLauncherProjectileState "NewEnumerator3")))))

(event Custom|MC_HitTarget
  (params (Instigator :type Pawn%20Object%20Reference) (Hit :type Hit%20Result%20Structure) (Destroyed :type Boolean) (ScoreValue :type Float%20%28single-precision%29))
  ;[1 1 1] MC Hit target - Client side hit FX
  (Audio|PlaySoundatLocation (select Destroyed "/Game/TargetRunner/Assets/Audio/PopShort_01.PopShort_01" 0) (.ImpactPoint (Collision|BreakHitResult Hit)) "0, 0, 0" 3.0 1.0 0.0 0 0 0)
  (if Destroyed
    (Effects|SpawnEmitteratLocation "/Game/TargetRunner/Assets/FX/Particles/TR_TargetExplode_01.TR_TargetExplode_01" (Transformation|GetWorldLocation (Variables|Default|GetStaticMesh)))
    (else
      (CallFunction|UpdateMeshbyState))))

(event EventBeginPlay
  ;[1 1 1] BeginPlay
  (Utilities|FlowControl|Sequence))

(event EventOnShootableTargetHit
  (params (Instigator :type Pawn%20Object%20Reference) (Hit :type Hit%20Result%20Structure) (Damage :type Float%20%28single-precision%29))
  (bind _scorevalue (CallFunction|GetScore))
  ;[1 1 1] Shootable Target Hit
  (Networking|SwitchHasAuthority
    (:Authority
      (if (> (Variables|Default|GetCurrentHealth) 0.0)
        (Variables|Default|SetCurrentHealth (- (Variables|Default|GetCurrentHealth) Damage))
        (bind _astr_player_controller_base_bp (Utilities|Casting|CastToTR_PlayerController_Base_BP (Pawn|GetController Instigator)))
        (Default|OnTargetHit (Variables|/Game/TargetRunner/Blueprints/Player/TR_PlayerController_Base_BP.TR_PlayerController_Base_BP_C|GetMyPlayerState _astr_player_controller_base_bp) _scorevalue true)
        (CallFunction|MCHitTarget Instigator Hit (<= (Variables|Default|GetCurrentHealth) 0.0) _scorevalue)
        (if (<= (Variables|Default|GetCurrentHealth) 0.0)
          (Actor|DestroyActor))))))

(event EventTick
  (params (DeltaSeconds :type Float%20%28single-precision%29))
  ;[1 1 1] Tick
  (switch Utilities|FlowControl|Switch|SwitchonLauncherProjectileState (Variables|Default|GetLauncherProjectileState)
    (:NewEnumerator0
      (CallFunction|ExpandTargetMesh DeltaSeconds))
    (:NewEnumerator3
      ;;[1 1 1] Check every DelayTime to see if we've "stopped"
      (Networking|SwitchHasAuthority
        (:Authority
          (Utilities|FlowControl|DoOnce false :!label _label
            (:Completed
              (if (<= (Math|Vector|VectorLength (Transformation|GetVelocity)) 125.0)
                (Variables|Default|SetLauncherProjectileState "NewEnumerator2")
                (else
                  (Utilities|FlowControl|Delay 0.2)
                  (goto _label Reset))))))))
    (:NewEnumerator2
      ;;[1 1 1] Slow rotation
      (if (> (Variables|Default|GetRotationMultiplier) 0.0)
        (Variables|Default|SetRotationMultiplier (Math|Interpolation|FInterpTo (Variables|Default|GetRotationMultiplier) 0.0 DeltaSeconds 2.0))
        (Variables|/Script/Engine.RotatingMovementComponent|SetRotationRate (Variables|Default|GetRotatingMovement) (* (Variables|Default|GetBaseRotationRate) (Variables|Default|GetRotationMultiplier)))))))

(fn ConstructionScript
  (Variables|Default|SetCurrentHealth (Variables|Default|GetMaxHealth))
  (Variables|/Script/Engine.RotatingMovementComponent|SetRotationRate (Variables|Default|GetRotatingMovement) (Variables|Default|GetBaseRotationRate))
  (CallFunction|UpdateMeshbyState))

(fn ExpandTargetMesh
  (params (DeltaSeconds :type Float%20%28single-precision%29))
  (switch Utilities|FlowControl|Switch|SwitchonLauncherProjectileState (Variables|Default|GetLauncherProjectileState)
    (:NewEnumerator0
      (Variables|Default|SetExpandTimeSum (+ DeltaSeconds (Variables|Default|GetExpandTimeSum)))
      (if (== (Class|KismetMathLibrary|FInterpEaseinOut (.X (Math|Vector|BreakVector (Transformation|GetActorScale3D))) (Variables|Default|GetFinalScale) (/ (Variables|Default|GetExpandTimeSum) (Variables|Default|GetExpandTime)) 1.5) (Variables|Default|GetFinalScale))
        (Transformation|SetActorScale3D (* "1.000000,1.000000,1.000000" (Variables|Default|GetFinalScale)))
        (Variables|Default|SetLauncherProjectileState "NewEnumerator1")
        (else
          (Transformation|SetActorScale3D (* "1.000000,1.000000,1.000000" (Class|KismetMathLibrary|FInterpEaseinOut (.X (Math|Vector|BreakVector (Transformation|GetActorScale3D))) (Variables|Default|GetFinalScale) (/ (Variables|Default|GetExpandTimeSum) (Variables|Default|GetExpandTime)) 1.5))))))))

(fn GetScore
  (LocalVariables|SettmpScore (Utilities|Select :Index (Variables|Default|GetLauncherProjectileState) :NewEnumerator0 (* (Variables|Default|GetBaseDestroyScoreValue) 2.0) :NewEnumerator1 (Variables|Default|GetBaseDestroyScoreValue) :NewEnumerator3 0.0 :NewEnumerator2 (/ (Variables|Default|GetBaseDestroyScoreValue) 3.0)))
  (if (> (Variables|Default|GetCurrentHealth) 0.0)
    (return (/ (LocalVariables|GettmpScore) (Variables|Default|GetCurrentHealth)))
    (else
      (return (LocalVariables|GettmpScore)))))

(fn OnRepProjectileState
  (CallFunction|UpdateMeshbyState))

(fn UpdateMeshbyState
  (bind _color (Variables|Default|GetColor))
  (Rendering|Material|SetVectorParameterValueonMaterials (Variables|Default|GetStaticMesh) "DiffuseColor" (Math|Conversions|ToVector(LinearColor) (Class|KismetMathLibrary|LinearColorDesaturated (Utilities|Select :Index (Variables|Default|GetLauncherProjectileState) :NewEnumerator0 _color :NewEnumerator1 _color :NewEnumerator3 _color :NewEnumerator2 (Variables|Default|GetStoppedColor)) (- 1.0 (Math|Float|Square (/ (Variables|Default|GetCurrentHealth) (Variables|Default|GetMaxHealth))))))))

(fn EdGraph51
  (if (Variables|Default|GetStopped)
    (return (Variables|Default|GetBaseDestroyScoreValue) 0.0)
    (else
      (return (/ (Variables|Default|GetBaseDestroyScoreValue) 3.0) 0.0))))

(fn GetTargetMesh
  (return 0))
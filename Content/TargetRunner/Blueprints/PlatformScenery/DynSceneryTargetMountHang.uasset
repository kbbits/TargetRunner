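; Dynamic platform scenery mount that hangs a shootable target from two cables.
; On BeginPlay it initializes from its platform, waits briefly, then gets the target mesh from its child actor through the IShootableTarget interface.
; Both cable ends attach to that mesh and become visible, and physics simulation is enabled on it.
; An unused branch that attaches the child actor component to the top bar remains in the graph.
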(event EventBeginPlay
  (bind _cable (Variables|Default|GetCable))
  (CallFunction|InitfromPlatform)
  (Utilities|FlowControl|Delay 0.2)
  (bind _asishootable_target (Utilities|Casting|CastToIShootableTarget (Variables|/Script/Engine.ChildActorComponent|GetChildActor (Variables|Default|GetChildActor_CAC))))
  (bind _mesh (Default|GetTargetMesh _asishootable_target))
  (Utilities|IsValid _mesh
    (:Is%20Valid
      (Class|CableComponent|SetAttachEndtoComponent _cable _mesh "None")
      (Rendering|SetVisibility _cable true false)
      (if (not (Physics|IsSimulatingPhysics _mesh "None"))
        (Physics|SetSimulatePhysics _mesh true)))))

(fn ConstructionScript
  (|CallParentFunction))
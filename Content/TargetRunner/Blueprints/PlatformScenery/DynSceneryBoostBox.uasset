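; Boost box scenery actor that boosts projectiles and launches the player character when they hit it.
; Its scene object's hit event calls OnBoost on base projectiles.
; For a first-person character, it adds a velocity-change impulse along the negated hit normal, scaled much stronger horizontally than vertically.
; Input-vector, movement-mode and reflection-vector nodes are left over and never run.
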(event OnComponentHit(SceneObject)
  (params (HitComponent :type Primitive%20Component%20Object%20Reference) (OtherActor :type Actor%20Object%20Reference) (OtherComp :type Primitive%20Component%20Object%20Reference) (NormalImpulse :type Vector :default "0, 0, 0") (Hit :type Hit%20Result%20Structure%20%28by%20ref%29))
  (bind _astr_projectile_base_bp (Utilities|Casting|CastToTR_Projectile_Base_BP OtherActor)
    (:then
      (Default|OnBoost _astr_projectile_base_bp 1.0))
    (:CastFailed
      (bind _astr_first_person_character (Utilities|Casting|CastToTR_FirstPersonCharacter OtherActor))
      (Physics|AddImpulse (Variables|/Script/Engine.Character|GetCharacterMovement _astr_first_person_character) (* (.Normal (Collision|BreakHitResult Hit)) "-2500.000000,-2500.000000,-250.000000") true))))

(event EventBeginPlay)

(fn ConstructionScript
  (|CallParentFunction))
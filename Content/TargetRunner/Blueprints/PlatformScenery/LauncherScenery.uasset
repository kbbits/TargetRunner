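; LauncherScenery is a platform scenery piece that hosts a launcher child actor and configures it for its owning platform.
; Its construction script runs InitFromPlatform, which requires a valid DynamicPlatform and an already positive DifficultyModifier.
; It hands the platform's LauncherTargetBox child actor to the launcher.
; It then refreshes DifficultyModifier from the game mode's multiplier for that platform and applies it to the launcher.
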(event EventTick
  (params (DeltaSeconds :type Float%20%28single-precision%29)))

(fn ConstructionScript
  (|CallParentFunction)
  (CallFunction|InitfromPlatform))

(fn SetLaucherTargetBox
  (params (TargetBox :type Launcher%20Target%20Box%20Object%20Reference))
  (bind _aslauncher_base (Utilities|Casting|CastToLauncher_Base (Variables|/Script/Engine.ChildActorComponent|GetChildActor (Variables|Default|GetLauncher_CAC))))
  (Variables|/Game/TargetRunner/Blueprints/Launcher/Launcher_Base.Launcher_Base_C|SetTargetBox _aslauncher_base TargetBox))

(fn GetLauncher
  (bind _aslauncher_base (Utilities|Casting|CastToLauncher_Base (Variables|/Script/Engine.ChildActorComponent|GetChildActor (Variables|Default|GetLauncher_CAC)))
    (:then
      (return _aslauncher_base))
    (:CastFailed
      (return 0))))

(fn InitfromPlatform
  (Utilities|IsValid (Variables|Default|GetPlatform)
    (:Is%20Valid
      (if (> (Variables|Default|GetDifficultyModifier) 0.0)
        (bind _asdynamic_platform (Utilities|Casting|CastToDynamicPlatform (Variables|Default|GetPlatform)))
        (LocalVariables|SettmpPlatform _asdynamic_platform)
        (LocalVariables|SettmpLauncher (CallFunction|GetLauncher))
        (Utilities|FlowControl|Sequence
          (:then_0
            (bind _aslauncher_target_box (Utilities|Casting|CastToLauncherTargetBox (Variables|/Script/Engine.ChildActorComponent|GetChildActor (Variables|/Game/TargetRunner/Blueprints/Platform/DynamicPlatform.DynamicPlatform_C|GetLauncherTargetBox_CAC (LocalVariables|GettmpPlatform)))))
            (CallFunction|SetLaucherTargetBox _aslauncher_target_box))
          (:then_1
            (bind _astr_game_mode_base_bp (Utilities|Casting|CastToTR_GameMode_Base_BP (Game|GetGameMode)))
            (bind _output_get (Variables|Default|SetDifficultyModifier (Default|DifficultyMultiplierforPlatform _astr_game_mode_base_bp (LocalVariables|GettmpPlatform))))
            (Default|SetDifficulty (LocalVariables|GettmpLauncher) _output_get)))))))
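; Scenery mesh placed on a dynamic platform, with an optional static mesh override applied in the construction script.
; SetScale extends the parent's logic on the server, drawing random X, Y and Z sizes between min and max limits from the platform's scenery random stream.
; It converts those sizes to world scale by dividing by the mesh's bounds, skipping this when both limits are zero.
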(fn ConstructionScript
  (|CallParentFunction)
  (Utilities|IsValid (Variables|Default|GetSceneMeshOverride)
    (:Is%20Valid
      (Components|StaticMesh|SetStaticMesh (Variables|Default|GetSceneObject) (Variables|Default|GetSceneMeshOverride)))))

(fn SetScale
  (bind _sceneobject (Variables|Default|GetSceneObject))
  (bind _minsizes (Variables|Default|GetMinSizes))
  (bind _maxsizes (Variables|Default|GetMaxSizes))
  (bind (_x _y _z) (Math|Vector|BreakVector _maxsizes))
  (bind _boxextent (Collision|GetComponentBounds _sceneobject))
  (bind (_x_2 _y_2 _z_2) (Math|Vector|BreakVector _minsizes))
  (bind _returnvalue (* _boxextent 2.0))
  (bind (_x_3 _y_3 _z_3) (Math|Vector|BreakVector _returnvalue))
  (|CallParentFunction)
  (if (Networking|IsServer)
    (bind _asdynamic_platform (Utilities|Casting|CastToDynamicPlatform (Variables|Default|GetPlatform)))
    (LocalVariables|SettmpSceneryStream (Variables|/Game/TargetRunner/Blueprints/Platform/DynamicPlatform.DynamicPlatform_C|GetSceneryStream _asdynamic_platform))
    (if (or (Class|KismetMathLibrary|NotEqualExactlyVectorVector (Variables|Default|GetMinSizes) "0, 0, 0") (Class|KismetMathLibrary|NotEqualExactlyVectorVector (Variables|Default|GetMaxSizes) "0, 0, 0"))
      (Utilities|FlowControl|Sequence
        (:then_0
          (LocalVariables|SettmpXSize (Math|Random|RandomFloatinRangefromStream _x_2 _x (LocalVariables|GettmpSceneryStream)))
          (LocalVariables|SettmpYSize (Math|Random|RandomFloatinRangefromStream _y_2 _y (LocalVariables|GettmpSceneryStream)))
          (LocalVariables|SettmpZSize (Math|Random|RandomFloatinRangefromStream _z_2 _z (LocalVariables|GettmpSceneryStream))))
        (:then_1
          (Transformation|SetWorldScale3D (Variables|Default|GetObjectsScene) (Math|Vector|MakeVector (/ (LocalVariables|GettmpXSize) _x_3) (/ (LocalVariables|GettmpYSize) _y_3) (/ (LocalVariables|GettmpZSize) _z_3))))
        (:then_2
          (return true)))
      (else
        (return true)))))
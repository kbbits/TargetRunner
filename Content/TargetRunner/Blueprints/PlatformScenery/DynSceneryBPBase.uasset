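; Base Blueprint for dynamic scenery objects that belong to a platform in TargetRunner.
; It stores its Platform and caches that platform's grid coordinates, both at construction and when SetMyPlatform assigns one.
; Construction and the ScaletoPlatform event call SetScale, which here is a stub returning false.
; Getters expose the platform, the placeable SceneObject and a flag marking it as an ISM template.
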(event EventSetMyPlatform
  (params (Platform :type Platform%20Base%20Object%20Reference))
  (bind _output_get (Variables|Default|SetPlatform Platform))
  (bind _returnvalue (Class|PlatformBase|GetGridCoordinates _output_get))
  (Variables|Default|SetMyPlatformGridCoords _returnvalue))

(event EventScaletoPlatform
  (CallFunction|SetScale))

(fn ConstructionScript
  (bind _platform (Variables|Default|GetPlatform))
  (Utilities|IsValid _platform
    (:Is%20Valid
      (bind _returnvalue (Class|PlatformBase|GetGridCoordinates _platform))
      (Variables|Default|SetMyPlatformGridCoords _returnvalue))
    (:Is%20Not%20Valid
      _))
  (CallFunction|SetScale))

(fn SetScale
  (return false))

(fn GetMyPlatform
  (return (Variables|Default|GetPlatform)))

(fn GetPlaceableMesh
  (return (Variables|Default|GetSceneObject)))

(fn IsTemplateforISM
  (return (Variables|Default|GetTemplateForISM?)))
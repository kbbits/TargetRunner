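; Dynamic platform scenery piece that builds a horizontal row of shootable targets.
; On the authority, SetScale uses the platform's seeded scenery stream to pick the row's length within its size limits, with axis and sign setting alignment and direction.
; It fits the collision box to the row and adds evenly spaced target child actors.
; The collision box is destroyed once the piece is placed on a platform.
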(event EventBeginPlay)

(event Collision|EventActorBeginOverlap
  (params (OtherActor :type Actor%20Object%20Reference)))

(event EventTick
  (params (DeltaSeconds :type Float%20%28single-precision%29)))

(event EventOnPlacedonPlatform
  (params (Platform :type Platform%20Base%20Object%20Reference))
  (|CallParentFunction Platform)
  (Components|DestroyComponent (Variables|Default|GetDynSceneryCollisionBox)))

(fn ConstructionScript
  (|CallParentFunction))

(fn SetScale
  (bind _minsizes (Variables|Default|GetMinSizes))
  (bind _minsizes_2 (Variables|Default|GetMinSizes))
  (bind _dynscenerycollisionbox (Variables|Default|GetDynSceneryCollisionBox))
  (bind _x (Math|Vector|BreakVector _minsizes))
  (bind _y (Math|Vector|BreakVector _minsizes_2))
  (bind _boxextent (Variables|/Script/Engine.BoxComponent|GetBoxExtent _dynscenerycollisionbox))
  (bind (_x_2 _y_2 _z) (Math|Vector|BreakVector _boxextent))
  (|CallParentFunction)
  (Networking|SwitchHasAuthority
    (:Authority
      (bind _asdynamic_platform (Utilities|Casting|CastToDynamicPlatform (Variables|Default|GetPlatform))
        (:then
          (LocalVariables|SettmpSceneryStream (Variables|/Game/TargetRunner/Blueprints/Platform/DynamicPlatform.DynamicPlatform_C|GetSceneryStream _asdynamic_platform)))
        (:CastFailed
          (LocalVariables|SettmpSceneryStream (Math|Random|MakeRandomStream 0))))
      (Utilities|FlowControl|Sequence
        (:then_0
          ;[1 1 1] Determine target array alignment and length from extents
          (if (== (.Y (Math|Vector|BreakVector (Variables|Default|GetMinSizes))) 0.0)
            (LocalVariables|SettmpTargetsExtent (* (Math|Float|Sign(Float) _x) (Math|Random|RandomFloatinRangefromStream (Math|Float|Absolute(Float) _x) (Math|Float|Absolute(Float) (.X (Math|Vector|BreakVector (Variables|Default|GetMaxSizes)))) (LocalVariables|GettmpSceneryStream)))) ; From X extent
            (LocalVariables|SettmpTargetsDirection (Transformation|GetActorForwardVector))
            (LocalVariables|SettmpTargetRotation "0,90.000000, 0")
            (else
              (LocalVariables|SettmpTargetsExtent (* (Math|Float|Sign(Float) _y) (Math|Random|RandomFloatinRangefromStream (Math|Float|Absolute(Float) _y) (Math|Float|Absolute(Float) (.Y (Math|Vector|BreakVector (Variables|Default|GetMaxSizes)))) (LocalVariables|GettmpSceneryStream)))) ; From Y extent
              (LocalVariables|SettmpTargetsDirection (Math|Vector|GetRightVector (Variables|Default|GetObjectsScene)))
              (LocalVariables|SettmpTargetRotation "0, 0, 0"))))
        (:then_1
          ;[1 1 1] Negative extents means rotate 180 - so target array goes the opposite direction.
          (if (< (LocalVariables|GettmpTargetsExtent) 0.0)
            (LocalVariables|SettmpTargetsDirection (* (LocalVariables|GettmpTargetsDirection) -1.0))))
        (:then_2
          (LocalVariables|SettmpNumTargets (select (< (Math|Float|Truncate (/ (- (Math|Float|Absolute(Float) (LocalVariables|GettmpTargetsExtent)) (Variables|Default|GetFirstTargetOffset)) (Variables|Default|GetTargetSpacing))) 1) 1 (Math|Float|Truncate (/ (- (Math|Float|Absolute(Float) (LocalVariables|GettmpTargetsExtent)) (Variables|Default|GetFirstTargetOffset)) (Variables|Default|GetTargetSpacing)))))
          (Transformation|AddRelativeLocation (Variables|Default|GetDynSceneryCollisionBox) (* (LocalVariables|GettmpTargetsDirection) (/ (+ (* (- (LocalVariables|GettmpNumTargets) 1) (Variables|Default|GetTargetSpacing)) (Variables|Default|GetFirstTargetOffset) (Variables|Default|GetTargetWidth)) 2.0)) false true)
          (Components|Box|SetBoxExtent (Variables|Default|GetDynSceneryCollisionBox) (Math|Vector|MakeVector (/ (+ (* (- (LocalVariables|GettmpNumTargets) 1) (Variables|Default|GetTargetSpacing)) (Variables|Default|GetFirstTargetOffset) (Variables|Default|GetTargetWidth)) 2.0) _y_2 _z) true)
          (Transformation|AddRelativeRotation (Variables|Default|GetDynSceneryCollisionBox) (Math|Conversions|RotationFromXVector (LocalVariables|GettmpTargetsDirection)) false false))
        (:then_3
          ;[1 1 1 1 14] One target every 2 meters. (200 units)
          (for _index (range 0 (- (LocalVariables|GettmpNumTargets) 1))
            (Utilities|FlowControl|Sequence
              (:then_0
                (LocalVariables|SettmpTargetLocation (+ (* (LocalVariables|GettmpTargetsDirection) (+ (* _index (Variables|Default|GetTargetSpacing)) (Variables|Default|GetFirstTargetOffset))) (Variables|/Script/Engine.SceneComponent|GetRelativeLocation (Variables|Default|GetSceneObject)))))
              (:then_1
                (bind _returnvalue (AddComponent|AddChildActorComponent false (Math|Transform|MakeTransform (LocalVariables|GettmpTargetLocation) (LocalVariables|GettmpTargetRotation))))
                (ChildActorComponent|SetChildActorClass _returnvalue "/Game/TargetRunner/Blueprints/Shootables/ShootableTarget_Base.ShootableTarget_Base_C")))))
        (:then_4
          (return true))))))
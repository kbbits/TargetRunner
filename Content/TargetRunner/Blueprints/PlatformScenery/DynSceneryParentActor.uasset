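; DynSceneryParentActor is a platform scenery actor that hosts a configurable child actor and passes platform-specific settings to it.
; On construction or when its platform is set, it applies the child class override to its ChildActorComponent.
; For a DynamicPlatform, it sends the game mode's difficulty multiplier and the platform's scenery random stream through ISceneryChild.
; Child actors lacking that interface are cleared when fetched during this initialization.
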(event EventSetMyPlatform
  (params (Platform :type Platform%20Base%20Object%20Reference))
  (|CallParentFunction Platform)
  (CallFunction|InitfromPlatform))

(event EventTick
  (params (DeltaSeconds :type Float%20%28single-precision%29)))

(fn ConstructionScript
  (|CallParentFunction)
  (CallFunction|InitfromPlatform))

(fn GetSceneryChild
  (bind _asiscenery_child (Utilities|Casting|CastToISceneryChild (Variables|/Script/Engine.ChildActorComponent|GetChildActor (Variables|Default|GetChildActor_CAC)))
    (:then
      (return _asiscenery_child))
    (:CastFailed
      (Utilities|IsValid (Variables|/Script/Engine.ChildActorComponent|GetChildActor (Variables|Default|GetChildActor_CAC))
        (:Is%20Valid
          (ChildActorComponent|SetChildActorClass (Variables|Default|GetChildActor_CAC) 0))
        (:Is%20Not%20Valid
          _))
      (return 0))))

(fn InitfromPlatform
  (Utilities|FlowControl|Sequence
    (:then_0
      (if (!= (Variables|Default|GetChildActorClassOverride) (Variables|/Script/Engine.ChildActorComponent|GetChildActorClass (Variables|Default|GetChildActor_CAC)))
        (ChildActorComponent|SetChildActorClass (Variables|Default|GetChildActor_CAC) (Variables|Default|GetChildActorClassOverride))))
    (:then_1
      (Utilities|IsValid (Variables|Default|GetPlatform)
        (:Is%20Valid
          (bind _asdynamic_platform (Utilities|Casting|CastToDynamicPlatform (Variables|Default|GetPlatform)))
          (LocalVariables|SettmpPlatform _asdynamic_platform)
          (bind _output_get (LocalVariables|SettmpChild (CallFunction|GetSceneryChild)))
          (Utilities|IsValid (Utilities|ToObject(Interface) _output_get)
            (:Is%20Valid
              (Utilities|FlowControl|Sequence
                (:then_0
                  (bind _astr_game_mode_base_bp (Utilities|Casting|CastToTR_GameMode_Base_BP (Game|GetGameMode)))
                  (bind _output_get_2 (Variables|Default|SetDifficultyModifier (Default|DifficultyMultiplierforPlatform _astr_game_mode_base_bp (LocalVariables|GettmpPlatform))))
                  (Default|SetDifficulty (LocalVariables|GettmpChild) _output_get_2))
                (:then_1
                  (Default|SetRandomStream (LocalVariables|GettmpChild) (Variables|/Game/TargetRunner/Blueprints/Platform/DynamicPlatform.DynamicPlatform_C|GetSceneryStream (LocalVariables|GettmpPlatform))))))))))))
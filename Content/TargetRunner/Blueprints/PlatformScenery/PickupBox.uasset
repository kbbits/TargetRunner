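; PickupBox is a pulsing, rotating scenery pillar that dispenses pickup awards when GiveAwards is called.
; A looping or one-shot timeline drives its emissive material and point light.
; GiveAwards spawns each Awards class in a quantity scaled by Difficulty, launching pickups outward at random yaw around the mesh.
; It then greys out, stops pulsing and rotating, and the authority destroys it after a short delay.
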(event Custom|GiveAwards
  (bind _keys (Utilities|Map|Keys (Variables|Default|GetAwards)))
  (for _array_element _keys
    (for _index (range 1 (Math|Float|Truncate (* (.Value (Utilities|Map|Find (Variables|Default|GetAwards) _array_element)) (Variables|Default|GetDifficulty))))
      (CallFunction|SpawnSingleAward _array_element)))
  (Utilities|FlowControl|Delay 0.5)
  (CallFunction|OnPillarDone))

(event Custom|OnPillarDone
  (Rendering|SetVisibility (Variables|Default|GetPointLight) false false)
  (Rendering|Material|SetVectorParameterValueonMaterials (Variables|Default|GetMesh) "BaseColor" (Math|Conversions|ToVector(LinearColor) "(R=0.385417,G=0.385417,B=0.385417,A=1.000000)"))
  (Rendering|Material|SetVectorParameterValueonMaterials (Variables|Default|GetMesh) "EmissiveColor" (Math|Conversions|ToVector(LinearColor) "(R=0.604167,G=0.604167,B=0.604167,A=1.000000)"))
  (Audio|Components|Audio|Stop (Variables|Default|GetPulseTimeline))
  (Variables|/Script/Engine.RotatingMovementComponent|SetRotationRate (Variables|Default|GetRotatingMovement) "0, 0, 0")
  (Networking|SwitchHasAuthority
    (:Authority
      (Utilities|FlowControl|Delay 2.0)
      (Actor|DestroyActor))))

(event EventBeginPlay
  (bind _pulsevalue (Timeline|PulseTimeline PlayFromStart)
    (:Update
      (Rendering|Material|SetScalarParameterValueonMaterials (Variables|Default|GetMesh) "EmissiveFactor" _pulsevalue)
      (Rendering|Components|Light|SetIntensity (Variables|Default|GetPointLight) (* _pulsevalue 3.2e+03)))))

(event EventSetDifficulty
  (params (Difficulty :type Float%20%28single-precision%29))
  (Variables|Default|SetDifficulty Difficulty))

(event EventSetRandomStream
  (params (RandomStream :type Random%20Stream%20Structure%20%28by%20ref%29))
  (Variables|Default|SetRandStream RandomStream))

(fn ConstructionScript)

(fn SpawnSingleAward
  (params (PickupClass :type Pickup%20Base%20BP%20Class%20Reference))
  (LocalVariables|SettmpPickupClass PickupClass)
  (LocalVariables|SettmpSpawnDirection (Math|Rotator|MakeRotator 0.0 0.0 (Math|Random|RandomFloatinRange 0.0 3.6e+02)))
  (bind _returnvalue (Game|SpawnActorfromClass (LocalVariables|GettmpPickupClass) (Math|Transform|MakeTransform (+ (Transformation|GetWorldLocation (Variables|Default|GetPickupSpawnPoint)) (* (Math|Vector|GetForwardVector (LocalVariables|GettmpSpawnDirection)) (* (.X (Math|Vector|BreakVector (.BoxExtent (Collision|GetComponentBounds (Variables|Default|GetMesh))))) 1.2))) (LocalVariables|GettmpSpawnDirection)) "AdjustIfPossibleButAlwaysSpawn" 0 0))
  (Game|Components|ProjectileMovement|SetVelocityinLocalSpace (Variables|/Game/TargetRunner/Blueprints/Pickups/Pickup_Base_BP.Pickup_Base_BP_C|GetProjectileMovement _returnvalue) "250.000000, 0, 0") ; "shoot" them out a bit from the pillar
)
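; Base Blueprint for dynamic scenery pieces that belong to a grid platform in TargetRunner.
; It stores its platform and that platform's grid coordinates, captured through SetMyPlatform or refreshed in the construction script.
; SetScale is a stub returning false, called on construction and by ScaletoPlatform, while getters expose the platform, placeable mesh and ISM-template flag.
; Unconnected logic would recover a missing platform from the GameState's grid manager using the saved coordinates.
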(event EventSetMyPlatform
  (params (Platform :type Platform%20Base%20Object%20Reference))
  (bind _output_get (Variables|Default|SetMyPlatform Platform))
  (bind _returnvalue (Class|PlatformBase|GetGridCoordinates _output_get))
  (Variables|Default|SetMyPlatformGridCoords _returnvalue))

(event EventScaletoPlatform
  (CallFunction|SetScale))

(fn ConstructionScript
  (bind _myplatform (Variables|Default|GetMyPlatform))
  (Utilities|IsValid _myplatform
    (:Is%20Valid
      (bind _returnvalue (Class|PlatformBase|GetGridCoordinates _myplatform))
      (Variables|Default|SetMyPlatformGridCoords _returnvalue))
    (:Is%20Not%20Valid
      _))
  (CallFunction|SetScale))

(fn SetScale
  (return false))

(fn GetMyPlatform
  (return (Variables|Default|GetMyPlatform)))

(fn GetPlaceableMesh
  (return (Variables|Default|GetSceneObject)))

(fn IsTemplateforISM
  (return (Variables|Default|GetTemplateForISM?)))
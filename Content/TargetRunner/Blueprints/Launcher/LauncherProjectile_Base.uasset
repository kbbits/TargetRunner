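; Base launcher projectile that grows to its final scale after spawning.
; On BeginPlay it sets the static mesh's relative rotation to the inverse of the box collision's world rotation.
; Tick accumulates time and eases uniform actor scale from its current value toward FinalScale over ExpandTime, then flags it as expanded once the target is reached.
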(event EventBeginPlay
  (Transformation|SetRelativeRotation (Variables|Default|GetStaticMesh) (Class|KismetMathLibrary|NegateRotator (Transformation|GetWorldRotation (Variables|Default|GetBoxCollision))) false false))

(event EventTick
  (params (DeltaSeconds :type Float%20%28single-precision%29))
  (Variables|Default|SetExpandTimeSum (+ DeltaSeconds (Variables|Default|GetExpandTimeSum)))
  (if (not (Variables|Default|GetExpanded))
    (if (== (Class|KismetMathLibrary|FInterpEaseinOut (.X (Math|Vector|BreakVector (Transformation|GetActorScale3D))) (Variables|Default|GetFinalScale) (/ (Variables|Default|GetExpandTimeSum) (Variables|Default|GetExpandTime)) 1.5) (Variables|Default|GetFinalScale))
      (Transformation|SetActorScale3D (* "1.000000,1.000000,1.000000" (Variables|Default|GetFinalScale)))
      (Variables|Default|SetExpanded true)
      (else
        (Transformation|SetActorScale3D (* "1.000000,1.000000,1.000000" (Class|KismetMathLibrary|FInterpEaseinOut (.X (Math|Vector|BreakVector (Transformation|GetActorScale3D))) (Variables|Default|GetFinalScale) (/ (Variables|Default|GetExpandTimeSum) (Variables|Default|GetExpandTime)) 1.5)))))))

(fn ConstructionScript)
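; LauncherTargetBox is a box volume actor that supplies random target points, apparently for a launcher.
; GetBoxBounds returns the bounds of its Box component.
; GetRandomLocation takes a random stream and offsets the box origin by a random value within the extent on each axis, so points are reproducible from the stream.
; It has no active event or construction logic.
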(event EventBeginPlay)

(event Collision|EventActorBeginOverlap
  (params (OtherActor :type Actor%20Object%20Reference)))

(event EventTick
  (params (DeltaSeconds :type Float%20%28single-precision%29)))

(fn ConstructionScript)

(fn GetBoxBounds
  (bind _box (Variables|Default|GetBox))
  (bind (_origin _boxextent _sphereradius) (Collision|GetComponentBounds _box))
  (return (Utilities|Struct|MakeBoxSphereBounds _origin _boxextent _sphereradius)))

(fn GetRandomLocation
  (params (RandStream :type Random%20Stream%20Structure%20%28by%20ref%29))
  (bind _box (Variables|Default|GetBox))
  (bind (_origin _boxextent) (Collision|GetComponentBounds _box))
  (LocalVariables|SettmpRandStream RandStream)
  (LocalVariables|SettmpMaxs _boxextent)
  (LocalVariables|SettmpMins (* _boxextent -1.0))
  (return (+ _origin (Math|Vector|MakeVector (Math|Random|RandomFloatinRangefromStream (.X (Math|Vector|BreakVector (LocalVariables|GettmpMins))) (.X (Math|Vector|BreakVector (LocalVariables|GettmpMaxs))) (LocalVariables|GettmpRandStream)) (Math|Random|RandomFloatinRangefromStream (.Y (Math|Vector|BreakVector (LocalVariables|GettmpMins))) (.Y (Math|Vector|BreakVector (LocalVariables|GettmpMaxs))) (LocalVariables|GettmpRandStream)) (Math|Random|RandomFloatinRangefromStream (.Z (Math|Vector|BreakVector (LocalVariables|GettmpMins))) (.Z (Math|Vector|BreakVector (LocalVariables|GettmpMaxs))) (LocalVariables|GettmpRandStream))))))
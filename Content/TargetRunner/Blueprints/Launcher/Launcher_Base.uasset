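; Base launcher actor that aims its barrel at random points in a target box and fires projectiles that serve as scalable, health-bearing targets.
; A server-driven state machine loops through delay, interpolated aiming and multicast firing until locations run out, then signals done.
; Projectile classes come from a cached weighted list using a seeded random stream.
; Replicated state recolors the sphere, and difficulty scales pacing, aim speed, health, size and count from class defaults.
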(event Custom|NextTarget
  (bind _targetlocations (Variables|Default|GetTargetLocations))
  (bind _returnvalue (Utilities|Array|LastIndex _targetlocations))
  ;[1 1 1] Next Target
  (Variables|Default|SetCurrentTargetLocation "0, 0, 0")
  (if (> (Variables|Default|GetDelayBetweenLaunches) 0.5)
    (Utilities|FlowControl|Delay 0.5))
  (if (>= (Utilities|Array|LastIndex (Variables|Default|GetTargetLocations)) 0)
    (CallFunction|ServerSetLauncherState "NewEnumerator5")
    (Utilities|FlowControl|Delay (select (> (Variables|Default|GetDelayBetweenLaunches) 0.5) (- (Variables|Default|GetDelayBetweenLaunches) 0.5) (Variables|Default|GetDelayBetweenLaunches)))
    (CallFunction|ServerSetLauncherState "NewEnumerator1")
    (Variables|Default|SetCurrentTargetLocation (Utilities|Array|Get(acopy) _targetlocations _returnvalue))
    (Utilities|Array|RemoveIndex (Variables|Default|GetTargetLocations) _returnvalue)
    (Variables|Default|SetCurrentTargetRotation (Math|Rotator|FindLookatRotation (Transformation|GetWorldLocation (Variables|Default|GetBarrelScene)) (Variables|Default|GetCurrentTargetLocation)))
    (else
      (Variables|Default|SetCurrentTargetRotation "0, 0, 0")
      (CallFunction|ServerSetLauncherState "NewEnumerator4"))))

(event Custom|StartLaunching
  (params (StartedManually :type Boolean))
  ;[1 1 1] Start Launching
  (Variables|Default|SetbWasStartedManually StartedManually)
  (switch Utilities|FlowControl|Switch|SwitchonLauncherState (Variables|Default|GetCurrentState)
    (:NewEnumerator0
      _)
    (:NewEnumerator3
      _))
  (if (> (Utilities|Array|Length (Variables|Default|GetTargetLocations)) 0)
    _
    (else
      (CallFunction|FindRandomTargets)))
  (CallFunction|NextTarget))

(event Custom|MC_FireProjectile
  ;[1 1 1] MC Fire projectiile
  (Networking|SwitchHasAuthority
    (:Authority
      (CallFunction|FireProjectileImpl))
    (:Remote
      _))
  (Math|Integer|IncrementInt (Variables|Default|GetTargetsLaunched)
    (:%20%20
      (Audio|PlaySoundatLocation "/Game/TargetRunner/Assets/Audio/WeaponFire.WeaponFire" (Transformation|GetActorLocation) "0, 0, 0" 1.0 0.5 0.0 0 0 0))))

(event Custom|ServerSetLauncherState
  (params (NewState :type LauncherState%20Enum :default "NewEnumerator0"))
  ;[1 1 1] ServerSetLauncherState
  (Variables|Default|SetCurrentState NewState)
  (if (Utilities|Enum|Equal(Enum) (Variables|Default|GetCurrentState) "NewEnumerator4")
    (Default|CallOnLauncherDone self)))

(event EventTick
  (params (DeltaSeconds :type Float%20%28single-precision%29))
  ;[1 1 1] Tick
  (Networking|SwitchHasAuthority
    (:Authority
      (switch Utilities|FlowControl|Switch|SwitchonLauncherState (Variables|Default|GetCurrentState)
        (:NewEnumerator1
          _)
        (:NewEnumerator3
          _)
        (:NewEnumerator4
          _))
      (if (Utilities|Enum|NotEqual(Enum) (Transformation|GetWorldRotation (Variables|Default|GetBarrelScene)) (Variables|Default|GetCurrentTargetRotation) 1.0)
        ;;[1 1 1] Rotate towards target
        (Transformation|SetWorldRotation (Variables|Default|GetBarrelScene) (Math|Interpolation|RInterpTo (Transformation|GetWorldRotation (Variables|Default|GetBarrelScene)) (Variables|Default|GetCurrentTargetRotation) DeltaSeconds (Variables|Default|GetAimSpeed)) false false)
        (else
          (switch Utilities|FlowControl|Switch|SwitchonLauncherState (Variables|Default|GetCurrentState)
            (:NewEnumerator1
              (CallFunction|ServerSetLauncherState "NewEnumerator2")
              (CallFunction|MCFireProjectile)
              (Variables|Default|SetCurrentTargetLocation "0, 0, 0")
              (CallFunction|NextTarget))
            (:NewEnumerator3
              (CallFunction|ServerSetLauncherState "NewEnumerator4"))))))))

(event EventBeginPlay
  ;[1 1 1] Begin Play
  (CallFunction|UpdatebyState)
  (if (Networking|IsServer)
    (if (>= (Variables|Default|GetDelayBeforeStart) 0.0)
      (Utilities|FlowControl|Delay (Variables|Default|GetDelayBeforeStart))
      (CallFunction|StartLaunching false))))

(fn ConstructionScript
  (CallFunction|UpdatebyState))

(fn FindRandomTargets
  (Utilities|Array|Clear (Variables|Default|GetTargetLocations))
  (Utilities|IsValid (Variables|Default|GetTargetBox)
    (:Is%20Valid
      (for _index (range 1 (- (Variables|Default|GetBaseTargetsToSpawn) (Variables|Default|GetTargetsLaunched)))
        (bind _location (Default|GetRandomLocationinBox (Variables|Default|GetTargetBox) (Variables|Default|GetRandStream)))
        (Utilities|Array|Add (Variables|Default|GetTargetLocations) _location)))))

(fn Fire
  (Utilities|FlowControl|Sequence
    (:then_0
      (CallFunction|MCFireProjectile))))

(fn GetLaunchDurationEstimate
  (LocalVariables|SettmpEstimate (+ (Variables|Default|GetDelayBeforeStart) (* (- (Variables|Default|GetBaseTargetsToSpawn) 1) (+ (Variables|Default|GetDelayBetweenLaunches) (/ 5.0 (Variables|Default|GetAimSpeed))))))
  (return (select (< (LocalVariables|GettmpEstimate) 0.0) 0.0 (LocalVariables|GettmpEstimate))))

(fn UpdatebyState
  (bind _targetingcolor (Variables|Default|GetTargetingColor))
  (bind _returnvalue (Math|Conversions|ToVector(LinearColor) _targetingcolor))
  (if (Utilities|Enum|Equal(Enum) (Variables|Default|GetCurrentState) "NewEnumerator4")
    (Utilities|Array|Clear (Variables|Default|GetCachedProjectilesByWeight)))
  (Rendering|Material|SetVectorParameterValueonMaterials (Variables|Default|GetSphere) "DiffuseColor" (Utilities|Select :Index (Variables|Default|GetCurrentState) :NewEnumerator0 (Math|Conversions|ToVector(LinearColor) (Variables|Default|GetWaitingToStartColor)) :NewEnumerator1 _returnvalue :NewEnumerator2 (Math|Conversions|ToVector(LinearColor) (Variables|Default|GetFiringColor)) :NewEnumerator5 _returnvalue :NewEnumerator3 (Math|Conversions|ToVector(LinearColor) (Variables|Default|GetIdleColor)) :NewEnumerator4 (Math|Conversions|ToVector(LinearColor) (Variables|Default|GetDoneColor)))))

(fn OnRepCurrentState
  (CallFunction|UpdatebyState))

(fn GetProjectileClass
  (if (== (Utilities|Array|Length (Variables|Default|GetCachedProjectilesByWeight)) 0)
    ;[1 1 1] Convert the map to a cahced array of classes, one entry per "weight point"
    (bind _keys (Utilities|Map|Keys (Variables|Default|GetProjectileClassWeights)))
    (for _array_element _keys
      (for _index (range 1 (.Value (Utilities|Map|Find (Variables|Default|GetProjectileClassWeights) _array_element)))
        (Utilities|Array|Add (Variables|Default|GetCachedProjectilesByWeight) _array_element))))
  (return (Utilities|Array|Get(acopy) (Variables|Default|GetCachedProjectilesByWeight) (Math|Random|RandomIntegerinRangefromStream 0 (Utilities|Array|LastIndex (Variables|Default|GetCachedProjectilesByWeight)) (Variables|Default|GetRandStream)))))

(fn FireProjectileImpl
  (LocalVariables|SettmpProjectileClass (CallFunction|GetProjectileClass))
  (bind _returnvalue (Game|SpawnActorfromClass (LocalVariables|GettmpProjectileClass) (Math|Transform|MakeTransform (Transformation|GetSocketLocation (Variables|Default|GetBarrelMesh) "ProjectileSocket") (Variables|Default|GetCurrentTargetRotation) "0.010000,0.010000,0.010000") "AlwaysSpawn" self (Variables|Default|GetTargetScaleMultiplier) (Variables|Default|GetTargetBaseHealth) (Variables|Default|GetRandStream) (Variables|Default|GetDifficultyModifier) 0))
  (return _returnvalue))

(fn SetDifficulty
  (params (DifficultyModifier :type Float%20%28single-precision%29))
  (bind _self self)
  (bind _returnvalue (Utilities|GetClass _self))
  (bind (_targetlocations _currenttargetrotation _currenttargetlocation _basetargetstospawn _delaybetweenlaunches _aimspeed _delaybeforestart _currentstate _onlauncherdone _waitingtostartcolor _targetingcolor _firingcolor _idlecolor _donecolor _targetslaunched _targetbasehealth _targetscalemultiplier) (Utilities|GetClassDefaults _returnvalue))
  (Variables|Default|SetDifficultyModifier DifficultyModifier)
  (Utilities|FlowControl|Sequence
    (:then_0
      (Variables|Default|SetDelayBetweenLaunches (/ _delaybetweenlaunches (Variables|Default|GetDifficultyModifier))))
    (:then_1
      (Variables|Default|SetAimSpeed (* (Variables|Default|GetDifficultyModifier) _aimspeed)))
    (:then_2
      (Variables|Default|SetTargetBaseHealth (Math|Conversions|ToFloat(Integer) (Math|Float|Truncate (* (Variables|Default|GetDifficultyModifier) _targetbasehealth)))))
    (:then_3
      (Variables|Default|SetTargetScaleMultiplier (Math|Float|Clamp(Float) (* (/ _targetscalemultiplier (Math|Float|Power (Variables|Default|GetDifficultyModifier) 0.7)) (Math|Random|RandomFloatinRange 0.95 1.05)) 0.25 _targetscalemultiplier)))
    (:then_4
      (Variables|Default|SetBaseTargetsToSpawn (Math|Float|Round (* _basetargetstospawn (Variables|Default|GetDifficultyModifier)))))))

(fn GetRemainingShots
  (return (- (Variables|Default|GetBaseTargetsToSpawn) (Variables|Default|GetTargetsLaunched))))